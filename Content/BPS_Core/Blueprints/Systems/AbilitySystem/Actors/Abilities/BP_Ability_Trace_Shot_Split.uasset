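; Trace-based shot ability in the ability system that fires a single randomly deviated shot from the caster's aim.
; CastAbility refreshes shooting attributes and damage, then traces along the aim rotation with random pitch and yaw spread, ignoring specified actors, and checks any hit.
; ApplyHitDamageToActor scales randomized damage down with trace distance, clamped to a minimum fraction at long range, then applies it as critical-capable point damage.
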(event `/Game/BPS_Core/Blueprints/Systems/AbilitySystem/Actors/Abilities/BP_Ability_Base.CastAbility`
  (bind _returnvalue (`self.GetInstigator`))
  ;[1 1 1] Try to cast shot split ability.
  (`self.UpdateShootingAttributes`)
  (`self.CalculatePossibleDamage`)
  (bind (_success _startlocation _aimrotation) (`/Game/BPS_Core/Blueprints/Systems/AbilitySystem/Libraries/BP_Library_AbilitySystem.GetCasterAimVariables` _returnvalue))
  (if _success
    (bind _output_get (set `self.ActorsToIgnore` (`/Game/BPS_Core/Blueprints/Systems/CoreSystem/Libraries/BP_Library_CoreFunctions.GetActorsToIgnore` _returnvalue)))
    (bind (_hitresult _washit) (`self.TryShootTrace` _startlocation (`KismetMathLibrary.NormalizedDeltaRotator` _aimrotation (`KismetMathLibrary.MakeRotator` 0.0 (`KismetMathLibrary.RandomFloatInRange` -5.0 5.0) (`KismetMathLibrary.RandomFloatInRange` -5.0 5.0))) (`self.ShootingRange`) _output_get))
    (if _washit
      (`self.CheckHit` _hitresult))))

(fn `ApplyHitDamageToActor`
  (params (TargetActor :type "Actor Object Reference") (HitResult :type "HitResult Structure"))
  (returns (Success :type Boolean))
  (locals (LocalDistanceMultiplier :type "Float (double-precision)" :default 0.0))
  ;[1 1 1] Reduce damage by the distance to hit.
  (bind _output_get (set `local.LocalDistanceMultiplier` (`KismetMathLibrary.MapRangeClamped` (`/Game/BPS_Core/Blueprints/Systems/CoreSystem/Libraries/BP_Library_CoreFunctions.GetTraceDistance` HitResult) 400.0 1000.0 1.0 0.2)))
  (bind _damagedata (`/Game/BPS_Core/Blueprints/Systems/DamageSystem/Libraries/BP_Library_DamageSystem.MakeCommonDamageData` (* _output_get (`self.RandomizeDamage` (`self.ResultDamage`))) (`self.DamageType`) (`self.CriticalDamageMultiplier`)))
  (bind _success (`/Game/BPS_Core/Blueprints/Systems/DamageSystem/Libraries/BP_Library_DamageSystem.ApplyPointDamage` TargetActor _damagedata (`/Game/BPS_Core/Blueprints/Systems/CoreSystem/Libraries/BP_Library_CoreFunctions.GetHitFromDirection` HitResult) HitResult (`self.GetInstigatorController`) (`self.GetInstigator`)))
  (return _success))

(fn `UserConstructionScript`
  (`parent.UserConstructionScript`))