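; Status effect actor that changes its owner's health, energy, hunger and thirst over time.
; Attribute tags supply per-second rates, either directly or as overall amounts divided by Duration.
; On init it caches the owner's stat components, and each tick applies the rates scaled by delta time and stack count.
; The effect destroys itself when the owner has no valid health component or is not alive.
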(fn `InitStatusEffect`
  (returns (Success :type Boolean))
  ;[1 1 1] Init status effect and try to set stat components references.
  (bind _success (`parent.InitStatusEffect`))
  (`|ExecutionSequence`
    (:`then_0`
      (`|ExecutionSequence`
        (:`then_0`
          (bind (_found _component) (`/Game/BPS_Core/Blueprints/Systems/StatsSystem/Libraries/BP_Library_StatsSystem.FindHealthStatAttributeComponent` (`self.GetOwner`)))
          (if _found
            (set `self.HealthStatComponent` _component)))
        (:`then_1`
          (`|ExecutionSequence`
            (:`then_0`
              (if (or (!= (`self.EnergyPerSecond`) 0.0) (!= (`self.EnergyPerSecond%`) 0.0))
                (bind (_found_2 _component_2) (`/Game/BPS_Core/Blueprints/Systems/StatsSystem/Libraries/BP_Library_StatsSystem.FindEnergyStatAttributeComponent` (`self.GetOwner`)))
                (if _found_2
                  (set `self.EnergyStatComponent` _component_2))))
            (:`then_1`
              (`|ExecutionSequence`
                (:`then_0`
                  (if (or (!= (`self.HungerPerSecond`) 0.0) (!= (`self.HungerPerSecond%`) 0.0))
                    (bind (_found_3 _component_3) (`/Game/BPS_Core/Blueprints/Systems/StatsSystem/Libraries/BP_Library_StatsSystem.FindStatAttributeComponentByName` (`self.GetOwner`) "Hunger"))
                    (if _found_3
                      (set `self.HungerStatComponent` _component_3))))
                (:`then_1`
                  (if (or (!= (`self.ThirstPerSecond`) 0.0) (!= (`self.ThirstPerSecond%`) 0.0))
                    (bind (_found_4 _component_4) (`/Game/BPS_Core/Blueprints/Systems/StatsSystem/Libraries/BP_Library_StatsSystem.FindStatAttributeComponentByName` (`self.GetOwner`) "Thirst"))
                    (if _found_4
                      (set `self.ThirstStatComponent` _component_4))))))))))
    (:`then_1`
      (return _success))))

(fn `InitStatusEffectAttributes`
  (returns (Success :type Boolean))
  ;[1 1 1] Update change stats variables depending attributes.
  (bind _success (`parent.InitStatusEffectAttributes`))
  (if (`KismetArrayLibrary.Array_IsValidIndex` (`self.EffectAttributes`))
    (`|ExecutionSequence`
      (:`then_0`
        (`|ExecutionSequence`
          (:`then_0`
            (bind _success_2 (`/Game/BPS_Core/Blueprints/Systems/AttributesSystem/Libraries/BP_Library_Attributes.TrySetFloatVariableByAttribute` (`self.OverallHealth`) (`self.EffectAttributes`) (`self.OverallHealthAttributeTag`)))
            (if _success_2
              (set `self.HealthPerSecond` (/ (`self.OverallHealth`) (`self.Duration`)))
              (else
                (bind _success_3 (`/Game/BPS_Core/Blueprints/Systems/AttributesSystem/Libraries/BP_Library_Attributes.TrySetFloatVariableByAttribute` (`self.OverallHealth%`) (`self.EffectAttributes`) (`self.OverallHealth%AttributeTag`)))
                (if _success_3
                  (set `self.HealthPerSecond%` (/ (`self.OverallHealth%`) (`self.Duration`)))
                  (else
                    (bind _success_4 (`/Game/BPS_Core/Blueprints/Systems/AttributesSystem/Libraries/BP_Library_Attributes.TrySetFloatVariableByAttribute` (`self.HealthPerSecond`) (`self.EffectAttributes`) (`self.HealthPerSecondAttributeTag`)))
                    (if (not _success_4)
                      (`/Game/BPS_Core/Blueprints/Systems/AttributesSystem/Libraries/BP_Library_Attributes.TrySetFloatVariableByAttribute` (`self.HealthPerSecond%`) (`self.EffectAttributes`) (`self.HealthPerSecond%AttributeTag`))))))))
          (:`then_1`
            (`|ExecutionSequence`
              (:`then_0`
                (bind _success_5 (`/Game/BPS_Core/Blueprints/Systems/AttributesSystem/Libraries/BP_Library_Attributes.TrySetFloatVariableByAttribute` (`self.OverallEnergy`) (`self.EffectAttributes`) (`self.OverallEnergyAttributeTag`)))
                (if _success_5
                  (set `self.EnergyPerSecond` (/ (`self.OverallEnergy`) (`self.Duration`)))
                  (else
                    (bind _success_6 (`/Game/BPS_Core/Blueprints/Systems/AttributesSystem/Libraries/BP_Library_Attributes.TrySetFloatVariableByAttribute` (`self.OverallEnergy%`) (`self.EffectAttributes`) (`self.OverallEnergy%AttributeTag`)))
                    (if _success_6
                      (set `self.EnergyPerSecond%` (/ (`self.OverallEnergy%`) (`self.Duration`)))
                      (else
                        (bind _success_7 (`/Game/BPS_Core/Blueprints/Systems/AttributesSystem/Libraries/BP_Library_Attributes.TrySetFloatVariableByAttribute` (`self.EnergyPerSecond`) (`self.EffectAttributes`) (`self.EnergyPerSecondAttributeTag`)))
                        (if (not _success_7)
                          (`/Game/BPS_Core/Blueprints/Systems/AttributesSystem/Libraries/BP_Library_Attributes.TrySetFloatVariableByAttribute` (`self.EnergyPerSecond%`) (`self.EffectAttributes`) (`self.EnergyPerSecond%AttributeTag`))))))))
              (:`then_1`
                (`|ExecutionSequence`
                  (:`then_0`
                    (bind _success_8 (`/Game/BPS_Core/Blueprints/Systems/AttributesSystem/Libraries/BP_Library_Attributes.TrySetFloatVariableByAttribute` (`self.OverallHunger`) (`self.EffectAttributes`) (`self.OverallHungerAttributeTag`)))
                    (if _success_8
                      (set `self.HungerPerSecond` (/ (`self.OverallHunger`) (`self.Duration`)))
                      (else
                        (bind _success_9 (`/Game/BPS_Core/Blueprints/Systems/AttributesSystem/Libraries/BP_Library_Attributes.TrySetFloatVariableByAttribute` (`self.OverallHunger%`) (`self.EffectAttributes`) (`self.OverallHunger%AttributeTag`)))
                        (if _success_9
                          (set `self.HungerPerSecond%` (/ (`self.OverallHunger%`) (`self.Duration`)))
                          (else
                            (bind _success_10 (`/Game/BPS_Core/Blueprints/Systems/AttributesSystem/Libraries/BP_Library_Attributes.TrySetFloatVariableByAttribute` (`self.HungerPerSecond`) (`self.EffectAttributes`) (`self.HungerPerSecondAttributeTag`)))
                            (if (not _success_10)
                              (`/Game/BPS_Core/Blueprints/Systems/AttributesSystem/Libraries/BP_Library_Attributes.TrySetFloatVariableByAttribute` (`self.HungerPerSecond%`) (`self.EffectAttributes`) (`self.HungerPerSecond%AttributeTag`))))))))
                  (:`then_1`
                    (bind _success_11 (`/Game/BPS_Core/Blueprints/Systems/AttributesSystem/Libraries/BP_Library_Attributes.TrySetFloatVariableByAttribute` (`self.OverallThirst`) (`self.EffectAttributes`) (`self.OverallThirstAttributeTag`)))
                    (if _success_11
                      (set `self.ThirstPerSecond` (/ (`self.OverallThirst`) (`self.Duration`)))
                      (else
                        (bind _success_12 (`/Game/BPS_Core/Blueprints/Systems/AttributesSystem/Libraries/BP_Library_Attributes.TrySetFloatVariableByAttribute` (`self.OverallThirst%`) (`self.EffectAttributes`) (`self.OverallThirst%AttributeTag`)))
                        (if _success_12
                          (set `self.ThirstPerSecond%` (/ (`self.OverallThirst%`) (`self.Duration`)))
                          (else
                            (bind _success_13 (`/Game/BPS_Core/Blueprints/Systems/AttributesSystem/Libraries/BP_Library_Attributes.TrySetFloatVariableByAttribute` (`self.ThirstPerSecond`) (`self.EffectAttributes`) (`self.ThirstPerSecondAttributeTag`)))
                            (if (not _success_13)
                              (`/Game/BPS_Core/Blueprints/Systems/AttributesSystem/Libraries/BP_Library_Attributes.TrySetFloatVariableByAttribute` (`self.ThirstPerSecond%`) (`self.EffectAttributes`) (`self.ThirstPerSecond%AttributeTag`))))))))))))))
      (:`then_1`
        (return _success)))))

(fn `TickActions`
  (params (DeltaSeconds :type "Float (double-precision)"))
  (returns (Success :type Boolean))
  (locals (LocalDeltaSeconds :type "Float (double-precision)" :default 0.0))
  (bind _healthstatcomponent (`self.HealthStatComponent`))
  (bind _thirststatcomponent (`self.ThirstStatComponent`))
  (bind _energystatcomponent (`self.EnergyStatComponent`))
  (bind _energypersecond (`self.EnergyPerSecond`))
  (bind _energypersecond_ (`self.EnergyPerSecond%`))
  (bind _hungerstatcomponent (`self.HungerStatComponent`))
  (bind _hungerpersecond (`self.HungerPerSecond`))
  (bind _thirstpersecond (`self.ThirstPerSecond`))
  (bind _hungerpersecond_ (`self.HungerPerSecond%`))
  (bind _thirstpersecond_ (`self.ThirstPerSecond%`))
  (bind _healthstatcomponent_2 (`self.HealthStatComponent`))
  (bind _healthpersecond (`self.HealthPerSecond`))
  (bind _healthpersecond_ (`self.HealthPerSecond%`))
  (bind _returnvalue (!= _healthpersecond_ 0.0))
  (bind _returnvalue_2 (!= _thirstpersecond_ 0.0))
  (bind _returnvalue_3 (!= _hungerpersecond_ 0.0))
  (bind _returnvalue_4 (!= _energypersecond_ 0.0))
  ;[1 1 1] Try to change stats of the owner depending status effect variables.
  (set `local.LocalDeltaSeconds` DeltaSeconds)
  (`/Engine/EditorBlueprintResources/StandardMacros.IsValid` _healthstatcomponent
    (:`Is Valid`
      (if (`/Game/BPS_Core/Blueprints/Systems/StatsSystem/Components/BP_AC_StatAttribute_Health.IsAlive` _healthstatcomponent)
        (`|ExecutionSequence`
          (:`then_0`
            (`|ExecutionSequence`
              (:`then_0`
                (if (or (!= _healthpersecond 0.0) (!= _healthpersecond_ 0.0))
                  (`/Engine/EditorBlueprintResources/StandardMacros.IsValid` _healthstatcomponent_2
                    (:`Is Valid`
                      (`/Game/BPS_Core/Blueprints/Systems/StatsSystem/Components/BP_AC_StatAttribute.ChangeCurrentValue` _healthstatcomponent_2 "NewEnumerator0" (* (`local.LocalDeltaSeconds`) (select `bool` _returnvalue :`false` _healthpersecond :`true` _healthpersecond_) (`KismetMathLibrary.Conv_IntToDouble` (`self.Stack`))) _returnvalue)))))
              (:`then_1`
                (`|ExecutionSequence`
                  (:`then_0`
                    (if (or (!= _energypersecond 0.0) (!= _energypersecond_ 0.0))
                      (`/Engine/EditorBlueprintResources/StandardMacros.IsValid` _energystatcomponent
                        (:`Is Valid`
                          (`/Game/BPS_Core/Blueprints/Systems/StatsSystem/Components/BP_AC_StatAttribute.ChangeCurrentValue` _energystatcomponent "NewEnumerator0" (* (`local.LocalDeltaSeconds`) (select `bool` _returnvalue_4 :`false` _energypersecond :`true` _energypersecond_) (`KismetMathLibrary.Conv_IntToDouble` (`self.Stack`))) _returnvalue_4)))))
                  (:`then_1`
                    (`|ExecutionSequence`
                      (:`then_0`
                        (if (or (!= _hungerpersecond 0.0) (!= _hungerpersecond_ 0.0))
                          (`/Engine/EditorBlueprintResources/StandardMacros.IsValid` _hungerstatcomponent
                            (:`Is Valid`
                              (`/Game/BPS_Core/Blueprints/Systems/StatsSystem/Components/BP_AC_StatAttribute.ChangeCurrentValue` _hungerstatcomponent "NewEnumerator0" (* (`local.LocalDeltaSeconds`) (select `bool` _returnvalue_3 :`false` _hungerpersecond :`true` _hungerpersecond_) (`KismetMathLibrary.Conv_IntToDouble` (`self.Stack`))) _returnvalue_3)))))
                      (:`then_1`
                        (if (or (!= _thirstpersecond 0.0) (!= _thirstpersecond_ 0.0))
                          (`/Engine/EditorBlueprintResources/StandardMacros.IsValid` _thirststatcomponent
                            (:`Is Valid`
                              (`/Game/BPS_Core/Blueprints/Systems/StatsSystem/Components/BP_AC_StatAttribute.ChangeCurrentValue` _thirststatcomponent "NewEnumerator0" (* (`local.LocalDeltaSeconds`) (select `bool` _returnvalue_2 :`false` _thirstpersecond :`true` _thirstpersecond_) (`KismetMathLibrary.Conv_IntToDouble` (`self.Stack`))) _returnvalue_2)))))))))))
          (:`then_1`
            (return true)))
        (else
          (`self.K2_DestroyActor` :!label _label)
          (return true))))
    (:`Is Not Valid`
      (goto _label))))

(fn `UserConstructionScript`
  (`parent.UserConstructionScript`))