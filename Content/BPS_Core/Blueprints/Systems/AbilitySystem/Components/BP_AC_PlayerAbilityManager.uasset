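; Player ability manager component that relays status effect changes from a target ability manager to the client.
; Bind functions register local listeners and call server events that subscribe to the target's added, updated and removed events.
; Server handlers send status effect data through client events, which fire local dispatchers.
; Binding all events together also replays currently active effects as additions, while the single-event binds skip this sync.
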(event `BindStatusEffectEvents (Server)`
  (params (AbilityManager :type "/Game/BPS_Core/Blueprints/Systems/AbilitySystem/Components/BP_AC_AbilityManager Object Reference"))
  ;[1 1 1] Status effect management events.
  (`self.UpdateStatusEffectsData` AbilityManager)
  (add `/Game/BPS_Core/Blueprints/Systems/AbilitySystem/Components/BP_AC_AbilityManager.OnStatusEffectAdded` AbilityManager (`|CreateDelegate` :!event `Bind_OnStatusEffectAdded`))
  (add `/Game/BPS_Core/Blueprints/Systems/AbilitySystem/Components/BP_AC_AbilityManager.OnStatusEffectRemoved` AbilityManager (`|CreateDelegate` :!event `Bind_OnStatusEffectRemoved`))
  (add `/Game/BPS_Core/Blueprints/Systems/AbilitySystem/Components/BP_AC_AbilityManager.OnStatusEffectUpdated` AbilityManager (`|CreateDelegate` :!event `Bind_OnStatusEffectUpdated`)))

(event `BindStatusEffectAddedEvent (Server)`
  (params (AbilityManager :type "/Game/BPS_Core/Blueprints/Systems/AbilitySystem/Components/BP_AC_AbilityManager Object Reference"))
  ;[1 1 1] Status effect management events.
  (add `/Game/BPS_Core/Blueprints/Systems/AbilitySystem/Components/BP_AC_AbilityManager.OnStatusEffectAdded` AbilityManager (`|CreateDelegate` :!event `Bind_OnStatusEffectAdded`)))

(event `BindStatusEffectUpdatedEvent (Server)`
  (params (AbilityManager :type "/Game/BPS_Core/Blueprints/Systems/AbilitySystem/Components/BP_AC_AbilityManager Object Reference"))
  ;[1 1 1] Status effect management events.
  (add `/Game/BPS_Core/Blueprints/Systems/AbilitySystem/Components/BP_AC_AbilityManager.OnStatusEffectUpdated` AbilityManager (`|CreateDelegate` :!event `Bind_OnStatusEffectUpdated`)))

(event `BindStatusEffectRemovedEvent (Server)`
  (params (AbilityManager :type "/Game/BPS_Core/Blueprints/Systems/AbilitySystem/Components/BP_AC_AbilityManager Object Reference"))
  ;[1 1 1] Status effect management events.
  (add `/Game/BPS_Core/Blueprints/Systems/AbilitySystem/Components/BP_AC_AbilityManager.OnStatusEffectRemoved` AbilityManager (`|CreateDelegate` :!event `Bind_OnStatusEffectRemoved`)))

(event `Bind_OnStatusEffectAdded`
  (params (AbilityManager :type "/Game/BPS_Core/Blueprints/Systems/AbilitySystem/Components/BP_AC_AbilityManager Object Reference") (StatusEffect :type "/Game/BPS_Core/Blueprints/Systems/AbilitySystem/Actors/StatusEffects/BP_StatusEffect_Base Object Reference"))
  ;[1 1 1] Status effect management events.
  (`self.StatusEffectDataAdded (Client)` AbilityManager (`/Game/BPS_Core/Blueprints/Systems/AbilitySystem/Actors/StatusEffects/BP_StatusEffect_Base.GetStatusEffectData` StatusEffect)))

(event `Bind_OnStatusEffectUpdated`
  (params (AbilityManager :type "/Game/BPS_Core/Blueprints/Systems/AbilitySystem/Components/BP_AC_AbilityManager Object Reference") (StatusEffect :type "/Game/BPS_Core/Blueprints/Systems/AbilitySystem/Actors/StatusEffects/BP_StatusEffect_Base Object Reference"))
  ;[1 1 1] Status effect management events.
  (`self.StatusEffectDataUpdated (Client)` AbilityManager (`/Game/BPS_Core/Blueprints/Systems/AbilitySystem/Actors/StatusEffects/BP_StatusEffect_Base.GetStatusEffectData` StatusEffect)))

(event `Bind_OnStatusEffectRemoved`
  (params (AbilityManager :type "/Game/BPS_Core/Blueprints/Systems/AbilitySystem/Components/BP_AC_AbilityManager Object Reference") (StatusEffect :type "/Game/BPS_Core/Blueprints/Systems/AbilitySystem/Actors/StatusEffects/BP_StatusEffect_Base Object Reference"))
  ;[1 1 1] Status effect management events.
  (`self.StatusEffectDataRemoved (Client)` AbilityManager (`/Game/BPS_Core/Blueprints/Systems/AbilitySystem/Actors/StatusEffects/BP_StatusEffect_Base.GetStatusEffectData` StatusEffect)))

(event `StatusEffectDataAdded (Client)`
  (params (AbilityManager :type "/Game/BPS_Core/Blueprints/Systems/AbilitySystem/Components/BP_AC_AbilityManager Object Reference") (StatusEffectData :type "/Game/BPS_Core/Blueprints/Systems/AbilitySystem/Structures/STR_StatusEffectData Structure"))
  ;[1 1 1] Status effect management events.
  (`self.OnStatusEffectDataAdded` AbilityManager StatusEffectData))

(event `StatusEffectDataUpdated (Client)`
  (params (AbilityManager :type "/Game/BPS_Core/Blueprints/Systems/AbilitySystem/Components/BP_AC_AbilityManager Object Reference") (StatusEffectData :type "/Game/BPS_Core/Blueprints/Systems/AbilitySystem/Structures/STR_StatusEffectData Structure"))
  ;[1 1 1] Status effect management events.
  (`self.OnStatusEffectDataUpdated` AbilityManager StatusEffectData))

(event `StatusEffectDataRemoved (Client)`
  (params (AbilityManager :type "/Game/BPS_Core/Blueprints/Systems/AbilitySystem/Components/BP_AC_AbilityManager Object Reference") (StatusEffectData :type "/Game/BPS_Core/Blueprints/Systems/AbilitySystem/Structures/STR_StatusEffectData Structure"))
  ;[1 1 1] Status effect management events.
  (`self.OnStatusEffectDataRemoved` AbilityManager StatusEffectData))

(fn `BindStatusEffectAddedEvent`
  (params (AbilityManager :type "/Game/BPS_Core/Blueprints/Systems/AbilitySystem/Components/BP_AC_AbilityManager Object Reference") (OnAddedEvent :type "Delegate (by ref)"))
  (returns (Success :type Boolean))
  ;[1 1 1] Bind status effect added event of target ability manager.
  (`self.BindStatusEffectAddedEvent (Server)` AbilityManager)
  (add `self.OnStatusEffectDataAdded` OnAddedEvent)
  (return true))

(fn `BindStatusEffectEvents`
  (params (AbilityManager :type "/Game/BPS_Core/Blueprints/Systems/AbilitySystem/Components/BP_AC_AbilityManager Object Reference") (OnAddedEvent :type "Delegate (by ref)") (OnRemovedEvent :type "Delegate (by ref)") (OnUpdatedEvent :type "Delegate (by ref)"))
  (returns (Success :type Boolean))
  ;[1 1 1] Bind status effect events of target ability manager.
  (`self.BindStatusEffectEvents (Server)` AbilityManager)
  (add `self.OnStatusEffectDataAdded` OnAddedEvent)
  (add `self.OnStatusEffectDataRemoved` OnRemovedEvent)
  (add `self.OnStatusEffectDataUpdated` OnUpdatedEvent)
  (return true))

(fn `BindStatusEffectRemovedEvent`
  (params (AbilityManager :type "/Game/BPS_Core/Blueprints/Systems/AbilitySystem/Components/BP_AC_AbilityManager Object Reference") (OnRemovedEvent :type "Delegate (by ref)"))
  (returns (Success :type Boolean))
  ;[1 1 1] Bind status effect removed event of target ability manager.
  (`self.BindStatusEffectRemovedEvent (Server)` AbilityManager)
  (add `self.OnStatusEffectDataRemoved` OnRemovedEvent)
  (return true))

(fn `BindStatusEffectUpdatedEvent`
  (params (AbilityManager :type "/Game/BPS_Core/Blueprints/Systems/AbilitySystem/Components/BP_AC_AbilityManager Object Reference") (OnRemovedEvent :type "Delegate (by ref)"))
  (returns (Success :type Boolean))
  ;[1 1 1] Bind status effect updated event of target ability manager.
  (`self.BindStatusEffectUpdatedEvent (Server)` AbilityManager)
  (add `self.OnStatusEffectDataUpdated` OnRemovedEvent)
  (return true))

(fn `UpdateStatusEffectsData`
  (params (AbilityManager :type "/Game/BPS_Core/Blueprints/Systems/AbilitySystem/Components/BP_AC_AbilityManager Object Reference"))
  (returns (Success :type Boolean))
  (locals (LocalAbilityManager :type "/Game/BPS_Core/Blueprints/Systems/AbilitySystem/Components/BP_AC_AbilityManager Object Reference") (LocalStatusEffectData :type "Array of /Game/BPS_Core/Blueprints/Systems/AbilitySystem/Structures/STR_StatusEffectData Structure"))
  ;[1 1 1] Update status effects data of target ability manager for the client.
  (set `local.LocalAbilityManager` AbilityManager)
  (bind _output_get (set `local.LocalStatusEffectData` (`/Game/BPS_Core/Blueprints/Systems/AbilitySystem/Components/BP_AC_AbilityManager.GetActiveStatusEffectsData` AbilityManager)))
  (for _array_element _output_get
    (`self.StatusEffectDataAdded (Client)` (`local.LocalAbilityManager`) _array_element))
  (return true))