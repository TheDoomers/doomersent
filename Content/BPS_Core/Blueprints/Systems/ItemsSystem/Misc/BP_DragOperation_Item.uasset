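; Drag operation for inventory items, carrying source and target container slot data during a drag and drop.
; It relays drag start, cancel, enter, pre-drop and drop to global item drag events.
; Enter and pre-drop checks record the target widget and report whether listeners left them unhandled, via handled flags and types.
; Helpers resolve source and target slots from item size and grab offsets, supporting single-slot and multi-cell containers.
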(event `DragStarted`
  ;[1 1 1] Drag item events.
  (`self.OnItemDragStarted` self))

(event `self.DragCancelled`
  (params (PointerEvent :type "PointerEvent Structure (by ref)"))
  ;[1 1 1] Drag item events.
  (`self.OnItemDragCancelled` self))

(event `DragEnteredWidget`
  ;[1 1 1] Drag item events.
  (`self.OnItemDragEntered` self (`self.TargetWidget`)))

(event `self.Drop`
  (params (PointerEvent :type "PointerEvent Structure (by ref)"))
  ;[1 1 1] Drag item events.
  (`self.OnItemDragDropped` self (`self.TargetWidget`)))

(event `PreDropChecked`
  ;[1 1 1] Drag item events.
  (`self.OnItemDragPreDropped` self (`self.TargetWidget`)))

(fn `ClearTargetContainerSlot`
  (returns (Success :type Boolean))
  ;[1 1 1] Clear target container slot variables.
  (set `self.TargetContainer` null)
  (return true))

(fn `EnterWidget`
  (params (TargetWidget :type "UserWidget Object Reference"))
  (returns (IsNotHandled :type Boolean))
  ;[1 1 1] Calls the item drag entered event.
  (set `self.TargetWidget` TargetWidget)
  (`self.DragEnteredWidget`)
  (return (not (`self.EnterIsHandled`))))

(fn `GetFromSlots`
  (returns (Success :type Boolean) (FromSlots :type "Array of Integer"))
  (bind ((`SizeX_79_C6254F1744F2868A1546F0A15D5923A6` _sizex) (`SizeY_80_BFD867AB4ECDE5D200B6F3BB91506129` _sizey)) (break `/Game/BPS_Core/Blueprints/Systems/ItemsSystem/Structures/STR_ItemInstance` (`.ItemInstance_5_2012745D42F44D65DB4D5E9C2D7A90BD` (break `/Game/BPS_Core/Blueprints/Systems/ItemsSystem/Structures/STR_ItemData` (`self.ItemData`)))))
  ;[1 1 1] Returns slots that are taken by the dragged item.
  (bind (_success _containerslots) (`/Game/BPS_Core/Blueprints/Systems/ItemsSystem/Components/BP_AC_ContainerComponent.GetContainerSlotsBySizeForMainSlot` (`self.FromContainer`) (`self.FromSlotIndex`) _sizey _sizex))
  (return _success _containerslots))

(fn `GetTargetAndMainSlots`
  (returns (TargetContainer :type "/Game/BPS_Core/Blueprints/Systems/ItemsSystem/Components/BP_AC_ContainerComponent Object Reference") (TargetSlotIndex :type Integer) (MainSlotIndex :type Integer))
  (bind _targetslotindex (`self.TargetSlotIndex`))
  (bind _targetcontainer (`self.TargetContainer`))
  ;[1 1 1] Returns target and main slots for the dragged item.
  (`/Engine/EditorBlueprintResources/StandardMacros.IsValid` _targetcontainer
    (:`Is Valid`
      (if (`/Game/BPS_Core/Blueprints/Systems/ItemsSystem/Components/BP_AC_ContainerComponent.UseSingleSlots` _targetcontainer)
        (return (`self.TargetContainer`) _targetslotindex _targetslotindex)
        (else
          (return (`self.TargetContainer`) (`self.TargetSlotIndex`) (`/Game/BPS_Core/Blueprints/Systems/ItemsSystem/Components/BP_AC_ContainerComponent.GetMainSlotIndexByOffsets` _targetcontainer (`self.TargetSlotIndex`) (`self.RowOffset`) (`self.ColumnOffset`))))))
    (:`Is Not Valid`
      (return null 0 0))))

(fn `GetTargetSlots`
  (returns (Success :type Boolean) (TargetSlots :type "Array of Integer"))
  (bind _targetcontainer (`self.TargetContainer`))
  (bind ((`SizeX_79_C6254F1744F2868A1546F0A15D5923A6` _sizex) (`SizeY_80_BFD867AB4ECDE5D200B6F3BB91506129` _sizey)) (break `/Game/BPS_Core/Blueprints/Systems/ItemsSystem/Structures/STR_ItemInstance` (`.ItemInstance_5_2012745D42F44D65DB4D5E9C2D7A90BD` (break `/Game/BPS_Core/Blueprints/Systems/ItemsSystem/Structures/STR_ItemData` (`self.ItemData`)))))
  ;[1 1 1] Returns target slots for the dragged item.
  (`/Engine/EditorBlueprintResources/StandardMacros.IsValid` _targetcontainer
    (:`Is Valid`
      (bind (_success _containerslots) (`/Game/BPS_Core/Blueprints/Systems/ItemsSystem/Components/BP_AC_ContainerComponent.GetContainerSlotsBySize` _targetcontainer (+ (* (`self.RowOffset`) -1) (`self.TargetRowIndex`)) (+ (* (`self.ColumnOffset`) -1) (`self.TargetColumnIndex`)) _sizey _sizex))
      (return _success _containerslots))
    (:`Is Not Valid`
      (return false))))

(fn `HandleDrop`
  (params (IsHandled :type Boolean) (HandleType :type Name))
  (returns (Success :type Boolean))
  ;[1 1 1] Update variables which indicate that the drop item event is handled.
  (set `self.DropIsHandled` IsHandled)
  (set `self.DropHandleType` HandleType)
  (return true))

(fn `HandleEnter`
  (params (IsHandled :type Boolean) (HandleType :type Name))
  (returns (Success :type Boolean))
  ;[1 1 1] Update variables which indicate that the enter widget event is handled.
  (set `self.EnterIsHandled` IsHandled)
  (set `self.EnterHandleType` HandleType)
  (return true))

(fn `PreDropCheck`
  (params (TargetWidget :type "UserWidget Object Reference"))
  (returns (IsNotHandled :type Boolean))
  ;[1 1 1] Call the item drag pre dropped event.
  (set `self.TargetWidget` TargetWidget)
  (`self.PreDropChecked`)
  (return (not (`self.DropIsHandled`))))

(fn `SetTargetContainerSlot`
  (params (TargetContainer :type "/Game/BPS_Core/Blueprints/Systems/ItemsSystem/Components/BP_AC_ContainerComponent Object Reference") (TargetSlotIndex :type Integer) (TargetRowIndex :type Integer) (TargetColumnIndex :type Integer))
  (returns (Success :type Boolean))
  ;[1 1 1] Set target container slot variables.
  (set `self.TargetContainer` TargetContainer)
  (set `self.TargetSlotIndex` TargetSlotIndex)
  (set `self.TargetRowIndex` TargetRowIndex)
  (set `self.TargetColumnIndex` TargetColumnIndex)
  (return true))

(fn `StartDragOperation`
  (returns (Success :type Boolean))
  ;[1 1 1] Calls the item drag started event.
  (set `self.TargetContainer` (`self.FromContainer`))
  (`self.DragStarted`)
  (return true))