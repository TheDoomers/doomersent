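; Base actor for an item lying in the world, holding its stack data and handling pickup, impact sounds and save/load.
; The item handle resolves to an instance that clamps stats and supplies the mesh, async-loaded at runtime.
; For finite physics items, authority timers either decay the stack unit by unit, spawning decay items, or trigger a timed event.
; A level-wide utility refreshes items and flags or respawns wrong classes.
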(event `self.ReceiveBeginPlay`
  ;[1 1 1] Begin play. Destroy world item after some time.
  (`self.InitWorldItemSettings`)
  (`/Engine/EditorBlueprintResources/ActorMacros.Switch Has Authority`
    (:`Authority`
      (`self.CheckAndStartTimers`))))

(event `UpdateSimulatePhysicsDelayed`
  ;[1 1 1] Begin play. Destroy world item after some time.
  (`KismetSystemLibrary.RetriggerableDelay` 0.0)
  (`self.UpdatePhysicsSimulation`))

(event `CheckAndStartTimers`
  ;[1 1 1] Begin play. Destroy world item after some time.
  (if (and (`self.SimulatePhysics`) (not (`self.InfiniteItem`)))
    (if (> (`self.Decay`) 0.0)
      (bind _returnvalue (`KismetSystemLibrary.K2_SetTimerDelegate` (`|CreateDelegate` :!event `DecayTick`) (`self.Decay`)))
      (set `self.DecayTimer` _returnvalue)
      (else
        (`KismetSystemLibrary.K2_SetTimerDelegate` (`|CreateDelegate` :!event `DestroyWorldItem`) (`self.DestroyTime`))))))

(event `self.StaticMesh.OnComponentHit`
  (params (HitComponent :type "PrimitiveComponent Object Reference") (OtherActor :type "Actor Object Reference") (OtherComp :type "PrimitiveComponent Object Reference") (NormalImpulse :type "Vector Structure") (Hit :type "HitResult Structure (by ref)"))
  ;[1 1 1] Play drop sound.
  (if (`self.SimulatePhysics`)
    (if (`SceneComponent.IsSimulatingPhysics` HitComponent "None")
      (if (>= (/ (`KismetMathLibrary.VSize` NormalImpulse) (`PrimitiveComponent.GetMass` HitComponent)) 100.0)
        (`self.PlayDropSound` Hit)))))

(event `self.SaveObjectComponent.OnSaveData`
  (params (Component :type "/Game/BPS_Core/Blueprints/Systems/SaveLoadSystem/Components/BP_AC_SaveObjectComponent Object Reference") (SaveGame :type "SaveGame Object Reference"))
  ;[1 1 1] Save and load events.
  (bind _saveid (`/Game/BPS_Core/Blueprints/Systems/SaveLoadSystem/Components/BP_AC_SaveObjectComponent.GetSaveID` Component))
  (`/Game/BPS_Core/Blueprints/Systems/SaveLoadSystem/Components/BP_AC_SaveObjectComponent.SaveActorDataAdvanced` Component SaveGame (`GameplayStatics.GetObjectClass` self) (`SceneComponent.K2_GetComponentToWorld` (`self.StaticMesh`)))
  (message `/Game/BPS_Core/Blueprints/Systems/ItemsSystem/Interfaces/BPI_SaveGame_ItemsSystem.SetWorldItemSaveData_BPI` SaveGame _saveid (make `/Game/BPS_Core/Blueprints/Systems/ItemsSystem/Structures/STR_SaveData_WorldItem` (`self.ItemHandle`) (`self.Amount`) (`self.Charges`) (`self.Durability`) (`self.GetDecayTime`) (`self.Options`) (`self.Bonuses`) (`self.ContainerItems`))))

(event `self.SaveObjectComponent.OnLoadData`
  (params (Component :type "/Game/BPS_Core/Blueprints/Systems/SaveLoadSystem/Components/BP_AC_SaveObjectComponent Object Reference") (SaveGame :type "SaveGame Object Reference"))
  ;[1 1 1] Save and load events.
  (bind _saveid (`/Game/BPS_Core/Blueprints/Systems/SaveLoadSystem/Components/BP_AC_SaveObjectComponent.GetSaveID` Component))
  (bind (_success _savedata) (message `/Game/BPS_Core/Blueprints/Systems/ItemsSystem/Interfaces/BPI_SaveGame_ItemsSystem.GetWorldItemSaveData_BPI` SaveGame _saveid))
  (if _success
    (bind (_itemhandle _amount _charges _durability _decay _options _bonuses _containeritems) (break `/Game/BPS_Core/Blueprints/Systems/ItemsSystem/Structures/STR_SaveData_WorldItem` _savedata))
    (set `self.ItemHandle` _itemhandle)
    (set `self.Amount` _amount)
    (set `self.Charges` _charges)
    (set `self.Durability` _durability)
    (set `self.Decay` _decay)
    (set `self.Options` _options)
    (set `self.Bonuses` _bonuses)
    (set `self.ContainerItems` _containeritems)
    (`self.InitWorldItemSettings`)
    (`self.UpdateWorldItemMesh`)
    (`self.CheckAndStartTimers`)))

(fn `Bind_OnStaticMeshLoaded`
  (params (StaticMesh :type "StaticMesh Object Reference"))
  ;[1 1 1] Update static mesh on load and update physics simulation.
  (`StaticMeshComponent.SetStaticMesh` (`self.StaticMesh`) StaticMesh)
  (`self.UpdateSimulatePhysicsDelayed`))

(fn `CheckAndRefreshWorldItems`
  (locals (LocalWorldItemClass :type "/Game/BPS_Core/Blueprints/Systems/ItemsSystem/Actors/BP_WorldItem_Base Class Reference"))
  (bind _defaultworlditemclass (`self.DefaultWorldItemClass`))
  ;[1 1 1] Refresh settings for all world items on the level.
  (set `self.WrongWorldItem` null)
  (bind _outactors (`GameplayStatics.GetAllActorsOfClass` "BP_WorldItem_Base_C"))
  (for _array_element _outactors
    (`self.InitWorldItemSettings` _array_element)
    (bind (_isdefaultclass _worlditemclass) (`/Game/BPS_Core/Blueprints/Systems/ItemsSystem/Libraries/BP_Library_ItemsSystem.FindWorldItemClass` (`self.GetWorldItemData` _array_element) _defaultworlditemclass))
    (if (!= _defaultworlditemclass (`GameplayStatics.GetObjectClass` _array_element))
      (set `self.WrongWorldItem` _array_element)
      (if (`self.NeedRespawnItems`)
        (if _isdefaultclass
          (bind _output_get (set `local.LocalWorldItemClass` (`self.DefaultWorldItemClass`)))
          (else
            (set `local.LocalWorldItemClass` _worlditemclass)))
        (bind (_itemhandle _amount _charges _durability _decay _options _bonuses _containeritems) (break `/Game/BPS_Core/Blueprints/Systems/ItemsSystem/Structures/STR_ContainerItemData` (`/Game/BPS_Core/Blueprints/Systems/ItemsSystem/Libraries/BP_Library_ItemsSystem.GetContainerItemData` (`self.GetWorldItemData` _array_element))))
        (bind _returnvalue (`|SpawnActorFromClass` _output_get (`self.GetTransform` _array_element) "AdjustIfPossibleButAlwaysSpawn" "SelectDefaultAtRuntime" null _itemhandle _amount _charges _durability _decay _options _bonuses _containeritems (`/Game/BPS_Core/Blueprints/Systems/ItemsSystem/Actors/BP_WorldItem_Base.SimulatePhysics` _array_element) (`/Game/BPS_Core/Blueprints/Systems/ItemsSystem/Actors/BP_WorldItem_Base.InfiniteItem` _array_element) null))
        (`/Engine/EditorBlueprintResources/StandardMacros.IsValid` _returnvalue
          (:`Is Valid`
            (`self.K2_DestroyActor` _array_element)))
        (else
          (`KismetSystemLibrary.PrintText` (`|FormatText` "Check world item class of the {DisplayName}!" _array_element) true true (struct :`R` 1.0 :`A` 1.0) 30.0)
          (return)))))
  (if (not (`KismetSystemLibrary.IsValid` (`self.WrongWorldItem`)))
    (`KismetSystemLibrary.PrintText` "All world items were refreshed!" true true (struct :`G` 1.0 :`A` 1.0) 30.0)))

(fn `DecayTick`
  ;[1 1 1] Spawn decay item and destroy world item if required.
  (bind _output_get (set `self.Amount` (- (stale _output_get) 1)))
  (`|ExecutionSequence`
    (:`then_0`
      (bind (_handlefound _specifichandle) (`/Game/BPS_Core/Blueprints/Systems/ItemsSystem/Libraries/BP_Library_ItemsSystem.FindItemSpecificHandle` (`self.GetWorldItemData`) "DecayItem"))
      (if _handlefound
        (`/Game/BPS_Core/Blueprints/Systems/ItemsSystem/Libraries/BP_Library_ItemsSystem.SpawnWorldItemByData` (make `/Game/BPS_Core/Blueprints/Systems/ItemsSystem/Structures/STR_ContainerItemData` :`ItemHandle` _specifichandle :`Amount` 1) (`self.K2_GetActorLocation`))))
    (:`then_1`
      (`|ExecutionSequence`
        (:`then_0`
          (if (<= (`self.Amount`) 0)
            (`self.K2_DestroyActor`)))
        (:`then_1`
          (bind _returnvalue (`KismetSystemLibrary.K2_SetTimerDelegate` (`|CreateDelegate` :!event `DecayTick`) (`.DecayTime_23_874E41914012913BB7E3DDA9244F8D23` (break `/Game/BPS_Core/Blueprints/Systems/ItemsSystem/Structures/STR_ItemInstance` (`self.ItemInstance`)))))
          (set `self.DecayTimer` _returnvalue))))))

(fn `DestroyWorldItem`
  ;[1 1 1] Destroy world item.
  (`self.K2_DestroyActor`))

(fn `GetDecayTime`
  (returns (DecayTime :type "Float (double-precision)"))
  (bind _decaytimer (`self.DecayTimer`))
  ;[1 1 1] Returns current decay time of the item.
  (return (select `bool` (`KismetSystemLibrary.K2_IsValidTimerHandle` _decaytimer) :`false` (`self.Decay`) :`true` (`KismetSystemLibrary.K2_GetTimerRemainingTimeHandle` _decaytimer) :!type "Float (double-precision)")))

(fn `GetSaveObjectComponent_BPI`
  (returns (Success :type Boolean) (Component :type "/Game/BPS_Core/Blueprints/Systems/SaveLoadSystem/Components/BP_AC_SaveObjectComponent Object Reference"))
  ;[1 1 1] Returns save object component reference.
  (return true (`self.SaveObjectComponent`)))

(fn `GetWorldItemData`
  (returns (ItemData :type "/Game/BPS_Core/Blueprints/Systems/ItemsSystem/Structures/STR_ItemData Structure"))
  (bind _itemhandle (`self.ItemHandle`))
  ;[1 1 1] Returns current item data of the item.
  (bind (_success _iteminstance) (`/Game/BPS_Core/Blueprints/Systems/ItemsSystem/Libraries/BP_Library_ItemsSystem.MakeItemInstance` _itemhandle))
  (set `self.ItemInstance` _iteminstance)
  (return (make `/Game/BPS_Core/Blueprints/Systems/ItemsSystem/Structures/STR_ItemData` (make `/Game/BPS_Core/Blueprints/Systems/ItemsSystem/Structures/STR_ContainerItemData` _itemhandle (`self.Amount`) (`self.Charges`) (`self.Durability`) (`self.GetDecayTime`) (`self.Options`) (`self.Bonuses`) (`self.ContainerItems`)) _iteminstance)))

(fn `GetWorldItemLocation`
  (returns (ReturnValue :type "Vector Structure"))
  ;[1 1 1] Returns location of static mesh of the world item.
  (return (`SceneComponent.K2_GetComponentLocation` (`self.StaticMesh`))))

(fn `InitWorldItemSettings`
  (returns (Success :type Boolean))
  (bind _charges (`self.Charges`))
  (bind _amount (`self.Amount`))
  (bind _durability (`self.Durability`))
  (bind _decay (`self.Decay`))
  (bind ((`SizeX_79_C6254F1744F2868A1546F0A15D5923A6` _sizex) (`SizeY_80_BFD867AB4ECDE5D200B6F3BB91506129` _sizey) (`DecayTime_23_874E41914012913BB7E3DDA9244F8D23` _decaytime)) (break `/Game/BPS_Core/Blueprints/Systems/ItemsSystem/Structures/STR_ItemInstance` (`self.ItemInstance`)))
  (bind ((`SizeX_79_C6254F1744F2868A1546F0A15D5923A6` _sizex_2) (`SizeY_80_BFD867AB4ECDE5D200B6F3BB91506129` _sizey_2) (`MaxStack_16_34001C214490CFB1617C38BF8677A56A` _maxstack)) (break `/Game/BPS_Core/Blueprints/Systems/ItemsSystem/Structures/STR_ItemInstance` (`self.ItemInstance`)))
  (bind ((`SizeX_79_C6254F1744F2868A1546F0A15D5923A6` _sizex_3) (`SizeY_80_BFD867AB4ECDE5D200B6F3BB91506129` _sizey_3) (`MaxCharges_18_9318245D452FAEA5F486409F430BD29A` _maxcharges)) (break `/Game/BPS_Core/Blueprints/Systems/ItemsSystem/Structures/STR_ItemInstance` (`self.ItemInstance`)))
  (bind ((`SizeX_79_C6254F1744F2868A1546F0A15D5923A6` _sizex_4) (`SizeY_80_BFD867AB4ECDE5D200B6F3BB91506129` _sizey_4) (`MaxDurability_21_22E2DA524D169876ADFB13B005F181BF` _maxdurability)) (break `/Game/BPS_Core/Blueprints/Systems/ItemsSystem/Structures/STR_ItemInstance` (`self.ItemInstance`)))
  ;[1 1 1] Init world item settings and update item mesh.
  (bind (_success _iteminstance) (`/Game/BPS_Core/Blueprints/Systems/ItemsSystem/Libraries/BP_Library_ItemsSystem.MakeItemInstance` (`self.ItemHandle`)))
  (if _success
    (set `self.ItemInstance` _iteminstance)
    (`|ExecutionSequence`
      (:`then_0`
        (`self.UpdateWorldItemMesh`)
        (`self.UpdateSimulatePhysicsDelayed`)
        (`|ExecutionSequence`
          (:`then_0`
            (set `self.Amount` (`KismetMathLibrary.Clamp` (select `bool` (< _amount 0) :`false` _amount :`true` _maxstack) 1 _maxstack)))
          (:`then_1`
            (`|ExecutionSequence`
              (:`then_0`
                (set `self.Charges` (`KismetMathLibrary.Clamp` (select `bool` (< _charges 0) :`false` _charges :`true` _maxcharges) 0 _maxcharges)))
              (:`then_1`
                (`|ExecutionSequence`
                  (:`then_0`
                    (set `self.Durability` (`KismetMathLibrary.FClamp` (select `bool` (< _durability 0.0) :`false` _durability :`true` _maxdurability :!type "Float (double-precision)") 0.0 _maxdurability)))
                  (:`then_1`
                    (`|ExecutionSequence`
                      (:`then_0`
                        (set `self.Decay` (`KismetMathLibrary.FClamp` (select `bool` (> _decaytime 0.0) :`true` (select `bool` (< _decay 0.0) :`false` _decay :`true` _decaytime :!type "Float (double-precision)")) 0.0 _decaytime)))))))))))
      (:`then_1`
        (return true)))))

(fn `IsInfiniteItem`
  (returns (InfiniteItem :type Boolean))
  ;[1 1 1] Returns true if item is infinite.
  (return (`self.InfiniteItem`)))

(fn `OnRep_ItemHandle`
  ;[1 1 1] Update world item settings when item handle is changed.
  (`self.InitWorldItemSettings`))

(fn `PickUpItem`
  (params (RemainingItemData :type "/Game/BPS_Core/Blueprints/Systems/ItemsSystem/Structures/STR_ItemData Structure"))
  (returns (Success :type Boolean))
  (bind ((`Amount_5_B033629F4C4A0888FA5694A50E9C628E` _amount) (`Charges_7_DB1A78E249E9703585020C838A8AD10B` _charges) (`Durability_10_8638D6964EDC7593074331AB041540E2` _durability) (`Decay_12_8A5B83FE4DB7B2FDA61992B1FB038C84` _decay) (`Options_20_B9F9AFC44A1DB534FEA651ABDE8D0D8B` _options) (`Bonuses_24_1DDA9F474A23C147B9FF2A821AF568AF` _bonuses) (`ContainerItems_27_5D95EA904371F00AE4CBA18906A62B0B` _containeritems)) (break `/Game/BPS_Core/Blueprints/Systems/ItemsSystem/Structures/STR_ContainerItemData` (`.ContainerItemData_2_23C913CF4242D016411ABA9CA08BBD6D` (break `/Game/BPS_Core/Blueprints/Systems/ItemsSystem/Structures/STR_ItemData` RemainingItemData))))
  ;[1 1 1] Set remaining item data for the world item.
  (`self.PlayPickUpSound`)
  (if (not (`self.IsInfiniteItem`))
    (if (<= _amount 0)
      (`self.DestroyWorldItem`)
      (else
        (set `self.Amount` _amount)
        (set `self.Charges` _charges)
        (set `self.Durability` _durability)
        (set `self.Decay` _decay)
        (set `self.Options` _options)
        (set `self.Bonuses` _bonuses)
        (set `self.ContainerItems` _containeritems)))
    (return true)
    (else
      (return true))))

(fn `PlayDropSound`
  (params (HitResult :type "HitResult Structure"))
  (returns (Success :type Boolean))
  (bind _dropimpactpreset (`self.DropImpactPreset`))
  (bind _dropsound (`self.DropSound`))
  ;[1 1 1] Try to play drop impact effects.
  (if (`/Game/BPS_Core/Blueprints/Systems/CoreSystem/Libraries/BP_Library_CoreFunctions.HandleIsValid` _dropimpactpreset)
    (bind _success (`/Game/BPS_Core/Blueprints/Systems/ImpactSystem/Libraries/BP_Library_ImpactSystem.PlayImpactEffectsByHandleReplicated` _dropimpactpreset HitResult))
    (return _success)
    (else
      (`/Engine/EditorBlueprintResources/StandardMacros.IsValid` _dropsound
        (:`Is Valid`
          (`GameplayStatics.PlaySoundAtLocation` _dropsound (`SceneComponent.K2_GetComponentLocation` (`self.StaticMesh`)) (struct) 1.0 1.0 0.0 null null null null)
          (return true))
        (:`Is Not Valid`
          (return false))))))

(fn `PlayPickUpSound`
  (returns (Success :type Boolean))
  (bind _pickupsound (`self.PickUpSound`))
  ;[1 1 1] Try to play pick up sound.
  (`/Engine/EditorBlueprintResources/StandardMacros.IsValid` _pickupsound
    (:`Is Valid`
      (`/Game/BPS_Core/Blueprints/Systems/CoreSystem/Libraries/BP_Library_CoreFunctions.TrySpawnSoundAtLocationReplicated` _pickupsound (`SceneComponent.K2_GetComponentLocation` (`self.StaticMesh`)))
      (return true))
    (:`Is Not Valid`
      (return false))))

(fn `UpdatePhysicsSimulation`
  (bind _staticmesh (`self.StaticMesh`))
  ;[1 1 1] Update phisics simulation for static mesh of the world item.
  (`/Engine/EditorBlueprintResources/StandardMacros.IsValid` (`StaticMeshComponent.StaticMesh` _staticmesh)
    (:`Is Valid`
      (`PrimitiveComponent.SetSimulatePhysics` _staticmesh (`self.SimulatePhysics`)))))

(fn `UpdateWorldItemMesh`
  (bind ((`WorldStaticMesh_26_1ACE78EF456C54797887A8949DAA78DE` _worldstaticmesh) (`WorldStaticMeshSoft_29_AF5908594C56D24787B324BF59CBADB2` _worldstaticmeshsoft)) (break `/Game/BPS_Core/Blueprints/Systems/ItemsSystem/Structures/STR_ItemInstance` (`self.ItemInstance`)))
  ;[1 1 1] Update static mesh component of the world item. Try to load static mesh from soft object reference.
  (if (`KismetSystemLibrary.IsValidSoftObjectReference` _worldstaticmeshsoft)
    (if (`/Game/BPS_Core/Blueprints/Systems/CoreSystem/Libraries/BP_Library_CoreFunctions.RunInEditor`)
      (bind _returnvalue (`KismetSystemLibrary.LoadAsset_Blocking` _worldstaticmeshsoft))
      (bind _asstatic_mesh (cast `StaticMesh` _returnvalue))
      (`StaticMeshComponent.SetStaticMesh` (`self.StaticMesh`) _asstatic_mesh)
      (else
        (`/Game/BPS_Core/Blueprints/Systems/AsyncLoadSystem/Libraries/BP_Library_AsyncLoad.AsyncLoadStaticMeshDelegate` _worldstaticmeshsoft (`|CreateDelegate` :!event `Bind_OnStaticMeshLoaded`))))
    (else
      (`StaticMeshComponent.SetStaticMesh` (`self.StaticMesh`) _worldstaticmesh))))

(fn `UserConstructionScript`
  ;[1 1 1] Construction script. Init world item settings.
  (if (`/Game/BPS_Core/Blueprints/Systems/CoreSystem/Libraries/BP_Library_CoreFunctions.RunInEditor`)
    (`self.InitWorldItemSettings`)))