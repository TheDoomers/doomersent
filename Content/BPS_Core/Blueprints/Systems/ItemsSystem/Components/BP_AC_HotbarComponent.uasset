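; Hotbar component for the items system that tracks which container slot is selected and exposes that slot's index and item data.
; TrySelectHotbarSlot changes the index only when CanChangeSlot allows it, then fires the server change event, with new and previous indices passed swapped.
; The selected index uses RepNotify to fire the client change event.
; Item lookup checks that the index is valid before returning data.
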(fn `GetSelectedSlotIndex`
  (returns (SelectedSlotIndex :type Integer))
  ;[1 1 1] Returns selected slot index.
  (return (`self.SelectedSlotIndex`)))

(fn `GetValidSelectedItemData`
  (returns (Success :type Boolean) (ItemData :type "/Game/BPS_Core/Blueprints/Systems/ItemsSystem/Structures/STR_ItemData Structure"))
  (bind _selectedslotindex (`self.SelectedSlotIndex`))
  ;[1 1 1] Returns item data of selected container slot.
  (if (`KismetArrayLibrary.Array_IsValidIndex` (`self.ItemsData`) _selectedslotindex)
    (bind (_success _itemdata) (`self.GetValidItemData` _selectedslotindex))
    (return _success _itemdata)
    (else
      (return false))))

(fn `OnRep_SelectedSlotIndex`
  ;[1 1 1] Call the selected slot changed for all clients.
  (`self.OnSelectedSlotChanged_Client` self (`self.SelectedSlotIndex`)))

(fn `TrySelectHotbarSlot`
  (params (SlotIndex :type Integer))
  (returns (Success :type Boolean))
  (locals (LocalPrevSelectedSlot :type Integer :default 0))
  ;[1 1 1] Try to select container slot by index.
  (if (`self.CanChangeSlot`)
    (bind _output_get (set `local.LocalPrevSelectedSlot` (`self.SelectedSlotIndex`)))
    (bind _output_get_2 (set `self.SelectedSlotIndex` SlotIndex))
    (`self.OnSelectedSlotChanged_Server` self _output_get _output_get_2)
    (return true)))