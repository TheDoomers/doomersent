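; Actor component that spawns world item actors around a location, from an item handle or from full item data, singly or in batches.
; Each spawn resolves the item's data table row and uses its world item class, falling back to a default class.
; Looked-up rows are cached by row name, with a short timer set to clear the cache.
; Spawns get a randomized offset within range and height bounds plus random rotation.
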(fn `FindItemInstance`
  (params (ItemHandle :type "DataTableRowHandle Structure"))
  (returns (Found :type Boolean) (ItemInstance :type "/Game/BPS_Core/Blueprints/Systems/ItemsSystem/Structures/STR_ItemInstance Structure"))
  (locals (LocalItemInstance :type "/Game/BPS_Core/Blueprints/Systems/ItemsSystem/Structures/STR_ItemInstance Structure"))
  (bind (_datatable _rowname) (break `DataTableRowHandle` ItemHandle))
  (bind (_value _returnvalue) (`BlueprintMapLibrary.Map_Find` (`self.QuickItemInstances`) (`.RowName` (break `DataTableRowHandle` ItemHandle))))
  ;[1 1 1] Try to find a quick item instance or find it in data table.
  (if (not _returnvalue)
    (if (`/Game/BPS_Core/Blueprints/Systems/CoreSystem/Libraries/BP_Library_CoreFunctions.HandleIsValid` ItemHandle)
      (bind _returnvalue_2 (`|GetDataTableRow` _datatable _rowname)
        (:`then`
          (bind _output_get (set `local.LocalItemInstance` _returnvalue_2))
          (`BlueprintMapLibrary.Map_Add` (`self.QuickItemInstances`) _rowname _output_get)
          (`KismetSystemLibrary.K2_SetTimerDelegate` (`|CreateDelegate` :!event `ResetQuickItemInstances`) 3.0)
          (return true (`local.LocalItemInstance`))))
      (else
        (return false)))
    (else
      (return true _value))))

(fn `GetDefaultWorldItemClass`
  (returns (WorldItemClass :type "/Game/BPS_Core/Blueprints/Systems/ItemsSystem/Actors/BP_WorldItem_Base Class Reference"))
  ;[1 1 1] Returns default world item class.
  (return (`self.DefaultWorldItemClass`)))

(fn `GetWorldItemClass`
  (params (ItemInstance :type "/Game/BPS_Core/Blueprints/Systems/ItemsSystem/Structures/STR_ItemInstance Structure"))
  (returns (IsDefaultClass :type Boolean) (WorldItemClass :type "/Game/BPS_Core/Blueprints/Systems/ItemsSystem/Actors/BP_WorldItem_Base Class Reference"))
  (bind ((`WorldItemClass_13_F505D1B040FF7CD4B5815BBDA7052C02` _worlditemclass)) (break `/Game/BPS_Core/Blueprints/Systems/ItemsSystem/Structures/STR_ItemInstance` ItemInstance))
  ;[1 1 1] Returns default world item class.
  (if (not (`KismetSystemLibrary.IsValidClass` _worlditemclass))
    (return true (`self.GetDefaultWorldItemClass`))
    (else
      (return false _worlditemclass))))

(fn `MakeSpawnLocation`
  (params (Location :type "Vector Structure") (MinRange :type "Float (double-precision)") (MaxRange :type "Float (double-precision)") (MinHeight :type "Float (double-precision)") (MaxHeight :type "Float (double-precision)"))
  (returns (ResultLocation :type "Vector Structure"))
  (bind _returnvalue (`KismetMathLibrary.RandomFloatInRange` MinRange MaxRange))
  (bind _returnvalue_2 (`KismetMathLibrary.RandomFloatInRange` MinRange MaxRange))
  ;[1 1 1] Make spawn location in using specific range and height.
  (return (+ Location (`KismetMathLibrary.GreaterGreater_VectorRotator` (`KismetMathLibrary.MakeVector` (select `bool` (`KismetMathLibrary.RandomBool`) :`false` _returnvalue :`true` (* _returnvalue -1.0)) (select `bool` (`KismetMathLibrary.RandomBool`) :`false` _returnvalue_2 :`true` (* _returnvalue_2 -1.0)) (`KismetMathLibrary.RandomFloatInRange` MinHeight MaxHeight)) (`KismetMathLibrary.MakeRotator` 0.0 0.0 (`KismetMathLibrary.RandomFloatInRange` 0.0 360.0))))))

(fn `ResetQuickItemInstances`
  ;[1 1 1] Clears the quick item instances variable.
  (`BlueprintMapLibrary.Map_Clear` (`self.QuickItemInstances`)))

(fn `SpawnWorldItem`
  (params (ItemHandle :type "DataTableRowHandle Structure") (Location :type "Vector Structure") (MinRange :type "Float (double-precision)") (MaxRange :type "Float (double-precision)") (MinHeight :type "Float (double-precision)") (MaxHeight :type "Float (double-precision)"))
  (returns (WorldItem :type "/Game/BPS_Core/Blueprints/Systems/ItemsSystem/Actors/BP_WorldItem_Base Object Reference"))
  (locals (LocalSpawnLocation :type "Vector Structure" :default (0.0 0.0 0.0)))
  ;[1 1 1] Spawn world item by item handle in a specific location.
  (bind (_found _iteminstance) (`self.FindItemInstance` ItemHandle))
  (if _found
    (bind _output_get (set `local.LocalSpawnLocation` (`self.MakeSpawnLocation` Location MinRange MaxRange MinHeight MaxHeight)))
    (bind _returnvalue (`|SpawnActorFromClass` :`Class` (`.WorldItemClass` (`self.GetWorldItemClass` _iteminstance)) :`SpawnTransform` (`KismetMathLibrary.MakeTransform` _output_get (`KismetMathLibrary.RandomRotator` false)) :`CollisionHandlingOverride` "AdjustIfPossibleButAlwaysSpawn" :`TransformScaleMethod` "SelectDefaultAtRuntime" :`ItemHandle` (`.ItemHandle_2_77EA4FE84F6A8B0D2A1BE6BCE8F2CE43` (break `/Game/BPS_Core/Blueprints/Systems/ItemsSystem/Structures/STR_ItemInstance` _iteminstance)) :`Instigator` null))
    (return _returnvalue)))

(fn `SpawnWorldItemByData`
  (params (ItemData :type "/Game/BPS_Core/Blueprints/Systems/ItemsSystem/Structures/STR_ContainerItemData Structure") (Location :type "Vector Structure") (MinRange :type "Float (double-precision)") (MaxRange :type "Float (double-precision)") (MinHeight :type "Float (double-precision)") (MaxHeight :type "Float (double-precision)"))
  (returns (WorldItem :type "/Game/BPS_Core/Blueprints/Systems/ItemsSystem/Actors/BP_WorldItem_Base Object Reference"))
  (locals (LocalItemData :type "/Game/BPS_Core/Blueprints/Systems/ItemsSystem/Structures/STR_ContainerItemData Structure") (LocalSpawnLocation :type "Vector Structure"))
  (bind (_itemhandle _amount _charges _durability _decay _options _bonuses _containeritems) (break `/Game/BPS_Core/Blueprints/Systems/ItemsSystem/Structures/STR_ContainerItemData` (`local.LocalItemData`)))
  ;[1 1 1] Spawn world item by item data in a specific location.
  (set `local.LocalItemData` ItemData)
  (bind (_found _iteminstance) (`self.FindItemInstance` (`.ItemHandle_2_AC01AFE74D1662F3E4302B94A89F111E` (break `/Game/BPS_Core/Blueprints/Systems/ItemsSystem/Structures/STR_ContainerItemData` ItemData))))
  (if _found
    (bind _output_get (set `local.LocalSpawnLocation` (`self.MakeSpawnLocation` Location MinRange MaxRange MinHeight MaxHeight)))
    (bind _returnvalue (`|SpawnActorFromClass` (`.WorldItemClass` (`self.GetWorldItemClass` _iteminstance)) (`KismetMathLibrary.MakeTransform` _output_get (`KismetMathLibrary.RandomRotator` false)) "AdjustIfPossibleButAlwaysSpawn" "SelectDefaultAtRuntime" null _itemhandle _amount _charges _durability _decay _options _bonuses _containeritems true false null))
    (return _returnvalue)))

(fn `SpawnWorldItemsByData`
  (params (ItemData :type "Array of /Game/BPS_Core/Blueprints/Systems/ItemsSystem/Structures/STR_ContainerItemData Structure") (Location :type "Vector Structure") (MinRange :type "Float (double-precision)") (MaxRange :type "Float (double-precision)") (MinHeight :type "Float (double-precision)") (MaxHeight :type "Float (double-precision)"))
  (returns (WorldItems :type "Array of /Game/BPS_Core/Blueprints/Systems/ItemsSystem/Actors/BP_WorldItem_Base Object Reference"))
  (locals (LocalWorldItems :type "Array of /Game/BPS_Core/Blueprints/Systems/ItemsSystem/Actors/BP_WorldItem_Base Object Reference"))
  ;[1 1 1] Spawn world items by item data in a specific location.
  (for _array_element ItemData
    (bind _worlditem (`self.SpawnWorldItemByData` _array_element Location MinRange MaxRange MinHeight MaxHeight))
    (`KismetArrayLibrary.Array_Add` (`local.LocalWorldItems`) _worlditem))
  (return (`local.LocalWorldItems`)))