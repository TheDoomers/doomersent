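; Actor component that turns its owner into a trader, buying and selling items against a currency item.
; On init it finds the owner's trading container by ID and applies a data-table trading list (loot, filters, cost multiplier).
; Buy/sell checks costs, moves items between containers, then transfers currency, with slot-targeted variants falling back to any slot.
; A server timer restocks the container, postponing while tracked active players are trading.
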(event `self.ReceiveBeginPlay`
  ;[1 1 1] Begin play. Try init component.
  (if (`self.InitOnBeginPlay`)
    (`self.TryInitComponent`)))

(fn `AddActivePlayer`
  (params (PlayerController :type "PlayerController Object Reference (by ref)"))
  (returns (Success :type Boolean))
  (bind _activeplayers (`self.ActivePlayers`))
  ;[1 1 1] Add active player to the list and call events.
  (if (`KismetSystemLibrary.IsServer`)
    (if (`KismetArrayLibrary.Array_Contains` _activeplayers PlayerController)
      _
      (else
        (`KismetArrayLibrary.Array_Add` _activeplayers PlayerController)
        (`self.OnActivePlayersChanged` self)
        (if (== (`KismetArrayLibrary.Array_Length` _activeplayers) 1)
          (`self.OnTradingOpened` self)
          (return true)
          (else
            (return false))))))
  (return false))

(fn `Bind_RefreshTimerTIck`
  ;[1 1 1] Refresh trading items if there are no active players.
  (if (not (`KismetArrayLibrary.Array_IsValidIndex` (`self.ActivePlayers`)))
    (`self.RefreshTradingList`)
    (else
      (`KismetSystemLibrary.K2_SetTimerDelegate` (`|CreateDelegate` :!event `Bind_RefreshTimerTIck`) 5.0))))

(fn `CheckItemToBuy`
  (params (ItemData :type "/Game/BPS_Core/Blueprints/Systems/ItemsSystem/Structures/STR_ItemData Structure"))
  (returns (Success :type Boolean))
  ;[1 1 1] Returns true if item data can be bought.
  (return (not (`/Game/BPS_Core/Blueprints/Systems/CoreSystem/Libraries/BP_Library_CoreFunctions.HandlesAreEqual` (`/Game/BPS_Core/Blueprints/Systems/ItemsSystem/Libraries/BP_Library_ItemsSystem.GetItemHandle` ItemData) (`.CurrencyItemHandle_31_5E371F044E6817B246DB19B6FB700707` (break `/Game/BPS_Core/Blueprints/Systems/ItemsSystem/Structures/STR_TradingList` (`self.TradingListData`)))))))

(fn `CheckItemToSell`
  (params (ItemData :type "/Game/BPS_Core/Blueprints/Systems/ItemsSystem/Structures/STR_ItemData Structure"))
  (returns (Success :type Boolean))
  (bind _itemhandle (`/Game/BPS_Core/Blueprints/Systems/ItemsSystem/Libraries/BP_Library_ItemsSystem.GetItemHandle` ItemData))
  (bind ((`CurrencyItemHandle_31_5E371F044E6817B246DB19B6FB700707` _currencyitemhandle) (`TradingLootList_32_82943E7948B5F2C3BC3489925EF18355` _tradinglootlist) (`CanSellItems_30_CC0B26D444B29D4298E092BAD1F2E33E` _cansellitems) (`InterestedItems_26_E2FA82FF4AF28E9BF3DE9BA64892BED4` _interesteditems) (`NotInterestedItems_25_F43767254D06E1AB414C1280EF478791` _notinteresteditems)) (break `/Game/BPS_Core/Blueprints/Systems/ItemsSystem/Structures/STR_TradingList` (`self.TradingListData`)))
  ;[1 1 1] Returns true if item data can be sold.
  (if _cansellitems
    (if (not (`/Game/BPS_Core/Blueprints/Systems/CoreSystem/Libraries/BP_Library_CoreFunctions.HandlesAreEqual` _itemhandle _currencyitemhandle))
      (if (`KismetArrayLibrary.Array_IsValidIndex` _interesteditems)
        (return (`KismetArrayLibrary.Array_Contains` _interesteditems _itemhandle))
        (else
          (return (not (`KismetArrayLibrary.Array_Contains` _notinteresteditems _itemhandle)))))
      (else
        _)))
  (return false))

(fn `FindBuyCost`
  (params (ItemData :type "/Game/BPS_Core/Blueprints/Systems/ItemsSystem/Structures/STR_ItemData Structure"))
  (returns (Found :type Boolean) (RequiredItem :type "/Game/BPS_Core/Blueprints/Systems/ItemsSystem/Structures/STR_RequiredItem Structure"))
  (bind ((`CurrencyItemHandle_31_5E371F044E6817B246DB19B6FB700707` _currencyitemhandle)) (break `/Game/BPS_Core/Blueprints/Systems/ItemsSystem/Structures/STR_TradingList` (`self.TradingListData`)))
  ;[1 1 1] Try to make required item for buy interaction.
  (if (`/Game/BPS_Core/Blueprints/Systems/CoreSystem/Libraries/BP_Library_CoreFunctions.HandleIsValid` _currencyitemhandle)
    (return true (make `/Game/BPS_Core/Blueprints/Systems/ItemsSystem/Structures/STR_RequiredItem` :`ItemHandle` _currencyitemhandle :`RequiredAmount` (`KismetMathLibrary.FTrunc` (* (* (`/Game/BPS_Core/Blueprints/Systems/ItemsSystem/Libraries/BP_Library_ItemsSystem.GetItemAmount` ItemData) (`self.GetBuyCostMultiplier`)) (`/Game/BPS_Core/Blueprints/Systems/ItemsSystem/Libraries/BP_Library_ItemsSystem.GetItemCostMultiplier` ItemData)))))
    (else
      (return false))))

(fn `FindSellCost`
  (params (ItemData :type "/Game/BPS_Core/Blueprints/Systems/ItemsSystem/Structures/STR_ItemData Structure"))
  (returns (Found :type Boolean) (RequiredItem :type "/Game/BPS_Core/Blueprints/Systems/ItemsSystem/Structures/STR_RequiredItem Structure"))
  (bind ((`CurrencyItemHandle_31_5E371F044E6817B246DB19B6FB700707` _currencyitemhandle)) (break `/Game/BPS_Core/Blueprints/Systems/ItemsSystem/Structures/STR_TradingList` (`self.TradingListData`)))
  ;[1 1 1] Try to make required item for sell interaction.
  (if (`/Game/BPS_Core/Blueprints/Systems/CoreSystem/Libraries/BP_Library_CoreFunctions.HandleIsValid` _currencyitemhandle)
    (return true (make `/Game/BPS_Core/Blueprints/Systems/ItemsSystem/Structures/STR_RequiredItem` :`ItemHandle` _currencyitemhandle :`RequiredAmount` (`KismetMathLibrary.FTrunc` (* (`/Game/BPS_Core/Blueprints/Systems/ItemsSystem/Libraries/BP_Library_ItemsSystem.GetItemAmount` ItemData) (`/Game/BPS_Core/Blueprints/Systems/ItemsSystem/Libraries/BP_Library_ItemsSystem.GetItemCostMultiplier` ItemData)))))
    (else
      (return false))))

(fn `GetBuyCostMultiplier`
  (returns (BuyCostMultiplier :type "Float (double-precision)"))
  ;[1 1 1] Returns cost multiplier for buy interaction.
  (return (`.BuyCostMultiplier_20_919D27AB41F383C2A249ED993D8C9710` (break `/Game/BPS_Core/Blueprints/Systems/ItemsSystem/Structures/STR_TradingList` (`self.TradingListData`)))))

(fn `GetTradingContainer`
  (returns (TradingContainer :type "/Game/BPS_Core/Blueprints/Systems/ItemsSystem/Components/BP_AC_ContainerComponent Object Reference"))
  ;[1 1 1] Returns trading container reference.
  (return (`self.TradingContainerComponent`)))

(fn `InitComponent`
  (returns (Success :type Boolean))
  (bind (_datatable _rowname) (break `DataTableRowHandle` (`self.TradingListHandle`)))
  ;[1 1 1] Init trading component.
  (for _array_element (`Actor.K2_GetComponentsByClass` (`self.GetOwner`) "/Game/BPS_Core/Blueprints/Systems/ItemsSystem/Components/BP_AC_ContainerComponent.BP_AC_ContainerComponent_C")
    (if (== (`/Game/BPS_Core/Blueprints/Systems/ItemsSystem/Components/BP_AC_ContainerComponent.InitContainerID` _array_element) (`self.TradingContainerID`))
      (bind _output_get (set `self.TradingContainerComponent` _array_element))
      (`/Engine/EditorBlueprintResources/StandardMacros.IsValid` _datatable
        (:`Is Valid`
          (bind _returnvalue (`|GetDataTableRow` _datatable _rowname)
            (:`then`
              (bind _output_get_2 (set `self.TradingListData` _returnvalue))
              (set `/Game/BPS_Core/Blueprints/Systems/ItemsSystem/Components/BP_AC_ContainerComponent.StartingLootHandle` (`.TradingLootList_32_82943E7948B5F2C3BC3489925EF18355` (break `/Game/BPS_Core/Blueprints/Systems/ItemsSystem/Structures/STR_TradingList` _output_get_2)) _output_get)))))))
  (`/Engine/EditorBlueprintResources/StandardMacros.IsValid` (`self.TradingContainerComponent`)
    (:`Is Valid`
      (`self.StartRefreshTimer`)
      (bind _output_get_3 (set `self.IsInitialized` true))
      (return _output_get_3))
    (:`Is Not Valid`
      (return false))))

(fn `RefreshTradingList`
  (returns (Success :type Boolean))
  (bind _tradingcontainercomponent (`self.TradingContainerComponent`))
  ;[1 1 1] Refresh items in the trading container.
  (if (`/Game/BPS_Core/Blueprints/Systems/ItemsSystem/Components/BP_AC_ContainerComponent.IsInitialized` _tradingcontainercomponent)
    (`/Game/BPS_Core/Blueprints/Systems/ItemsSystem/Components/BP_AC_ContainerComponent.ClearItemsData` _tradingcontainercomponent)
    (`/Game/BPS_Core/Blueprints/Systems/ItemsSystem/Components/BP_AC_ContainerComponent.InitContainerLoot` _tradingcontainercomponent (`.TradingLootList_32_82943E7948B5F2C3BC3489925EF18355` (break `/Game/BPS_Core/Blueprints/Systems/ItemsSystem/Structures/STR_TradingList` (`self.TradingListData`)))))
  (`self.StartRefreshTimer`)
  (return true))

(fn `RemoveActivePlayer`
  (params (PlayerController :type "PlayerController Object Reference (by ref)"))
  (returns (Success :type Boolean))
  (bind _activeplayers (`self.ActivePlayers`))
  ;[1 1 1] Remove player from the list and call events.
  (if (`KismetSystemLibrary.IsServer`)
    (bind _returnvalue (`KismetArrayLibrary.Array_RemoveItem` _activeplayers PlayerController))
    (if _returnvalue
      (`self.OnActivePlayersChanged` self)
      (if (== (`KismetArrayLibrary.Array_Length` _activeplayers) 0)
        (`self.OnTradingClosed` self)
        (return true)
        (else
          (return false)))
      (else
        _)))
  (return false))

(fn `StartRefreshTimer`
  (returns (Success :type Boolean))
  ;[1 1 1] Start refresh trading loot timer on server.
  (if (`KismetSystemLibrary.IsServer`)
    (`KismetSystemLibrary.K2_SetTimerDelegate` (`|CreateDelegate` :!event `Bind_RefreshTimerTIck`) (`.RefreshTime_13_27B36EB5473DA9CF6E7500ABBCE56768` (break `/Game/BPS_Core/Blueprints/Systems/ItemsSystem/Structures/STR_TradingList` (`self.TradingListData`))))
    (return true)))

(fn `TryBuyContainerItem`
  (params (FromContainer :type "/Game/BPS_Core/Blueprints/Systems/ItemsSystem/Components/BP_AC_ContainerComponent Object Reference") (FromSlot :type Integer) (ToContainer :type "/Game/BPS_Core/Blueprints/Systems/ItemsSystem/Components/BP_AC_ContainerComponent Object Reference") (Amount :type Integer) (PlayerContainer :type "/Game/BPS_Core/Blueprints/Systems/ItemsSystem/Components/BP_AC_ContainerComponent Object Reference"))
  (returns (Success :type Boolean))
  (locals (LocalFromContainer :type "/Game/BPS_Core/Blueprints/Systems/ItemsSystem/Components/BP_AC_ContainerComponent Object Reference") (LocalFromSlot :type Integer) (LocalToContainer :type "/Game/BPS_Core/Blueprints/Systems/ItemsSystem/Components/BP_AC_ContainerComponent Object Reference") (LocalAmount :type Integer) (LocalPlayerContainer :type "/Game/BPS_Core/Blueprints/Systems/ItemsSystem/Components/BP_AC_ContainerComponent Object Reference") (LocalFromItem :type "/Game/BPS_Core/Blueprints/Systems/ItemsSystem/Structures/STR_ItemData Structure") (LocalRequiredItem :type "/Game/BPS_Core/Blueprints/Systems/ItemsSystem/Structures/STR_RequiredItem Structure"))
  (bind _localrequireditem (`local.LocalRequiredItem`))
  (bind ((`ItemHandle_2_1A1AFDBD41B476FF4CC5F4BEE895C742` _itemhandle) (`RequiredAmount_5_BAC5EC5349E2BD29FBFECA8B2B7A94D6` _requiredamount)) (break `/Game/BPS_Core/Blueprints/Systems/ItemsSystem/Structures/STR_RequiredItem` _localrequireditem))
  ;[1 1 1] Try to buy item. Move item to the trading container and remove cost item from the player container.
  (bind _output_get (set `local.LocalFromContainer` FromContainer))
  (bind _output_get_2 (set `local.LocalFromSlot` FromSlot))
  (set `local.LocalToContainer` ToContainer)
  (bind _output_get_3 (set `local.LocalAmount` Amount))
  (set `local.LocalPlayerContainer` PlayerContainer)
  (bind (_success _itemdata) (`/Game/BPS_Core/Blueprints/Systems/ItemsSystem/Components/BP_AC_ContainerComponent.GetValidItemData` _output_get _output_get_2))
  (if _success
    (bind _resultdata (`/Game/BPS_Core/Blueprints/Systems/ItemsSystem/Libraries/BP_Library_ItemsSystem.SetItemAmount` _itemdata _output_get_3))
    (bind _output_get_4 (set `local.LocalFromItem` _resultdata))
    (bind _success_2 (`self.CheckItemToBuy` _output_get_4))
    (if _success_2
      (bind (_found _requireditem) (`self.FindBuyCost` _output_get_4))
      (if _found
        (bind _output_get_5 (set `local.LocalRequiredItem` _requireditem))
        (bind _result (`/Game/BPS_Core/Blueprints/Systems/ItemsSystem/Components/BP_AC_ContainerComponent.CheckRequiredItem` (`local.LocalPlayerContainer`) _output_get_5))
        (if _result
          (bind _success_3 (`/Game/BPS_Core/Blueprints/Systems/ItemsSystem/Components/BP_AC_ContainerComponent.TryMoveItemToContainer` (`local.LocalFromContainer`) (`local.LocalFromSlot`) (`local.LocalToContainer`) (`local.LocalAmount`) true))
          (if _success_3
            (`/Game/BPS_Core/Blueprints/Systems/ItemsSystem/Components/BP_AC_ContainerComponent.RemoveRequiredItem` (`local.LocalPlayerContainer`) _localrequireditem (`|MakeArray`))
            (bind _containeritems (`/Game/BPS_Core/Blueprints/Systems/ItemsSystem/Libraries/BP_Library_ItemsSystem.MakeContainerItemsFromListItem` (make `/Game/BPS_Core/Blueprints/Systems/ItemsSystem/Structures/STR_ListItem` _itemhandle _requiredamount)))
            (`/Game/BPS_Core/Blueprints/Systems/ItemsSystem/Components/BP_AC_ContainerComponent.TryAddItems` (`self.TradingContainerComponent`) _containeritems)
            (`self.OnItemBought` self)
            (return true)
            (else
              (return false)))
          (else
            _)))))
  (return false))

(fn `TryBuyContainerItemToSlot`
  (params (FromContainer :type "/Game/BPS_Core/Blueprints/Systems/ItemsSystem/Components/BP_AC_ContainerComponent Object Reference") (FromSlot :type Integer) (ToContainer :type "/Game/BPS_Core/Blueprints/Systems/ItemsSystem/Components/BP_AC_ContainerComponent Object Reference") (ToSlot :type Integer) (Amount :type Integer) (PlayerContainer :type "/Game/BPS_Core/Blueprints/Systems/ItemsSystem/Components/BP_AC_ContainerComponent Object Reference"))
  (returns (Success :type Boolean))
  (locals (LocalFromContainer :type "/Game/BPS_Core/Blueprints/Systems/ItemsSystem/Components/BP_AC_ContainerComponent Object Reference") (LocalFromSlot :type Integer) (LocalToContainer :type "/Game/BPS_Core/Blueprints/Systems/ItemsSystem/Components/BP_AC_ContainerComponent Object Reference") (LocalToSlot :type Integer) (LocalAmount :type Integer) (LocalPlayerContainer :type "/Game/BPS_Core/Blueprints/Systems/ItemsSystem/Components/BP_AC_ContainerComponent Object Reference") (LocalFromItem :type "/Game/BPS_Core/Blueprints/Systems/ItemsSystem/Structures/STR_ItemData Structure") (LocalRequiredItem :type "/Game/BPS_Core/Blueprints/Systems/ItemsSystem/Structures/STR_RequiredItem Structure"))
  (bind _localrequireditem (`local.LocalRequiredItem`))
  (bind ((`ItemHandle_2_1A1AFDBD41B476FF4CC5F4BEE895C742` _itemhandle) (`RequiredAmount_5_BAC5EC5349E2BD29FBFECA8B2B7A94D6` _requiredamount)) (break `/Game/BPS_Core/Blueprints/Systems/ItemsSystem/Structures/STR_RequiredItem` _localrequireditem))
  ;[1 1 1] Try to buy item. Move item to specific trading container slot and remove cost item from the player container.
  (bind _output_get (set `local.LocalFromContainer` FromContainer))
  (bind _output_get_2 (set `local.LocalFromSlot` FromSlot))
  (set `local.LocalToContainer` ToContainer)
  (set `local.LocalToSlot` ToSlot)
  (bind _output_get_3 (set `local.LocalAmount` Amount))
  (set `local.LocalPlayerContainer` PlayerContainer)
  (bind (_success _itemdata) (`/Game/BPS_Core/Blueprints/Systems/ItemsSystem/Components/BP_AC_ContainerComponent.GetValidItemData` _output_get _output_get_2))
  (if _success
    (bind _resultdata (`/Game/BPS_Core/Blueprints/Systems/ItemsSystem/Libraries/BP_Library_ItemsSystem.SetItemAmount` _itemdata _output_get_3))
    (bind _output_get_4 (set `local.LocalFromItem` _resultdata))
    (bind _success_2 (`self.CheckItemToBuy` _output_get_4))
    (if _success_2
      (bind (_found _requireditem) (`self.FindBuyCost` _output_get_4))
      (if _found
        (bind _output_get_5 (set `local.LocalRequiredItem` _requireditem))
        (bind _result (`/Game/BPS_Core/Blueprints/Systems/ItemsSystem/Components/BP_AC_ContainerComponent.CheckRequiredItem` (`local.LocalPlayerContainer`) _output_get_5))
        (if _result
          (bind (_rowspan _columnspan) (`/Game/BPS_Core/Blueprints/Systems/ItemsSystem/Libraries/BP_Library_ItemsSystem.GetItemSizes` _output_get_4))
          (bind _success_3 (`/Game/BPS_Core/Blueprints/Systems/ItemsSystem/Components/BP_AC_ContainerComponent.CheckContainerSlotsForMove` (`local.LocalToContainer`) (`local.LocalToSlot`) _rowspan _columnspan (`|MakeArray`)))
          (if _success_3
            (bind _success_4 (`/Game/BPS_Core/Blueprints/Systems/ItemsSystem/Components/BP_AC_ContainerComponent.TryMoveItemToContainerSlot` (`local.LocalFromContainer`) (`local.LocalFromSlot`) (`local.LocalToContainer`) (`local.LocalToSlot`) (`local.LocalAmount`) true))
            (if _success_4
              _
              (else
                (return false)))
            (else
              (bind _success_5 (`/Game/BPS_Core/Blueprints/Systems/ItemsSystem/Components/BP_AC_ContainerComponent.TryMoveItemToContainer` (`local.LocalFromContainer`) (`local.LocalFromSlot`) (`local.LocalToContainer`) (`local.LocalAmount`) true))
              (if _success_5
                _
                (else
                  (return false)))))
          (`/Game/BPS_Core/Blueprints/Systems/ItemsSystem/Components/BP_AC_ContainerComponent.RemoveRequiredItem` (`local.LocalPlayerContainer`) _localrequireditem (`|MakeArray`))
          (bind _containeritems (`/Game/BPS_Core/Blueprints/Systems/ItemsSystem/Libraries/BP_Library_ItemsSystem.MakeContainerItemsFromListItem` (make `/Game/BPS_Core/Blueprints/Systems/ItemsSystem/Structures/STR_ListItem` _itemhandle _requiredamount)))
          (`/Game/BPS_Core/Blueprints/Systems/ItemsSystem/Components/BP_AC_ContainerComponent.TryAddItems` (`self.TradingContainerComponent`) _containeritems)
          (`self.OnItemBought` self)
          (return true)
          (else
            _)))))
  (return false))

(fn `TryInitComponent`
  (returns (Success :type Boolean))
  ;[1 1 1] Try init trading component.
  (if (not (`self.IsInitialized`))
    (bind _success (`self.InitComponent`))
    (return _success)
    (else
      (return true))))

(fn `TrySellContainerItem`
  (params (FromContainer :type "/Game/BPS_Core/Blueprints/Systems/ItemsSystem/Components/BP_AC_ContainerComponent Object Reference") (FromSlot :type Integer) (ToContainer :type "/Game/BPS_Core/Blueprints/Systems/ItemsSystem/Components/BP_AC_ContainerComponent Object Reference") (Amount :type Integer) (PlayerContainer :type "/Game/BPS_Core/Blueprints/Systems/ItemsSystem/Components/BP_AC_ContainerComponent Object Reference"))
  (returns (Success :type Boolean))
  (locals (LocalFromContainer :type "/Game/BPS_Core/Blueprints/Systems/ItemsSystem/Components/BP_AC_ContainerComponent Object Reference") (LocalFromSlot :type Integer) (LocalToContainer :type "/Game/BPS_Core/Blueprints/Systems/ItemsSystem/Components/BP_AC_ContainerComponent Object Reference") (LocalAmount :type Integer) (LocalPlayerContainer :type "/Game/BPS_Core/Blueprints/Systems/ItemsSystem/Components/BP_AC_ContainerComponent Object Reference") (LocalFromItem :type "/Game/BPS_Core/Blueprints/Systems/ItemsSystem/Structures/STR_ItemData Structure") (LocalRequiredItem :type "/Game/BPS_Core/Blueprints/Systems/ItemsSystem/Structures/STR_RequiredItem Structure"))
  (bind _localrequireditem (`local.LocalRequiredItem`))
  (bind ((`ItemHandle_2_1A1AFDBD41B476FF4CC5F4BEE895C742` _itemhandle) (`RequiredAmount_5_BAC5EC5349E2BD29FBFECA8B2B7A94D6` _requiredamount)) (break `/Game/BPS_Core/Blueprints/Systems/ItemsSystem/Structures/STR_RequiredItem` _localrequireditem))
  ;[1 1 1] Try to sell item. Move item to the specific container and add cost item to the player container.
  (bind _output_get (set `local.LocalFromContainer` FromContainer))
  (bind _output_get_2 (set `local.LocalFromSlot` FromSlot))
  (set `local.LocalToContainer` ToContainer)
  (bind _output_get_3 (set `local.LocalAmount` Amount))
  (set `local.LocalPlayerContainer` PlayerContainer)
  (bind (_success _itemdata) (`/Game/BPS_Core/Blueprints/Systems/ItemsSystem/Components/BP_AC_ContainerComponent.GetValidItemData` _output_get _output_get_2))
  (if _success
    (bind _resultdata (`/Game/BPS_Core/Blueprints/Systems/ItemsSystem/Libraries/BP_Library_ItemsSystem.SetItemAmount` _itemdata _output_get_3))
    (bind _output_get_4 (set `local.LocalFromItem` _resultdata))
    (bind _success_2 (`self.CheckItemToSell` _output_get_4))
    (if _success_2
      (bind (_found _requireditem) (`self.FindSellCost` _output_get_4))
      (if _found
        (bind _output_get_5 (set `local.LocalRequiredItem` _requireditem))
        (bind _result (`/Game/BPS_Core/Blueprints/Systems/ItemsSystem/Components/BP_AC_ContainerComponent.CheckRequiredItem` (`self.TradingContainerComponent`) _output_get_5))
        (if _result
          (bind _success_3 (`/Game/BPS_Core/Blueprints/Systems/ItemsSystem/Components/BP_AC_ContainerComponent.TryMoveItemToContainer` (`local.LocalFromContainer`) (`local.LocalFromSlot`) (`local.LocalToContainer`) (`local.LocalAmount`) true))
          (if _success_3
            (`/Game/BPS_Core/Blueprints/Systems/ItemsSystem/Components/BP_AC_ContainerComponent.RemoveRequiredItem` (`self.TradingContainerComponent`) _localrequireditem (`|MakeArray`))
            (bind _containeritems (`/Game/BPS_Core/Blueprints/Systems/ItemsSystem/Libraries/BP_Library_ItemsSystem.MakeContainerItemsFromListItem` (make `/Game/BPS_Core/Blueprints/Systems/ItemsSystem/Structures/STR_ListItem` _itemhandle _requiredamount)))
            (`/Game/BPS_Core/Blueprints/Systems/ItemsSystem/Components/BP_AC_ContainerComponent.TryAddItems` (`local.LocalPlayerContainer`) _containeritems)
            (`self.OnItemSold` self)
            (return true)
            (else
              (return false)))
          (else
            _)))))
  (return false))

(fn `TrySellContainerItemToSlot`
  (params (FromContainer :type "/Game/BPS_Core/Blueprints/Systems/ItemsSystem/Components/BP_AC_ContainerComponent Object Reference") (FromSlot :type Integer) (ToContainer :type "/Game/BPS_Core/Blueprints/Systems/ItemsSystem/Components/BP_AC_ContainerComponent Object Reference") (ToSlot :type Integer) (Amount :type Integer) (PlayerContainer :type "/Game/BPS_Core/Blueprints/Systems/ItemsSystem/Components/BP_AC_ContainerComponent Object Reference"))
  (returns (Success :type Boolean))
  (locals (LocalFromContainer :type "/Game/BPS_Core/Blueprints/Systems/ItemsSystem/Components/BP_AC_ContainerComponent Object Reference") (LocalFromSlot :type Integer) (LocalToContainer :type "/Game/BPS_Core/Blueprints/Systems/ItemsSystem/Components/BP_AC_ContainerComponent Object Reference") (LocalToSlot :type Integer) (LocalAmount :type Integer) (LocalPlayerContainer :type "/Game/BPS_Core/Blueprints/Systems/ItemsSystem/Components/BP_AC_ContainerComponent Object Reference") (LocalFromItem :type "/Game/BPS_Core/Blueprints/Systems/ItemsSystem/Structures/STR_ItemData Structure") (LocalRequiredItem :type "/Game/BPS_Core/Blueprints/Systems/ItemsSystem/Structures/STR_RequiredItem Structure"))
  (bind _localrequireditem (`local.LocalRequiredItem`))
  (bind ((`ItemHandle_2_1A1AFDBD41B476FF4CC5F4BEE895C742` _itemhandle) (`RequiredAmount_5_BAC5EC5349E2BD29FBFECA8B2B7A94D6` _requiredamount)) (break `/Game/BPS_Core/Blueprints/Systems/ItemsSystem/Structures/STR_RequiredItem` _localrequireditem))
  ;[1 1 1] Try to sell item. Move item to the specific container slot and add cost item to the player container.
  (bind _output_get (set `local.LocalFromContainer` FromContainer))
  (bind _output_get_2 (set `local.LocalFromSlot` FromSlot))
  (set `local.LocalToContainer` ToContainer)
  (set `local.LocalToSlot` ToSlot)
  (bind _output_get_3 (set `local.LocalAmount` Amount))
  (set `local.LocalPlayerContainer` PlayerContainer)
  (bind (_success _itemdata) (`/Game/BPS_Core/Blueprints/Systems/ItemsSystem/Components/BP_AC_ContainerComponent.GetValidItemData` _output_get _output_get_2))
  (if _success
    (bind _resultdata (`/Game/BPS_Core/Blueprints/Systems/ItemsSystem/Libraries/BP_Library_ItemsSystem.SetItemAmount` _itemdata _output_get_3))
    (bind _output_get_4 (set `local.LocalFromItem` _resultdata))
    (bind _success_2 (`self.CheckItemToSell` _output_get_4))
    (if _success_2
      (bind (_found _requireditem) (`self.FindSellCost` _output_get_4))
      (if _found
        (bind _output_get_5 (set `local.LocalRequiredItem` _requireditem))
        (bind _result (`/Game/BPS_Core/Blueprints/Systems/ItemsSystem/Components/BP_AC_ContainerComponent.CheckRequiredItem` (`self.TradingContainerComponent`) _output_get_5))
        (if _result
          (bind (_rowspan _columnspan) (`/Game/BPS_Core/Blueprints/Systems/ItemsSystem/Libraries/BP_Library_ItemsSystem.GetItemSizes` _output_get_4))
          (bind _success_3 (`/Game/BPS_Core/Blueprints/Systems/ItemsSystem/Components/BP_AC_ContainerComponent.CheckContainerSlotsForMove` (`local.LocalToContainer`) (`local.LocalToSlot`) _rowspan _columnspan (`|MakeArray`)))
          (if _success_3
            (bind _success_4 (`/Game/BPS_Core/Blueprints/Systems/ItemsSystem/Components/BP_AC_ContainerComponent.TryMoveItemToContainerSlot` (`local.LocalFromContainer`) (`local.LocalFromSlot`) (`local.LocalToContainer`) (`local.LocalToSlot`) (`local.LocalAmount`) true))
            (if _success_4
              _
              (else
                (return false)))
            (else
              (bind _success_5 (`/Game/BPS_Core/Blueprints/Systems/ItemsSystem/Components/BP_AC_ContainerComponent.TryMoveItemToContainer` (`local.LocalFromContainer`) (`local.LocalFromSlot`) (`local.LocalToContainer`) (`local.LocalAmount`) true))
              (if _success_5
                _
                (else
                  (return false)))))
          (`/Game/BPS_Core/Blueprints/Systems/ItemsSystem/Components/BP_AC_ContainerComponent.RemoveRequiredItem` (`self.TradingContainerComponent`) _localrequireditem (`|MakeArray`))
          (bind _containeritems (`/Game/BPS_Core/Blueprints/Systems/ItemsSystem/Libraries/BP_Library_ItemsSystem.MakeContainerItemsFromListItem` (make `/Game/BPS_Core/Blueprints/Systems/ItemsSystem/Structures/STR_ListItem` _itemhandle _requiredamount)))
          (`/Game/BPS_Core/Blueprints/Systems/ItemsSystem/Components/BP_AC_ContainerComponent.TryAddItems` (`local.LocalPlayerContainer`) _containeritems)
          (`self.OnItemSold` self)
          (return true)
          (else
            _)))))
  (return false))