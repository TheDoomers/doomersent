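; Player camera manager that orbits the view target at a set yaw, pitch and zoom distance.
; BlueprintUpdateCamera derives the target position from those values and interpolates toward it with an eased speed, snapping after initialization or SetCameraRotation.
; Yaw and pitch input also update control rotation, while zoom input is clamped between length limits.
; Turn mode gates yaw input and raises the target interpolation speed for tighter following.
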(fn `AddCameraInputPitch`
  (params (Value :type "Float (double-precision)"))
  (returns (Success :type Boolean))
  ;[1 1 1] Add camera input pitch value and update control rotation of the player.
  (bind _output_get (set `self.TargetCameraPitch` (+ (`self.TargetCameraPitch`) (* Value (`PlayerController.GetDeprecatedInputPitchScale` (`self.GetOwningPlayerController`))))))
  (`Controller.SetControlRotation` (`self.GetOwningPlayerController`) (`KismetMathLibrary.MakeRotator` 0.0 _output_get (`self.TargetCameraYaw`)))
  (return true))

(fn `AddCameraInputYaw`
  (params (Value :type "Float (double-precision)"))
  (returns (Success :type Boolean))
  ;[1 1 1] Add camera input yaw value and update control rotation of the player.
  (if (`self.InTurnMode`)
    (bind _output_get (set `self.TargetCameraYaw` (+ (`self.TargetCameraYaw`) (* Value (`PlayerController.GetDeprecatedInputYawScale` (`self.GetOwningPlayerController`))))))
    (`Controller.SetControlRotation` (`self.GetOwningPlayerController`) (`KismetMathLibrary.MakeRotator` 0.0 (`self.TargetCameraPitch`) _output_get))
    (return true)))

(fn `AddCameraInputZoom`
  (params (Value :type "Float (double-precision)"))
  (returns (Success :type Boolean))
  ;[1 1 1] Add camera input zoom value and update target camera length.
  (set `self.TargetCameraLength` (`KismetMathLibrary.FClamp` (+ (`self.TargetCameraLength`) (* Value (`self.ZoomInputScale`))) (`self.MinCameraLength`) (`self.MaxCameraLength`)))
  (return true))

(fn `BlueprintUpdateCamera`
  (params (CameraTarget :type "Actor Object Reference"))
  (returns (NewCameraLocation :type "Vector Structure") (NewCameraRotation :type "Rotator Structure") (NewCameraFOV :type "Float (single-precision)") (ReturnValue :type Boolean))
  (locals (LocalTargetLocation :type "Vector Structure" :default (0.0 0.0 0.0)) (LocalTargetRotation :type "Rotator Structure" :default (struct)))
  (bind _returnvalue (`GameplayStatics.GetWorldDeltaSeconds`))
  (bind _currentinterpspeed (`self.CurrentInterpSpeed`))
  ;[1 1 1] Update camera location and rotation
  (bind (_targetlocation _targetrotation) (`self.CalculateTargetCameraPosition` CameraTarget))
  (bind _output_get (set `local.LocalTargetLocation` _targetlocation))
  (bind _output_get_2 (set `local.LocalTargetRotation` _targetrotation))
  (if (`self.ForceUpdateCameraPosition`)
    (set `self.CurrentCameraLocation` _output_get)
    (set `self.CurrentCameraRotation` _output_get_2)
    (set `self.ForceUpdateCameraPosition` false)
    (else
      (set `self.CurrentInterpSpeed` (`KismetMathLibrary.FInterpTo` (`self.CurrentInterpSpeed`) (`self.TargetInterpSpeed`) _returnvalue 5.0))
      (set `self.CurrentCameraLocation` (`KismetMathLibrary.VInterpTo` (`self.CurrentCameraLocation`) (`local.LocalTargetLocation`) _returnvalue _currentinterpspeed))
      (set `self.CurrentCameraRotation` (`KismetMathLibrary.RInterpTo` (`self.CurrentCameraRotation`) (`local.LocalTargetRotation`) _returnvalue _currentinterpspeed))))
  (return (`self.CurrentCameraLocation`) (`self.CurrentCameraRotation`) (`self.DefaultFOV`) true))

(fn `CalculateTargetCameraPosition`
  (params (CameraTarget :type "Actor Object Reference"))
  (returns (TargetLocation :type "Vector Structure") (TargetRotation :type "Rotator Structure"))
  ;[1 1 1] Calculate target camera location and rotation.
  (return (+ (`self.K2_GetActorLocation` CameraTarget) (* (`KismetMathLibrary.GetForwardVector` (`KismetMathLibrary.MakeRotator` 0.0 (- 180.0 (`self.TargetCameraPitch`)) (`self.TargetCameraYaw`))) (`self.TargetCameraLength`))) (`KismetMathLibrary.MakeRotator` 0.0 (* (`self.TargetCameraPitch`) -1.0) (`self.TargetCameraYaw`))))

(fn `InitCameraManagerVariables`
  (returns (Success :type Boolean))
  ;[1 1 1] Init camera manager variables.
  (set `self.TargetCameraYaw` (`self.InitialCameraYaw`))
  (set `self.TargetCameraPitch` (`self.InitialCameraPitch`))
  (set `self.TargetCameraLength` (`self.InitialCameraLength`))
  (set `self.CurrentInterpSpeed` (`self.InitialInterpSpeed`))
  (set `self.ForceUpdateCameraPosition` true)
  (return true))

(fn `SetCameraManagerVariables`
  (params (InitialCameraPitch :type "Float (double-precision)") (InitialCameraYaw :type "Float (double-precision)") (InitialCameraLength :type "Float (double-precision)") (InitialInterpSpeed :type "Float (double-precision)") (ZoomInputScale :type "Float (double-precision)") (MinCameraLength :type "Float (double-precision)") (MaxCameraLength :type "Float (double-precision)"))
  (returns (Success :type Boolean))
  ;[1 1 1] Set initial camera manager variables.
  (set `self.InitialCameraPitch` InitialCameraPitch)
  (set `self.InitialCameraYaw` InitialCameraYaw)
  (set `self.InitialCameraLength` InitialCameraLength)
  (set `self.InitialInterpSpeed` InitialInterpSpeed)
  (set `self.ZoomInputScale` ZoomInputScale)
  (set `self.MinCameraLength` MinCameraLength)
  (set `self.MaxCameraLength` MaxCameraLength)
  (`self.InitCameraManagerVariables`)
  (return true))

(fn `SetCameraRotation`
  (params (Rotation :type "Rotator Structure"))
  (returns (Success :type Boolean))
  ;[1 1 1] Set camera rotation.
  (set `self.TargetCameraPitch` Rotation_Pitch)
  (set `self.TargetCameraYaw` Rotation_Yaw)
  (set `self.ForceUpdateCameraPosition` true)
  (return true))

(fn `SetCameraTurnModeEnabled`
  (params (TurnMode :type Boolean))
  (returns (Success :type Boolean))
  ;[1 1 1] Set turn mode and update player input mode.
  (bind _output_get (set `self.InTurnMode` TurnMode))
  (if _output_get
    (set `self.TargetInterpSpeed` 30.0)
    (else
      (set `self.TargetInterpSpeed` (`self.InitialInterpSpeed`))))
  (return true))

(fn `UserConstructionScript`
  ;[1 1 1] Init player camera manager variables.
  (`self.InitCameraManagerVariables`))