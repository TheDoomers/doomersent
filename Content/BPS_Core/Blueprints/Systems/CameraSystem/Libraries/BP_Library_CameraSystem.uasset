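; Blueprint function library that gives global access to the local player's camera system for yaw, pitch, zoom and turn mode control.
; A finder function looks up the camera manager component on player controller 0.
; Each wrapper forwards its value to that component and returns its result, or false when no manager is found.
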(fn `AddCameraInputPitch`
  (params (Value :type "Float (double-precision)"))
  (returns (Success :type Boolean))
  ;[1 1 1] Add camera input pitch value and update control rotation of the player.
  (bind (_found _manager) (`self.FindCameraManager` null))
  (if _found
    (bind _success (`/Game/BPS_Core/Blueprints/Systems/CameraSystem/Components/BP_AC_CameraManagerComponent.AddCameraInputPitch` _manager Value))
    (return _success)
    (else
      (return false))))

(fn `AddCameraInputYaw`
  (params (Value :type "Float (double-precision)"))
  (returns (Success :type Boolean))
  ;[1 1 1] Add camera input yaw value and update control rotation of the player.
  (bind (_found _manager) (`self.FindCameraManager` null))
  (if _found
    (bind _success (`/Game/BPS_Core/Blueprints/Systems/CameraSystem/Components/BP_AC_CameraManagerComponent.AddCameraInputYaw` _manager Value))
    (return _success)
    (else
      (return false))))

(fn `AddCameraInputZoom`
  (params (Value :type "Float (double-precision)"))
  (returns (Success :type Boolean))
  ;[1 1 1] Add camera input zoom value and update target camera length.
  (bind (_found _manager) (`self.FindCameraManager` null))
  (if _found
    (bind _success (`/Game/BPS_Core/Blueprints/Systems/CameraSystem/Components/BP_AC_CameraManagerComponent.AddCameraInputZoom` _manager Value))
    (return _success)
    (else
      (return false))))

(fn `FindCameraManager`
  (returns (Found :type Boolean) (Manager :type "/Game/BPS_Core/Blueprints/Systems/CameraSystem/Components/BP_AC_CameraManagerComponent Object Reference"))
  (locals (LocalCameraManager :type "/Game/BPS_Core/Blueprints/Systems/CameraSystem/Components/BP_AC_CameraManagerComponent Object Reference"))
  ;[1 1 1] Try to find camera manager component of local player controller.
  (bind _output_get (set `local.LocalCameraManager` (`Actor.GetComponentByClass` (`GameplayStatics.GetPlayerController` null) "/Game/BPS_Core/Blueprints/Systems/CameraSystem/Components/BP_AC_CameraManagerComponent.BP_AC_CameraManagerComponent_C")))
  (`/Engine/EditorBlueprintResources/StandardMacros.IsValid` _output_get
    (:`Is Valid`
      (return true _output_get))
    (:`Is Not Valid`
      (return false null))))

(fn `SetCameraTurnModeEnabled`
  (params (TurnMode :type Boolean))
  (returns (Success :type Boolean))
  ;[1 1 1] Set turn mode and update player input mode.
  (bind (_found _manager) (`self.FindCameraManager` null))
  (if _found
    (bind _success (`/Game/BPS_Core/Blueprints/Systems/CameraSystem/Components/BP_AC_CameraManagerComponent.SetCameraTurnModeEnabled` _manager TurnMode))
    (return _success)
    (else
      (return false))))