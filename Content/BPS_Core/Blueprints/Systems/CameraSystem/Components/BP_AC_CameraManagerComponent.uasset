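; Player controller component that configures and fronts the custom BP_PlayerCameraManager for camera rotation, zoom and turn mode.
; On BeginPlay it pushes initial pitch, yaw, length and zoom settings to the manager, then after a Delay(0) sets the starting control rotation.
; Input functions forward yaw, pitch and zoom to the manager.
; Turn mode changes fire a notification and can switch between game-only and game-and-UI input, toggling the cursor.
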(event `self.ReceiveBeginPlay`
  (bind (_returnvalue_roll _returnvalue_pitch _returnvalue_yaw) (`KismetMathLibrary.BreakRotator` (`Controller.GetControlRotation` (`self.PlayerController`))))
  ;[1 1 1] Begin Play. Init component.
  (`self.TryInitComponent`)
  (`KismetSystemLibrary.Delay` 0.0)
  (if (`self.UseInitialPlayerControlRotation`)
    (`self.SetCameraControlRotation` (`KismetMathLibrary.MakeRotator` _returnvalue_roll _returnvalue_pitch _returnvalue_yaw))
    (else
      (`self.SetCameraControlRotation` (`KismetMathLibrary.MakeRotator` 0.0 (`self.InitialCameraPitch`) (select `bool` (`self.UseInitialPlayerYaw`) :`false` (`self.InitialCameraYaw`) :`true` _returnvalue_yaw :!type "Float (double-precision)"))))))

(fn `AddCameraInputPitch`
  (params (Value :type "Float (double-precision)"))
  (returns (Success :type Boolean))
  (bind _playercameramanager (`self.PlayerCameraManager`))
  ;[1 1 1] Add camera input pitch value and update control rotation of the player.
  (`/Engine/EditorBlueprintResources/StandardMacros.IsValid` _playercameramanager
    (:`Is Valid`
      (bind _success (`/Game/BPS_Core/Blueprints/Systems/CameraSystem/Actors/BP_PlayerCameraManager.AddCameraInputPitch` _playercameramanager Value))
      (return _success))
    (:`Is Not Valid`
      (return false))))

(fn `AddCameraInputYaw`
  (params (Value :type "Float (double-precision)"))
  (returns (Success :type Boolean))
  (bind _playercameramanager (`self.PlayerCameraManager`))
  ;[1 1 1] Add camera input yaw value and update control rotation of the player.
  (`/Engine/EditorBlueprintResources/StandardMacros.IsValid` _playercameramanager
    (:`Is Valid`
      (bind _success (`/Game/BPS_Core/Blueprints/Systems/CameraSystem/Actors/BP_PlayerCameraManager.AddCameraInputYaw` _playercameramanager Value))
      (return _success))
    (:`Is Not Valid`
      (return false))))

(fn `AddCameraInputZoom`
  (params (Value :type "Float (double-precision)"))
  (returns (Success :type Boolean))
  (bind _playercameramanager (`self.PlayerCameraManager`))
  ;[1 1 1] Add camera input zoom value and update target camera length.
  (`/Engine/EditorBlueprintResources/StandardMacros.IsValid` _playercameramanager
    (:`Is Valid`
      (bind _success (`/Game/BPS_Core/Blueprints/Systems/CameraSystem/Actors/BP_PlayerCameraManager.AddCameraInputZoom` _playercameramanager Value))
      (return _success))
    (:`Is Not Valid`
      (return false))))

(fn `InitComponent`
  (returns (Success :type Boolean))
  ;[1 1 1] Try init camera manager component.
  (bind _asplayer_controller (cast `PlayerController` (`self.GetOwner`))
    (:`then`
      (bind _output_get (set `self.PlayerController` _asplayer_controller))
      (bind _asbp_player_camera_manager (cast `/Game/BPS_Core/Blueprints/Systems/CameraSystem/Actors/BP_PlayerCameraManager` (`PlayerController.PlayerCameraManager` _output_get))
        (:`then`
          (bind _output_get_2 (set `self.PlayerCameraManager` _asbp_player_camera_manager))
          (`/Engine/EditorBlueprintResources/StandardMacros.IsValid` _output_get_2
            (:`Is Valid`
              (`/Game/BPS_Core/Blueprints/Systems/CameraSystem/Actors/BP_PlayerCameraManager.SetCameraManagerVariables` _output_get_2 (`self.InitialCameraPitch`) (`self.InitialCameraYaw`) (`self.InitialCameraLength`) (`self.InitialInterpSpeed`) (`self.ZoomInputScale`) (`self.MinCameraLength`) (`self.MaxCameraLength`))
              (`self.SetCameraTurnModeEnabled` (`self.InitialTurnModeEnabled`))
              (return true))
            (:`Is Not Valid`
              _)))
        (:`CastFailed`
          _)))
    (:`CastFailed`
      _))
  (return false))

(fn `SetCameraControlRotation`
  (params (Rotation :type "Rotator Structure"))
  (returns (Success :type Boolean))
  ;[1 1 1] Set camera control rotation.
  (bind _success (`/Game/BPS_Core/Blueprints/Systems/CameraSystem/Actors/BP_PlayerCameraManager.SetCameraRotation` (`self.PlayerCameraManager`) Rotation))
  (`Controller.SetControlRotation` (`self.PlayerController`) Rotation)
  (return _success))

(fn `SetCameraTurnModeEnabled`
  (params (TurnMode :type Boolean))
  (returns (Success :type Boolean))
  (bind _playercameramanager (`self.PlayerCameraManager`))
  (bind _playercontroller (`self.PlayerController`))
  (bind _playercontroller_2 (`self.PlayerController`))
  ;[1 1 1] Set turn mode and update player input mode.
  (`/Engine/EditorBlueprintResources/StandardMacros.IsValid` _playercameramanager
    (:`Is Valid`
      (if (!= (`self.TurnModeIsEnabled`) TurnMode)
        (bind _output_get (set `self.TurnModeIsEnabled` TurnMode))
        (`/Game/BPS_Core/Blueprints/Systems/CameraSystem/Actors/BP_PlayerCameraManager.SetCameraTurnModeEnabled` _playercameramanager _output_get)
        (`|ExecutionSequence`
          (:`then_0`
            (`self.OnTurnModeChanged` self (`self.TurnModeIsEnabled`)))
          (:`then_1`
            (`|ExecutionSequence`
              (:`then_0`
                (if (`self.ChangePlayerInputsOnTurnMode`)
                  (if (`self.TurnModeIsEnabled`)
                    (`WidgetBlueprintLibrary.SetInputMode_GameOnly` _playercontroller_2)
                    (set `PlayerController.bShowMouseCursor` false _playercontroller_2)
                    (else
                      (`WidgetBlueprintLibrary.SetInputMode_GameAndUIEx` _playercontroller null "LockAlways" false)
                      (set `PlayerController.bShowMouseCursor` true _playercontroller)))))
              (:`then_1`
                (return true)))))))))

(fn `TryInitComponent`
  (returns (Success :type Boolean))
  ;[1 1 1] Try init camera manager component.
  (if (not (`self.IsInitialized`))
    (bind _success (`self.InitComponent`))
    (bind _output_get (set `self.IsInitialized` _success))
    (return _output_get)
    (else
      (return true))))

(fn `UpdateCameraControlRotation`
  (returns (Success :type Boolean))
  (bind _playercameramanager (`self.PlayerCameraManager`))
  ;[1 1 1] Update camera control rotation.
  (bind _success (`self.SetCameraControlRotation` (`KismetMathLibrary.MakeRotator` 0.0 (`/Game/BPS_Core/Blueprints/Systems/CameraSystem/Actors/BP_PlayerCameraManager.TargetCameraPitch` _playercameramanager) (`/Game/BPS_Core/Blueprints/Systems/CameraSystem/Actors/BP_PlayerCameraManager.TargetCameraYaw` _playercameramanager))))
  (return _success))