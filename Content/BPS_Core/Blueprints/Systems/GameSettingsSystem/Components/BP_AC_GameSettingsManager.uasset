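; Actor component that manages player game settings, loading or creating a settings save game and saving changes to its slot.
; Typed get/set accessors reach named variables in the save object through Blueprint interface messages, with default maps seeding new saves.
; Audio volumes apply through sound mix class overrides, graphics through GameUserSettings and a volumetric fog console command.
; Init can run a one-time hardware benchmark, reusing texture quality as fog quality.
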(event `self.ReceiveBeginPlay`
  ;[1 1 1] Begin play. Init game settings.
  (if (`self.InitOnBeginPlay`)
    (`self.InitGameSettings`)))

(fn `ApplyAudioSettings`
  (returns (Success :type Boolean))
  ;[1 1 1] Apply, update and save audio settings in current settings save game.
  (`self.UpdateAudioSettings`)
  (`self.SaveGameSettings`)
  (return true))

(fn `ApplyAudioTypeSettings`
  (params (VolumeType :type Name :default "MasterVolume") (VolumeValue :type "Float (double-precision)" :default 1.0))
  (returns (Success :type Boolean))
  (bind (_value _returnvalue) (`BlueprintMapLibrary.Map_Find` (`self.SoundMixes`) VolumeType))
  ;[1 1 1] Apply a specific audio settings and update it in appropriated audio classes.
  (if _returnvalue
    (`GameplayStatics.SetSoundMixClassOverride` _value (`BlueprintMapLibrary.Map_Find` (`self.SoundClasses`) VolumeType) VolumeValue 1.0 0.5)
    (return true)
    (else
      (return false))))

(fn `ApplyGraphicSettings`
  (returns (Success :type Boolean))
  ;[1 1 1] Apply, update and save graphic settings in current settings save game.
  (bind _returnvalue (`GameUserSettings.GetGameUserSettings`))
  (`GameUserSettings.ApplySettings` _returnvalue false)
  (`self.UpdateGraphicSettings`)
  (`self.SaveGameSettings`)
  (return true))

(fn `ApplyGraphicTypeSettings`
  (params (SettingsType :type Name) (SettingsValue :type Integer))
  (returns (Success :type Boolean))
  ;[1 1 1] Apply a specific graphic settings and update for the user.
  (switch `name` SettingsType
    (:`Default`
      (return false))
    (:`VolumetricFogQuality`
      (`KismetSystemLibrary.ExecuteConsoleCommand` (select `int` SettingsValue :`0` "r.VolumetricFog.GridPixelSize 64" :`1` "r.VolumetricFog.GridPixelSize 64" :`2` "r.VolumetricFog.GridPixelSize 32" :`3` "r.VolumetricFog.GridPixelSize 16") null)
      (return true))))

(fn `CheckHardware`
  (returns (Success :type Boolean))
  ;[1 1 1] Checks hardware and updates graphic settings for user.
  (bind (_success _value) (`self.GetBooleanVariable` "HardwareIsChecked"))
  (if (not _value)
    (bind _returnvalue (`GameUserSettings.GetGameUserSettings`))
    (`GameUserSettings.RunHardwareBenchmark` _returnvalue 10 1.0 1.0)
    (`GameUserSettings.ApplyHardwareBenchmarkResults` _returnvalue)
    (bind _returnvalue_2 (`GameUserSettings.GetTextureQuality` _returnvalue))
    (`self.ApplyGraphicTypeSettings` "VolumetricFogQuality" _returnvalue_2)
    (`self.SetIntegerVariable` "VolumetricFogQuality" _returnvalue_2)
    (`self.SetBooleanVariable` "HardwareIsChecked" true)
    (`self.SaveGameSettings`)
    (return true)
    (else
      (return true))))

(fn `CreateSettingsSaveGame`
  (returns (Success :type Boolean))
  ;[1 1 1] Create settings save game object and set default settings to it.
  (bind _returnvalue (`GameplayStatics.CreateSaveGameObject` (`self.SettingsSaveGameClass`)))
  (bind _output_get (set `self.SettingsSaveGame` _returnvalue))
  (bind _success (message `/Game/BPS_Core/Blueprints/Systems/GameSettingsSystem/Interfaces/BPI_SaveGame_Settings.SetDefaultGameSettings_BPI` _output_get (`self.DefaultBooleanSettings`) (`self.DefaultByteSettings`) (`self.DefaultIntegerSettings`) (`self.DefaultFloatSettings`) (`self.DefaultStringSettings`)))
  (if _success
    (`|ExecutionSequence`
      (:`then_0`
        (bind _keys (`BlueprintMapLibrary.Map_Keys` (`self.DefaultAudioSettings`)))
        (for _array_element _keys
          (`self.SetFloatVariable` _array_element (`BlueprintMapLibrary.Map_Find` (`self.DefaultAudioSettings`) _array_element))))
      (:`then_1`
        (`self.SaveGameSettings`)
        (return true)))
    (else
      (return false))))

(fn `GetBooleanVariable`
  (params (VariableName :type Name))
  (returns (Success :type Boolean) (Value :type Boolean))
  ;[1 1 1] Returns a specific boolean variable from the current settings save game.
  (bind (_success _value) (message `/Game/BPS_Core/Blueprints/Systems/GameSettingsSystem/Interfaces/BPI_SaveGame_Settings.GetBooleanGameSettingsVariable_BPI` (`self.GetSettingsSaveGame`) VariableName))
  (return _success _value))

(fn `GetByteVariable`
  (params (VariableName :type Name))
  (returns (Success :type Boolean) (Value :type Byte))
  ;[1 1 1] Returns a specific byte variable from the current settings save game.
  (bind (_success _value) (message `/Game/BPS_Core/Blueprints/Systems/GameSettingsSystem/Interfaces/BPI_SaveGame_Settings.GetByteGameSettingsVariable_BPI` (`self.GetSettingsSaveGame`) VariableName))
  (return _success _value))

(fn `GetFloatVariable`
  (params (VariableName :type Name))
  (returns (Success :type Boolean) (Value :type "Float (double-precision)"))
  ;[1 1 1] Returns a specific float variable from the current settings save game.
  (bind (_success _value) (message `/Game/BPS_Core/Blueprints/Systems/GameSettingsSystem/Interfaces/BPI_SaveGame_Settings.GetFloatGameSettingsVariable_BPI` (`self.GetSettingsSaveGame`) VariableName))
  (return _success _value))

(fn `GetIntegerVariable`
  (params (VariableName :type Name))
  (returns (Success :type Boolean) (Value :type Integer))
  ;[1 1 1] Returns a specific integer variable from the current settings save game.
  (bind (_success _value) (message `/Game/BPS_Core/Blueprints/Systems/GameSettingsSystem/Interfaces/BPI_SaveGame_Settings.GetIntegerGameSettingsVariable_BPI` (`self.GetSettingsSaveGame`) VariableName))
  (return _success _value))

(fn `GetSettingsSaveGame`
  (returns (SettingsSaveGame :type "SaveGame Object Reference"))
  ;[1 1 1] Returns settings save game object reference. Creates the new one if save game object is does not exist.
  (`/Engine/EditorBlueprintResources/StandardMacros.IsValid` (`self.SettingsSaveGame`)
    (:`Is Valid`
      _)
    (:`Is Not Valid`
      (bind _returnvalue (`GameplayStatics.LoadGameFromSlot` (`self.SettingsSaveSlotName`)))
      (`/Engine/EditorBlueprintResources/StandardMacros.IsValid` _returnvalue
        (:`Is Valid`
          (set `self.SettingsSaveGame` _returnvalue))
        (:`Is Not Valid`
          (`self.CreateSettingsSaveGame`)))))
  (return (`self.SettingsSaveGame`)))

(fn `GetStringVariable`
  (params (VariableName :type Name))
  (returns (Success :type Boolean) (Value :type String))
  ;[1 1 1] Returns a specific string variable from the current settings save game.
  (bind (_success _value) (message `/Game/BPS_Core/Blueprints/Systems/GameSettingsSystem/Interfaces/BPI_SaveGame_Settings.GetStringGameSettingsVariable_BPI` (`self.GetSettingsSaveGame`) VariableName))
  (return _success _value))

(fn `InitGameSettings`
  (returns (Success :type Boolean))
  ;[1 1 1] Init and update game settings. Also check hardware if required.
  (set `self.SettingsSaveGame` (`self.GetSettingsSaveGame`))
  (`|ExecutionSequence`
    (:`then_0`
      (if (`self.CheckHardwareOnInit`)
        (`self.CheckHardware`)))
    (:`then_1`
      (`|ExecutionSequence`
        (:`then_0`
          (`GameplayStatics.SetBaseSoundMix` (`self.BaseSoundMix`))
          (`self.UpdateAudioSettings`))
        (:`then_1`
          (return true))))))

(fn `ResetAudioSettings`
  (returns (Success :type Boolean))
  ;[1 1 1] Reset audio settings to default values and save it to settings save game.
  (bind _keys (`BlueprintMapLibrary.Map_Keys` (`self.DefaultAudioSettings`)))
  (for _array_element _keys
    (`self.SetFloatVariable` _array_element (`BlueprintMapLibrary.Map_Find` (`self.DefaultAudioSettings`) _array_element)))
  (`self.UpdateAudioSettings`)
  (`self.SaveGameSettings`)
  (return true))

(fn `ResetGameSettings`
  (returns (Success :type Boolean))
  ;[1 1 1] Reset game settings in current settings save game.
  (bind _success (message `/Game/BPS_Core/Blueprints/Systems/GameSettingsSystem/Interfaces/BPI_SaveGame_Settings.ResetGameSettings_BPI` (`self.GetSettingsSaveGame`)))
  (if _success
    (`self.SaveGameSettings`)
    (return true)
    (else
      (return false))))

(fn `SaveGameSettings`
  (returns (Success :type Boolean))
  ;[1 1 1] Save game settings in settings save game.
  (`GameplayStatics.SaveGameToSlot` (`self.GetSettingsSaveGame`) (`self.SettingsSaveSlotName`))
  (return true))

(fn `SetBooleanVariable`
  (params (VariableName :type Name) (VariableValue :type Boolean))
  (returns (Success :type Boolean))
  ;[1 1 1] Set a specific boolean variable to the current settings save game.
  (bind _success (message `/Game/BPS_Core/Blueprints/Systems/GameSettingsSystem/Interfaces/BPI_SaveGame_Settings.SetBooleanGameSettingsVariable_BPI` (`self.GetSettingsSaveGame`) VariableName VariableValue))
  (return _success))

(fn `SetByteVariable`
  (params (VariableName :type Name) (VariableValue :type Byte))
  (returns (Success :type Boolean))
  ;[1 1 1] Set a specific byte variable to the current settings save game.
  (bind _success (message `/Game/BPS_Core/Blueprints/Systems/GameSettingsSystem/Interfaces/BPI_SaveGame_Settings.SetByteGameSettingsVariable_BPI` (`self.GetSettingsSaveGame`) VariableName VariableValue))
  (return _success))

(fn `SetFloatVariable`
  (params (VariableName :type Name) (VariableValue :type "Float (double-precision)"))
  (returns (Success :type Boolean))
  ;[1 1 1] Set a specific float variable to the current settings save game.
  (bind _success (message `/Game/BPS_Core/Blueprints/Systems/GameSettingsSystem/Interfaces/BPI_SaveGame_Settings.SetFloatGameSettingsVariable_BPI` (`self.GetSettingsSaveGame`) VariableName VariableValue))
  (return _success))

(fn `SetIntegerVariable`
  (params (VariableName :type Name) (VariableValue :type Integer))
  (returns (Success :type Boolean))
  ;[1 1 1] Set a specific integer variable to the current settings save game.
  (bind _success (message `/Game/BPS_Core/Blueprints/Systems/GameSettingsSystem/Interfaces/BPI_SaveGame_Settings.SetIntegerGameSettingsVariable_BPI` (`self.GetSettingsSaveGame`) VariableName VariableValue))
  (return _success))

(fn `SetStringVariable`
  (params (VariableName :type Name) (VariableValue :type String))
  (returns (Success :type Boolean))
  ;[1 1 1] Set a specific string variable to the current settings save game.
  (bind _success (message `/Game/BPS_Core/Blueprints/Systems/GameSettingsSystem/Interfaces/BPI_SaveGame_Settings.SetStringGameSettingsVariable_BPI` (`self.GetSettingsSaveGame`) VariableName VariableValue))
  (return _success))

(fn `UpdateAudioSettings`
  (returns (Success :type Boolean))
  (bind _soundmixes (`self.SoundMixes`))
  ;[1 1 1] Update audio settings for all audio classes.
  (bind _keys (`BlueprintMapLibrary.Map_Keys` _soundmixes))
  (`BlueprintMapLibrary.Map_Values` _soundmixes)
  (for _array_element _keys
    (bind (_success _value) (`self.GetFloatVariable` _array_element))
    (if _success
      (bind (_value_2 _returnvalue) (`BlueprintMapLibrary.Map_Find` (`self.SoundMixes`) _array_element))
      (if _returnvalue
        (`GameplayStatics.SetSoundMixClassOverride` _value_2 (`BlueprintMapLibrary.Map_Find` (`self.SoundClasses`) _array_element) _value 1.0 0.2))))
  (return true))

(fn `UpdateGraphicSettings`
  (returns (Success :type Boolean))
  ;[1 1 1] Update custom graphic settings.
  (bind (_success _value) (`self.GetIntegerVariable` "VolumetricFogQuality"))
  (`KismetSystemLibrary.ExecuteConsoleCommand` (select `int` _value :`0` "r.VolumetricFog.GridPixelSize 64" :`1` "r.VolumetricFog.GridPixelSize 64" :`2` "r.VolumetricFog.GridPixelSize 32" :`3` "r.VolumetricFog.GridPixelSize 16") null)
  (return true))