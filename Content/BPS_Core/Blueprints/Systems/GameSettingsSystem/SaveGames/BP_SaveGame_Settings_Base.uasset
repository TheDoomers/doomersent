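; Base SaveGame Blueprint that stores game settings for the settings system as name-keyed maps of boolean, byte, integer, float and string values.
; Interface functions read a value with a success flag or write it into the matching saved map.
; A separate set of default maps is supplied from outside, and reset copies those defaults over the saved values.
; Writing to or loading from disk is not handled here.
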(fn `GetBooleanGameSettingsVariable_BPI`
  (params (VariableName :type Name))
  (returns (Success :type Boolean) (Value :type Boolean))
  (bind (_value _returnvalue) (`BlueprintMapLibrary.Map_Find` (`self.SavedBooleanVariables`) VariableName))
  ;[1 1 1] Returns boolean value of specific game settings variable.
  (return _returnvalue _value))

(fn `GetByteGameSettingsVariable_BPI`
  (params (VariableName :type Name))
  (returns (Success :type Boolean) (Value :type Byte))
  (bind (_value _returnvalue) (`BlueprintMapLibrary.Map_Find` (`self.SavedByteVariables`) VariableName))
  ;[1 1 1] Returns byte value of specific game settings variable.
  (return _returnvalue _value))

(fn `GetFloatGameSettingsVariable_BPI`
  (params (VariableName :type Name))
  (returns (Success :type Boolean) (Value :type "Float (double-precision)"))
  (bind (_value _returnvalue) (`BlueprintMapLibrary.Map_Find` (`self.SavedFloatVariables`) VariableName))
  ;[1 1 1] Returns float value of specific game settings variable.
  (return _returnvalue _value))

(fn `GetIntegerGameSettingsVariable_BPI`
  (params (VariableName :type Name))
  (returns (Success :type Boolean) (Value :type Integer))
  (bind (_value _returnvalue) (`BlueprintMapLibrary.Map_Find` (`self.SavedIntegerVariables`) VariableName))
  ;[1 1 1] Returns integer value of specific game settings variable.
  (return _returnvalue _value))

(fn `GetStringGameSettingsVariable_BPI`
  (params (VariableName :type Name))
  (returns (Success :type Boolean) (Value :type String))
  (bind (_value _returnvalue) (`BlueprintMapLibrary.Map_Find` (`self.SavedStringVariables`) VariableName))
  ;[1 1 1] Returns string value of specific game settings variable.
  (return _returnvalue _value))

(fn `ResetGameSettings_BPI`
  (returns (Success :type Boolean))
  ;[1 1 1] Reset values of game settings variables.
  (set `self.SavedBooleanVariables` (`self.DefaultBooleanVariables`))
  (set `self.SavedByteVariables` (`self.DefaultByteVariables`))
  (set `self.SavedIntegerVariables` (`self.DefaultIntegerVariables`))
  (set `self.SavedFloatVariables` (`self.DefaultFloatVariables`))
  (set `self.SavedStringVariables` (`self.DefaultStringVariables`))
  (return true))

(fn `SetBooleanGameSettingsVariable_BPI`
  (params (VariableName :type Name) (VariableValue :type Boolean))
  (returns (Success :type Boolean))
  ;[1 1 1] Set boolean value of specific variable in game settings.
  (`BlueprintMapLibrary.Map_Add` (`self.SavedBooleanVariables`) VariableName VariableValue)
  (return true))

(fn `SetByteGameSettingsVariable_BPI`
  (params (VariableName :type Name) (VariableValue :type Byte))
  (returns (Success :type Boolean))
  ;[1 1 1] Set byte value of specific variable in game settings.
  (`BlueprintMapLibrary.Map_Add` (`self.SavedByteVariables`) VariableName VariableValue)
  (return true))

(fn `SetDefaultGameSettings_BPI`
  (params (BooleanVariables :type "Map of Name to Boolean") (ByteVariables :type "Map of Name to Byte") (IntegerVariables :type "Map of Name to Integer") (FloatVariables :type "Map of Name to Float (double-precision)") (StringVariables :type "Map of Name to String"))
  (returns (Success :type Boolean))
  ;[1 1 1] Set default values of game settings variables.
  (set `self.DefaultBooleanVariables` BooleanVariables)
  (set `self.DefaultByteVariables` ByteVariables)
  (set `self.DefaultIntegerVariables` IntegerVariables)
  (set `self.DefaultFloatVariables` FloatVariables)
  (set `self.DefaultStringVariables` StringVariables)
  (return true))

(fn `SetFloatGameSettingsVariable_BPI`
  (params (VariableName :type Name) (VariableValue :type "Float (double-precision)"))
  (returns (Success :type Boolean))
  ;[1 1 1] Set float value of specific variable in game settings.
  (`BlueprintMapLibrary.Map_Add` (`self.SavedFloatVariables`) VariableName VariableValue)
  (return true))

(fn `SetIntegerGameSettingsVariable_BPI`
  (params (VariableName :type Name) (VariableValue :type Integer))
  (returns (Success :type Boolean))
  ;[1 1 1] Set integer value of specific variable in game settings.
  (`BlueprintMapLibrary.Map_Add` (`self.SavedIntegerVariables`) VariableName VariableValue)
  (return true))

(fn `SetStringGameSettingsVariable_BPI`
  (params (VariableName :type Name) (VariableValue :type String))
  (returns (Success :type Boolean))
  ;[1 1 1] Set string value of specific variable in game settings.
  (`BlueprintMapLibrary.Map_Add` (`self.SavedStringVariables`) VariableName VariableValue)
  (return true))