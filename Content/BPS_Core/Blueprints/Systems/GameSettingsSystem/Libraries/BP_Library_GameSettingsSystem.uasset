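; Blueprint function library that gives global access to the game settings system through BP_AC_GameSettingsManager on the Game State.
; Each function finds that component and forwards the call, returning false or default values when it is missing.
; Wrappers cover saving, resetting, updating and applying audio or graphic settings, plus typed access to save-game variables by name.
; UpdateGraphicSettings calls the component's UpdateAudioSettings rather than a graphics update.
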(fn `ApplyAudioSettings`
  (returns (Success :type Boolean))
  ;[1 1 1] Try to apply current audio settings.
  (bind (_success _component) (`self.FindGameSettingsManager` null))
  (if _success
    (bind _success_2 (`/Game/BPS_Core/Blueprints/Systems/GameSettingsSystem/Components/BP_AC_GameSettingsManager.ApplyAudioSettings` _component))
    (return _success_2)
    (else
      (return false))))

(fn `ApplyGraphicSettings`
  (returns (Success :type Boolean))
  ;[1 1 1] Try to apply current graphic settings.
  (bind (_success _component) (`self.FindGameSettingsManager` null))
  (if _success
    (bind _success_2 (`/Game/BPS_Core/Blueprints/Systems/GameSettingsSystem/Components/BP_AC_GameSettingsManager.ApplyGraphicSettings` _component))
    (return _success_2)
    (else
      (return false))))

(fn `FindGameSettingsManager`
  (returns (Success :type Boolean) (Component :type "/Game/BPS_Core/Blueprints/Systems/GameSettingsSystem/Components/BP_AC_GameSettingsManager Object Reference"))
  (locals (LocalGameSettingsManager :type "/Game/BPS_Core/Blueprints/Systems/GameSettingsSystem/Components/BP_AC_GameSettingsManager Object Reference"))
  ;[1 1 1] Try to find game settings manager component from the game state class.
  (bind _output_get (set `local.LocalGameSettingsManager` (`Actor.GetComponentByClass` (`GameplayStatics.GetGameState` null) "/Game/BPS_Core/Blueprints/Systems/GameSettingsSystem/Components/BP_AC_GameSettingsManager.BP_AC_GameSettingsManager_C")))
  (`/Engine/EditorBlueprintResources/StandardMacros.IsValid` _output_get
    (:`Is Valid`
      (return true (`local.LocalGameSettingsManager`)))
    (:`Is Not Valid`
      (`KismetSystemLibrary.PrintText` null "Game settings manager component is not found! \nGame settings manager component should be a part of the game state class." true true (struct :`R` 1.0 :`A` 1.0) 10.0)
      (return false null))))

(fn `GetBooleanGameSettingsVariable`
  (params (VariableName :type Name))
  (returns (Success :type Boolean) (Value :type Boolean))
  ;[1 1 1] Returns a specific boolean variable from the current settings save game.
  (bind (_success _component) (`self.FindGameSettingsManager` null))
  (if _success
    (bind (_success_2 _value) (`/Game/BPS_Core/Blueprints/Systems/GameSettingsSystem/Components/BP_AC_GameSettingsManager.GetBooleanVariable` _component VariableName))
    (return _success_2 _value)
    (else
      (return false false))))

(fn `GetByteGameSettingsVariable`
  (params (VariableName :type Name))
  (returns (Success :type Boolean) (Value :type Byte))
  ;[1 1 1] Returns a specific byte variable from the current settings save game.
  (bind (_success _component) (`self.FindGameSettingsManager` null))
  (if _success
    (bind (_success_2 _value) (`/Game/BPS_Core/Blueprints/Systems/GameSettingsSystem/Components/BP_AC_GameSettingsManager.GetByteVariable` _component VariableName))
    (return _success_2 _value)
    (else
      (return false 0))))

(fn `GetFloatGameSettingsVariable`
  (params (VariableName :type Name))
  (returns (Success :type Boolean) (Value :type "Float (double-precision)"))
  ;[1 1 1] Returns a specific float variable from the current settings save game.
  (bind (_success _component) (`self.FindGameSettingsManager` null))
  (if _success
    (bind (_success_2 _value) (`/Game/BPS_Core/Blueprints/Systems/GameSettingsSystem/Components/BP_AC_GameSettingsManager.GetFloatVariable` _component VariableName))
    (return _success_2 _value)
    (else
      (return false 0.0))))

(fn `GetIntegerGameSettingsVariable`
  (params (VariableName :type Name))
  (returns (Success :type Boolean) (Value :type Integer))
  ;[1 1 1] Returns a specific integer variable from the current settings save game.
  (bind (_success _component) (`self.FindGameSettingsManager` null))
  (if _success
    (bind (_success_2 _value) (`/Game/BPS_Core/Blueprints/Systems/GameSettingsSystem/Components/BP_AC_GameSettingsManager.GetIntegerVariable` _component VariableName))
    (return _success_2 _value)
    (else
      (return false 0))))

(fn `GetStringGameSettingsVariable`
  (params (VariableName :type Name))
  (returns (Success :type Boolean) (Value :type String))
  ;[1 1 1] Returns a specific string variable from the current settings save game.
  (bind (_success _component) (`self.FindGameSettingsManager` null))
  (if _success
    (bind (_success_2 _value) (`/Game/BPS_Core/Blueprints/Systems/GameSettingsSystem/Components/BP_AC_GameSettingsManager.GetStringVariable` _component VariableName))
    (return _success_2 _value)
    (else
      (return false ""))))

(fn `ResetAudioSettings`
  (returns (Success :type Boolean))
  ;[1 1 1] Try to reset current audio settings.
  (bind (_success _component) (`self.FindGameSettingsManager` null))
  (if _success
    (bind _success_2 (`/Game/BPS_Core/Blueprints/Systems/GameSettingsSystem/Components/BP_AC_GameSettingsManager.ResetAudioSettings` _component))
    (return _success_2)
    (else
      (return false))))

(fn `ResetGameSettings`
  (returns (Success :type Boolean))
  ;[1 1 1] Try to reset current game settings.
  (bind (_success _component) (`self.FindGameSettingsManager` null))
  (if _success
    (bind _success_2 (`/Game/BPS_Core/Blueprints/Systems/GameSettingsSystem/Components/BP_AC_GameSettingsManager.ResetGameSettings` _component))
    (return _success_2)
    (else
      (return false))))

(fn `SaveGameSettings`
  (returns (Success :type Boolean))
  ;[1 1 1] Try to save current game settings.
  (bind (_success _component) (`self.FindGameSettingsManager` null))
  (if _success
    (bind _success_2 (`/Game/BPS_Core/Blueprints/Systems/GameSettingsSystem/Components/BP_AC_GameSettingsManager.SaveGameSettings` _component))
    (return _success_2)
    (else
      (return false))))

(fn `SetAudioTypeSettings`
  (params (VolumeType :type Name :default "MasterVolume") (VolumeValue :type "Float (double-precision)" :default 1.0))
  (returns (Success :type Boolean))
  ;[1 1 1] Try to set and apply a specific audio settings.
  (bind (_success _component) (`self.FindGameSettingsManager` null))
  (if _success
    (bind _success_2 (`/Game/BPS_Core/Blueprints/Systems/GameSettingsSystem/Components/BP_AC_GameSettingsManager.ApplyAudioTypeSettings` _component VolumeType VolumeValue))
    (return _success_2)
    (else
      (return false))))

(fn `SetBooleanGameSettingsVariable`
  (params (VariableName :type Name) (VariableValue :type Boolean))
  (returns (Success :type Boolean))
  ;[1 1 1] Set a specific boolean variable to the current settings save game.
  (bind (_success _component) (`self.FindGameSettingsManager` null))
  (if _success
    (bind _success_2 (`/Game/BPS_Core/Blueprints/Systems/GameSettingsSystem/Components/BP_AC_GameSettingsManager.SetBooleanVariable` _component VariableName VariableValue))
    (return _success_2)
    (else
      (return false))))

(fn `SetByteGameSettingsVariable`
  (params (VariableName :type Name) (VariableValue :type Byte))
  (returns (Success :type Boolean))
  ;[1 1 1] Set a specific byte variable to the current settings save game.
  (bind (_success _component) (`self.FindGameSettingsManager` null))
  (if _success
    (bind _success_2 (`/Game/BPS_Core/Blueprints/Systems/GameSettingsSystem/Components/BP_AC_GameSettingsManager.SetByteVariable` _component VariableName VariableValue))
    (return _success_2)
    (else
      (return false))))

(fn `SetFloatGameSettingsVariable`
  (params (VariableName :type Name) (VariableValue :type "Float (double-precision)" :default 0.0))
  (returns (Success :type Boolean))
  ;[1 1 1] Set a specific float variable to the current settings save game.
  (bind (_success _component) (`self.FindGameSettingsManager` null))
  (if _success
    (bind _success_2 (`/Game/BPS_Core/Blueprints/Systems/GameSettingsSystem/Components/BP_AC_GameSettingsManager.SetFloatVariable` _component VariableName VariableValue))
    (return _success_2)
    (else
      (return false))))

(fn `SetGraphicTypeSettings`
  (params (SettingsType :type Name) (SettingsValue :type Integer))
  (returns (Success :type Boolean))
  ;[1 1 1] Try to set and apply a specific graphic settings.
  (bind (_success _component) (`self.FindGameSettingsManager` null))
  (if _success
    (bind _success_2 (`/Game/BPS_Core/Blueprints/Systems/GameSettingsSystem/Components/BP_AC_GameSettingsManager.ApplyGraphicTypeSettings` _component SettingsType SettingsValue))
    (return _success_2)
    (else
      (return false))))

(fn `SetIntegerGameSettingsVariable`
  (params (VariableName :type Name) (VariableValue :type Integer))
  (returns (Success :type Boolean))
  ;[1 1 1] Set a specific integer variable to the current settings save game.
  (bind (_success _component) (`self.FindGameSettingsManager` null))
  (if _success
    (bind _success_2 (`/Game/BPS_Core/Blueprints/Systems/GameSettingsSystem/Components/BP_AC_GameSettingsManager.SetIntegerVariable` _component VariableName VariableValue))
    (return _success_2)
    (else
      (return false))))

(fn `SetStringGameSettingsVariable`
  (params (VariableName :type Name) (VariableValue :type String))
  (returns (Success :type Boolean))
  ;[1 1 1] Set a specific string variable to the current settings save game.
  (bind (_success _component) (`self.FindGameSettingsManager` null))
  (if _success
    (bind _success_2 (`/Game/BPS_Core/Blueprints/Systems/GameSettingsSystem/Components/BP_AC_GameSettingsManager.SetStringVariable` _component VariableName VariableValue))
    (return _success_2)
    (else
      (return false))))

(fn `UpdateAudioSettings`
  (returns (Success :type Boolean))
  ;[1 1 1] Try to update current audio settings.
  (bind (_success _component) (`self.FindGameSettingsManager` null))
  (if _success
    (bind _success_2 (`/Game/BPS_Core/Blueprints/Systems/GameSettingsSystem/Components/BP_AC_GameSettingsManager.UpdateAudioSettings` _component))
    (return _success_2)
    (else
      (return false))))

(fn `UpdateGraphicSettings`
  (returns (Success :type Boolean))
  ;[1 1 1] Try to update current graphic settings.
  (bind (_success _component) (`self.FindGameSettingsManager` null))
  (if _success
    (bind _success_2 (`/Game/BPS_Core/Blueprints/Systems/GameSettingsSystem/Components/BP_AC_GameSettingsManager.UpdateAudioSettings` _component))
    (return _success_2)
    (else
      (return false))))