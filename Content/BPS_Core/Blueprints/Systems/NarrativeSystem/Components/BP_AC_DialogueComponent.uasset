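; Actor component that makes its owner a dialogue speaker with name, icon and voice, starting conversations through the player's narrative manager.
; It tracks the manager and target, firing started and ended events, and fading audio on end.
; Replies come from DataTable rows, preferring a context-based DialogueWave over a plain sound, played 2D or attached.
; The audio component is shared with the manager; multicast replication always requests attached playback.
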(event `PlayDialogueReply (Multicast)`
  (params (ReplyHandle :type "DataTableRowHandle Structure") (TargetActors :type "Array of Actor Object Reference") (PlaySound2D :type Boolean))
  ;[1 1 1] Play dialogue reply for everyone.
  (`self.PlayDialogueReply` ReplyHandle TargetActors PlaySound2D))

(fn `DestroyAudioComponent`
  (returns (Success :type Boolean))
  (bind _audiocomponent (`self.AudioComponent`))
  ;[1 1 1] Destroy audio component.
  (`/Engine/EditorBlueprintResources/StandardMacros.IsValid` _audiocomponent
    (:`Is Valid`
      (`self.K2_DestroyComponent` _audiocomponent))
    (:`Is Not Valid`
      _))
  (return true))

(fn `EndDialogue`
  (returns (Success :type Boolean))
  (bind _audiocomponent (`self.AudioComponent`))
  ;[1 1 1] Set dialogue ended variables and call dialogue ended event.
  (`/Engine/EditorBlueprintResources/StandardMacros.IsValid` _audiocomponent
    (:`Is Valid`
      (`AudioComponent.FadeOut` _audiocomponent 0.5 0.0 "Linear"))
    (:`Is Not Valid`
      _))
  (`self.SetNarrativeManager` null)
  (`self.SetDialogueTarget` null)
  (if (`self.DialogueIsStarted`)
    (set `self.DialogueIsStarted` false)
    (`self.OnDialogueEnded` self))
  (return true))

(fn `GetSpeakerIcon`
  (returns (SpeakerIcon :type "Texture2D Object Reference"))
  ;[1 1 1] Returns speaker icon.
  (return (`self.SpeakerIcon`)))

(fn `GetSpeakerName`
  (returns (SpeakerName :type Text))
  ;[1 1 1] Returns speaker name.
  (return (`self.SpeakerName`)))

(fn `GetSpeakerVoice`
  (returns (SpeakerVoice :type "DialogueVoice Object Reference"))
  ;[1 1 1] Returns speaker voice.
  (return (`self.SpeakerVoice`)))

(fn `GetTargetActor`
  (returns (TargetActor :type "Actor Object Reference"))
  ;[1 1 1] Returns target actor.
  (return (`self.TargetActor`)))

(fn `PlayDialogueReply`
  (params (ReplyHandle :type "DataTableRowHandle Structure") (TargetActors :type "Array of Actor Object Reference") (PlaySound2D :type Boolean))
  (returns (Success :type Boolean))
  (locals (LocalReplyHandle :type "DataTableRowHandle Structure") (LocalTargetActors :type "Array of Actor Object Reference") (LocalDialogueReply :type "/Game/BPS_Core/Blueprints/Systems/NarrativeSystem/Structures/STR_DialogueReply Structure") (LocalPlaySound2D :type Boolean))
  (bind _localplaysound2d (`local.LocalPlaySound2D`))
  ;[1 1 1] Play dialogue reply sound and call the on dialogue reply played event.
  (bind _output_get (set `local.LocalReplyHandle` ReplyHandle))
  (set `local.LocalTargetActors` TargetActors)
  (set `local.LocalPlaySound2D` PlaySound2D)
  (bind (_datatable _rowname) (break `DataTableRowHandle` _output_get))
  (`/Engine/EditorBlueprintResources/StandardMacros.IsValid` _datatable
    (:`Is Valid`
      (bind _returnvalue (`|GetDataTableRow` _datatable _rowname)
        (:`then`
          (set `local.LocalDialogueReply` _returnvalue)
          (bind ((`ReplySound_44_1A8FD76E44A73F8FAE32929DABBE06C4` _replysound) (`ReplyWave_43_EC92078447479115FF1F459ADCB62598` _replywave)) (break `/Game/BPS_Core/Blueprints/Systems/NarrativeSystem/Structures/STR_DialogueReply` _returnvalue))
          (`/Engine/EditorBlueprintResources/StandardMacros.IsValid` _replywave
            (:`Is Valid`
              (bind (_success _dialoguecontext) (`/Game/BPS_Core/Blueprints/Systems/NarrativeSystem/Libraries/BP_Library_NarrativeSystem.MakeDialogueContext` (`self.GetOwner`) (`local.LocalTargetActors`)))
              (if _success
                (`self.PlayDialogueWave` _replywave _dialoguecontext _localplaysound2d)
                (`self.OnDialogueReplyPlayed` self (`local.LocalDialogueReply`) :!label _label)
                (return true)
                (else
                  _)))
            (:`Is Not Valid`
              (`/Engine/EditorBlueprintResources/StandardMacros.IsValid` _replysound
                (:`Is Valid`
                  (`self.PlayDialogueSound` _replysound _localplaysound2d)
                  (goto _label))
                (:`Is Not Valid`
                  _))))
          (return false))
        (:`RowNotFound`
          _)))
    (:`Is Not Valid`
      _))
  (return false))

(fn `PlayDialogueReplyReplicated`
  (params (ReplyHandle :type "DataTableRowHandle Structure") (TargetActors :type "Array of Actor Object Reference (by ref)") (PlaySound2D :type Boolean))
  (returns (Success :type Boolean))
  ;[1 1 1] Try to play dialogue reply for everyone.
  (`self.PlayDialogueReply (Multicast)` ReplyHandle TargetActors)
  (return true))

(fn `PlayDialogueSound`
  (params (DialogueSound :type "SoundBase Object Reference") (PlaySound2D :type Boolean))
  (returns (Success :type Boolean))
  ;[1 1 1] Try to play dialogue sound.
  (`self.DestroyAudioComponent`)
  (if PlaySound2D
    (bind _returnvalue (`GameplayStatics.SpawnSound2D` DialogueSound 1.0 1.0 0.0 null))
    (`self.SetAudioComponent` _returnvalue)
    (return true)
    (else
      (bind _returnvalue_2 (`GameplayStatics.SpawnSoundAttached` DialogueSound (`Actor.RootComponent` (`self.GetOwner`)) "None" (0.0 0.0 0.0) (struct) "KeepRelativeOffset" true 1.0 1.0 0.0 null null))
      (`self.SetAudioComponent` _returnvalue_2)
      (return true))))

(fn `PlayDialogueWave`
  (params (DialogueWave :type "DialogueWave Object Reference") (DialogueContext :type "DialogueContext Structure") (PlaySound2D :type Boolean))
  (returns (Success :type Boolean))
  ;[1 1 1] Try to play dialogue wave.
  (`self.DestroyAudioComponent`)
  (if PlaySound2D
    (bind _returnvalue (`GameplayStatics.SpawnDialogue2D` DialogueWave DialogueContext))
    (`self.SetAudioComponent` _returnvalue)
    (return true)
    (else
      (bind _returnvalue_2 (`GameplayStatics.SpawnDialogueAttached` DialogueWave DialogueContext (`Actor.RootComponent` (`self.GetOwner`)) "None" (0.0 0.0 0.0) (struct) "KeepRelativeOffset" true 1.0 1.0 0.0 null))
      (`self.SetAudioComponent` _returnvalue_2)
      (return true))))

(fn `SetAudioComponent`
  (params (AudioComponent :type "AudioComponent Object Reference"))
  (returns (Success :type Boolean))
  (bind _narrativemanager (`self.NarrativeManager`))
  ;[1 1 1] Set audio component reference.
  (bind _output_get (set `self.AudioComponent` AudioComponent))
  (`/Engine/EditorBlueprintResources/StandardMacros.IsValid` _narrativemanager
    (:`Is Valid`
      (`/Game/BPS_Core/Blueprints/Systems/NarrativeSystem/Components/BP_AC_NarrativeManager.SetAudioComponent` _narrativemanager _output_get))
    (:`Is Not Valid`
      _))
  (return true))

(fn `SetDialogueTarget`
  (params (TargetActor :type "Actor Object Reference"))
  (returns (Success :type Boolean))
  ;[1 1 1] Set dialogue target reference.
  (set `self.TargetActor` TargetActor)
  (return true))

(fn `SetNarrativeManager`
  (params (NarrativeManager :type "/Game/BPS_Core/Blueprints/Systems/NarrativeSystem/Components/BP_AC_NarrativeManager Object Reference"))
  (returns (Success :type Boolean))
  ;[1 1 1] Set narrative manager component reference.
  (set `self.NarrativeManager` NarrativeManager)
  (return true))

(fn `StartDialogue`
  (params (DialogueManager :type "/Game/BPS_Core/Blueprints/Systems/NarrativeSystem/Components/BP_AC_NarrativeManager Object Reference") (TargetActor :type "Actor Object Reference"))
  (returns (Success :type Boolean))
  ;[1 1 1] Set dialogue started variables and call dialogue started event.
  (`self.SetNarrativeManager` DialogueManager)
  (`self.SetDialogueTarget` TargetActor)
  (if (not (`self.DialogueIsStarted`))
    (set `self.DialogueIsStarted` true)
    (`self.OnDialogueStarted` self))
  (return true))

(fn `TryStartDialogue`
  (params (PlayerController :type "PlayerController Object Reference"))
  (returns (Success :type Boolean))
  ;[1 1 1] Try to start dialogue for the player.
  (if (`/Game/BPS_Core/Blueprints/Systems/CoreSystem/Libraries/BP_Library_CoreFunctions.HandleIsValid` (`self.DialogueHandle`))
    (bind (_found _manager) (`/Game/BPS_Core/Blueprints/Systems/NarrativeSystem/Libraries/BP_Library_NarrativeSystem.FindNarrativeManager` PlayerController))
    (if _found
      (`/Game/BPS_Core/Blueprints/Systems/NarrativeSystem/Components/BP_AC_NarrativeManager.TryStartDialogue` _manager (`self.DialogueHandle`) (`self.GetOwner`))
      (return true)
      (else
        (return false)))))