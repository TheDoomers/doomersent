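; Blueprint function library for the narrative system, providing helpers for quests and dialogue.
; Lookup functions find the narrative manager and dialogue components on an actor.
; MakeDialogueContext gathers speaker and target voices from dialogue components, failing if any participant lacks one.
; Quest helpers find the manager on the player controller and forward requests to start a quest or a specific stage, with optional restart.
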(fn `FindDialogueComponent`
  (params (TargetActor :type "Actor Object Reference"))
  (returns (Found :type Boolean) (Component :type "/Game/BPS_Core/Blueprints/Systems/NarrativeSystem/Components/BP_AC_DialogueComponent Object Reference"))
  (locals (LocalDialogueComponent :type "/Game/BPS_Core/Blueprints/Systems/NarrativeSystem/Components/BP_AC_DialogueComponent Object Reference"))
  ;[1 1 1] Try to find dialogue component.
  (bind _output_get (set `local.LocalDialogueComponent` (`Actor.GetComponentByClass` TargetActor "/Game/BPS_Core/Blueprints/Systems/NarrativeSystem/Components/BP_AC_DialogueComponent.BP_AC_DialogueComponent_C")))
  (`/Engine/EditorBlueprintResources/StandardMacros.IsValid` _output_get
    (:`Is Valid`
      (return true _output_get))
    (:`Is Not Valid`
      (return false null))))

(fn `FindNarrativeManager`
  (params (TargetActor :type "Actor Object Reference"))
  (returns (Found :type Boolean) (Manager :type "/Game/BPS_Core/Blueprints/Systems/NarrativeSystem/Components/BP_AC_NarrativeManager Object Reference"))
  (locals (LocalNarrativeManager :type "/Game/BPS_Core/Blueprints/Systems/NarrativeSystem/Components/BP_AC_NarrativeManager Object Reference"))
  ;[1 1 1] Try to find narrative manager component.
  (bind _output_get (set `local.LocalNarrativeManager` (`Actor.GetComponentByClass` TargetActor "/Game/BPS_Core/Blueprints/Systems/NarrativeSystem/Components/BP_AC_NarrativeManager.BP_AC_NarrativeManager_C")))
  (`/Engine/EditorBlueprintResources/StandardMacros.IsValid` _output_get
    (:`Is Valid`
      (return true _output_get))
    (:`Is Not Valid`
      (return false null))))

(fn `MakeDialogueContext`
  (params (SpeakerActor :type "Actor Object Reference") (TargetActors :type "Array of Actor Object Reference"))
  (returns (Success :type Boolean) (DialogueContext :type "DialogueContext Structure"))
  (locals (LocalSpeakerVoice :type "DialogueVoice Object Reference") (TargetVoices :type "Array of DialogueVoice Object Reference"))
  ;[1 1 1] Make dialogue context for dialogue.
  (bind (_found _component) (`self.FindDialogueComponent` SpeakerActor))
  (if _found
    (set `local.LocalSpeakerVoice` (`/Game/BPS_Core/Blueprints/Systems/NarrativeSystem/Components/BP_AC_DialogueComponent.GetSpeakerVoice` _component))
    (for _array_element TargetActors
      (bind (_found_2 _component_2) (`self.FindDialogueComponent` _array_element))
      (if _found_2
        (`KismetArrayLibrary.Array_Add` (`local.TargetVoices`) (`/Game/BPS_Core/Blueprints/Systems/NarrativeSystem/Components/BP_AC_DialogueComponent.GetSpeakerVoice` _component_2))
        (else
          (return false))))
    (return true (make `DialogueContext` (`local.LocalSpeakerVoice`) (`local.TargetVoices`)))
    (else
      (return false))))

(fn `TryStartQuestForPlayer`
  (params (PlayerController :type "Actor Object Reference") (QuestHandle :type "DataTableRowHandle Structure") (AllowRestart :type Boolean))
  (returns (Success :type Boolean))
  ;[1 1 1] Try to start quest for player.
  (bind (_found _manager) (`self.FindNarrativeManager` PlayerController))
  (if _found
    (bind _success (`/Game/BPS_Core/Blueprints/Systems/NarrativeSystem/Components/BP_AC_NarrativeManager.StartQuest` _manager QuestHandle AllowRestart))
    (return _success)))

(fn `TryStartQuestStageForPlayer`
  (params (PlayerController :type "Actor Object Reference") (QuestHandle :type "DataTableRowHandle Structure") (StageName :type Name) (StageTag :type "GameplayTag Structure") (AllowRestart :type Boolean))
  (returns (Success :type Boolean))
  ;[1 1 1] Try to start quest stage for player.
  (bind (_found _manager) (`self.FindNarrativeManager` PlayerController))
  (if _found
    (bind _success (`/Game/BPS_Core/Blueprints/Systems/NarrativeSystem/Components/BP_AC_NarrativeManager.StartQuestStage` _manager QuestHandle StageName StageTag AllowRestart))
    (return _success)))