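; BP_Dialogue_Base is the base dialogue actor that loads its settings from a data table row on begin play.
; It gates replies on player and GameState tag queries, all/any gameplay conditions and a named custom condition.
; Reply events add or remove tags on both, then trigger player gameplay events and a named custom event.
; Child dialogue classes can override both custom hooks, which return true by default.
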(event `self.ReceiveBeginPlay`
  (bind _dialoguehandle (`self.DialogueHandle`))
  (bind (_datatable _rowname) (break `DataTableRowHandle` _dialoguehandle))
  ;[1 1 1] Begin play. Init dialogue.
  (if (`/Game/BPS_Core/Blueprints/Systems/CoreSystem/Libraries/BP_Library_CoreFunctions.HandleIsValid` _dialoguehandle)
    (bind _returnvalue (`|GetDataTableRow` _datatable _rowname)
      (:`then`
        (set `self.DialogueSettings` _returnvalue)))))

(fn `CheckCustomReplyCondition`
  (params (ConditionName :type Name))
  (returns (Success :type Boolean))
  ;[1 1 1] Returns true if custom conditions complete. Can be overridden in child dialogue class.
  (return true))

(fn `CheckReplyConditions`
  (params (ReplyConditions :type "/Game/BPS_Core/Blueprints/Systems/NarrativeSystem/Structures/STR_DialogueReplyConditions Structure"))
  (returns (Success :type Boolean))
  (locals (LocalPlayerController :type "PlayerController Object Reference") (LocalReplyConditions :type "/Game/BPS_Core/Blueprints/Systems/NarrativeSystem/Structures/STR_DialogueReplyConditions Structure"))
  ;[1 1 1] Check player tags, game tags, and other conditions. Returns true if all conditions are completed.
  (set `local.LocalReplyConditions` ReplyConditions)
  (`|ExecutionSequence`
    (:`then_0`
      (bind _result (`/Game/BPS_Core/Blueprints/Systems/CoreSystem/Libraries/BP_Library_CoreFunctions.CheckActorGameplayTagQuery` (`self.PlayerController`) (`.PlayerTagsQuery_2_29FFE61A4ACA8FFF0A40CBB7CD7AC1AD` (break `/Game/BPS_Core/Blueprints/Systems/NarrativeSystem/Structures/STR_DialogueReplyConditions` (`local.LocalReplyConditions`))) true))
      (if (not _result)
        (return false)))
    (:`then_1`
      (`|ExecutionSequence`
        (:`then_0`
          (bind _result_2 (`/Game/BPS_Core/Blueprints/Systems/CoreSystem/Libraries/BP_Library_CoreFunctions.CheckActorGameplayTagQuery` (`GameplayStatics.GetGameState`) (`.GameTagsQuery_4_4EA6665B4A9BE27069EFFAB89F2C595A` (break `/Game/BPS_Core/Blueprints/Systems/NarrativeSystem/Structures/STR_DialogueReplyConditions` (`local.LocalReplyConditions`))) true))
          (if (not _result_2)
            (return false)))
        (:`then_1`
          (`|ExecutionSequence`
            (:`then_0`
              (bind _success (`/Game/BPS_Core/Blueprints/Systems/CoreSystem/Libraries/BP_Library_CoreFunctions.CheckGameplayConditions` self (`self.PlayerController`) (`.RequiredConditionsAll_21_84E7174B4F1F6C15B26D2EAC2AAA44F8` (break `/Game/BPS_Core/Blueprints/Systems/NarrativeSystem/Structures/STR_DialogueReplyConditions` (`local.LocalReplyConditions`)))))
              (if (not _success)
                (return false)))
            (:`then_1`
              (`|ExecutionSequence`
                (:`then_0`
                  (bind _success_2 (`/Game/BPS_Core/Blueprints/Systems/CoreSystem/Libraries/BP_Library_CoreFunctions.CheckGameplayConditions` self (`self.PlayerController`) (`.RequiredConditionsAny_22_EB60ABA644F79EC45A147B8DF24CD109` (break `/Game/BPS_Core/Blueprints/Systems/NarrativeSystem/Structures/STR_DialogueReplyConditions` (`local.LocalReplyConditions`))) true))
                  (if (not _success_2)
                    (return false)))
                (:`then_1`
                  (`|ExecutionSequence`
                    (:`then_0`
                      (bind _success_3 (`self.CheckCustomReplyCondition` (`.CustomConditionName_23_F38F0DE54E35540B098900BE123EF72B` (break `/Game/BPS_Core/Blueprints/Systems/NarrativeSystem/Structures/STR_DialogueReplyConditions` (`local.LocalReplyConditions`)))))
                      (if (not _success_3)
                        (return false)))
                    (:`then_1`
                      (return true))))))))))))

(fn `TryRunCustomReplyEvents`
  (params (EventName :type Name))
  (returns (Success :type Boolean))
  ;[1 1 1] Try to call custom reply events. Can be overridden in child dialogue class.
  (return true))

(fn `TryRunReplyEvents`
  (params (ReplyEvents :type "/Game/BPS_Core/Blueprints/Systems/NarrativeSystem/Structures/STR_DialogueReplyEvents Structure"))
  (returns (Success :type Boolean))
  (locals (LocalReplyEvents :type "/Game/BPS_Core/Blueprints/Systems/NarrativeSystem/Structures/STR_DialogueReplyEvents Structure"))
  (bind _returnvalue (`GameplayStatics.GetGameState`))
  (bind _playercontroller (`self.PlayerController`))
  (bind ((`PlayerTagsToAdd_25_29FFE61A4ACA8FFF0A40CBB7CD7AC1AD` _playertagstoadd) (`PlayerTagsToRemove_26_EB92DB2A494C8766F41ACBA9FF85A905` _playertagstoremove)) (break `/Game/BPS_Core/Blueprints/Systems/NarrativeSystem/Structures/STR_DialogueReplyEvents` (`local.LocalReplyEvents`)))
  (bind ((`GameTagsToAdd_35_4EA6665B4A9BE27069EFFAB89F2C595A` _gametagstoadd) (`GameTagsToRemove_28_C8873645463245D5A762EE882D723D1D` _gametagstoremove)) (break `/Game/BPS_Core/Blueprints/Systems/NarrativeSystem/Structures/STR_DialogueReplyEvents` (`local.LocalReplyEvents`)))
  ;[1 1 1] Try to run reply events for player controller.
  (set `local.LocalReplyEvents` ReplyEvents)
  (`|ExecutionSequence`
    (:`then_0`
      (`/Game/BPS_Core/Blueprints/Systems/CoreSystem/Libraries/BP_Library_CoreFunctions.AddActorGameplayTags` _playercontroller _playertagstoadd)
      (`/Game/BPS_Core/Blueprints/Systems/CoreSystem/Libraries/BP_Library_CoreFunctions.RemoveActorGameplayTags` _playercontroller _playertagstoremove))
    (:`then_1`
      (`|ExecutionSequence`
        (:`then_0`
          (`/Game/BPS_Core/Blueprints/Systems/CoreSystem/Libraries/BP_Library_CoreFunctions.AddActorGameplayTags` _returnvalue _gametagstoadd)
          (`/Game/BPS_Core/Blueprints/Systems/CoreSystem/Libraries/BP_Library_CoreFunctions.RemoveActorGameplayTags` _returnvalue _gametagstoremove))
        (:`then_1`
          (`|ExecutionSequence`
            (:`then_0`
              (`/Game/BPS_Core/Blueprints/Systems/CoreSystem/Libraries/BP_Library_CoreFunctions.TryRunPlayerGameplayEvents` (`self.PlayerController`) (`.EventsToCall_36_84E7174B4F1F6C15B26D2EAC2AAA44F8` (break `/Game/BPS_Core/Blueprints/Systems/NarrativeSystem/Structures/STR_DialogueReplyEvents` (`local.LocalReplyEvents`)))))
            (:`then_1`
              (`|ExecutionSequence`
                (:`then_0`
                  (`self.TryRunCustomReplyEvents` (`.CustomEventName_33_F38F0DE54E35540B098900BE123EF72B` (break `/Game/BPS_Core/Blueprints/Systems/NarrativeSystem/Structures/STR_DialogueReplyEvents` (`local.LocalReplyEvents`)))))
                (:`then_1`
                  (return true))))))))))

(fn `UserConstructionScript`)