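; Player controller component that manages the map and minimap: open and enabled state, display settings, active marks, pan and zoom.
; It spawns a map render actor that follows a center target, replicated from the server and applied on the local client, and switches it between map and minimap modes.
; A sphere trace at that actor selects map selection volumes that update render settings.
; It also spawns an optional local player mark.
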(event `self.ReceiveBeginPlay`
  ;[1 1 1] Begin play. Init component.
  (if (`self.InitOnBeginPlay`)
    (`self.TryInitComponent`)))

(event `SetMapCenterTarget (Server)`
  (params (TargetActor :type "Actor Object Reference"))
  ;[1 1 1] Network events.
  (set `self.ReplicatedMapCenterTarget` TargetActor))

(event `self.ReceiveEndPlay`
  (params (EndPlayReason :type "EEndPlayReason Enum" :default "Destroyed"))
  (bind _maprenderactor (`self.MapRenderActor`))
  (bind _playermark (`self.PlayerMark`))
  ;[1 1 1] End play. Destroy actors.
  (`|ExecutionSequence`
    (:`then_0`
      (`/Engine/EditorBlueprintResources/StandardMacros.IsValid` _maprenderactor
        (:`Is Valid`
          (`Actor.K2_DestroyActor` _maprenderactor))))
    (:`then_1`
      (`/Engine/EditorBlueprintResources/StandardMacros.IsValid` _playermark
        (:`Is Valid`
          (`Actor.K2_DestroyActor` _playermark))))))

(fn `Bind_OnMarkDestroyed`
  (params (DestroyedActor :type "Actor Object Reference"))
  (for (_array_element _array_index) (`self.ActiveMapMarks`)
    (if (== _array_element DestroyedActor)
      (`KismetArrayLibrary.Array_Remove` (`self.ActiveMapMarks`) _array_index)
      (return))))

(fn `ChangeMapRenderOffset`
  (params (DeltaValue :type "Vector2D Structure"))
  (returns (Success :type Boolean))
  (bind _maprenderactor (`self.MapRenderActor`))
  (bind (_x _y) (`KismetMathLibrary.BreakVector2D` (* DeltaValue (`self.MapNavigationMultiplier`))))
  ;[1 1 1] Try to change offset of map render actor for map navigation.
  (if (`self.GetMapIsOpened`)
    (`/Engine/EditorBlueprintResources/StandardMacros.IsValid` _maprenderactor
      (:`Is Valid`
        (`/Game/BPS_Core/Blueprints/Systems/MapSystem/Actors/BP_MapRenderActor.ChangeRenderOffset` _maprenderactor (`KismetMathLibrary.MakeVector` _x _y))
        (`/Game/BPS_Core/Blueprints/Systems/MapSystem/Actors/BP_MapRenderActor.SetFollowToTarget` _maprenderactor false)
        (return true))
      (:`Is Not Valid`
        _)))
  (return false))

(fn `ChangeMapRenderWidth`
  (params (DeltaWidth :type "Float (double-precision)"))
  (returns (Success :type Boolean))
  (bind _maprenderactor (`self.MapRenderActor`))
  ;[1 1 1] Try to change render width of the map render actor.
  (if (`self.GetMapIsOpened`)
    (`/Engine/EditorBlueprintResources/StandardMacros.IsValid` _maprenderactor
      (:`Is Valid`
        (`/Game/BPS_Core/Blueprints/Systems/MapSystem/Actors/BP_MapRenderActor.ChangeRenderWidth` _maprenderactor (* DeltaWidth (`self.MapZoomMultiplier`)))
        (return true))
      (:`Is Not Valid`
        _)))
  (return false))

(fn `CreatePlayerMark`
  (returns (Success :type Boolean))
  (bind _playercontroller (`self.PlayerController`))
  ;[1 1 1] Create player mark.
  (if (`self.UsePlayerMark`)
    (if (`Controller.IsLocalPlayerController` _playercontroller)
      (`self.DestroyPlayerMark`)
      (bind _returnvalue (`|SpawnActorFromClass` "/Game/BPS_Core/Blueprints/Systems/MapSystem/Actors/BP_MapMark.BP_MapMark_C" (`Actor.GetTransform` _playercontroller) "AlwaysSpawn" "OverrideRootScale" null "PlayerMark" "Player" (`self.PlayerMarkIcon`) false true true false (select `bool` (`self.AttachPlayerMarkToController`) :`false` (`Controller.K2_GetPawn` _playercontroller) :`true` _playercontroller :!type "Actor Object Reference") 100.0 true null))
      (set `self.PlayerMark` _returnvalue)
      (return true)
      (else
        _)))
  (return true))

(fn `DestroyPlayerMark`
  (returns (Success :type Boolean))
  (bind _playermark (`self.PlayerMark`))
  ;[1 1 1] Destroy player mark.
  (`/Engine/EditorBlueprintResources/StandardMacros.IsValid` _playermark
    (:`Is Valid`
      (`Actor.K2_DestroyActor` _playermark))
    (:`Is Not Valid`
      _))
  (return true))

(fn `FindMapMarks`
  (returns (MapMarks :type "Array of /Game/BPS_Core/Blueprints/Systems/MapSystem/Actors/BP_MapMark Object Reference"))
  ;[1 1 1] Finds and returns active map marks.
  (return (`self.ActiveMapMarks`)))

(fn `FindMapRenderActor`
  (returns (Found :type Boolean) (MapRenderActor :type "/Game/BPS_Core/Blueprints/Systems/MapSystem/Actors/BP_MapRenderActor Object Reference"))
  (bind _maprenderactor (`self.MapRenderActor`))
  ;[1 1 1] Returns the map render actor if it is valid.
  (`/Engine/EditorBlueprintResources/StandardMacros.IsValid` _maprenderactor
    (:`Is Valid`
      (return true _maprenderactor))
    (:`Is Not Valid`
      (return false null))))

(fn `FindMapSelectionVolume`
  (params (Location :type "Vector Structure"))
  (returns (Success :type Boolean))
  (locals (LocalHitVolumes :type "Array of /Game/BPS_Core/Blueprints/Systems/MapSystem/Actors/BP_MapSelectionVolume Object Reference") (LocalResultVolumes :type "Array of /Game/BPS_Core/Blueprints/Systems/MapSystem/Actors/BP_MapSelectionVolume Object Reference"))
  (bind _localhitvolumes (`local.LocalHitVolumes`))
  ;[1 1 1] Try to find and select map selection volume in target location.
  (bind _outhits (`KismetSystemLibrary.SphereTraceMultiForObjects` Location Location 5.0 (`|MakeArray` "ObjectTypeQuery2" :!type "EObjectTypeQuery Enum")))
  (for _array_element _outhits
    (bind _asbp_map_selection_volume (cast `/Game/BPS_Core/Blueprints/Systems/MapSystem/Actors/BP_MapSelectionVolume` (`/Game/BPS_Core/Blueprints/Systems/CoreSystem/Libraries/BP_Library_CoreFunctions.GetHitActor` _array_element)))
    (`KismetArrayLibrary.Array_Add` (`local.LocalHitVolumes`) _asbp_map_selection_volume))
  (set `local.LocalResultVolumes` _localhitvolumes)
  (for _array_element_2 _localhitvolumes
    (`KismetArrayLibrary.Array_RemoveItem` (`local.LocalResultVolumes`) (`/Game/BPS_Core/Blueprints/Systems/MapSystem/Actors/BP_MapSelectionVolume.OutMapVolume` _array_element_2)))
  (for _array_element_3 (`local.LocalResultVolumes`)
    (`self.SetMapSelectionVolume` _array_element_3))
  (return true))

(fn `GetMapIsEnabled`
  (returns (MapIsOpened :type Boolean))
  ;[1 1 1] Returns true if map is enabled.
  (return (`self.MapIsEnabled`)))

(fn `GetMapIsEnabledByDefault`
  (returns (MapIsOpened :type Boolean))
  ;[1 1 1] Returns true if map is enabled by default.
  (return (`self.MapIsEnabledByDefault`)))

(fn `GetMapIsOpened`
  (returns (MapIsOpened :type Boolean))
  ;[1 1 1] Returns true if map is opened.
  (return (`self.MapIsOpened`)))

(fn `GetMapMarks`
  (returns (MapMarks :type "Array of /Game/BPS_Core/Blueprints/Systems/MapSystem/Actors/BP_MapMark Object Reference"))
  ;[1 1 1] Returns active map marks.
  (bind _mapmarks (`self.FindMapMarks`))
  (return _mapmarks))

(fn `GetMinimapIsEnabled`
  (returns (MapIsOpened :type Boolean))
  ;[1 1 1] Returns true if minimap is enabled.
  (return (`self.MinimapIsEnabled`)))

(fn `GetMinimapIsEnabledByDefault`
  (returns (MapIsOpened :type Boolean))
  ;[1 1 1] Returns true if minimap is enabled by default.
  (return (`self.MinimapIsEnabledByDefault`)))

(fn `GetShowMarksSettings`
  (returns (ShowMarks :type Boolean))
  ;[1 1 1] Returns the show marks property of the map render settings.
  (return (`self.ShowMarks`)))

(fn `GetShowMinimapSettings`
  (returns (ShowMinimap :type Boolean))
  ;[1 1 1] Returns the show minimap property of the map render settings.
  (return (`self.ShowMinimap`)))

(fn `InitComponent`
  (returns (Success :type Boolean))
  ;[1 1 1] Try to init map manager component.
  (bind _asplayer_controller (cast `PlayerController` (`self.GetOwner`))
    (:`then`
      (set `self.PlayerController` _asplayer_controller)
      (`self.CreatePlayerMark`)
      (set `self.MapIsEnabled` (`self.GetMapIsEnabledByDefault`))
      (set `self.MinimapIsEnabled` (`self.GetMinimapIsEnabledByDefault`))
      (`self.SetMapSelectionVolume` (`self.MapSelectionVolume`))
      (bind _output_get (set `self.IsInitialized` true))
      (return _output_get))
    (:`CastFailed`
      (`KismetSystemLibrary.PrintText` "The map manager component is designed only for player controllers!" true true (struct :`R` 1.0 :`A` 1.0) 10.0)
      (bind _output_get_2 (set `self.IsInitialized` false))
      (return _output_get_2))))

(fn `InitMapMarkInManager`
  (params (Mark :type "/Game/BPS_Core/Blueprints/Systems/MapSystem/Actors/BP_MapMark Object Reference"))
  (returns (Success :type Boolean))
  (locals (LocalMapMark :type "/Game/BPS_Core/Blueprints/Systems/MapSystem/Actors/BP_MapMark Object Reference"))
  (bind _localmapmark (`local.LocalMapMark`))
  ;[1 1 1] Init map mark in the map manager.
  (set `local.LocalMapMark` Mark)
  (if (not (`KismetArrayLibrary.Array_Contains` (`self.ActiveMapMarks`) Mark))
    (`KismetArrayLibrary.Array_Add` (`self.ActiveMapMarks`) _localmapmark)
    (add `Actor.OnDestroyed` _localmapmark (`|CreateDelegate` :!event `Bind_OnMarkDestroyed`))
    (return true)
    (else
      (return true))))

(fn `OnRep_ReplicatedMapCenterTarget`
  ;[1 1 1] Set map target actor on clients.
  (`self.TryInitComponent`)
  (if (`Controller.IsLocalPlayerController` (`self.PlayerController`))
    (`self.SetMapCenterTarget` (`self.ReplicatedMapCenterTarget`))))

(fn `SetMapCenterTarget`
  (params (TargetActor :type "Actor Object Reference"))
  (returns (Success :type Boolean))
  ;[1 1 1] Spawn map render actor and set map center target.
  (if (!= TargetActor (`self.MapCenterTargetActor`))
    (bind _output_get (set `self.MapCenterTargetActor` TargetActor))
    (bind _maprenderactor (`self.SpawnMapRenderActor`))
    (`/Game/BPS_Core/Blueprints/Systems/MapSystem/Actors/BP_MapRenderActor.SetTargetActor` _maprenderactor _output_get)
    (for _array_element (`self.ActiveMapMarks`)
      (`/Game/BPS_Core/Blueprints/Systems/MapSystem/Actors/BP_MapRenderActor.AddActorToRenderList` _maprenderactor _array_element))
    (`self.FindMapSelectionVolume` (`Actor.K2_GetActorLocation` _maprenderactor))
    (return true)))

(fn `SetMapEnabled`
  (params (NewEnabled :type Boolean))
  (returns (Success :type Boolean))
  ;[1 1 1] Set the map is enabled variable and if it is changed then call the map is enabled changed event.
  (if (!= NewEnabled (`self.MapIsEnabled`))
    (bind _output_get (set `self.MapIsEnabled` NewEnabled))
    (`self.OnMapIsEnabledChanged` self _output_get))
  (return true))

(fn `SetMapIsOpened`
  (params (MapIsOpened :type Boolean))
  (returns (Success :type Boolean))
  (bind _maprenderactor (`self.MapRenderActor`))
  ;[1 1 1] Set the map is opened variable and call the on map is opened changed event.
  (if (!= MapIsOpened (`self.MapIsOpened`))
    (bind _output_get (set `self.MapIsOpened` MapIsOpened))
    (`self.OnMapIsOpenedChanged` self _output_get)
    (`/Engine/EditorBlueprintResources/StandardMacros.IsValid` _maprenderactor
      (:`Is Valid`
        (if (`self.MapIsOpened`)
          (`/Game/BPS_Core/Blueprints/Systems/MapSystem/Actors/BP_MapRenderActor.SelectMapMode` _maprenderactor)
          (else
            (`/Game/BPS_Core/Blueprints/Systems/MapSystem/Actors/BP_MapRenderActor.SelectMinimapMode` _maprenderactor))))
      (:`Is Not Valid`
        _)))
  (return true))

(fn `SetMapSelectionVolume`
  (params (MapSelectionVolume :type "/Game/BPS_Core/Blueprints/Systems/MapSystem/Actors/BP_MapSelectionVolume Object Reference"))
  (returns (Success :type Boolean))
  (bind _playercontroller (`self.PlayerController`))
  ;[1 1 1] Set map selection volume and update map render settings.
  (bind _output_get (set `self.MapSelectionVolume` MapSelectionVolume))
  (`/Engine/EditorBlueprintResources/StandardMacros.IsValid` _output_get
    (:`Is Valid`
      (`/Engine/EditorBlueprintResources/StandardMacros.IsValid` _playercontroller
        (:`Is Valid`
          (`/Game/BPS_Core/Blueprints/Systems/MapSystem/Actors/BP_MapSelectionVolume.UpdateMapRenderSettingsForPlayer` _output_get _playercontroller)
          (return true))
        (:`Is Not Valid`
          _)))
    (:`Is Not Valid`
      (`self.SetMapEnabled` (`self.GetMapIsEnabledByDefault`))
      (`self.SetMinimapEnabled` (`self.GetMinimapIsEnabledByDefault`))
      (bind (_found _maprenderactor) (`self.FindMapRenderActor`))
      (if _found
        (`/Game/BPS_Core/Blueprints/Systems/MapSystem/Actors/BP_MapRenderActor.ResetRenderSettings` _maprenderactor)
        (return true)
        (else
          _))))
  (return false))

(fn `SetMinimapEnabled`
  (params (NewEnabled :type Boolean))
  (returns (Success :type Boolean))
  ;[1 1 1] Set the minimap is enabled variable and if it is changed then call the minimap is enabled changed event.
  (if (!= NewEnabled (`self.MinimapIsEnabled`))
    (bind _output_get (set `self.MinimapIsEnabled` NewEnabled))
    (`self.OnMinimapIsEnabledChanged` self _output_get))
  (return true))

(fn `SetShowMarksSettings`
  (params (ShowMarks :type Boolean))
  (returns (Success :type Boolean))
  ;[1 1 1] Set the show marks property of the map render settings.
  (bind _output_get (set `self.ShowMarks` ShowMarks))
  (`self.OnShowMarksSettingsChanged` self _output_get)
  (return true))

(fn `SetShowMinimapSettings`
  (params (ShowMinimap :type Boolean))
  (returns (Success :type Boolean))
  ;[1 1 1] Set the show minimap property of the map render settings.
  (bind _output_get (set `self.ShowMinimap` ShowMinimap))
  (`self.OnShowMinimapSettingsChanged` self _output_get)
  (return true))

(fn `SpawnMapRenderActor`
  (returns (MapRenderActor :type "/Game/BPS_Core/Blueprints/Systems/MapSystem/Actors/BP_MapRenderActor Object Reference"))
  ;[1 1 1] Spawn and return map render actor if it is not exist.
  (`/Engine/EditorBlueprintResources/StandardMacros.IsValid` (`self.MapRenderActor`)
    (:`Is Valid`
      (return (`self.MapRenderActor`)))
    (:`Is Not Valid`
      (bind _returnvalue (`|SpawnActorFromClass` (`self.MapRenderActorClass`) (`KismetMathLibrary.MakeTransform` (0.0 0.0 0.0)) "Undefined" "SelectDefaultAtRuntime" null (`self.RenderMapSprites`) (`self.RenderMapMarks`) null (`self.MinRenderWidth`) (`self.MaxRenderWidth`) (`self.MinimapRenderWidth`) (`self.MapRenderWidth`) null))
      (bind _output_get (set `self.MapRenderActor` _returnvalue))
      (if (`self.MapIsOpened`)
        (`/Game/BPS_Core/Blueprints/Systems/MapSystem/Actors/BP_MapRenderActor.SetRenderWidth` _output_get (`self.MapRenderWidth`) true)
        (else
          (`/Game/BPS_Core/Blueprints/Systems/MapSystem/Actors/BP_MapRenderActor.SetRenderWidth` _output_get (`self.MinimapRenderWidth`) false)))
      (return _output_get))))

(fn `TryCloseMap`
  (returns (Success :type Boolean))
  ;[1 1 1] Try to close map.
  (if (`self.MapIsOpened`)
    (`self.SetMapIsOpened` false)
    (return true)
    (else
      (return true))))

(fn `TryInitComponent`
  (returns (Success :type Boolean))
  ;[1 1 1] Try to init map manager component.
  (if (not (`self.IsInitialized`))
    (bind _success (`self.InitComponent`))
    (bind _output_get (set `self.IsInitialized` _success))
    (return _output_get)
    (else
      (return true))))

(fn `TryOpenMap`
  (returns (Success :type Boolean))
  ;[1 1 1] Try to open map if it can be opened.
  (if (and (`self.MapIsEnabled`) (not (`self.MapIsOpened`)))
    (`self.SetMapIsOpened` true)
    (return true)
    (else
      (return true))))

(fn `TryToggleMap`
  (returns (Success :type Boolean))
  ;[1 1 1] Try to open or close map.
  (if (not (`self.MapIsOpened`))
    (bind _success (`self.TryOpenMap`))
    (return _success)
    (else
      (bind _success_2 (`self.TryCloseMap`))
      (return _success_2))))