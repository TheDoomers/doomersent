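; Client-only trigger volume that selects which map sprite, render settings and map/minimap availability apply while a local player's character is inside it.
; On overlap it registers itself with the player controller's BP_AC_MapManager, and on exit hands over to OutMapVolume or clears the selection.
; UpdateMapRenderSettingsForPlayer applies optional overrides to the map render actor and manager.
; ClampSpriteBox derives render clamp bounds from the sprite and collision, drawing a debug box.
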(event `self.ReceiveBeginPlay`
  ;[1 1 1] Begin play. Destroy actor on dedicated server.
  (if (`KismetSystemLibrary.IsDedicatedServer`)
    (`self.K2_DestroyActor`)))

(event `self.CollisionComponent.OnComponentBeginOverlap`
  (params (OverlappedComponent :type "PrimitiveComponent Object Reference") (OtherActor :type "Actor Object Reference") (OtherComp :type "PrimitiveComponent Object Reference") (OtherBodyIndex :type Integer) (bFromSweep :type Boolean) (SweepResult :type "HitResult Structure (by ref)"))
  ;[1 1 1] Begin and end overlap map selection collision.
  (`/Engine/EditorBlueprintResources/StandardMacros.IsValid` OtherActor
    (:`Is Valid`
      (bind _ascharacter (cast `Character` OtherActor))
      (bind _returnvalue (`Pawn.GetController` _ascharacter))
      (bind _asplayer_controller (cast `PlayerController` _returnvalue))
      (if (`Controller.IsLocalPlayerController` _returnvalue)
        (bind _returnvalue_2 (`self.GetComponentByClass` _asplayer_controller "/Game/BPS_Core/Blueprints/Systems/MapSystem/Components/BP_AC_MapManager.BP_AC_MapManager_C"))
        (`/Engine/EditorBlueprintResources/StandardMacros.IsValid` _returnvalue_2
          (:`Is Valid`
            (`/Game/BPS_Core/Blueprints/Systems/MapSystem/Components/BP_AC_MapManager.SetMapSelectionVolume` _returnvalue_2 self)))))))

(event `self.CollisionComponent.OnComponentEndOverlap`
  (params (OverlappedComponent :type "PrimitiveComponent Object Reference") (OtherActor :type "Actor Object Reference") (OtherComp :type "PrimitiveComponent Object Reference") (OtherBodyIndex :type Integer))
  (bind _outmapvolume (`self.OutMapVolume`))
  ;[1 1 1] Begin and end overlap map selection collision.
  (`/Engine/EditorBlueprintResources/StandardMacros.IsValid` OtherActor
    (:`Is Valid`
      (bind _ascharacter (cast `Character` OtherActor))
      (bind _returnvalue (`Pawn.GetController` _ascharacter))
      (bind _asplayer_controller (cast `PlayerController` _returnvalue))
      (if (`Controller.IsLocalPlayerController` _returnvalue)
        (bind _returnvalue_2 (`self.GetComponentByClass` _asplayer_controller "/Game/BPS_Core/Blueprints/Systems/MapSystem/Components/BP_AC_MapManager.BP_AC_MapManager_C"))
        (`/Engine/EditorBlueprintResources/StandardMacros.IsValid` _returnvalue_2
          (:`Is Valid`
            (`/Engine/EditorBlueprintResources/StandardMacros.IsValid` _outmapvolume
              (:`Is Valid`
                (`/Game/BPS_Core/Blueprints/Systems/MapSystem/Components/BP_AC_MapManager.SetMapSelectionVolume` _returnvalue_2 _outmapvolume))
              (:`Is Not Valid`
                (`/Game/BPS_Core/Blueprints/Systems/MapSystem/Components/BP_AC_MapManager.SetMapSelectionVolume` _returnvalue_2 null)))))))))

(fn `CheckMapEnabled`
  (params (PlayerController :type "Controller Object Reference"))
  (locals (LocalMapManager :type "/Game/BPS_Core/Blueprints/Systems/MapSystem/Components/BP_AC_MapManager Object Reference"))
  ;[1 1 1] Check and disable map.
  (`/Engine/EditorBlueprintResources/StandardMacros.IsValid` PlayerController
    (:`Is Valid`
      (if (`self.OverrideMapIsEnabled`)
        (bind _output_get (set `local.LocalMapManager` (`self.GetComponentByClass` PlayerController "/Game/BPS_Core/Blueprints/Systems/MapSystem/Components/BP_AC_MapManager.BP_AC_MapManager_C")))
        (`/Engine/EditorBlueprintResources/StandardMacros.IsValid` _output_get
          (:`Is Valid`
            (`/Game/BPS_Core/Blueprints/Systems/MapSystem/Components/BP_AC_MapManager.SetMapEnabled` _output_get (`self.MapIsEnabledInVolume`))))))))

(fn `CheckMinimapEnabled`
  (params (PlayerController :type "Controller Object Reference"))
  (locals (LocalMapManager :type "/Game/BPS_Core/Blueprints/Systems/MapSystem/Components/BP_AC_MapManager Object Reference"))
  ;[1 1 1] Check and disable minimap.
  (`/Engine/EditorBlueprintResources/StandardMacros.IsValid` PlayerController
    (:`Is Valid`
      (if (`self.OverrideMinimapIsEnabled`)
        (bind _output_get (set `local.LocalMapManager` (`self.GetComponentByClass` PlayerController "/Game/BPS_Core/Blueprints/Systems/MapSystem/Components/BP_AC_MapManager.BP_AC_MapManager_C")))
        (`/Engine/EditorBlueprintResources/StandardMacros.IsValid` _output_get
          (:`Is Valid`
            (`/Game/BPS_Core/Blueprints/Systems/MapSystem/Components/BP_AC_MapManager.SetMinimapEnabled` _output_get (`self.MinimapIsEnabledInVolume`))))))))

(fn `CheckRenderSettings`
  (params (PlayerController :type "Controller Object Reference"))
  (locals (LocalMapManager :type "/Game/BPS_Core/Blueprints/Systems/MapSystem/Components/BP_AC_MapManager Object Reference"))
  ;[1 1 1] Check and show map sprite.
  (`/Engine/EditorBlueprintResources/StandardMacros.IsValid` PlayerController
    (:`Is Valid`
      (if (`self.OverrideRenderSettings`)
        (bind _output_get (set `local.LocalMapManager` (`self.GetComponentByClass` PlayerController "/Game/BPS_Core/Blueprints/Systems/MapSystem/Components/BP_AC_MapManager.BP_AC_MapManager_C")))
        (`/Engine/EditorBlueprintResources/StandardMacros.IsValid` _output_get
          (:`Is Valid`
            (bind (_found _maprenderactor) (`/Game/BPS_Core/Blueprints/Systems/MapSystem/Components/BP_AC_MapManager.FindMapRenderActor` _output_get))
            (if _found
              (`/Game/BPS_Core/Blueprints/Systems/MapSystem/Actors/BP_MapRenderActor.SetRenderSettings` _maprenderactor (`self.RenderMapSprites`) (`self.RenderMapMarks`) (`self.MapSprite`) (`self.ClampRenderLocation`) (`self.ClampBoxOrigin`) (`self.ClampBoxExtent`)))))))))

(fn `ClampSpriteBox`
  (bind _mapsprite (`self.MapSprite`))
  (bind (_origin _boxextent) (`KismetSystemLibrary.GetComponentBounds` (`self.CollisionComponent`)))
  (bind (_origin_2 _boxextent_2) (`self.GetActorBounds` _mapsprite false false))
  ;[1 1 1] Initialize clamp variables for the selected map sprite.
  (`/Engine/EditorBlueprintResources/StandardMacros.IsValid` _mapsprite
    (:`Is Valid`
      (set `self.ClampRenderLocation` true)
      (set `self.ClampBoxOrigin` (`KismetMathLibrary.MakeVector` (.x _origin_2) (.y _origin_2) (.z _origin)))
      (set `self.ClampBoxExtent` (`KismetMathLibrary.MakeVector` (.x _boxextent_2) (.y _boxextent_2) (.z _boxextent)))
      (`self.DrawClampBox`))
    (:`Is Not Valid`
      (set `self.ClampRenderLocation` false))))

(fn `DrawClampBox`
  ;[1 1 1] Draw debug box for the selected map sprite.
  (`KismetSystemLibrary.DrawDebugBox` (`self.ClampBoxOrigin`) (`self.ClampBoxExtent`) (struct :`R` 1.0 :`A` 1.0) (struct) 5.0))

(fn `UpdateMapRenderSettingsForPlayer`
  (params (PlayerController :type "PlayerController Object Reference"))
  ;[1 1 1] Update map selection for the player.
  (`self.CheckRenderSettings` PlayerController)
  (`self.CheckMapEnabled` PlayerController)
  (`self.CheckMinimapEnabled` PlayerController))

(fn `UserConstructionScript`)