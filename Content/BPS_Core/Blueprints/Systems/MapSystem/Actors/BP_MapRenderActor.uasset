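; Map render actor that moves an orthographic scene capture to render both the minimap and the full map.
; Minimap mode follows a target actor; map mode supports panning, zooming and interpolating to a selected actor.
; Render settings choose between legacy capture and a show-only list of map sprite and BP_MapMark actors.
; Optional box clamping keeps the open map's view within bounds and filters which actors join that list.
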(event `self.ReceiveTick`
  (params (DeltaSeconds :type "Float (single-precision)"))
  ;[1 1 1] Update map render location.
  (`self.UpdateLocation`))

(fn `AddActorToRenderList`
  (params (Actor :type "Actor Object Reference"))
  (returns (Success :type Boolean))
  ;[1 1 1] Try to add actor to render list.
  (if (`self.ClampRender`)
    (if (`KismetMathLibrary.IsPointInBox` (`self.K2_GetActorLocation` Actor) (`self.SelectedMapBoxOrigin`) (`self.SelectedMapBoxExtent`))
      _
      (else
        (return false))))
  (`KismetArrayLibrary.Array_AddUnique` (`SceneCaptureComponent.ShowOnlyActors` (`self.MapSceneCapture`)) Actor)
  (return true))

(fn `ChangeRenderOffset`
  (params (DeltaLocation :type "Vector Structure"))
  ;[1 1 1] Add actor location world offset.
  (`self.SetRenderLocation` (+ DeltaLocation (`self.K2_GetActorLocation`))))

(fn `ChangeRenderWidth`
  (params (DeltaWidth :type "Float (double-precision)"))
  ;[1 1 1] Change render width.
  (`self.SetRenderWidth` (- (`self.CurrentRenderWidth`) DeltaWidth)))

(fn `ResetRenderSettings`
  ;[1 1 1] Reset render settings to default.
  (`self.SetRenderSettings` (`self.RenderMapSpritesByDefault`) (`self.RenderMapMarksByDefault`)))

(fn `SelectMapMode`
  ;[1 1 1] Set render map settings.
  (set `self.MapIsOpened` true)
  (`self.SetFollowToTarget` false)
  (`self.SetRenderWidth` (`self.MapRenderWidth`) false))

(fn `SelectMinimapMode`
  ;[1 1 1] Set minimap render settings.
  (set `self.MapIsOpened` false)
  (`self.SetFollowToTarget` true)
  (`self.SetRenderWidth` (`self.MinimapRenderWidth`) false))

(fn `SetFollowToTarget`
  (params (FollowToTarget :type Boolean))
  ;[1 1 1] Set follow to target state.
  (set `self.FollowToTarget` FollowToTarget)
  (set `self.SelectedActor` null))

(fn `SetRenderLocation`
  (params (NewLocation :type "Vector Structure"))
  (bind _z (.z NewLocation))
  (bind (_selectedmapboxorigin_x _selectedmapboxorigin_y) (`KismetMathLibrary.BreakVector` (`self.SelectedMapBoxOrigin`)))
  (bind (_selectedmapboxextent_x _selectedmapboxextent_y) (`KismetMathLibrary.BreakVector` (`self.SelectedMapBoxExtent`)))
  (bind (_selectedmapboxorigin_x_2 _selectedmapboxorigin_y_2) (`KismetMathLibrary.BreakVector` (`self.SelectedMapBoxOrigin`)))
  (bind _returnvalue (/ (`self.CurrentRenderWidth`) 2.0))
  (bind _x (.x (- (`self.SelectedMapBoxExtent`) (/ (`self.CurrentRenderWidth`) 2.0))))
  (bind _y (.y (- (`self.SelectedMapBoxExtent`) (/ (`self.CurrentRenderWidth`) 2.0))))
  ;[1 1 1] Set render location. If map is open clamp location in selected map sprite bounds.
  (if (`self.MapIsOpened`)
    (if (`self.ClampRender`)
      (`self.K2_SetActorLocation` (select `bool` (and (< _returnvalue _selectedmapboxextent_x) (< _returnvalue _selectedmapboxextent_y)) :`false` (`KismetMathLibrary.MakeVector` _selectedmapboxorigin_x _selectedmapboxorigin_y _z) :`true` (`KismetMathLibrary.MakeVector` (`KismetMathLibrary.FClamp` (.x NewLocation) (- _selectedmapboxorigin_x_2 _x) (+ _selectedmapboxorigin_x_2 _x)) (`KismetMathLibrary.FClamp` (.y NewLocation) (- _selectedmapboxorigin_y_2 _y) (+ _selectedmapboxorigin_y_2 _y)) _z)) false true)
      (else
        (`self.K2_SetActorLocation` NewLocation false true :!label _label)))
    (else
      (goto _label))))

(fn `SetRenderSettings`
  (params (RenderMapSprites :type Boolean) (RenderMapMarks :type Boolean) (MapSpriteActor :type "Actor Object Reference") (ClampRenderLocation :type Boolean) (ClampBoxOrigin :type "Vector Structure") (ClampBoxExtent :type "Vector Structure"))
  (bind _mapscenecapture (`self.MapSceneCapture`))
  (bind _selectedmapsprite (`self.SelectedMapSprite`))
  ;[1 1 1] Select target map sprite and update clamp render variables.
  (set `self.RenderMapSprites` RenderMapSprites)
  (set `self.RenderMapMarks` RenderMapMarks)
  (set `self.SelectedMapSprite` MapSpriteActor)
  (set `self.ClampRender` ClampRenderLocation)
  (set `self.SelectedMapBoxOrigin` ClampBoxOrigin)
  (set `self.SelectedMapBoxExtent` ClampBoxExtent)
  (`KismetArrayLibrary.Array_Clear` (`SceneCaptureComponent.ShowOnlyActors` (`self.MapSceneCapture`)))
  (if (`self.RenderMapSprites`)
    (set `SceneCaptureComponent.PrimitiveRenderMode` "PRM_UseShowOnlyList" _mapscenecapture)
    (`/Engine/EditorBlueprintResources/StandardMacros.IsValid` _selectedmapsprite
      (:`Is Valid`
        (`self.AddActorToRenderList` _selectedmapsprite))
      (:`Is Not Valid`
        _))
    (else
      (set `SceneCaptureComponent.PrimitiveRenderMode` "PRM_LegacySceneCapture" _mapscenecapture)))
  (if (`self.RenderMapMarks`)
    (bind _outactors (`GameplayStatics.GetAllActorsOfClass` "/Game/BPS_Core/Blueprints/Systems/MapSystem/Actors/BP_MapMark.BP_MapMark_C"))
    (for _array_element _outactors
      (bind _success (`self.AddActorToRenderList` _array_element))
      (set `/Game/BPS_Core/Blueprints/Systems/MapSystem/Actors/BP_MapMark.RenderOnMap` _success _array_element))))

(fn `SetRenderWidth`
  (params (Width :type "Float (double-precision)" :default 3000.0) (Clamp :type Boolean :default true))
  ;[1 1 1] Set map render ortho width and update render location.
  (bind _output_get (set `SceneCaptureComponent2D.OrthoWidth` (select `bool` Clamp :`false` Width :`true` (`KismetMathLibrary.FClamp` Width (`self.MinRenderWidth`) (`self.MaxRenderWidth`))) (`self.MapSceneCapture`)))
  (set `self.CurrentRenderWidth` _output_get)
  (`self.SetRenderLocation` (`self.K2_GetActorLocation`)))

(fn `SetSelectedActor`
  (params (SelectedActor :type "Actor Object Reference"))
  ;[1 1 1] Select actor to follow.
  (set `self.SelectedActor` SelectedActor))

(fn `SetTargetActor`
  (params (TargetActor :type "Actor Object Reference"))
  (returns (Success :type Boolean))
  ;[1 1 1] Set target actor reference and set follow to target flag.
  (set `self.TargetActor` TargetActor)
  (`self.SetFollowToTarget` true)
  (return true))

(fn `UpdateLocation`
  (bind _targetactor (`self.TargetActor`))
  (bind _selectedactor (`self.SelectedActor`))
  ;[1 1 1] Update render actor location.
  (if (`self.FollowToTarget`)
    (`/Engine/EditorBlueprintResources/StandardMacros.IsValid` _targetactor
      (:`Is Valid`
        (`self.SetRenderLocation` (`self.K2_GetActorLocation` _targetactor))))
    (else
      (`/Engine/EditorBlueprintResources/StandardMacros.IsValid` _selectedactor
        (:`Is Valid`
          (`self.SetRenderLocation` (`KismetMathLibrary.VInterpTo` (`self.K2_GetActorLocation`) (`self.K2_GetActorLocation` _selectedactor) (`GameplayStatics.GetWorldDeltaSeconds`) 5.0)))))))

(fn `UserConstructionScript`
  (bind _mapscenecapture (`self.MapSceneCapture`))
  ;[1 1 1] Set render width on construction script.
  (set `self.RenderMapSprites` (`self.RenderMapSpritesByDefault`))
  (set `self.RenderMapMarks` (`self.RenderMapMarksByDefault`))
  (`self.SetRenderWidth` (`SceneCaptureComponent2D.OrthoWidth` _mapscenecapture))
  (set `SceneCaptureComponent.PrimitiveRenderMode` (select `bool` (`self.RenderMapSpritesByDefault`) :`false` "PRM_LegacySceneCapture" :`true` "PRM_UseShowOnlyList" :!type "ESceneCapturePrimitiveRenderMode Enum") _mapscenecapture)
  (if (`self.RenderMapMarksByDefault`)
    (bind _outactors (`GameplayStatics.GetAllActorsOfClass` "/Game/BPS_Core/Blueprints/Systems/MapSystem/Actors/BP_MapMark.BP_MapMark_C"))
    (for _array_element _outactors
      (bind _success (`self.AddActorToRenderList` _array_element))
      (set `/Game/BPS_Core/Blueprints/Systems/MapSystem/Actors/BP_MapMark.RenderOnMap` _success _array_element))))