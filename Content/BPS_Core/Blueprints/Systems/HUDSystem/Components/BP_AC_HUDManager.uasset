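; HUD manager component that creates and tracks a player's on-screen widgets: HUD, pause menu, loading screen, message box and custom mouse cursors.
; A single main-widget slot swaps HUD and pause menu, and closing the menu restores the HUD.
; Widget classes and cursors can be looked up by profile.
; Loading screens and message boxes are driven through interface messages, with Run*Event functions relaying their events to dispatchers and clearing references.
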(event `self.ReceiveBeginPlay`
  ;[1 1 1] Begin play event. Try init component.
  (if (`self.InitOnBeginPlay`)
    (`self.InitComponent`)))

(fn `AddLoadingScreen`
  (params (PlayShowAnimation :type Boolean) (AnimationSpeed :type "Float (double-precision)" :default 1.0))
  (returns (Success :type Boolean) (UserWidget :type "UserWidget Object Reference"))
  (locals (LocalPlayShowAnimation :type Boolean) (LocalAnimationSpeed :type "Float (double-precision)" :default 1.0))
  ;[1 1 1] Try to show loading screen widget for player.
  (set `local.LocalPlayShowAnimation` PlayShowAnimation)
  (set `local.LocalAnimationSpeed` AnimationSpeed)
  (if (not (`KismetSystemLibrary.IsValid` (`self.LoadingScreenWidget`)))
    (bind (_success _userwidget) (`self.AddWidgetToViewport` (`self.LoadingScreenWidgetClass`) 100))
    (if _success
      (bind _output_get (set `self.LoadingScreenWidget` _userwidget))
      (if (`local.LocalPlayShowAnimation`)
        (message `/Game/BPS_Core/Blueprints/Systems/HUDSystem/Interfaces/BPI_UI_LoadingScreen.PlayShowAnimation_BPI` _output_get (`local.LocalAnimationSpeed`)))
      (return true (`self.LoadingScreenWidget`))
      (else
        _)))
  (return false null))

(fn `AddLoadingScreenCallback`
  (params (AnimationSpeed :type "Float (double-precision)" :default 1.0) (ShowEndedEvent :type "Delegate (by ref)"))
  (returns (Success :type Boolean) (UserWidget :type "UserWidget Object Reference"))
  ;[1 1 1] Try to show loading screen widget for player. Call ended event when the show animation ended.
  (bind (_success _userwidget) (`self.AddLoadingScreen` true AnimationSpeed))
  (if _success
    (add `self.OnShowLoadingScreenEnded` self ShowEndedEvent)
    (return true _userwidget)
    (else
      (return false null))))

(fn `AddMainWidgetToViewport`
  (params (WidgetClass :type "UserWidget Class Reference") (ZOrder :type Integer))
  (returns (Success :type Boolean) (UserWidget :type "UserWidget Object Reference"))
  ;[1 1 1] Create and add specific widget to player's viewport. Remove previous main widget.
  (bind _returnvalue (`|CreateWidget` WidgetClass))
  (bind (_success _userwidget) (`self.SetMainWidgetForViewport` _returnvalue ZOrder))
  (return _success _userwidget))

(fn `AddMainWidgetToViewportByProfile`
  (params (Profile :type Name) (ZOrder :type Integer))
  (returns (Success :type Boolean) (UserWidget :type "UserWidget Object Reference"))
  (bind (_value _returnvalue) (`BlueprintMapLibrary.Map_Find` (`self.WidgetClassProfiles`) Profile))
  ;[1 1 1] Create and add a widget by the specific profile to the player's viewport. Remove previous main widget.
  (if _returnvalue
    (bind (_success _userwidget) (`self.AddMainWidgetToViewport` _value ZOrder))
    (return _success _userwidget)
    (else
      (return false null))))

(fn `AddMessageBox`
  (params (MessageText :type Text :default "NSLOCTEXT(\"[60BEFEAF43E5BE1DB35FC5BF83DB72FB]\", \"2711C336424B21970D5A6097D6114C91\", \"Message\")") (ShowCancelButton :type Boolean :default true) (OkButtonText :type Text :default "NSLOCTEXT(\"[60BEFEAF43E5BE1DB35FC5BF83DB72FB]\", \"D630AFE34C08ABD48C55BDB8EC872C9F\", \"Ok\")") (CancelButtonText :type Text :default "NSLOCTEXT(\"[60BEFEAF43E5BE1DB35FC5BF83DB72FB]\", \"D7C22D054E04623C3009DB8CBB305A70\", \"Cancel\")"))
  (returns (Success :type Boolean) (UserWidget :type "UserWidget Object Reference"))
  (bind _messageboxwidget (`self.MessageBoxWidget`))
  ;[1 1 1] Try to add message box widget to the player's viewport.
  (if (not (`KismetSystemLibrary.IsValid` (`self.MessageBoxWidget`)))
    (bind (_success _userwidget) (`self.AddWidgetToViewport` (`self.MessageBoxWidgetClass`) 10))
    (if _success
      (bind _output_get (set `self.MessageBoxWidget` _userwidget))
      (message `/Game/BPS_Core/Blueprints/Systems/HUDSystem/Interfaces/BPI_UI_MessageBox.SetMessageBoxVariables_BPI` _output_get MessageText ShowCancelButton OkButtonText CancelButtonText)
      (`self.OnMessageBoxAdded` self _messageboxwidget)
      (return true _messageboxwidget)
      (else
        _)))
  (return false null))

(fn `AddMessageBoxCallback`
  (params (MessageText :type Text :default "NSLOCTEXT(\"[60BEFEAF43E5BE1DB35FC5BF83DB72FB]\", \"FF19ECFF40232CD575A400924641D638\", \"Message\")") (ShowCancelButton :type Boolean :default true) (OkButtonText :type Text :default "NSLOCTEXT(\"[60BEFEAF43E5BE1DB35FC5BF83DB72FB]\", \"48329C5E43F5D7B1A7C67F9574833B45\", \"Ok\")") (CancelButtonText :type Text :default "NSLOCTEXT(\"[60BEFEAF43E5BE1DB35FC5BF83DB72FB]\", \"F7EDAB8D4EF59BAD042ADE9459072B6D\", \"Cancel\")") (OkButtonClickedEvent :type "Delegate (by ref)") (CancelButtonClickedEvent :type "Delegate (by ref)"))
  (returns (Success :type Boolean) (UserWidget :type "UserWidget Object Reference"))
  ;[1 1 1] Try to add message box widget to the player's viewport. Allows to bind on ok and cancel buttons clicked events.
  (bind (_success _userwidget) (`self.AddMessageBox` MessageText ShowCancelButton OkButtonText CancelButtonText))
  (if _success
    (add `self.OnMessageBoxOkButtonClicked` OkButtonClickedEvent)
    (add `self.OnMessageBoxCancelButtonClicked` CancelButtonClickedEvent)
    (return true _userwidget)
    (else
      (return false null))))

(fn `AddWidgetToViewport`
  (params (WidgetClass :type "UserWidget Class Reference") (ZOrder :type Integer))
  (returns (Success :type Boolean) (UserWidget :type "UserWidget Object Reference"))
  ;[1 1 1] Create and add specific widget to player's viewport.
  (bind _returnvalue (`|CreateWidget` WidgetClass))
  (`/Engine/EditorBlueprintResources/StandardMacros.IsValid` _returnvalue
    (:`Is Valid`
      (`UserWidget.AddToViewport` _returnvalue ZOrder)
      (return true _returnvalue))
    (:`Is Not Valid`
      (return false null))))

(fn `AddWidgetToViewportByProfile`
  (params (Profile :type Name) (ZOrder :type Integer))
  (returns (Success :type Boolean) (UserWidget :type "UserWidget Object Reference"))
  (bind (_value _returnvalue) (`BlueprintMapLibrary.Map_Find` (`self.WidgetClassProfiles`) Profile))
  ;[1 1 1] Create and add a widget by the specific profile to the player's viewport.
  (if _returnvalue
    (bind (_success _userwidget) (`self.AddWidgetToViewport` _value ZOrder))
    (return _success _userwidget)
    (else
      (return false null))))

(fn `ClearLoadingScreen`
  (returns (Success :type Boolean))
  ;[1 1 1] Clear loading screen widget from the player's viewport.
  (`Widget.RemoveFromParent` (`self.LoadingScreenWidget`))
  (set `self.LoadingScreenWidget` null)
  (return true))

(fn `HideLoadingScreen`
  (params (PlayHideAnimation :type Boolean) (AnimationSpeed :type "Float (double-precision)" :default 1.0))
  (returns (Success :type Boolean) (UserWidget :type "UserWidget Object Reference"))
  (locals (LocalPlayHideAnimation :type Boolean) (LocalAnimationSpeed :type "Float (double-precision)" :default 1.0))
  ;[1 1 1] Try to hide loading screen widget for player.
  (set `local.LocalPlayHideAnimation` PlayHideAnimation)
  (set `local.LocalAnimationSpeed` AnimationSpeed)
  (if (not (`KismetSystemLibrary.IsValid` (`self.LoadingScreenWidget`)))
    (if (`local.LocalPlayHideAnimation`)
      (bind (_success _userwidget) (`self.AddWidgetToViewport` (`self.LoadingScreenWidgetClass`) 100))
      (if _success
        (bind _output_get (set `self.LoadingScreenWidget` _userwidget))
        (else
          (return false null)))
      (else
        (return true null)))
    (elif (`local.LocalPlayHideAnimation`)
      _
      (else
        (`self.ClearLoadingScreen`)
        (return true null))))
  (message `/Game/BPS_Core/Blueprints/Systems/HUDSystem/Interfaces/BPI_UI_LoadingScreen.PlayHideAnimation_BPI` _output_get (`local.LocalAnimationSpeed`))
  (return true (`self.LoadingScreenWidget`)))

(fn `HideLoadingScreenCallback`
  (params (AnimationSpeed :type "Float (double-precision)" :default 1.0) (HideEndedEvent :type "Delegate (by ref)"))
  (returns (Success :type Boolean) (UserWidget :type "UserWidget Object Reference"))
  ;[1 1 1] Try to hide loading screen widget for player. Call ended event when the hide animation ended.
  (bind (_success _userwidget) (`self.HideLoadingScreen` true AnimationSpeed))
  (if _success
    (add `self.OnHideLoadingScreenEnded` self HideEndedEvent)
    (return true _userwidget)
    (else
      (return false null))))

(fn `InitComponent`
  (returns (Success :type Boolean))
  (bind _hudwidgetclass (`self.HUDWidgetClass`))
  ;[1 1 1] Try init HUD manager component and add widget to the player's viewport.
  (if (`KismetSystemLibrary.IsValidClass` (`self.HUDWidgetClass`))
    (if (`self.HUDIsMainWidget`)
      (bind (_success _userwidget) (`self.AddMainWidgetToViewport` _hudwidgetclass))
      (if _success
        (set `self.HUDWidget` _userwidget)
        (return true)
        (else
          (return false)))
      (else
        (bind (_success_2 _userwidget_2) (`self.AddWidgetToViewport` _hudwidgetclass))
        (if _success_2
          (set `self.HUDWidget` _userwidget_2)
          (return true))))
    (else
      (return false))))

(fn `InitHUDForCharacter`
  (params (Character :type "Character Object Reference"))
  (returns (Success :type Boolean))
  (locals (LocalCharacter :type "Character Object Reference"))
  (bind _hudwidgetclass (`self.HUDWidgetClass`))
  ;[1 1 1] Try init HUD for player and call init character event.
  (set `local.LocalCharacter` Character)
  (if (`self.HUDIsMainWidget`)
    (bind (_success _userwidget) (`self.AddMainWidgetToViewport` _hudwidgetclass))
    (if _success
      (set `self.HUDWidget` _userwidget)
      (`self.OnInitHUDForCharacter` self (`local.LocalCharacter`) :!label _label)
      (return true)
      (else
        _))
    (else
      (bind (_success_2 _userwidget_2) (`self.AddWidgetToViewport` _hudwidgetclass))
      (if _success_2
        (set `self.HUDWidget` _userwidget_2)
        (goto _label)
        (else
          _))))
  (return false))

(fn `PlayCustomEvent`
  (params (EventName :type Name) (SubType :type Name))
  (returns (Success :type Boolean))
  ;[1 1 1] Play and call custom HUD event.
  (`self.OnEventPlayed` self EventName SubType)
  (return true))

(fn `ResetMouseCursor`
  (params (PlayerController :type "PlayerController Object Reference"))
  (returns (Success :type Boolean))
  (bind (_locationx _locationy) (`PlayerController.GetMousePosition` PlayerController))
  ;[1 1 1] Reset mouse cursor for player.
  (set `PlayerController.CurrentMouseCursor` "Default" PlayerController)
  (`PlayerController.SetMouseLocation` PlayerController (`KismetMathLibrary.FTrunc` _locationx) (`KismetMathLibrary.FTrunc` _locationy))
  (return true))

(fn `ReturnHUDWidgetToViewport`
  (params (ZOrder :type Integer))
  (returns (Success :type Boolean))
  (bind _hudwidget (`self.HUDWidget`))
  ;[1 1 1] Try to return HUD widget to player's viewport.
  (`/Engine/EditorBlueprintResources/StandardMacros.IsValid` _hudwidget
    (:`Is Valid`
      (`UserWidget.AddToViewport` _hudwidget ZOrder)
      (return true))
    (:`Is Not Valid`
      (return false))))

(fn `RunLoadingScreenEvent`
  (params (EventName :type Name))
  (returns (Success :type Boolean))
  ;[1 1 1] Try to run specific loading screen event.
  (switch `name` EventName
    (:`OnShowEnded`
      (`self.OnShowLoadingScreenEnded` self (`self.LoadingScreenWidget`))
      (return true))
    (:`OnHideEnded`
      (`self.OnHideLoadingScreenEnded` self (`self.LoadingScreenWidget`))
      (`self.ClearLoadingScreen`)
      (return true))))

(fn `RunMessageBoxEvent`
  (params (EventName :type Name))
  (returns (Success :type Boolean))
  ;[1 1 1] Try to run specific message box event.
  (switch `name` EventName
    (:`Destruct`
      (`self.OnMessageBoxRemoved` self (`self.MessageBoxWidget`))
      (set `self.MessageBoxWidget` null)
      (`self.UnbindMessageBox`)
      (return true))
    (:`OkButtonClicked`
      (`self.OnMessageBoxOkButtonClicked` self (`self.MessageBoxWidget`))
      (return true))
    (:`CancelButtonClicked`
      (`self.OnMessageBoxCancelButtonClicked` self (`self.MessageBoxWidget`))
      (return true))))

(fn `SetCustomMouseCursorByProfile`
  (params (PlayerController :type "PlayerController Object Reference") (MouseCursorType :type "EMouseCursor Enum" :default "None") (ProfileName :type Name))
  (returns (Success :type Boolean))
  (locals (LocalPlayerController :type "PlayerController Object Reference") (LocalNewMouseCursor :type "EMouseCursor Enum" :default "None"))
  (bind _localplayercontroller (`local.LocalPlayerController`))
  (bind _localnewmousecursor (`local.LocalNewMouseCursor`))
  (bind (_locationx _locationy) (`PlayerController.GetMousePosition` _localplayercontroller))
  (bind (_value _returnvalue) (`BlueprintMapLibrary.Map_Find` (`self.CustomMouseCursorsByProfile`) ProfileName))
  ;[1 1 1] Try to set custom mouse cursor by specific profile for player.
  (set `local.LocalPlayerController` PlayerController)
  (set `local.LocalNewMouseCursor` MouseCursorType)
  (if _returnvalue
    (bind _returnvalue_2 (`|CreateWidget` _value))
    (`PlayerController.SetMouseCursorWidget` _localplayercontroller _localnewmousecursor _returnvalue_2)
    (set `PlayerController.CurrentMouseCursor` _localnewmousecursor _localplayercontroller)
    (`PlayerController.SetMouseLocation` _localplayercontroller (`KismetMathLibrary.FTrunc` _locationx) (`KismetMathLibrary.FTrunc` _locationy))
    (return true)
    (else
      (return false))))

(fn `SetCustomMouseCursorByType`
  (params (PlayerController :type "PlayerController Object Reference") (MouseCursorType :type "EMouseCursor Enum" :default "None"))
  (returns (Success :type Boolean))
  (locals (LocalPlayerController :type "PlayerController Object Reference") (LocalNewMouseCursor :type "EMouseCursor Enum" :default "None"))
  (bind _localplayercontroller (`local.LocalPlayerController`))
  (bind _localnewmousecursor (`local.LocalNewMouseCursor`))
  (bind (_locationx _locationy) (`PlayerController.GetMousePosition` _localplayercontroller))
  (bind (_value _returnvalue) (`BlueprintMapLibrary.Map_Find` (`self.CustomMouseCursorsByType`) MouseCursorType))
  ;[1 1 1] Try to set custom mouse cursor by specific type for player.
  (set `local.LocalPlayerController` PlayerController)
  (set `local.LocalNewMouseCursor` MouseCursorType)
  (if _returnvalue
    (bind _returnvalue_2 (`|CreateWidget` _value))
    (`PlayerController.SetMouseCursorWidget` _localplayercontroller _localnewmousecursor _returnvalue_2))
  (set `PlayerController.CurrentMouseCursor` _localnewmousecursor _localplayercontroller)
  (`PlayerController.SetMouseLocation` _localplayercontroller (`KismetMathLibrary.FTrunc` _locationx) (`KismetMathLibrary.FTrunc` _locationy))
  (return true))

(fn `SetMainWidgetForViewport`
  (params (NewMainWidget :type "UserWidget Object Reference") (ZOrder :type Integer))
  (returns (Success :type Boolean) (UserWidget :type "UserWidget Object Reference"))
  (bind _mainwidget (`self.MainWidget`))
  ;[1 1 1] Set main widget and add it to player's viewport. Remove previous main widget.
  (`/Engine/EditorBlueprintResources/StandardMacros.IsValid` _mainwidget
    (:`Is Valid`
      (`Widget.RemoveFromParent` _mainwidget))
    (:`Is Not Valid`
      _))
  (bind _output_get (set `self.MainWidget` NewMainWidget))
  (`/Engine/EditorBlueprintResources/StandardMacros.IsValid` _output_get
    (:`Is Valid`
      (`UserWidget.AddToViewport` _output_get ZOrder)
      (return true _output_get))
    (:`Is Not Valid`
      (return false null))))

(fn `TryClosePauseMenu`
  (returns (Success :type Boolean))
  (bind _hudwidget (`self.HUDWidget`))
  ;[1 1 1] Try close pause menu widget for player.
  (if (`KismetSystemLibrary.IsValid` (`self.PauseMenuWidget`))
    (`Widget.RemoveFromParent` (`self.PauseMenuWidget`))
    (set `self.PauseMenuWidget` null))
  (`/Engine/EditorBlueprintResources/StandardMacros.IsValid` _hudwidget
    (:`Is Valid`
      (if (not (`Widget.IsInViewport` _hudwidget))
        (set `self.MainWidget` _hudwidget)
        (`UserWidget.AddToViewport` _hudwidget 0)
        (return true)
        (else
          _)))
    (:`Is Not Valid`
      _))
  (return false))

(fn `TryOpenPauseMenu`
  (returns (Success :type Boolean))
  ;[1 1 1] Try to open pause menu widget for player.
  (if (not (`KismetSystemLibrary.IsValid` (`self.PauseMenuWidget`)))
    (bind (_success _userwidget) (`self.AddMainWidgetToViewport` (`self.PauseMenuWidgetClass`)))
    (if _success
      (set `self.PauseMenuWidget` _userwidget)
      (return true)
      (else
        _)))
  (return false))

(fn `UnbindMessageBox`
  (returns (Success :type Boolean))
  ;[1 1 1] Unbind message box events.
  (clear `self.OnMessageBoxOkButtonClicked`)
  (clear `self.OnMessageBoxCancelButtonClicked`)
  (return true))