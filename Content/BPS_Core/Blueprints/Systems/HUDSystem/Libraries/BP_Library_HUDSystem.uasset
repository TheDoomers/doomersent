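; Blueprint function library for the HUD system, giving global access to a player's loading screens, message boxes and custom mouse cursors.
; FindHUDManager locates the BP_AC_HUDManager component on the PlayerController's HUD actor.
; Every other function is a thin wrapper that forwards to that manager and reports failure when none is found.
; Callback variants pass events through for animation completion and OK/Cancel clicks.
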(fn `AddLoadingScreen`
  (params (PlayerController :type "PlayerController Object Reference") (PlayShowAnimation :type Boolean) (AnimationSpeed :type "Float (double-precision)" :default 1.0))
  (returns (Success :type Boolean) (UserWidget :type "UserWidget Object Reference"))
  ;[1 1 1] Try to show loading screen widget for player.
  (bind (_found _manager) (`self.FindHUDManager` PlayerController))
  (if _found
    (bind (_success _userwidget) (`/Game/BPS_Core/Blueprints/Systems/HUDSystem/Components/BP_AC_HUDManager.AddLoadingScreen` _manager PlayShowAnimation AnimationSpeed))
    (return _success _userwidget)
    (else
      (return false null))))

(fn `AddLoadingScreenCallback`
  (params (PlayerController :type "PlayerController Object Reference") (AnimationSpeed :type "Float (double-precision)" :default 1.0) (ShowEndedEvent :type "Delegate (by ref)"))
  (returns (Success :type Boolean) (UserWidget :type "UserWidget Object Reference"))
  ;[1 1 1] Try to show loading screen widget for player. Call ended event when the show animation ended.
  (bind (_found _manager) (`self.FindHUDManager` PlayerController))
  (if _found
    (bind (_success _userwidget) (`/Game/BPS_Core/Blueprints/Systems/HUDSystem/Components/BP_AC_HUDManager.AddLoadingScreenCallback` _manager AnimationSpeed ShowEndedEvent))
    (return _success _userwidget)
    (else
      (return false null))))

(fn `AddMessageBox`
  (params (PlayerController :type "PlayerController Object Reference") (MessageText :type Text :default "NSLOCTEXT(\"[9A71C29342219C45A35488A7269D6D19]\", \"5B0B428E4C1815358E5C62BDCAE3B748\", \"Message\")") (ShowCancelButton :type Boolean :default true) (OkButtonText :type Text :default "NSLOCTEXT(\"[9A71C29342219C45A35488A7269D6D19]\", \"D74E843545382F3002EA639036486326\", \"Ok\")") (CancelButtonText :type Text :default "NSLOCTEXT(\"[9A71C29342219C45A35488A7269D6D19]\", \"2D32C3C44FA7CA98CBE75F8CD3B77FB6\", \"Cancel\")"))
  (returns (Success :type Boolean) (UserWidget :type "UserWidget Object Reference"))
  ;[1 1 1] Try to add message box widget to the player's viewport.
  (bind (_found _manager) (`self.FindHUDManager` PlayerController))
  (if _found
    (bind (_success _userwidget) (`/Game/BPS_Core/Blueprints/Systems/HUDSystem/Components/BP_AC_HUDManager.AddMessageBox` _manager MessageText ShowCancelButton OkButtonText CancelButtonText))
    (return _success _userwidget)
    (else
      (return false null))))

(fn `AddMessageBoxCallback`
  (params (PlayerController :type "PlayerController Object Reference") (MessageText :type Text :default "NSLOCTEXT(\"[9A71C29342219C45A35488A7269D6D19]\", \"D9DD16164DB5194EECF257B5560FE404\", \"Message\")") (ShowCancelButton :type Boolean :default true) (OkButtonText :type Text :default "NSLOCTEXT(\"[9A71C29342219C45A35488A7269D6D19]\", \"952D6075464A0EFD458ED18A5E12697F\", \"Ok\")") (CancelButtonText :type Text :default "NSLOCTEXT(\"[9A71C29342219C45A35488A7269D6D19]\", \"51FADFCD45C43F3116CDB08A260377F0\", \"Cancel\")") (OkButtonClickedEvent :type "Delegate (by ref)") (CancelButtonClickedEvent :type "Delegate (by ref)"))
  (returns (Success :type Boolean) (UserWidget :type "UserWidget Object Reference"))
  ;[1 1 1] Try to add message box widget to the player's viewport. Allows to bind on ok and cancel buttons clicked events.
  (bind (_found _manager) (`self.FindHUDManager` PlayerController))
  (if _found
    (bind (_success _userwidget) (`/Game/BPS_Core/Blueprints/Systems/HUDSystem/Components/BP_AC_HUDManager.AddMessageBoxCallback` _manager MessageText ShowCancelButton OkButtonText CancelButtonText OkButtonClickedEvent CancelButtonClickedEvent))
    (return _success _userwidget)
    (else
      (return false null))))

(fn `FindHUDManager`
  (params (PlayerController :type "PlayerController Object Reference"))
  (returns (Found :type Boolean) (Manager :type "/Game/BPS_Core/Blueprints/Systems/HUDSystem/Components/BP_AC_HUDManager Object Reference"))
  (locals (LocalManager :type "/Game/BPS_Core/Blueprints/Systems/HUDSystem/Components/BP_AC_HUDManager Object Reference"))
  (bind _returnvalue (`PlayerController.GetHUD` PlayerController))
  ;[1 1 1] Find HUD manager component.
  (`/Engine/EditorBlueprintResources/StandardMacros.IsValid` _returnvalue
    (:`Is Valid`
      (bind _output_get (set `local.LocalManager` (`Actor.GetComponentByClass` _returnvalue "/Game/BPS_Core/Blueprints/Systems/HUDSystem/Components/BP_AC_HUDManager.BP_AC_HUDManager_C")))
      (`/Engine/EditorBlueprintResources/StandardMacros.IsValid` _output_get
        (:`Is Valid`
          (return true _output_get))
        (:`Is Not Valid`
          _)))
    (:`Is Not Valid`
      _))
  (return false null))

(fn `HideLoadingScreen`
  (params (PlayerController :type "PlayerController Object Reference") (PlayHideAnimation :type Boolean) (AnimationSpeed :type "Float (double-precision)" :default 1.0))
  (returns (Success :type Boolean) (UserWidget :type "UserWidget Object Reference"))
  ;[1 1 1] Try to hide loading screen widget for player.
  (bind (_found _manager) (`self.FindHUDManager` PlayerController))
  (if _found
    (bind (_success _userwidget) (`/Game/BPS_Core/Blueprints/Systems/HUDSystem/Components/BP_AC_HUDManager.HideLoadingScreen` _manager PlayHideAnimation AnimationSpeed))
    (return _success _userwidget)
    (else
      (return false null))))

(fn `HideLoadingScreenCallback`
  (params (PlayerController :type "PlayerController Object Reference") (AnimationSpeed :type "Float (double-precision)" :default 1.0) (HideEndedEvent :type "Delegate (by ref)"))
  (returns (Success :type Boolean) (UserWidget :type "UserWidget Object Reference"))
  ;[1 1 1] Try to hide loading screen widget for player. Call ended event when the hide animation ended.
  (bind (_found _manager) (`self.FindHUDManager` PlayerController))
  (if _found
    (bind (_success _userwidget) (`/Game/BPS_Core/Blueprints/Systems/HUDSystem/Components/BP_AC_HUDManager.HideLoadingScreenCallback` _manager AnimationSpeed HideEndedEvent))
    (return _success _userwidget)
    (else
      (return false null))))

(fn `ResetMouseCursor`
  (params (PlayerController :type "PlayerController Object Reference"))
  (returns (Success :type Boolean))
  ;[1 1 1] Reset mouse cursor for player.
  (bind (_found _manager) (`self.FindHUDManager` PlayerController))
  (if _found
    (bind _success (`/Game/BPS_Core/Blueprints/Systems/HUDSystem/Components/BP_AC_HUDManager.ResetMouseCursor` _manager PlayerController))
    (return _success)
    (else
      (return false))))

(fn `SetCustomMouseCursorByProfile`
  (params (PlayerController :type "PlayerController Object Reference") (MouseCursorType :type "EMouseCursor Enum" :default "None") (ProfileName :type Name))
  (returns (Success :type Boolean))
  ;[1 1 1] Try to set custom mouse cursor by specific profile for player.
  (bind (_found _manager) (`self.FindHUDManager` PlayerController))
  (if _found
    (bind _success (`/Game/BPS_Core/Blueprints/Systems/HUDSystem/Components/BP_AC_HUDManager.SetCustomMouseCursorByProfile` _manager PlayerController MouseCursorType ProfileName))
    (return _success)
    (else
      (return false))))

(fn `SetCustomMouseCursorByType`
  (params (PlayerController :type "PlayerController Object Reference") (MouseCursorType :type "EMouseCursor Enum" :default "None"))
  (returns (Success :type Boolean))
  ;[1 1 1] Try to set custom mouse cursor by specific type for player.
  (bind (_found _manager) (`self.FindHUDManager` PlayerController))
  (if _found
    (bind _success (`/Game/BPS_Core/Blueprints/Systems/HUDSystem/Components/BP_AC_HUDManager.SetCustomMouseCursorByType` _manager PlayerController MouseCursorType))
    (return _success)
    (else
      (return false))))