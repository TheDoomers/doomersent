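; Actor component that gives its owner faction identity and classifies other actors as friend, threat or enemy.
; Initialization takes faction tags and friendly/enemy tag queries from a data table row or the InitialRelationships struct, overridable at runtime.
; Checks match queries against the target's faction tags, though friendship short-circuits when GroupActors contains GroupLeader, and any non-friend other than the owner counts as a threat.
; Adding or removing tags fires a change event.
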(event `self.ReceiveBeginPlay`
  ;[1 1 1] Begin play. Init component.
  (if (`self.InitOnBeginPlay`)
    (`self.TryInitComponent`)))

(fn `AddFactionTag`
  (params (NewFactionTag :type "GameplayTag Structure"))
  (returns (Success :type Boolean))
  (locals (LocalPrevTags :type "GameplayTagContainer Structure"))
  (bind _factiontags (`self.FactionTags`))
  ;[1 1 1] Add the new faction tag.
  (set `local.LocalPrevTags` _factiontags)
  (if (not (`BlueprintGameplayTagLibrary.HasTag` _factiontags NewFactionTag))
    (`BlueprintGameplayTagLibrary.AddGameplayTag` (`self.FactionTags`) NewFactionTag)
    (`self.OnFactionTagsChanged` self (`self.FactionTags`) (`local.LocalPrevTags`)))
  (return true))

(fn `CheckTargetIsEnemy`
  (params (TargetActor :type "Actor Object Reference"))
  (returns (IsEnemy :type Boolean))
  (locals (LocalTargetActor :type "Actor Object Reference"))
  (bind _enemyquery (`self.EnemyQuery`))
  ;[1 1 1] Returns true if target actor is enemy.
  (bind _output_get (set `local.LocalTargetActor` TargetActor))
  (if (!= _output_get (`self.GetOwner`))
    (bind _isfriend (`self.CheckTargetIsFriend` (`local.LocalTargetActor`)))
    (if (not _isfriend)
      (bind (_found _component) (`/Game/BPS_Core/Blueprints/Systems/BehaviorSystem/Libraries/BPI_Library_BehaviorSystem.FindFactionComponent` (`local.LocalTargetActor`)))
      (if _found
        (if (not (`BlueprintGameplayTagLibrary.IsTagQueryEmpty` _enemyquery))
          (return (`BlueprintGameplayTagLibrary.DoesContainerMatchTagQuery` (`self.GetFactionTags` _component) _enemyquery))
          (else
            _)))))
  (return false))

(fn `CheckTargetIsFriend`
  (params (TargetActor :type "Actor Object Reference"))
  (returns (IsFriend :type Boolean))
  (locals (LocalTargetActor :type "Actor Object Reference"))
  (bind _friendlyquery (`self.FriendlyQuery`))
  ;[1 1 1] Returns true if target actor is friend.
  (bind _output_get (set `local.LocalTargetActor` TargetActor))
  (bind (_found _component) (`/Game/BPS_Core/Blueprints/Systems/BehaviorSystem/Libraries/BPI_Library_BehaviorSystem.FindFactionComponent` _output_get))
  (if (and _found (!= _output_get (`self.GetOwner`)))
    (if (`KismetArrayLibrary.Array_Contains` (`self.GroupActors`) (`self.GroupLeader`))
      (return true)
      (elif (not (`BlueprintGameplayTagLibrary.IsTagQueryEmpty` _friendlyquery))
        (return (`BlueprintGameplayTagLibrary.DoesContainerMatchTagQuery` (`self.GetFactionTags` _component) _friendlyquery))
        (else
          _))))
  (return false))

(fn `CheckTargetIsThreat`
  (params (TargetActor :type "Actor Object Reference"))
  (returns (IsThreat :type Boolean))
  (locals (LocalTargetActor :type "Actor Object Reference"))
  ;[1 1 1] Returns true if target actor is threat.
  (bind _output_get (set `local.LocalTargetActor` TargetActor))
  (if (!= _output_get (`self.GetOwner`))
    (bind _isfriend (`self.CheckTargetIsFriend` (`local.LocalTargetActor`)))
    (if (not _isfriend)
      (return true)
      (else
        _)))
  (return false))

(fn `GetEnemyQuery`
  (returns (EnemyQuery :type "GameplayTagQuery Structure"))
  ;[1 1 1] Returns enemy query of the actor.
  (return (`self.EnemyQuery`)))

(fn `GetFactionTags`
  (returns (FactionTags :type "GameplayTagContainer Structure"))
  ;[1 1 1] Returns faction tags of the actor.
  (return (`self.FactionTags`)))

(fn `GetFriendlyQuery`
  (returns (FriendlyQuery :type "GameplayTagQuery Structure"))
  ;[1 1 1] Returns friendly query of the actor.
  (return (`self.FriendlyQuery`)))

(fn `GetGroupActors`
  (returns (GroupActors :type "Array of Actor Object Reference"))
  ;[1 1 1] Returns actors that are in a group of the actor.
  (return (`self.GroupActors`)))

(fn `GetGroupLeader`
  (returns (GroupLeader :type "Actor Object Reference"))
  ;[1 1 1] Returns group leader of the actor.
  (return (`self.GroupLeader`)))

(fn `InitComponent`
  (returns (Success :type Boolean))
  ;[1 1 1] Try init relationships.
  (bind _success (`self.InitRelationships`))
  (bind _output_get (set `self.IsInitialized` _success))
  (return _output_get))

(fn `InitRelationships`
  (returns (Success :type Boolean))
  (bind (_datatable _rowname) (break `DataTableRowHandle` (`self.RelationshipsHandle`)))
  ;[1 1 1] Init relationships settings from the data table.
  (`/Engine/EditorBlueprintResources/StandardMacros.IsValid` _datatable
    (:`Is Valid`
      (bind _returnvalue (`|GetDataTableRow` _datatable _rowname)
        (:`then`
          (bind _output_get (set `self.InitialRelationships` _returnvalue)))
        (:`RowNotFound`
          _)))
    (:`Is Not Valid`
      _))
  (bind (_factiontags _friendlyquery _enemyquery) (break `/Game/BPS_Core/Blueprints/Systems/BehaviorSystem/Structures/STR_Relationships` _output_get))
  (set `self.FactionTags` _factiontags)
  (set `self.FriendlyQuery` _friendlyquery)
  (set `self.EnemyQuery` _enemyquery)
  (return true))

(fn `OverrideRelationships`
  (params (RelationshipsHandle :type "DataTableRowHandle Structure") (Relationships :type "/Game/BPS_Core/Blueprints/Systems/BehaviorSystem/Structures/STR_Relationships Structure"))
  (returns (Success :type Boolean))
  ;[1 1 1] Override relationships.
  (set `self.RelationshipsHandle` RelationshipsHandle)
  (set `self.InitialRelationships` Relationships)
  (`self.InitRelationships`)
  (return true))

(fn `RemoveFactionTag`
  (params (FactionTag :type "GameplayTag Structure"))
  (returns (Success :type Boolean))
  (locals (LocalPrevTags :type "GameplayTagContainer Structure"))
  (bind _factiontags (`self.FactionTags`))
  ;[1 1 1] Remove the specific faction tag.
  (set `local.LocalPrevTags` _factiontags)
  (if (`BlueprintGameplayTagLibrary.HasTag` _factiontags FactionTag)
    (`BlueprintGameplayTagLibrary.RemoveGameplayTag` (`self.FactionTags`) FactionTag)
    (`self.OnFactionTagsChanged` self (`self.FactionTags`) (`local.LocalPrevTags`)))
  (return true))

(fn `TryInitComponent`
  (returns (Success :type Boolean))
  ;[1 1 1] Try init component.
  (if (not (`self.IsInitialized`))
    (bind _success (`self.InitComponent`))
    (return _success)
    (else
      (return true))))