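; Base actor for restricted areas in the behavior system that reports whether the area is restricted for a given actor inside it.
; On BeginPlay it loads friendly and enemy tag queries, optionally from a data table row, and binds overlap events on all its primitive components.
; Overlaps track actors that have a faction component.
; Restriction checks match their faction tags against those queries, treating any non-friend as a threat.
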(event `self.ReceiveBeginPlay`
  ;[1 1 1] Begin play. Init variables.
  (`self.InitRestrictedArea`))

(fn `Bind_OnBeginOverlap`
  (params (OverlappedComponent :type "PrimitiveComponent Object Reference") (OtherActor :type "Actor Object Reference") (OtherComp :type "PrimitiveComponent Object Reference") (OtherBodyIndex :type Integer) (bFromSweep :type Boolean) (SweepResult :type "HitResult Structure (by ref)"))
  ;[1 1 1] Add actor to the list of overlapped actors.
  (bind _found (`/Game/BPS_Core/Blueprints/Systems/BehaviorSystem/Libraries/BPI_Library_BehaviorSystem.FindFactionComponent` OtherActor))
  (if _found
    (`KismetArrayLibrary.Array_AddUnique` (`self.OverlappedActors`) OtherActor)))

(fn `Bind_OnEndOverlap`
  (params (OverlappedComponent :type "PrimitiveComponent Object Reference") (OtherActor :type "Actor Object Reference") (OtherComp :type "PrimitiveComponent Object Reference") (OtherBodyIndex :type Integer))
  ;[1 1 1] Remove actor from the list of overlapped actors.
  (bind _found (`/Game/BPS_Core/Blueprints/Systems/BehaviorSystem/Libraries/BPI_Library_BehaviorSystem.FindFactionComponent` OtherActor))
  (if _found
    (`KismetArrayLibrary.Array_RemoveItem` (`self.OverlappedActors`) OtherActor)))

(fn `CheckRestrictionForTarget`
  (params (TargetActor :type "Actor Object Reference") (CheckIsEnemy :type Boolean))
  (returns (IsRestricted :type Boolean))
  ;[1 1 1] Returns true if area is restricted for target actor.
  (bind _result (`self.CheckTargetIsInArea` TargetActor))
  (if _result
    (if CheckIsEnemy
      (bind _isenemy (`self.CheckTargetIsEnemy` TargetActor))
      (return _isenemy)
      (else
        (bind _isthreat (`self.CheckTargetIsThreat` TargetActor))
        (return _isthreat)))
    (else
      (return false))))

(fn `CheckTargetIsEnemy`
  (params (TargetActor :type "Actor Object Reference"))
  (returns (IsEnemy :type Boolean))
  (bind _enemyquery (`self.EnemyQuery`))
  ;[1 1 1] Returns true if target actor is enemy.
  (bind (_found _component) (`/Game/BPS_Core/Blueprints/Systems/BehaviorSystem/Libraries/BPI_Library_BehaviorSystem.FindFactionComponent` TargetActor))
  (if (and _found (not (`BlueprintGameplayTagLibrary.IsTagQueryEmpty` _enemyquery)))
    (return (`BlueprintGameplayTagLibrary.DoesContainerMatchTagQuery` (`/Game/BPS_Core/Blueprints/Systems/BehaviorSystem/Components/BP_AC_FactionComponent.GetFactionTags` _component) _enemyquery))
    (else
      (return false))))

(fn `CheckTargetIsFriend`
  (params (TargetActor :type "Actor Object Reference"))
  (returns (IsFriend :type Boolean))
  (bind _friendlyquery (`self.FriendlyQuery`))
  ;[1 1 1] Returns true if target actor is friend.
  (bind (_found _component) (`/Game/BPS_Core/Blueprints/Systems/BehaviorSystem/Libraries/BPI_Library_BehaviorSystem.FindFactionComponent` TargetActor))
  (if (and _found (not (`BlueprintGameplayTagLibrary.IsTagQueryEmpty` _friendlyquery)))
    (return (`BlueprintGameplayTagLibrary.DoesContainerMatchTagQuery` (`/Game/BPS_Core/Blueprints/Systems/BehaviorSystem/Components/BP_AC_FactionComponent.GetFactionTags` _component) _friendlyquery))
    (else
      (return false))))

(fn `CheckTargetIsInArea`
  (params (TargetActor :type "Actor Object Reference"))
  (returns (Result :type Boolean))
  ;[1 1 1] Returns true if target actor is in area.
  (return (`KismetArrayLibrary.Array_Contains` (`self.OverlappedActors`) TargetActor)))

(fn `CheckTargetIsThreat`
  (params (TargetActor :type "Actor Object Reference"))
  (returns (IsThreat :type Boolean))
  ;[1 1 1] Returns true if target actor is threat.
  (bind _isfriend (`self.CheckTargetIsFriend` TargetActor))
  (return (not _isfriend)))

(fn `InitRelationships`
  (returns (Success :type Boolean))
  (bind (_datatable _rowname) (break `DataTableRowHandle` (`self.RelationshipsHandle`)))
  ;[1 1 1] Try to load relationship settings from the data table.
  (`/Engine/EditorBlueprintResources/StandardMacros.IsValid` _datatable
    (:`Is Valid`
      (bind _returnvalue (`|GetDataTableRow` _datatable _rowname)
        (:`then`
          (bind _output_get (set `self.InitialRelationships` _returnvalue)))
        (:`RowNotFound`
          _)))
    (:`Is Not Valid`
      _))
  (bind ((`FriendlyQuery_18_7969CEA745B06EDA5F9F9B9ABC96EF6D` _friendlyquery) (`EnemyQuery_20_BF0016A94578303F8A9BCAAD83679AA6` _enemyquery)) (break `/Game/BPS_Core/Blueprints/Systems/BehaviorSystem/Structures/STR_Relationships` _output_get))
  (set `self.FriendlyQuery` _friendlyquery)
  (set `self.EnemyQuery` _enemyquery)
  (return true))

(fn `InitRestrictedArea`
  (returns (Success :type Boolean))
  ;[1 1 1] Init relationship settings and bind events.
  (`self.InitRelationships`)
  (for _array_element (`self.K2_GetComponentsByClass` "/Script/Engine.PrimitiveComponent")
    (add `PrimitiveComponent.OnComponentBeginOverlap` _array_element (`|CreateDelegate` :!event `Bind_OnBeginOverlap`))
    (add `PrimitiveComponent.OnComponentEndOverlap` _array_element (`|CreateDelegate` :!event `Bind_OnEndOverlap`)))
  (return true))

(fn `UserConstructionScript`)