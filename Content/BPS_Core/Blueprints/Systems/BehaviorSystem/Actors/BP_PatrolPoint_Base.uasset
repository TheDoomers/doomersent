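; BP_PatrolPoint_Base is a base patrol point actor for the behavior system, marked by a billboard icon.
; SetPatrolPointForCharacter finds the behavior manager on its target character, assigns itself as that manager's patrol point and prints success or failure messages.
; GetFocalPoint returns a location a fixed distance along the actor's forward vector.
; An interface function exposes its SaveObject component to other systems.
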(fn `GetFocalPoint`
  (returns (ReturnValue :type "Vector Structure"))
  ;[1 1 1] Returns focal point.
  (return (+ (`self.K2_GetActorLocation`) (* (`KismetMathLibrary.GetForwardVector` (`self.K2_GetActorRotation`)) 500.0))))

(fn `GetSaveObjectComponent_BPI`
  (returns (Success :type Boolean) (Component :type "/Game/BPS_Core/Blueprints/Systems/SaveLoadSystem/Components/BP_AC_SaveObjectComponent Object Reference"))
  ;[1 1 1] Returns save object component.
  (return true (`self.SaveObject`)))

(fn `SetPatrolPointForCharacter`
  (bind _targetcharacter (`self.TargetCharacter`))
  ;[1 1 1] Try to set patrol point for the character.
  (`/Engine/EditorBlueprintResources/StandardMacros.IsValid` _targetcharacter
    (:`Is Valid`
      (bind (_found _component) (`/Game/BPS_Core/Blueprints/Systems/BehaviorSystem/Libraries/BPI_Library_BehaviorSystem.FindBehaviorManager` _targetcharacter))
      (if _found
        (set `/Game/BPS_Core/Blueprints/Systems/BehaviorSystem/Components/BP_AC_BehaviorManager.PatrolPoint` self _component)
        (`KismetSystemLibrary.PrintText` "Patrol point is set!" true true (struct :`G` 1.0 :`A` 1.0) 10.0)
        (else
          (`KismetSystemLibrary.PrintText` "Behavior manager is not found!" true true (struct :`R` 1.0 :`A` 1.0) 10.0))))
    (:`Is Not Valid`
      (`KismetSystemLibrary.PrintText` "Select the target character!" true true (struct :`R` 1.0 :`A` 1.0) 10.0))))

(fn `UserConstructionScript`
  ;[1 1 1] Set billboard sprite texture.
  (`BillboardComponent.SetSprite` (`self.Billboard`) (`self.PointIcon`)))