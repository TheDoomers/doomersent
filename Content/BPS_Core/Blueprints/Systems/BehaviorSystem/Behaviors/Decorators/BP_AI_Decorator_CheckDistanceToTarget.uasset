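; Behavior tree decorator that passes when the AI pawn is within an acceptance radius of its target.
; The radius comes from a fixed value, a Blackboard float or the sum of both.
; It either measures distance to a Blackboard actor, falling back to a location vector, and caches it in the Blackboard, or compares against the distance already stored there.
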(fn `PerformConditionCheckAI`
  (params (OwnerController :type "AIController Object Reference") (ControlledPawn :type "Pawn Object Reference"))
  (returns (ReturnValue :type Boolean))
  (locals (LocalTargetActor :type "Actor Object Reference") (LocalDistanceToTarget :type "Float (double-precision)" :default 0.0))
  (bind _targetactororlocation (`self.TargetActorOrLocation`))
  ;[1 1 1] Return true if distance to target in result acceptance radius.
  (`self.UpdateAcceptanceRadius`)
  (if (`self.CalculateDistanceToTarget`)
    (bind _output_get (set `local.LocalTargetActor` (`BTFunctionLibrary.GetBlackboardValueAsActor` _targetactororlocation)))
    (`/Engine/EditorBlueprintResources/StandardMacros.IsValid` _output_get
      (:`Is Valid`
        (bind _output_get_2 (set `local.LocalDistanceToTarget` (`Actor.GetDistanceTo` _output_get ControlledPawn))))
      (:`Is Not Valid`
        (set `local.LocalDistanceToTarget` (`KismetMathLibrary.Vector_Distance` (`Actor.K2_GetActorLocation` ControlledPawn) (`BTFunctionLibrary.GetBlackboardValueAsVector` _targetactororlocation)))))
    (`BTFunctionLibrary.SetBlackboardValueAsFloat` (`self.DistanceToTarget`) _output_get_2)
    (return (<= (`local.LocalDistanceToTarget`) (`self.ResultAcceptanceRadius`)))
    (else
      (return (<= (`BTFunctionLibrary.GetBlackboardValueAsFloat` (`self.DistanceToTarget`)) (`self.ResultAcceptanceRadius`))))))

(fn `UpdateAcceptanceRadius`
  (bind _acceptanceradius (`self.AcceptanceRadius`))
  (bind _returnvalue (`BTFunctionLibrary.GetBlackboardValueAsFloat` (`self.BlackboardRadius`)))
  ;[1 1 1] Update acceptance radius.
  (if (`self.UseBlackboardRadius`)
    (set `self.ResultAcceptanceRadius` (select `bool` (`self.SumRadiusValues`) :`false` _returnvalue :`true` (+ _acceptanceradius _returnvalue) :!type "Float (double-precision)"))
    (else
      (set `self.ResultAcceptanceRadius` _acceptanceradius))))