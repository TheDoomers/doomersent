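; Behavior task that uses an EQS query to find a position with a clear line to the AI's suspicious location.
; It checks results best-first with offset sphere traces from slightly above each point, ignoring the pawn and its attached actors.
; The first clear point becomes the TargetLocation blackboard value, otherwise the task fails.
; With FinishOnAnySuccess off, the obstacle check reports blocked even when every trace is clear.
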(event `self.ReceiveExecuteAI`
  (params (OwnerController :type "AIController Object Reference") (ControlledPawn :type "Pawn Object Reference"))
  ;[1 1 1] Try to find and update suspicious location for the controlled pawn.
  (bind _output_get (set `self.ControlledPawn` ControlledPawn))
  (bind _returnvalue (`EnvQueryManager.RunEQSQuery` (`self.QueryTemplate`) _output_get (`self.QueryRunMode`)))
  (add `EnvQueryInstanceBlueprintWrapper.OnQueryFinishedEvent` _returnvalue (delegate `OnQueryFinished`)))

(event `OnQueryFinished`
  (params (QueryInstance :type "EnvQueryInstanceBlueprintWrapper Object Reference") (QueryStatus :type "EEnvQueryStatus Enum" :default "Processing"))
  ;[1 1 1] Try to find and update suspicious location for the controlled pawn.
  (bind (_success _sortedlocations) (`/Game/BPS_Core/Blueprints/Systems/BehaviorSystem/Libraries/BPI_Library_BehaviorSystem.GetResultLocationsSortedByMax` QueryInstance))
  (if _success
    (set `self.ExecutionSuccessed` false)
    (for _array_element _sortedlocations
      (bind _targetisblocked (`self.CheckObstacle` (+ _array_element (0.0 0.0 50.0)) (`BTFunctionLibrary.GetBlackboardValueAsVector` (`self.SuspiciousLocation`))))
      (if (not _targetisblocked)
        (`BTFunctionLibrary.SetBlackboardValueAsVector` (`self.TargetLocation`) _array_element)
        (set `self.ExecutionSuccessed` true)
        (break)))
    (if (`self.ExecutionSuccessed`)
      (`self.FinishExecute` true)
      (else
        (`self.FinishExecute` false)))
    (else
      (`self.FinishExecute` false))))

(fn `CheckObstacle`
  (params (StartLocation :type "Vector Structure") (TargetLocation :type "Vector Structure"))
  (returns (TargetIsBlocked :type Boolean))
  (locals (LocalTargetLocation :type "Vector Structure") (LocalTargetActors :type "Array of Actor Object Reference") (LocalActorsToIgnore :type "Array of Actor Object Reference") (LocalStartLocation :type "Vector Structure") (LocalEndLocation :type "Vector Structure") (LocalTraceOffsets :type "Array of Vector Structure") (LocalTargetIsBlocked :type Boolean) (LocalTraceOffset :type "Vector Structure"))
  (bind _controlledpawn (`self.ControlledPawn`))
  (bind _finishonanysuccess (`self.FinishOnAnySuccess`))
  (bind _localstartlocation (`local.LocalStartLocation`))
  ;[1 1 1] Check obstacle between start location and target location.
  (set `local.LocalStartLocation` StartLocation)
  (set `local.LocalTargetLocation` TargetLocation)
  (bind _output_get (set `local.LocalActorsToIgnore` (`Actor.GetAttachedActors` _controlledpawn true false)))
  (`KismetArrayLibrary.Array_Add` _output_get _controlledpawn)
  (set `local.LocalStartLocation` _localstartlocation)
  (set `local.LocalEndLocation` (`self.GetTraceEnd` _localstartlocation (`local.LocalTargetLocation`)))
  (bind _output_get_2 (set `local.LocalTraceOffsets` (`self.TraceOffsets`)))
  (`KismetArrayLibrary.Array_Insert` _output_get_2 (`self.FirstTraceOffset`))
  (set `local.LocalTargetIsBlocked` true)
  (for _array_element _output_get_2
    (bind _output_get_3 (set `local.LocalTraceOffset` _array_element))
    (bind (_outhits _returnvalue) (`KismetSystemLibrary.SphereTraceMultiForObjects` (+ (`local.LocalStartLocation`) _output_get_3) (+ (`local.LocalEndLocation`) _output_get_3) (`self.TraceRadius`) (`self.ObstacleObjectTypes`) false (`local.LocalActorsToIgnore`)))
    (if (not _returnvalue)
      (if _finishonanysuccess
        (return false))
      (elif (not _finishonanysuccess)
        (return true))))
  (return (`local.LocalTargetIsBlocked`)))

(fn `GetTraceEnd`
  (params (StartLocation :type "Vector Structure") (TargetLocation :type "Vector Structure"))
  (returns (TraceEnd :type "Vector Structure"))
  (bind _returnvalue (- TargetLocation StartLocation))
  ;[1 1 1] Returns trace end location.
  (return (+ StartLocation (* (`KismetMathLibrary.Normal` _returnvalue) (`KismetMathLibrary.VSize` _returnvalue)))))