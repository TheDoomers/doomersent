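; Behavior tree task that writes the controlled pawn's current distance to its target into a blackboard float key.
; The target key is read as an actor first, using actor-to-actor distance when valid.
; Otherwise it is read as a vector and measured against the pawn's location.
; The task then finishes immediately with success.
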(event `self.ReceiveExecuteAI`
  (params (OwnerController :type "AIController Object Reference") (ControlledPawn :type "Pawn Object Reference"))
  (bind _distancetotarget (`self.DistanceToTarget`))
  (bind _targetactororlocation (`self.TargetActorOrLocation`))
  (bind _returnvalue (`BTFunctionLibrary.GetBlackboardValueAsActor` _targetactororlocation))
  ;[1 1 1] Update distance to target blackboard value.
  (`/Engine/EditorBlueprintResources/StandardMacros.IsValid` _returnvalue
    (:`Is Valid`
      (`BTFunctionLibrary.SetBlackboardValueAsFloat` _distancetotarget (`Actor.GetDistanceTo` _returnvalue ControlledPawn)))
    (:`Is Not Valid`
      (`BTFunctionLibrary.SetBlackboardValueAsFloat` _distancetotarget (`KismetMathLibrary.Vector_Distance` (`BTFunctionLibrary.GetBlackboardValueAsVector` _targetactororlocation) (`Actor.K2_GetActorLocation` ControlledPawn)))))
  (`self.FinishExecute` true))