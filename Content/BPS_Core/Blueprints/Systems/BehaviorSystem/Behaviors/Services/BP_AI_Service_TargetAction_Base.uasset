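; Base behavior tree service that makes an AI pawn attempt a special action related to its target actor.
; Each tick runs optional gates in order: cooldown, distance, facing angle and interaction tag queries on pawn and target, with distance, range and rotation optionally read from the Blackboard.
; When all pass, it asks the pawn's Behavior Manager to play the configured action and starts that action type's cooldown on success.
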(event `self.ReceiveTickAI`
  (params (OwnerController :type "AIController Object Reference") (ControlledPawn :type "Pawn Object Reference") (DeltaSeconds :type "Float (single-precision)"))
  ;[1 1 1] Check action conditions and do action on service tick.
  (set `self.OwnerController` OwnerController)
  (set `self.ControlledPawn` ControlledPawn)
  (bind _success (`self.CheckConditions`))
  (if _success
    (`self.TryPlayActions`)))

(fn `CheckConditions`
  (returns (Success :type Boolean))
  ;[1 1 1] Check action conditions.
  (`|ExecutionSequence`
    (:`then_0`
      (bind _success (`self.CheckCooldown`))
      (if (not _success)
        (return false)))
    (:`then_1`
      (`|ExecutionSequence`
        (:`then_0`
          (bind _success_2 (`self.CheckDistanceToTarget`))
          (if (not _success_2)
            (return false)))
        (:`then_1`
          (`|ExecutionSequence`
            (:`then_0`
              (bind _success_3 (`self.CheckTargetInSight`))
              (if (not _success_3)
                (return false)))
            (:`then_1`
              (`|ExecutionSequence`
                (:`then_0`
                  (bind _success_4 (`self.CheckInteractionTags`))
                  (if (not _success_4)
                    (return false)))
                (:`then_1`
                  (return true))))))))))

(fn `CheckCooldown`
  (returns (Success :type Boolean))
  ;[1 1 1] Check action conditions.
  (if (!= (`self.CooldownActionType`) "None")
    (bind (_found _component) (`/Game/BPS_Core/Blueprints/Systems/BehaviorSystem/Libraries/BPI_Library_BehaviorSystem.FindBehaviorManager` (`self.ControlledPawn`)))
    (if _found
      (bind _success (`/Game/BPS_Core/Blueprints/Systems/BehaviorSystem/Components/BP_AC_BehaviorManager.CheckActionCooldown` _component (`self.CooldownActionType`)))
      (return _success)
      (else
        (return false)))
    (else
      (return true))))

(fn `CheckDistanceToTarget`
  (returns (Success :type Boolean))
  ;[1 1 1] Check distance to target actor.
  (if (`self.CheckDistance`)
    (bind (_success _distance) (`self.GetDistanceToTarget`))
    (if _success
      (bind _returnvalue (<= _distance (`self.GetTargetRange`)))
      (return (select `bool` (`self.InRange`) :`false` (not _returnvalue) :`true` _returnvalue))
      (else
        (return false)))
    (else
      (return true))))

(fn `CheckInteractionTags`
  (returns (Success :type Boolean))
  ;[1 1 1] Check interaction tags and return true if queries are complete.
  (`|ExecutionSequence`
    (:`then_0`
      (if (not (`BlueprintGameplayTagLibrary.IsTagQueryEmpty` (`self.SelfQuery`)))
        (bind (_found _component) (`/Game/BPS_Core/Blueprints/Systems/CharacterSystem/Libraries/BP_Library_CharacterSystem.FindInteractionManager` (`self.ControlledPawn`)))
        (if _found
          (bind _result (`/Game/BPS_Core/Blueprints/Systems/CharacterSystem/Components/BP_AC_InteractionManager.CheckInteractionTags` _component (`self.SelfQuery`)))
          (if (not _result)
            (return false))
          (else
            (return false)))))
    (:`then_1`
      (`|ExecutionSequence`
        (:`then_0`
          (if (not (`BlueprintGameplayTagLibrary.IsTagQueryEmpty` (`self.TargetQuery`)))
            (bind (_found_2 _component_2) (`/Game/BPS_Core/Blueprints/Systems/CharacterSystem/Libraries/BP_Library_CharacterSystem.FindInteractionManager` (`BTFunctionLibrary.GetBlackboardValueAsActor` (`self.TargetActor`))))
            (if _found_2
              (bind _result_2 (`/Game/BPS_Core/Blueprints/Systems/CharacterSystem/Components/BP_AC_InteractionManager.CheckInteractionTags` _component_2 (`self.TargetQuery`)))
              (if (not _result_2)
                (return false))
              (else
                (return false)))))
        (:`then_1`
          (return true))))))

(fn `CheckTargetInSight`
  (returns (Success :type Boolean))
  (locals (LocalInSight :type Boolean :default false))
  (bind _controlledpawn (`self.ControlledPawn`))
  (bind _localinsight (`local.LocalInSight`))
  (bind _sightangle (`self.SightAngle`))
  (bind (_returnvalue_roll _returnvalue_pitch _returnvalue_yaw) (`KismetMathLibrary.BreakRotator` (`BTFunctionLibrary.GetBlackboardValueAsRotator` (`self.RotationToTarget`))))
  (bind (_returnvalue_roll_2 _returnvalue_pitch_2 _returnvalue_yaw_2) (`KismetMathLibrary.BreakRotator` (`Actor.K2_GetActorRotation` _controlledpawn)))
  (bind _returnvalue (`KismetMathLibrary.MakeRotator` 0.0 0.0 _returnvalue_yaw_2))
  (bind (_returnvalue_roll_3 _returnvalue_pitch_3 _returnvalue_yaw_3) (`KismetMathLibrary.BreakRotator` (`KismetMathLibrary.FindLookAtRotation` (`Actor.K2_GetActorLocation` _controlledpawn) (`Actor.K2_GetActorLocation` (`BTFunctionLibrary.GetBlackboardValueAsActor` (`self.TargetActor`))))))
  ;[1 1 1] Check that the target actor in sight of the pawn.
  (if (`self.CheckSight`)
    (`/Engine/EditorBlueprintResources/StandardMacros.IsValid` (`BTFunctionLibrary.GetBlackboardValueAsActor` (`self.TargetActor`))
      (:`Is Valid`
        (if (`self.UseBlackboardRotation`)
          (set `local.LocalInSight` (== (`KismetMathLibrary.MakeRotator` 0.0 0.0 _returnvalue_yaw) _returnvalue :`ErrorTolerance` _sightangle))
          (else
            (set `local.LocalInSight` (== _returnvalue (`KismetMathLibrary.MakeRotator` 0.0 0.0 _returnvalue_yaw_3) :`ErrorTolerance` _sightangle))))
        (return (select `bool` (`self.InSight`) :`false` (not _localinsight) :`true` _localinsight)))
      (:`Is Not Valid`
        (return false)))
    (else
      (return true))))

(fn `GetDistanceToTarget`
  (returns (Success :type Boolean) (Distance :type "Float (double-precision)"))
  (bind _returnvalue (`BTFunctionLibrary.GetBlackboardValueAsActor` (`self.TargetActor`)))
  ;[1 1 1] Returns distance to target value.
  (if (`self.UseBlackboardDistance`)
    (return true (`BTFunctionLibrary.GetBlackboardValueAsFloat` (`self.DistanceToTarget`)))
    (else
      (`/Engine/EditorBlueprintResources/StandardMacros.IsValid` _returnvalue
        (:`Is Valid`
          (return true (`Actor.GetDistanceTo` _returnvalue (`self.ControlledPawn`))))
        (:`Is Not Valid`
          (return false 0.0))))))

(fn `GetTargetRange`
  (returns (AcceptanceRadius :type "Float (double-precision)"))
  (bind _range (`self.Range`))
  (bind _returnvalue (`BTFunctionLibrary.GetBlackboardValueAsFloat` (`self.AcceptanceRange`)))
  ;[1 1 1] Returns target range value.
  (if (`self.UseBlackboardRange`)
    (return (select `bool` (`self.SumRangeValues`) :`false` _returnvalue :`true` (+ _range _returnvalue) :!type "Float (double-precision)"))
    (else
      (return _range))))

(fn `StartCooldown`
  (returns (Success :type Boolean))
  ;[1 1 1] Check action conditions.
  (if (and (!= (`self.CooldownActionType`) "None") (> (`self.CooldownTime`) 0.0))
    (bind (_found _component) (`/Game/BPS_Core/Blueprints/Systems/BehaviorSystem/Libraries/BPI_Library_BehaviorSystem.FindBehaviorManager` (`self.ControlledPawn`)))
    (if _found
      (bind _success (`/Game/BPS_Core/Blueprints/Systems/BehaviorSystem/Components/BP_AC_BehaviorManager.StartActionCooldown` _component (`self.CooldownActionType`) (`self.CooldownTime`)))
      (return _success))
    (else
      (return true))))

(fn `TryPlayActions`
  (returns (Success :type Boolean))
  ;[1 1 1] Do actions and start cooldown.
  (bind (_found _component) (`/Game/BPS_Core/Blueprints/Systems/BehaviorSystem/Libraries/BPI_Library_BehaviorSystem.FindBehaviorManager` (`self.ControlledPawn`)))
  (if _found
    (bind _success (`/Game/BPS_Core/Blueprints/Systems/BehaviorSystem/Components/BP_AC_BehaviorManager.TryPlaySpecialAction` _component (`self.ActionTypeTag`) (`self.ActionType`)))
    (if _success
      (`self.StartCooldown`))
    (return true)
    (else
      (return false))))