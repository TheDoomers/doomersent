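; Behavior tree service that validates the AI's current order target on every AI tick.
; It reads the OrderTarget blackboard actor and checks that it is valid and alive.
; If the target is missing or dead, it finds the pawn's behavior manager component and calls ClearOrder.
; The check returns true for a living target or a cleared order, and false only when no manager is found.
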(event `self.ReceiveTickAI`
  (params (OwnerController :type "AIController Object Reference") (ControlledPawn :type "Pawn Object Reference") (DeltaSeconds :type "Float (single-precision)"))
  ;[1 1 1] Check order target on tick.
  (`self.CheckOrderTarget` OwnerController ControlledPawn))

(fn `CheckOrderTarget`
  (params (OwnerController :type "AIController Object Reference") (ControlledPawn :type "Pawn Object Reference"))
  (returns (Success :type Boolean))
  (locals (LocalOrderTarget :type "Actor Object Reference"))
  ;[1 1 1] Checks order target and returns true if target is alive.
  (bind _output_get (set `local.LocalOrderTarget` (`BTFunctionLibrary.GetBlackboardValueAsActor` (`self.OrderTarget`))))
  (`/Engine/EditorBlueprintResources/StandardMacros.IsValid` _output_get
    (:`Is Valid`
      (bind _isalive (`/Game/BPS_Core/Blueprints/Systems/StatsSystem/Libraries/BP_Library_StatsSystem.CheckActorIsAlive` _output_get))
      (if (not _isalive)
        (bind (_found _component) (`/Game/BPS_Core/Blueprints/Systems/BehaviorSystem/Libraries/BPI_Library_BehaviorSystem.FindBehaviorManager` ControlledPawn :!label _label))
        (if _found
          (`/Game/BPS_Core/Blueprints/Systems/BehaviorSystem/Components/BP_AC_BehaviorManager.ClearOrder` _component)
          (else
            (return false)))))
    (:`Is Not Valid`
      (goto _label)))
  (return true))