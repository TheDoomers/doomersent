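; Behavior tree service that keeps an AI pawn's threat target up to date by dropping threats that no longer apply.
; Each tick it reads the ThreatActor from the blackboard and finds the pawn's behavior manager component.
; If the actor is dead or the manager no longer considers it a threat, the manager clears it.
; An invalid actor or missing manager leaves everything untouched.
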(event `self.ReceiveTickAI`
  (params (OwnerController :type "AIController Object Reference") (ControlledPawn :type "Pawn Object Reference") (DeltaSeconds :type "Float (single-precision)"))
  ;[1 1 1] Check threat actor on tick.
  (`self.CheckThreatActor` OwnerController ControlledPawn))

(fn `CheckThreatActor`
  (params (OwnerController :type "AIController Object Reference") (ControlledPawn :type "Pawn Object Reference"))
  (returns (Success :type Boolean))
  (locals (LocalTargetActor :type "Actor Object Reference"))
  (bind _localtargetactor (`local.LocalTargetActor`))
  ;[1 1 1] Check that the threat actor is alive and it is threat for the controlled pawn.
  (bind _output_get (set `local.LocalTargetActor` (`BTFunctionLibrary.GetBlackboardValueAsActor` (`self.ThreatActor`))))
  (`/Engine/EditorBlueprintResources/StandardMacros.IsValid` _output_get
    (:`Is Valid`
      (bind (_found _component) (`/Game/BPS_Core/Blueprints/Systems/BehaviorSystem/Libraries/BPI_Library_BehaviorSystem.FindBehaviorManager` ControlledPawn))
      (if _found
        (bind _isalive (`/Game/BPS_Core/Blueprints/Systems/StatsSystem/Libraries/BP_Library_StatsSystem.CheckActorIsAlive` _localtargetactor))
        (if _isalive
          (bind _isthreat (`/Game/BPS_Core/Blueprints/Systems/BehaviorSystem/Components/BP_AC_BehaviorManager.CheckTargetIsThreat` _component _localtargetactor))
          (if (not _isthreat)
            (`/Game/BPS_Core/Blueprints/Systems/BehaviorSystem/Components/BP_AC_BehaviorManager.ClearThreatActor` _component :!label _label))
          (else
            (goto _label)))
        (return true)
        (else
          _)))
    (:`Is Not Valid`
      _))
  (return true))