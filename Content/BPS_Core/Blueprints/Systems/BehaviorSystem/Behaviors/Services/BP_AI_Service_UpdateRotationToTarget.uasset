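; Behavior tree service that keeps a blackboard rotation pointing from the controlled pawn toward its target.
; On each AI tick it reads the TargetActorOrLocation key as an actor, falling back to a vector when no valid actor is found.
; It writes the look-at rotation from the pawn's location to that point into the RotationToTarget key, without rotating the pawn itself.
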(event `self.ReceiveTickAI`
  (params (OwnerController :type "AIController Object Reference") (ControlledPawn :type "Pawn Object Reference") (DeltaSeconds :type "Float (single-precision)"))
  ;[1 1 1] Update rotation to target actor on tick.
  (`self.UpdateRotationToTarget` OwnerController ControlledPawn))

(fn `UpdateRotationToTarget`
  (params (OwnerController :type "AIController Object Reference") (ControlledPawn :type "Pawn Object Reference"))
  (returns (Success :type Boolean))
  (locals (LocalOrderTarget :type "Actor Object Reference") (LocalTargetActor :type "Actor Object Reference"))
  (bind _returnvalue (`Actor.K2_GetActorLocation` ControlledPawn))
  (bind _targetactororlocation (`self.TargetActorOrLocation`))
  ;[1 1 1] Update rotation to target blackboard value.
  (bind _output_get (set `local.LocalTargetActor` (`BTFunctionLibrary.GetBlackboardValueAsActor` _targetactororlocation)))
  (`/Engine/EditorBlueprintResources/StandardMacros.IsValid` _output_get
    (:`Is Valid`
      (`BTFunctionLibrary.SetBlackboardValueAsRotator` (`self.RotationToTarget`) (`KismetMathLibrary.FindLookAtRotation` _returnvalue (`Actor.K2_GetActorLocation` _output_get)))
      (return true))
    (:`Is Not Valid`
      (`BTFunctionLibrary.SetBlackboardValueAsRotator` (`self.RotationToTarget`) (`KismetMathLibrary.FindLookAtRotation` _returnvalue (`BTFunctionLibrary.GetBlackboardValueAsVector` _targetactororlocation)))
      (return true))))