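; Behavior tree service that validates the AI pawn's chased actor on every tick.
; It requires the blackboard target to be valid, alive and, when the distance check is enabled, within chasing distance of the guard location rather than the pawn.
; A passing target becomes the controller's focus.
; Otherwise the service clears the focus and, if the pawn has a behavior manager component, has it clear the chased actor.
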(event `self.ReceiveTickAI`
  (params (OwnerController :type "AIController Object Reference") (ControlledPawn :type "Pawn Object Reference") (DeltaSeconds :type "Float (single-precision)"))
  ;[1 1 1] Check target actor on tick.
  (`self.CheckChasedActor` OwnerController ControlledPawn))

(fn `CheckChasedActor`
  (params (OwnerController :type "AIController Object Reference") (ControlledPawn :type "Pawn Object Reference"))
  (returns (Success :type Boolean))
  (locals (LocalTargetActor :type "Actor Object Reference"))
  ;[1 1 1] Check that the target actor is alive and it is in the chasing distance range.
  (bind _output_get (set `local.LocalTargetActor` (`BTFunctionLibrary.GetBlackboardValueAsActor` (`self.ChasedActor`))))
  (`/Engine/EditorBlueprintResources/StandardMacros.IsValid` _output_get
    (:`Is Valid`
      (bind _isalive (`/Game/BPS_Core/Blueprints/Systems/StatsSystem/Libraries/BP_Library_StatsSystem.CheckActorIsAlive` _output_get))
      (if _isalive
        (bind _success (`self.CheckChasedDistance`))
        (if _success
          (`AIController.K2_SetFocus` OwnerController (`local.LocalTargetActor`))
          (return true)
          (else
            _))))
    (:`Is Not Valid`
      _))
  (bind (_found _component) (`/Game/BPS_Core/Blueprints/Systems/BehaviorSystem/Libraries/BPI_Library_BehaviorSystem.FindBehaviorManager` ControlledPawn))
  (if _found
    (`/Game/BPS_Core/Blueprints/Systems/BehaviorSystem/Components/BP_AC_BehaviorManager.ClearChasedActor` _component))
  (`AIController.K2_ClearFocus` OwnerController)
  (return true))

(fn `CheckChasedDistance`
  (returns (Success :type Boolean))
  (locals (LocalTargetActor :type "Actor Object Reference"))
  ;[1 1 1] Returns true if target actor is in chasing distance.
  (if (`BTFunctionLibrary.GetBlackboardValueAsBool` (`self.CheckChasingDistance`))
    (bind _output_get (set `local.LocalTargetActor` (`BTFunctionLibrary.GetBlackboardValueAsActor` (`self.ChasedActor`))))
    (`/Engine/EditorBlueprintResources/StandardMacros.IsValid` _output_get
      (:`Is Valid`
        (return (> (`BTFunctionLibrary.GetBlackboardValueAsFloat` (`self.ChasingDistance`)) (`KismetMathLibrary.VSize` (- (`Actor.K2_GetActorLocation` _output_get) (`BTFunctionLibrary.GetBlackboardValueAsVector` (`self.GuardLocation`)))))))
      (:`Is Not Valid`
        (return false)))
    (else
      (return true))))