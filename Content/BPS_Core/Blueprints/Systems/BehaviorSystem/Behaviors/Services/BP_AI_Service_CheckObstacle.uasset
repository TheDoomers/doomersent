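; Behavior tree service that checks on each tick whether obstacles block the AI pawn's view of its TargetActor.
; It runs parallel sphere traces on the Visibility channel from pawn to target at configurable offsets, ignoring the pawn and its attachments.
; A hit on the target or its attached actors clears the TargetIsBlocked blackboard value.
; FinishOnAnySuccess only stops tracing early, since any single success counts as unblocked.
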(event `self.ReceiveTickAI`
  (params (OwnerController :type "AIController Object Reference") (ControlledPawn :type "Pawn Object Reference") (DeltaSeconds :type "Float (single-precision)"))
  ;[1 1 1] Check target actor on tick.
  (`self.CheckObstacle` OwnerController ControlledPawn))

(fn `CheckObstacle`
  (params (OwnerController :type "AIController Object Reference") (ControlledPawn :type "Pawn Object Reference"))
  (returns (TargetIsBlocked :type Boolean))
  (locals (LocalOrderTarget :type "Actor Object Reference") (LocalTargetActor :type "Actor Object Reference") (LocalActorsToIgnore :type "Array of Actor Object Reference") (LocalStartLocation :type "Vector Structure" :default (0.0 0.0 0.0)) (LocalEndLocation :type "Vector Structure" :default (0.0 0.0 0.0)) (LocalTargetActors :type "Array of Actor Object Reference") (LocalTraceOffsets :type "Array of Vector Structure") (LocalTraceOffset :type "Vector Structure") (LocalTargetIsBlocked :type Boolean :default false))
  (bind _returnvalue (`Actor.K2_GetActorLocation` ControlledPawn))
  (bind _localtargetisblocked (`local.LocalTargetIsBlocked`))
  (bind _returnvalue_2 (`BTFunctionLibrary.GetBlackboardValueAsActor` (`self.TargetActor`)))
  ;[1 1 1] Check obstacle and update target is blocked blackboard value.
  (`/Engine/EditorBlueprintResources/StandardMacros.IsValid` _returnvalue_2
    (:`Is Valid`
      (bind _output_get (set `local.LocalTargetActor` _returnvalue_2))
      (bind _output_get_2 (set `local.LocalTargetActors` (`Actor.GetAttachedActors` _returnvalue_2 true false)))
      (bind _output_get_3 (set `local.LocalActorsToIgnore` (`Actor.GetAttachedActors` ControlledPawn true false)))
      (`KismetArrayLibrary.Array_Add` _output_get_2 _output_get)
      (`KismetArrayLibrary.Array_Add` _output_get_3 ControlledPawn)
      (set `local.LocalStartLocation` _returnvalue)
      (set `local.LocalEndLocation` (`self.GetTraceEnd` _returnvalue (`Actor.K2_GetActorLocation` _returnvalue_2)))
      (bind _output_get_4 (set `local.LocalTraceOffsets` (`self.TraceOffsets`)))
      (`KismetArrayLibrary.Array_Insert` _output_get_4 (`self.FirstTraceOffset`))
      (set `local.LocalTargetIsBlocked` true)
      (for _array_element _output_get_4
        (bind _output_get_5 (set `local.LocalTraceOffset` _array_element))
        (bind _outhit (`KismetSystemLibrary.SphereTraceSingle` (+ (`local.LocalStartLocation`) _output_get_5) (+ (`local.LocalEndLocation`) _output_get_5) 25.0 "TraceTypeQuery1" true (`local.LocalActorsToIgnore`) "None" true (struct :`R` 1.0 :`A` 1.0) (struct :`G` 1.0 :`A` 1.0) 1.0))
        (if (`KismetArrayLibrary.Array_Contains` (`local.LocalTargetActors`) (`.HitActor` (`GameplayStatics.BreakHitResult` _outhit)))
          (if (`self.FinishOnAnySuccess`)
            (`BTFunctionLibrary.SetBlackboardValueAsBool` (`self.TargetIsBlocked`))
            (return false)
            (else
              (set `local.LocalTargetIsBlocked` false)))))
      (`BTFunctionLibrary.SetBlackboardValueAsBool` (`self.TargetIsBlocked`) _localtargetisblocked)
      (return _localtargetisblocked))))

(fn `GetTraceEnd`
  (params (PawnLocation :type "Vector Structure") (TargetLocation :type "Vector Structure"))
  (returns (TraceEnd :type "Vector Structure"))
  (bind _returnvalue (- TargetLocation PawnLocation))
  ;[1 1 1] Returns trace end location.
  (return (+ PawnLocation (* (`KismetMathLibrary.Normal` _returnvalue) (`KismetMathLibrary.VSize` _returnvalue)))))