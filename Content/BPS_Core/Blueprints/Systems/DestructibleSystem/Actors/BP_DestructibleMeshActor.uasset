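; Base actor for a destructible mesh in the destructible system, configured from a data table row that sets its duration and hurt point offset.
; On BeginPlay it either async loads a soft class and replaces itself with that actor, or, unless mesh async loading is set, calls TryDestructActor and starts a timer.
; TryDestructActor is an empty stub here.
; Removal destroys the actor only when not recently rendered, otherwise it sets another timer.
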(event `self.ReceiveBeginPlay`
  ;[1 1 1] Begin play. Try to async load destructible mesh and actor class for soft references.
  (if (`self.AsyncLoadClass`)
    (bind _class (`|LoadAssetClass` (`.DestructibleClassSoft_8_7B2970864DDC6045B1616D9F2ED81E71` (break `/Game/BPS_Core/Blueprints/Systems/DestructibleSystem/Structures/STR_DestructibleSettings` (`self.DestructibleSettings`))))
      (:`Completed`
        (bind _asbp_destructible_mesh_actor (castclass `/Game/BPS_Core/Blueprints/Systems/DestructibleSystem/Actors/BP_DestructibleMeshActor` _class))
        (`|SpawnActorFromClass` _asbp_destructible_mesh_actor (`self.GetTransform`) "Undefined" "SelectDefaultAtRuntime" null (`self.DestructibleHandle`) false (`self.HurtData`) null)
        (`self.K2_DestroyActor`)))
    (elif (not (`self.LoadDestructibleMeshAsync`))
      (`self.TryDestructActor`)
      (`KismetSystemLibrary.K2_SetTimerDelegate` (`|CreateDelegate` :!event `TryRemoveDestructible`) (`self.TimeDuration`)))))

(event `TryRemoveDestructible`
  ;[1 1 1] Try to remove destructible from the game.
  (if (`self.WasRecentlyRendered` 5.0)
    (`KismetSystemLibrary.K2_SetTimerDelegate` (`|CreateDelegate` :!event `TryRemoveDestructible`) 3.0)
    (else
      (`self.K2_DestroyActor`))))

(fn `TryDestructActor`
  (returns (Success :type Boolean))
  (locals (LocalHurtData :type "/Game/BPS_Core/Blueprints/Systems/DestructibleSystem/Structures/STR_DestructibleHurtData Structure"))
  ;[1 1 1] Try to destruct actor using destructible hurt data.
)

(fn `UserConstructionScript`
  (bind (_datatable _rowname) (break `DataTableRowHandle` (`self.DestructibleHandle`)))
  ;[1 1 1] Init destructible settings from the data table.
  (`/Engine/EditorBlueprintResources/StandardMacros.IsValid` _datatable
    (:`Is Valid`
      (bind _returnvalue (`|GetDataTableRow` _datatable _rowname)
        (:`then`
          (bind _output_get (set `self.DestructibleSettings` _returnvalue))
          (bind ((`TimeDuration_17_595E8F1B42023870BBEF95BE328EDA2E` _timeduration) (`LocationOffset_28_50B0633E49294FDE670B64829631FEFF` _locationoffset)) (break `/Game/BPS_Core/Blueprints/Systems/DestructibleSystem/Structures/STR_DestructibleSettings` _output_get))
          (set `self.TimeDuration` _timeduration)
          (`SceneComponent.K2_SetRelativeLocation` (`self.HurtPoint`) _locationoffset false true))))))