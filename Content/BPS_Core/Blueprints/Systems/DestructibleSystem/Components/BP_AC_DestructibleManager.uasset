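; Actor component that manages spawning of destructible mesh actors, either locally or replicated to all clients.
; Replicated spawning runs only on the server, validates the data table handle and multicasts, with dedicated servers skipping the actual spawn.
; Each machine looks up the handle's row, resolves the destructible class and spawns it, passing along hurt data and an async class-load flag.
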(event `SpawnDestructible (Multicast)`
  (params (DestructibleHandle :type "DataTableRowHandle Structure") (SpawnTransform :type "Transform Structure") (HurtData :type "/Game/BPS_Core/Blueprints/Systems/DestructibleSystem/Structures/STR_DestructibleHurtData Structure"))
  ;[1 1 1] Spawn destructible for all clients.
  (if (not (`KismetSystemLibrary.IsDedicatedServer`))
    (`self.SpawnDestructible` DestructibleHandle SpawnTransform HurtData)))

(fn `SpawnDestructible`
  (params (DestructibleHandle :type "DataTableRowHandle Structure") (SpawnTransform :type "Transform Structure") (HurtData :type "/Game/BPS_Core/Blueprints/Systems/DestructibleSystem/Structures/STR_DestructibleHurtData Structure"))
  (returns (Success :type Boolean))
  (locals (LocalDestructibleHandle :type "DataTableRowHandle Structure") (LocalSpawnTransform :type "Transform Structure") (LocalHurtData :type "/Game/BPS_Core/Blueprints/Systems/DestructibleSystem/Structures/STR_DestructibleHurtData Structure"))
  ;[1 1 1] Try to spawn destructible mesh actor on local machine.
  (bind _output_get (set `local.LocalDestructibleHandle` DestructibleHandle))
  (set `local.LocalSpawnTransform` SpawnTransform)
  (set `local.LocalHurtData` HurtData)
  (bind (_datatable _rowname) (break `DataTableRowHandle` _output_get))
  (`/Engine/EditorBlueprintResources/StandardMacros.IsValid` _datatable
    (:`Is Valid`
      (bind _returnvalue (`|GetDataTableRow` _datatable _rowname)
        (:`then`
          (bind (_success _needload _destructibleclass) (`/Game/BPS_Core/Blueprints/Systems/DestructibleSystem/Libraries/BP_Library_DestructibleSystem.FindDestructibleClass` _returnvalue))
          (`|SpawnActorFromClass` _destructibleclass (`local.LocalSpawnTransform`) "AlwaysSpawn" "SelectDefaultAtRuntime" null (`local.LocalDestructibleHandle`) _needload (`local.LocalHurtData`) null)
          (return true))
        (:`RowNotFound`
          _)))
    (:`Is Not Valid`
      _))
  (return false))

(fn `SpawnDestructibleReplicated`
  (params (DestructibleHandle :type "DataTableRowHandle Structure") (SpawnTransform :type "Transform Structure") (HurtData :type "/Game/BPS_Core/Blueprints/Systems/DestructibleSystem/Structures/STR_DestructibleHurtData Structure"))
  (returns (Success :type Boolean))
  ;[1 1 1] Try to spawn destructible mesh actor for all clients.
  (if (`KismetSystemLibrary.IsServer`)
    (if (`/Game/BPS_Core/Blueprints/Systems/CoreSystem/Libraries/BP_Library_CoreFunctions.HandleIsValid` DestructibleHandle)
      (`self.SpawnDestructible (Multicast)` DestructibleHandle SpawnTransform HurtData)
      (return true)
      (else
        _)))
  (return false))