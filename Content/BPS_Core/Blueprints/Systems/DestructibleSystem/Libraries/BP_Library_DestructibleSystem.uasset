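; Blueprint function library for the destructible system, giving callers an entry point to spawn destructible mesh actors.
; It finds the destructible manager component on the game state, printing an error if missing, and forwards validated handles to its local or replicated spawn functions.
; A class resolver prefers the soft class from settings, flags when it still needs loading, and falls back to the default destructible mesh actor.
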(fn `FindDestructibleClass`
  (params (Settings :type "/Game/BPS_Core/Blueprints/Systems/DestructibleSystem/Structures/STR_DestructibleSettings Structure"))
  (returns (Success :type Boolean) (NeedLoad :type Boolean) (DestructibleClass :type "/Game/BPS_Core/Blueprints/Systems/DestructibleSystem/Actors/BP_DestructibleMeshActor Class Reference"))
  (bind (_destructibleclass _destructibleclasssoft) (break `/Game/BPS_Core/Blueprints/Systems/DestructibleSystem/Structures/STR_DestructibleSettings` Settings))
  (bind _output (`|ConvertAsset` _destructibleclasssoft))
  ;[1 1 1] Try to find destructible mesh actor class.
  (if (`KismetSystemLibrary.IsValidSoftClassReference` _destructibleclasssoft)
    (if (`KismetSystemLibrary.IsValidClass` _output)
      (return true false _output)
      (else
        (return true true "/Game/BPS_Core/Blueprints/Systems/DestructibleSystem/Actors/BP_DestructibleMeshActor.BP_DestructibleMeshActor_C")))
    (elif (`KismetSystemLibrary.IsValidClass` _destructibleclass)
      (return true false _destructibleclass)
      (else
        (return true false "/Game/BPS_Core/Blueprints/Systems/DestructibleSystem/Actors/BP_DestructibleMeshActor.BP_DestructibleMeshActor_C")))))

(fn `FindDestructibleManager`
  (returns (Success :type Boolean) (Component :type "/Game/BPS_Core/Blueprints/Systems/DestructibleSystem/Components/BP_AC_DestructibleManager Object Reference"))
  (locals (LocalDestructibleManager :type "/Game/BPS_Core/Blueprints/Systems/DestructibleSystem/Components/BP_AC_DestructibleManager Object Reference"))
  ;[1 1 1] Try to find destructible manager component.
  (bind _output_get (set `local.LocalDestructibleManager` (`Actor.GetComponentByClass` (`GameplayStatics.GetGameState` null) "/Game/BPS_Core/Blueprints/Systems/DestructibleSystem/Components/BP_AC_DestructibleManager.BP_AC_DestructibleManager_C")))
  (`/Engine/EditorBlueprintResources/StandardMacros.IsValid` _output_get
    (:`Is Valid`
      (return true (`local.LocalDestructibleManager`)))
    (:`Is Not Valid`
      (`KismetSystemLibrary.PrintText` null "Destructible manager component is not found! \nDestructible manager component should be a part of the game state class." true true (struct :`R` 1.0 :`A` 1.0) 10.0)
      (return false null))))

(fn `TrySpawnDestructible`
  (params (DestructibleHandle :type "DataTableRowHandle Structure") (SpawnTransform :type "Transform Structure") (HurtData :type "/Game/BPS_Core/Blueprints/Systems/DestructibleSystem/Structures/STR_DestructibleHurtData Structure"))
  (returns (Success :type Boolean))
  ;[1 1 1] Try to spawn destructible mesh actor on local machine.
  (if (`/Game/BPS_Core/Blueprints/Systems/CoreSystem/Libraries/BP_Library_CoreFunctions.HandleIsValid` DestructibleHandle)
    (bind (_success _component) (`self.FindDestructibleManager` null))
    (if _success
      (bind _success_2 (`/Game/BPS_Core/Blueprints/Systems/DestructibleSystem/Components/BP_AC_DestructibleManager.SpawnDestructible` _component DestructibleHandle SpawnTransform HurtData))
      (return _success_2)
      (else
        _)))
  (return false))

(fn `TrySpawnDestructibleReplicated`
  (params (DestructibleHandle :type "DataTableRowHandle Structure") (SpawnTransform :type "Transform Structure") (HurtData :type "/Game/BPS_Core/Blueprints/Systems/DestructibleSystem/Structures/STR_DestructibleHurtData Structure"))
  (returns (Success :type Boolean))
  ;[1 1 1] Try to spawn destructible mesh actor for all clients.
  (if (`/Game/BPS_Core/Blueprints/Systems/CoreSystem/Libraries/BP_Library_CoreFunctions.HandleIsValid` DestructibleHandle)
    (bind (_success _component) (`self.FindDestructibleManager` null))
    (if _success
      (bind _success_2 (`/Game/BPS_Core/Blueprints/Systems/DestructibleSystem/Components/BP_AC_DestructibleManager.SpawnDestructibleReplicated` _component DestructibleHandle SpawnTransform HurtData))
      (return _success_2)
      (else
        _)))
  (return false))