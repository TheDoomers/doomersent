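; Ownership component for the building system that tracks which players own the thing it is attached to.
; It stores owners as networked player IDs resolved from PlayerControllers, with functions to add, remove and check an owner.
; Adds are unique, and both edit functions reassign the OwnerIDs array to itself after changing it and always return true.
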(fn `AddPlayerOwner`
  (params (PlayerController :type "PlayerController Object Reference"))
  (returns (Success :type Boolean))
  ;[1 1 1] Add the networked player ID to the list of owner IDs.
  (`KismetArrayLibrary.Array_AddUnique` (`self.OwnerIDs`) (`/Game/BPS_Core/Blueprints/Systems/CoreSystem/Libraries/BP_Library_CoreFunctions.GetNetworkedPlayerID` PlayerController))
  (set `self.OwnerIDs` (`self.OwnerIDs`))
  (return true))

(fn `CheckPlayerIsOwner`
  (params (PlayerController :type "PlayerController Object Reference"))
  (returns (Result :type Boolean))
  ;[1 1 1] Returns true if player are in list of owners.
  (return (`KismetArrayLibrary.Array_Contains` (`self.OwnerIDs`) (`/Game/BPS_Core/Blueprints/Systems/CoreSystem/Libraries/BP_Library_CoreFunctions.GetNetworkedPlayerID` PlayerController))))

(fn `RemovePlayerOwner`
  (params (PlayerController :type "PlayerController Object Reference"))
  (returns (Success :type Boolean))
  ;[1 1 1] Remove the networked player ID from the list of owner IDs.
  (`KismetArrayLibrary.Array_RemoveItem` (`self.OwnerIDs`) (`/Game/BPS_Core/Blueprints/Systems/CoreSystem/Libraries/BP_Library_CoreFunctions.GetNetworkedPlayerID` PlayerController))
  (set `self.OwnerIDs` (`self.OwnerIDs`))
  (return true))