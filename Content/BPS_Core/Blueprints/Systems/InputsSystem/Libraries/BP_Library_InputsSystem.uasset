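; Blueprint function library that gives access to a player's input mapping management in the InputsSystem.
; FindInputsManager looks up the BP_AC_InputsManager component on a PlayerController, and the set, set-default, set-by-profile and reset mapping functions forward to it.
; These wrappers return false when no manager is found, otherwise the manager's result.
; A separate helper swaps the key in an Enhanced Input action key mapping struct.
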(fn `FindInputsManager`
  (params (PlayerController :type "PlayerController Object Reference"))
  (returns (Success :type Boolean) (Manager :type "/Game/BPS_Core/Blueprints/Systems/InputsSystem/Components/BP_AC_InputsManager Object Reference"))
  (locals (LocalInputsManager :type "/Game/BPS_Core/Blueprints/Systems/InputsSystem/Components/BP_AC_InputsManager Object Reference"))
  ;[1 1 1] Try to find inputs manager component.
  (bind _output_get (set `local.LocalInputsManager` (`Actor.GetComponentByClass` PlayerController "/Game/BPS_Core/Blueprints/Systems/InputsSystem/Components/BP_AC_InputsManager.BP_AC_InputsManager_C")))
  (`/Engine/EditorBlueprintResources/StandardMacros.IsValid` _output_get
    (:`Is Valid`
      (return true _output_get))
    (:`Is Not Valid`
      (return false null))))

(fn `RemapEnhancedActionKeyMapping`
  (params (KeyMapping :type "EnhancedActionKeyMapping Structure (by ref)") (NewKey :type "Key Structure" :default "None"))
  (returns (ResultMapping :type "EnhancedActionKeyMapping Structure"))
  (bind ((`Triggers` _triggers) (`Modifiers` _modifiers) (`Action` _action)) (break `EnhancedActionKeyMapping` KeyMapping))
  ;[1 1 1] Change mapping key in enhanced action key mapping structure.
  (bind _structout (setmembers `EnhancedActionKeyMapping` :`StructRef` KeyMapping :`Triggers` _triggers :`Modifiers` _modifiers :`Action` _action :`Key` NewKey))
  (return _structout))

(fn `ResetInputMapping`
  (params (PlayerController :type "PlayerController Object Reference"))
  (returns (Success :type Boolean))
  ;[1 1 1] Reset input mapping context to default value for the player.
  (bind (_success _manager) (`self.FindInputsManager` PlayerController))
  (if _success
    (bind _success_2 (`/Game/BPS_Core/Blueprints/Systems/InputsSystem/Components/BP_AC_InputsManager.ResetInputMapping` _manager))
    (return _success_2)
    (else
      (return false))))

(fn `SetDefaultInputMapping`
  (params (PlayerController :type "PlayerController Object Reference") (InputMapping :type "InputMappingContext Object Reference") (UseDefault :type Boolean))
  (returns (Success :type Boolean))
  ;[1 1 1] Set default input mapping for the player.
  (bind (_success _manager) (`self.FindInputsManager` PlayerController))
  (if _success
    (bind _success_2 (`/Game/BPS_Core/Blueprints/Systems/InputsSystem/Components/BP_AC_InputsManager.SetDefaultInputMapping` _manager InputMapping UseDefault))
    (return _success_2)
    (else
      (return false))))

(fn `SetInputMapping`
  (params (PlayerController :type "PlayerController Object Reference") (InputMapping :type "InputMappingContext Object Reference"))
  (returns (Success :type Boolean))
  ;[1 1 1] Set current input mapping for the player.
  (bind (_success _manager) (`self.FindInputsManager` PlayerController))
  (if _success
    (bind _success_2 (`/Game/BPS_Core/Blueprints/Systems/InputsSystem/Components/BP_AC_InputsManager.SetInputMapping` _manager InputMapping))
    (return _success_2)
    (else
      (return false))))

(fn `SetInputMappingByProfile`
  (params (PlayerController :type "PlayerController Object Reference") (ProfileName :type Name))
  (returns (Success :type Boolean))
  ;[1 1 1] Set current input mapping by profile for the player.
  (bind (_success _manager) (`self.FindInputsManager` PlayerController))
  (if _success
    (bind _success_2 (`/Game/BPS_Core/Blueprints/Systems/InputsSystem/Components/BP_AC_InputsManager.SetInputMappingByProfile` _manager ProfileName))
    (return _success_2)
    (else
      (return false))))