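; Save game object for the inputs system that stores the player's remapped Enhanced Input bindings.
; Adding a remap replaces, at the same index, any entry with the same input action and default key, or otherwise appends it.
; A getter returns the whole saved list, with both functions exposed as BPI-style calls that report success.
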(fn `AddRemappedEnhancedInput_BPI`
  (params (EnhancedInput :type "/Game/BPS_Core/Blueprints/Systems/InputsSystem/Structures/STR_SaveData_EnhancedInput Structure"))
  (returns (Success :type Boolean))
  (bind ((`InputAction_2_559B3733475CD3DD4F9828895737278D` _inputaction) (`DefaultInputKey_8_668973344234FD41BF4615AF0147A2EB` _defaultinputkey)) (break `/Game/BPS_Core/Blueprints/Systems/InputsSystem/Structures/STR_SaveData_EnhancedInput` EnhancedInput))
  (bind _remappedenhancedinputs (`self.RemappedEnhancedInputs`))
  ;[1 1 1] Add remapped enhanced input to the list.
  (for (_array_element _array_index) (`self.RemappedEnhancedInputs`)
    (bind ((`InputAction_2_559B3733475CD3DD4F9828895737278D` _inputaction_2) (`DefaultInputKey_8_668973344234FD41BF4615AF0147A2EB` _defaultinputkey_2)) (break `/Game/BPS_Core/Blueprints/Systems/InputsSystem/Structures/STR_SaveData_EnhancedInput` _array_element))
    (if (and (== _inputaction_2 _inputaction) (== _defaultinputkey_2 _defaultinputkey))
      (`KismetArrayLibrary.Array_Remove` _remappedenhancedinputs _array_index)
      (`KismetArrayLibrary.Array_Insert` _remappedenhancedinputs EnhancedInput _array_index)
      (return true)))
  (`KismetArrayLibrary.Array_Add` (`self.RemappedEnhancedInputs`) EnhancedInput)
  (return true))

(fn `GetRemappedEnhancedInputs_BPI`
  (returns (Success :type Boolean) (RemappedInputs :type "Array of /Game/BPS_Core/Blueprints/Systems/InputsSystem/Structures/STR_SaveData_EnhancedInput Structure"))
  ;[1 1 1] Returns the list of saved remapped inputs.
  (return true (`self.RemappedEnhancedInputs`)))