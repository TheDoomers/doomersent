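; Player controller component that manages Enhanced Input mapping contexts and key remapping.
; It keeps a permanent context alongside a current one, which is swapped directly or by profile name and resets to a default.
; Remaps edit mapping arrays in place across profile, initial and permanent contexts, then register in a settings save game.
; Init reapplies saved remaps before adding contexts; the save is lazily loaded or created through an interface-accessed object.
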(event `self.ReceiveBeginPlay`
  ;[1 1 1] Begin play. Init component.
  (if (`self.InitOnBeginPlay`)
    (`self.TryInitComponent`)))

(fn `CreateSettingsSaveGame`
  (returns (Success :type Boolean))
  ;[1 1 1] Create settings save game object reference.
  (bind _returnvalue (`GameplayStatics.CreateSaveGameObject` (`self.SettingsSaveGameClass`)))
  (set `self.SettingsSaveGame` _returnvalue)
  (`self.SaveSettingsSaveGame`)
  (return true))

(fn `GetCurrentInputMapping`
  (returns (CurrentInputMapping :type "InputMappingContext Object Reference"))
  ;[1 1 1] Returns current input mapping context.
  (return (`self.CurrentInputMapping`)))

(fn `GetSettingsSaveGame`
  (returns (SettingsSaveGame :type "SaveGame Object Reference"))
  (bind _settingssaveslotname (`self.SettingsSaveSlotName`))
  ;[1 1 1] Try to get settings save game object reference.
  (`/Engine/EditorBlueprintResources/StandardMacros.IsValid` (`self.SettingsSaveGame`)
    (:`Is Valid`
      _)
    (:`Is Not Valid`
      (bind _returnvalue (`GameplayStatics.DoesSaveGameExist` _settingssaveslotname))
      (if _returnvalue
        (bind _returnvalue_2 (`GameplayStatics.LoadGameFromSlot` _settingssaveslotname))
        (`/Engine/EditorBlueprintResources/StandardMacros.IsValid` _returnvalue_2
          (:`Is Valid`
            (set `self.SettingsSaveGame` _returnvalue_2))
          (:`Is Not Valid`
            (`self.CreateSettingsSaveGame` :!label _label)))
        (else
          (goto _label)))))
  (return (`self.SettingsSaveGame`)))

(fn `InitComponent`
  (returns (Success :type Boolean))
  ;[1 1 1] Try to init inputs manager component.
  (bind _asplayer_controller (cast `PlayerController` (`self.GetOwner`))
    (:`then`
      (bind _output_get (set `self.PlayerController` _asplayer_controller))
      (set `PlayerController.bShowMouseCursor` (`self.InitialShowMouseCursor`) _output_get)
      (`self.InitRemappedKeys`)
      (bind _success (`self.SetDefaultInputMapping` (`self.InitialInputMapping`) true))
      (`self.SetPermanentInputMapping` (`self.PermanentInputMapping`))
      (bind _output_get_2 (set `self.IsInitialized` _success))
      (return _output_get_2))
    (:`CastFailed`
      (`KismetSystemLibrary.PrintText` "The inputs manager component is designed only for player controllers!" true true (struct :`R` 1.0 :`A` 1.0) 5.0)
      (bind _output_get_3 (set `self.IsInitialized` false))
      (return _output_get_3))))

(fn `InitRemappedKeys`
  (returns (Success :type Boolean))
  (bind (_success _remappedinputs) (message `/Game/BPS_Core/Blueprints/Systems/InputsSystem/Interfaces/BPI_SaveGame_InputsSystem.GetRemappedEnhancedInputs_BPI` (`self.GetSettingsSaveGame`)))
  (if _success
    (for _array_element _remappedinputs
      (bind (_inputaction _newinputkey _defaultinputkey) (break `/Game/BPS_Core/Blueprints/Systems/InputsSystem/Structures/STR_SaveData_EnhancedInput` _array_element))
      (`self.RemapInputAction` _inputaction _newinputkey _defaultinputkey _defaultinputkey))
    (return true)
    (else
      (return false))))

(fn `RemapInputAction`
  (params (InputAction :type "InputAction Object Reference") (NewInputKey :type "Key Structure" :default "None") (PrevInputKey :type "Key Structure" :default "None") (DefaultInputKey :type "Key Structure" :default "None"))
  (returns (Success :type Boolean))
  (locals (LocalInputAction :type "InputAction Object Reference") (LocalNewInputKey :type "Key Structure" :default "None") (LocalPrevInputKey :type "Key Structure" :default "None") (LocalDefaultInputKey :type "Key Structure" :default "None") (LocalMappingContexts :type "Array of InputMappingContext Object Reference"))
  ;[1 1 1] Remap input action to another key and save it into inputs settings.
  (set `local.LocalInputAction` InputAction)
  (set `local.LocalNewInputKey` NewInputKey)
  (set `local.LocalPrevInputKey` PrevInputKey)
  (set `local.LocalDefaultInputKey` DefaultInputKey)
  (bind _values (`BlueprintMapLibrary.Map_Values` (`self.InputMappingProfiles`)))
  (bind _output_get (set `local.LocalMappingContexts` _values))
  (`KismetArrayLibrary.Array_Append` _output_get (`|MakeArray` (`self.InitialInputMapping`) (`self.PermanentInputMapping`)))
  (for _array_element _output_get
    (`self.RemapInputActionInMappingContext` (`local.LocalInputAction`) _array_element (`local.LocalNewInputKey`) (`local.LocalPrevInputKey`) (`local.LocalDefaultInputKey`)))
  (return true))

(fn `RemapInputActionInMappingContext`
  (params (InputAction :type "InputAction Object Reference") (MappingContext :type "InputMappingContext Object Reference") (NewInputKey :type "Key Structure" :default "None") (PrevInputKey :type "Key Structure" :default "None") (DefaultInputKey :type "Key Structure" :default "None"))
  (returns (Success :type Boolean))
  (locals (LocalInputAction :type "InputAction Object Reference") (LocalMappingContext :type "InputMappingContext Object Reference") (LocalNewInputKey :type "Key Structure" :default "None") (LocalPrevInputKey :type "Key Structure" :default "None") (LocalKeyMapping :type "EnhancedActionKeyMapping Structure") (LocalTargetIndex :type Integer) (LocalDefaultInputKey :type "Key Structure" :default "None"))
  ;[1 1 1] Remap input action to another key for specific mapping context and save it into inputs settings.
  (set `local.LocalInputAction` InputAction)
  (bind _output_get (set `local.LocalMappingContext` MappingContext))
  (set `local.LocalNewInputKey` NewInputKey)
  (set `local.LocalPrevInputKey` PrevInputKey)
  (set `local.LocalDefaultInputKey` DefaultInputKey)
  (`/Engine/EditorBlueprintResources/StandardMacros.IsValid` _output_get
    (:`Is Valid`
      (for (_array_element _array_index) (`InputMappingContext.Mappings` _output_get)
        (set `local.LocalKeyMapping` _array_element)
        (set `local.LocalTargetIndex` _array_index)
        (bind ((`Action` _action) (`Key` _key)) (break `EnhancedActionKeyMapping` _array_element))
        (if (and (== _action (`local.LocalInputAction`)) (== _key (`local.LocalPrevInputKey`)))
          (bind _resultmapping (`/Game/BPS_Core/Blueprints/Systems/InputsSystem/Libraries/BP_Library_InputsSystem.RemapEnhancedActionKeyMapping` (`local.LocalKeyMapping`) (`local.LocalNewInputKey`)))
          (`KismetArrayLibrary.Array_Set` (`InputMappingContext.Mappings` (`local.LocalMappingContext`)) (`local.LocalTargetIndex`) _resultmapping)
          (message `/Game/BPS_Core/Blueprints/Systems/InputsSystem/Interfaces/BPI_SaveGame_InputsSystem.AddRemappedEnhancedInput_BPI` (`self.GetSettingsSaveGame`) (make `/Game/BPS_Core/Blueprints/Systems/InputsSystem/Structures/STR_SaveData_EnhancedInput` (`local.LocalInputAction`) (`local.LocalNewInputKey`) (`local.LocalDefaultInputKey`)))
          (return true))))
    (:`Is Not Valid`
      _))
  (return false))

(fn `ResetInputMapping`
  (returns (Success :type Boolean))
  ;[1 1 1] Reset input mapping context to default value for the player.
  (bind _success (`self.SetInputMapping` (`self.DefaultInputMapping`)))
  (return _success))

(fn `SaveSettingsSaveGame`
  (returns (Success :type Boolean))
  ;[1 1 1] Save settings save game to the settings save slot.
  (`GameplayStatics.SaveGameToSlot` (`self.GetSettingsSaveGame`) (`self.SettingsSaveSlotName`))
  (return true))

(fn `SetDefaultInputMapping`
  (params (InputMapping :type "InputMappingContext Object Reference") (UseDefault :type Boolean))
  (returns (Success :type Boolean))
  ;[1 1 1] Set default input mapping context for the player.
  (set `self.DefaultInputMapping` InputMapping)
  (if UseDefault
    (`self.ResetInputMapping`))
  (return true))

(fn `SetInputMapping`
  (params (InputMapping :type "InputMappingContext Object Reference"))
  (returns (Success :type Boolean))
  (bind _playercontroller (`self.PlayerController`))
  (bind _returnvalue (pcsubsystem `EnhancedInputLocalPlayerSubsystem` _playercontroller))
  ;[1 1 1] Set current input mapping context for the player.
  (`/Engine/EditorBlueprintResources/StandardMacros.IsValid` _playercontroller
    (:`Is Valid`
      (`/Engine/EditorBlueprintResources/StandardMacros.IsValid` _returnvalue
        (:`Is Valid`
          (`EnhancedInputSubsystemInterface.RemoveMappingContext` _returnvalue (`self.CurrentInputMapping`) (struct)))
        (:`Is Not Valid`
          (return false))))
    (:`Is Not Valid`
      _))
  (bind _output_get (set `self.CurrentInputMapping` InputMapping))
  (`EnhancedInputSubsystemInterface.AddMappingContext` _returnvalue _output_get 0 (struct))
  (return true))

(fn `SetInputMappingByProfile`
  (params (ProfileName :type Name))
  (returns (Success :type Boolean))
  (bind (_value _returnvalue) (`BlueprintMapLibrary.Map_Find` (`self.InputMappingProfiles`) ProfileName))
  ;[1 1 1] Set current input mapping context by profile name for the player.
  (if _returnvalue
    (bind _success (`self.SetInputMapping` _value))
    (return _success)
    (else
      (return false))))

(fn `SetPermanentInputMapping`
  (params (InputMapping :type "InputMappingContext Object Reference"))
  (returns (Success :type Boolean))
  (bind _playercontroller (`self.PlayerController`))
  (bind _returnvalue (pcsubsystem `EnhancedInputLocalPlayerSubsystem` _playercontroller))
  ;[1 1 1] Set permanent input mapping context for the player.
  (`/Engine/EditorBlueprintResources/StandardMacros.IsValid` _playercontroller
    (:`Is Valid`
      (`/Engine/EditorBlueprintResources/StandardMacros.IsValid` _returnvalue
        (:`Is Valid`
          (`EnhancedInputSubsystemInterface.RemoveMappingContext` _returnvalue (`self.PermanentInputMapping`) (struct)))))
    (:`Is Not Valid`
      _))
  (bind _output_get (set `self.PermanentInputMapping` InputMapping))
  (`EnhancedInputSubsystemInterface.AddMappingContext` _returnvalue _output_get 0 (struct))
  (return true))

(fn `TryInitComponent`
  (returns (Success :type Boolean))
  ;[1 1 1] Try to init inputs manager component.
  (if (not (`self.IsInitialized`))
    (bind _success (`self.InitComponent`))
    (bind _output_get (set `self.IsInitialized` _success))
    (return _output_get)
    (else
      (return true))))