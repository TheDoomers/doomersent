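; Blueprint function library that starts async loads of generic assets, static meshes and skeletal meshes from soft references.
; Each function finds BP_AC_AsyncLoadManager on the GameState, creates a loader from it, then binds a callback or passes the target component.
; Component variants fall back to a blocking load and set the mesh directly when game instance or manager is missing, without firing any callback; delegate-only variants return false.
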(fn `AsyncLoadAssetDelegate`
  (params (SoftObjectReference :type "Object Soft Object Reference") (OnAssetLoaded :type "Delegate (by ref)"))
  (returns (Success :type Boolean))
  (locals (LocalSoftObjectReference :type "Object Soft Object Reference"))
  ;[1 1 1] Try to load asset from soft object reference.
  (set `local.LocalSoftObjectReference` SoftObjectReference)
  (`/Engine/EditorBlueprintResources/StandardMacros.IsValid` (`GameplayStatics.GetGameInstance` null)
    (:`Is Valid`
      (bind (_found _manager) (`self.FindAsyncLoadManager` null))
      (if _found
        (bind (_success _asyncloader) (`/Game/BPS_Core/Blueprints/Systems/AsyncLoadSystem/Components/BP_AC_AsyncLoadManager.CreateAsyncLoader` _manager))
        (if _success
          (add `/Game/BPS_Core/Blueprints/Systems/AsyncLoadSystem/Actors/BP_AsyncLoader.OnAssetLoaded` _asyncloader OnAssetLoaded)
          (`/Game/BPS_Core/Blueprints/Systems/AsyncLoadSystem/Actors/BP_AsyncLoader.AsyncLoadAsset` _asyncloader (`local.LocalSoftObjectReference`))
          (return true)
          (else
            _))))
    (:`Is Not Valid`
      _))
  (return false))

(fn `AsyncLoadSkeletalMeshDelegate`
  (params (SoftObjectReference :type "Object Soft Object Reference") (OnSkeletalMeshLoaded :type "Delegate (by ref)"))
  (returns (Success :type Boolean))
  (locals (LocalSoftObjectReference :type "Object Soft Object Reference"))
  ;[1 1 1] Try to load skeletal mesh from soft object reference.
  (set `local.LocalSoftObjectReference` SoftObjectReference)
  (`/Engine/EditorBlueprintResources/StandardMacros.IsValid` (`GameplayStatics.GetGameInstance` null)
    (:`Is Valid`
      (bind (_found _manager) (`self.FindAsyncLoadManager` null))
      (if _found
        (bind (_success _asyncloader) (`/Game/BPS_Core/Blueprints/Systems/AsyncLoadSystem/Components/BP_AC_AsyncLoadManager.CreateAsyncLoader` _manager))
        (if _success
          (add `/Game/BPS_Core/Blueprints/Systems/AsyncLoadSystem/Actors/BP_AsyncLoader.OnSkeletalMeshLoaded` _asyncloader OnSkeletalMeshLoaded)
          (`/Game/BPS_Core/Blueprints/Systems/AsyncLoadSystem/Actors/BP_AsyncLoader.AsyncLoadSkeletalMesh` _asyncloader (`local.LocalSoftObjectReference`))
          (return true)
          (else
            _))))
    (:`Is Not Valid`
      _))
  (return false))

(fn `AsyncLoadSkeletalMeshForComponent`
  (params (TargetComponent :type "SkeletalMeshComponent Object Reference") (SoftObjectReference :type "Object Soft Object Reference"))
  (returns (Success :type Boolean))
  (locals (LocalSkeletalMeshComponent :type "SkeletalMeshComponent Object Reference") (LocalSoftObjectReference :type "Object Soft Object Reference"))
  ;[1 1 1] Try to load and update skeletal mesh object for component from soft object reference.
  (set `local.LocalSkeletalMeshComponent` TargetComponent)
  (bind _output_get (set `local.LocalSoftObjectReference` SoftObjectReference))
  (`/Engine/EditorBlueprintResources/StandardMacros.IsValid` (`GameplayStatics.GetGameInstance` null)
    (:`Is Valid`
      (bind (_found _manager) (`self.FindAsyncLoadManager` null))
      (if _found
        (bind (_success _asyncloader) (`/Game/BPS_Core/Blueprints/Systems/AsyncLoadSystem/Components/BP_AC_AsyncLoadManager.CreateAsyncLoader` _manager))
        (if _success
          (`/Game/BPS_Core/Blueprints/Systems/AsyncLoadSystem/Actors/BP_AsyncLoader.AsyncLoadSkeletalMeshForComponent` _asyncloader (`local.LocalSkeletalMeshComponent`) (`local.LocalSoftObjectReference`))
          (return true)
          (else
            _))
        (else
          (bind _returnvalue (`KismetSystemLibrary.LoadAsset_Blocking` _output_get :!label _label))
          (bind _asskeletal_mesh (cast `SkeletalMesh` _returnvalue)
            (:`then`
              (`SkinnedMeshComponent.SetSkinnedAssetAndUpdate` (`local.LocalSkeletalMeshComponent`) _asskeletal_mesh true)
              (return true))
            (:`CastFailed`
              _)))))
    (:`Is Not Valid`
      (goto _label)))
  (return false))

(fn `AsyncLoadStaticMeshDelegate`
  (params (SoftObjectReference :type "Object Soft Object Reference") (OnStaticMeshLoaded :type "Delegate (by ref)"))
  (returns (Success :type Boolean))
  (locals (LocalSoftObjectReference :type "Object Soft Object Reference"))
  ;[1 1 1] Try to load static mesh from soft object reference.
  (set `local.LocalSoftObjectReference` SoftObjectReference)
  (`/Engine/EditorBlueprintResources/StandardMacros.IsValid` (`GameplayStatics.GetGameInstance` null)
    (:`Is Valid`
      (bind (_found _manager) (`self.FindAsyncLoadManager` null))
      (if _found
        (bind (_success _asyncloader) (`/Game/BPS_Core/Blueprints/Systems/AsyncLoadSystem/Components/BP_AC_AsyncLoadManager.CreateAsyncLoader` _manager))
        (if _success
          (add `/Game/BPS_Core/Blueprints/Systems/AsyncLoadSystem/Actors/BP_AsyncLoader.OnStaticMeshLoaded` _asyncloader OnStaticMeshLoaded)
          (`/Game/BPS_Core/Blueprints/Systems/AsyncLoadSystem/Actors/BP_AsyncLoader.AsyncLoadStaticMesh` _asyncloader (`local.LocalSoftObjectReference`))
          (return true)
          (else
            _))))
    (:`Is Not Valid`
      _))
  (return false))

(fn `AsyncLoadStaticMeshForComponent`
  (params (TargetComponent :type "StaticMeshComponent Object Reference") (SoftObjectReference :type "Object Soft Object Reference"))
  (returns (Success :type Boolean))
  (locals (LocalStaticMeshComponent :type "StaticMeshComponent Object Reference") (LocalSoftObjectReference :type "Object Soft Object Reference"))
  ;[1 1 1] Try to load and update static mesh object for component from soft object reference.
  (set `local.LocalStaticMeshComponent` TargetComponent)
  (bind _output_get (set `local.LocalSoftObjectReference` SoftObjectReference))
  (`/Engine/EditorBlueprintResources/StandardMacros.IsValid` (`GameplayStatics.GetGameInstance` null)
    (:`Is Valid`
      (bind (_found _manager) (`self.FindAsyncLoadManager` null))
      (if _found
        (bind (_success _asyncloader) (`/Game/BPS_Core/Blueprints/Systems/AsyncLoadSystem/Components/BP_AC_AsyncLoadManager.CreateAsyncLoader` _manager))
        (if _success
          (`/Game/BPS_Core/Blueprints/Systems/AsyncLoadSystem/Actors/BP_AsyncLoader.AsyncLoadStaticMeshForComponent` _asyncloader (`local.LocalStaticMeshComponent`) (`local.LocalSoftObjectReference`))
          (return true)
          (else
            _))
        (else
          (bind _returnvalue (`KismetSystemLibrary.LoadAsset_Blocking` _output_get :!label _label))
          (bind _asstatic_mesh (cast `StaticMesh` _returnvalue)
            (:`then`
              (bind _returnvalue_2 (`StaticMeshComponent.SetStaticMesh` (`local.LocalStaticMeshComponent`) _asstatic_mesh))
              (return _returnvalue_2))
            (:`CastFailed`
              _)))))
    (:`Is Not Valid`
      (goto _label)))
  (return false))

(fn `FindAsyncLoadManager`
  (returns (Found :type Boolean) (Manager :type "/Game/BPS_Core/Blueprints/Systems/AsyncLoadSystem/Components/BP_AC_AsyncLoadManager Object Reference"))
  (locals (LocalAsyncLoadManager :type "/Game/BPS_Core/Blueprints/Systems/AsyncLoadSystem/Components/BP_AC_AsyncLoadManager Object Reference"))
  (bind _returnvalue (`GameplayStatics.GetGameState` null))
  ;[1 1 1] Try to find async load manager component.
  (`/Engine/EditorBlueprintResources/StandardMacros.IsValid` _returnvalue
    (:`Is Valid`
      (bind _output_get (set `local.LocalAsyncLoadManager` (`Actor.GetComponentByClass` _returnvalue "/Game/BPS_Core/Blueprints/Systems/AsyncLoadSystem/Components/BP_AC_AsyncLoadManager.BP_AC_AsyncLoadManager_C")))
      (`/Engine/EditorBlueprintResources/StandardMacros.IsValid` _output_get
        (:`Is Valid`
          (return true (`local.LocalAsyncLoadManager`)))
        (:`Is Not Valid`
          (`KismetSystemLibrary.PrintText` null "Async load manager component is not found! \nAsync load manager component should be a part of the game state class." true true (struct :`R` 1.0 :`A` 1.0) 10.0)
          (return false null))))
    (:`Is Not Valid`
      (return false null))))

(fn `TryAsyncLoadSkeletalMeshForComponent`
  (params (SkeletalMeshComponent :type "SkeletalMeshComponent Object Reference") (SoftObjectReference :type "Object Soft Object Reference") (OnSkeletalMeshLoaded :type "Delegate (by ref)"))
  (returns (Success :type Boolean))
  (locals (LocalSoftObjectReference :type "Object Soft Object Reference"))
  ;[1 1 1] Try to load skeletal mesh from soft object reference.
  (set `local.LocalSoftObjectReference` SoftObjectReference)
  (`/Engine/EditorBlueprintResources/StandardMacros.IsValid` (`GameplayStatics.GetGameInstance` null)
    (:`Is Valid`
      (bind (_found _manager) (`self.FindAsyncLoadManager` null))
      (if _found
        (bind (_success _asyncloader) (`/Game/BPS_Core/Blueprints/Systems/AsyncLoadSystem/Components/BP_AC_AsyncLoadManager.CreateAsyncLoader` _manager))
        (if _success
          (add `/Game/BPS_Core/Blueprints/Systems/AsyncLoadSystem/Actors/BP_AsyncLoader.OnSkeletalMeshLoaded` _asyncloader OnSkeletalMeshLoaded)
          (`/Game/BPS_Core/Blueprints/Systems/AsyncLoadSystem/Actors/BP_AsyncLoader.AsyncLoadSkeletalMesh` _asyncloader (`local.LocalSoftObjectReference`))
          (return true)
          (else
            _))
        (else
          (bind _returnvalue (`KismetSystemLibrary.LoadAsset_Blocking` (`local.LocalSoftObjectReference`) :!label _label))
          (bind _asskeletal_mesh (cast `SkeletalMesh` _returnvalue)
            (:`then`
              (`SkinnedMeshComponent.SetSkinnedAssetAndUpdate` SkeletalMeshComponent _asskeletal_mesh true)
              (return true))
            (:`CastFailed`
              _)))))
    (:`Is Not Valid`
      (goto _label)))
  (return false))

(fn `TryAsyncLoadStaticMeshForComponent`
  (params (StaticMeshComponent :type "StaticMeshComponent Object Reference") (SoftObjectReference :type "Object Soft Object Reference") (OnStaticMeshLoaded :type "Delegate (by ref)"))
  (returns (Success :type Boolean))
  (locals (LocalSoftObjectReference :type "Object Soft Object Reference"))
  ;[1 1 1] Try to load static mesh from soft object reference.
  (set `local.LocalSoftObjectReference` SoftObjectReference)
  (`/Engine/EditorBlueprintResources/StandardMacros.IsValid` (`GameplayStatics.GetGameInstance` null)
    (:`Is Valid`
      (bind (_found _manager) (`self.FindAsyncLoadManager` null))
      (if _found
        (bind (_success _asyncloader) (`/Game/BPS_Core/Blueprints/Systems/AsyncLoadSystem/Components/BP_AC_AsyncLoadManager.CreateAsyncLoader` _manager))
        (if _success
          (add `/Game/BPS_Core/Blueprints/Systems/AsyncLoadSystem/Actors/BP_AsyncLoader.OnStaticMeshLoaded` _asyncloader OnStaticMeshLoaded)
          (`/Game/BPS_Core/Blueprints/Systems/AsyncLoadSystem/Actors/BP_AsyncLoader.AsyncLoadStaticMesh` _asyncloader (`local.LocalSoftObjectReference`))
          (return true)
          (else
            _))
        (else
          (bind _returnvalue (`KismetSystemLibrary.LoadAsset_Blocking` (`local.LocalSoftObjectReference`) :!label _label))
          (bind _asstatic_mesh (cast `StaticMesh` _returnvalue)
            (:`then`
              (`StaticMeshComponent.SetStaticMesh` StaticMeshComponent _asstatic_mesh)
              (return true))
            (:`CastFailed`
              _)))))
    (:`Is Not Valid`
      (goto _label)))
  (return false))