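; BP_AsyncLoader is a one-shot helper actor that asynchronously loads assets from soft references.
; Separate events handle generic assets, static meshes and skeletal meshes, with component variants that apply the loaded mesh to a supplied component if it is still valid.
; Successful loads are reported through OnAssetLoaded, OnStaticMeshLoaded or OnSkeletalMeshLoaded dispatchers.
; The actor destroys itself when any load completes, even if the cast or component check fails.
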(event `AsyncLoadAsset`
  (params (SoftObjectReference :type "Object Soft Object Reference"))
  ;[1 1 1] Async load assets with delegates.
  (bind _object (`|LoadAsset` SoftObjectReference)
    (:`Completed`
      (`self.OnAssetLoaded` _object)
      (`self.K2_DestroyActor`))))

(event `AsyncLoadStaticMeshForComponent`
  (params (StaticMeshComponent :type "StaticMeshComponent Object Reference") (SoftObjectReference :type "Object Soft Object Reference"))
  ;[1 1 1] Async load assets and update components.
  (bind _object (`|LoadAsset` SoftObjectReference)
    (:`Completed`
      (bind _asstatic_mesh (cast `StaticMesh` _object)
        (:`then`
          (`/Engine/EditorBlueprintResources/StandardMacros.IsValid` StaticMeshComponent
            (:`Is Valid`
              (`StaticMeshComponent.SetStaticMesh` StaticMeshComponent _asstatic_mesh)
              (`self.OnStaticMeshLoaded` _asstatic_mesh))
            (:`Is Not Valid`
              _)))
        (:`CastFailed`
          _))
      (`self.K2_DestroyActor`))))

(event `AsyncLoadStaticMesh`
  (params (SoftObjectReference :type "Object Soft Object Reference"))
  ;[1 1 1] Async load assets with delegates.
  (bind _object (`|LoadAsset` SoftObjectReference)
    (:`Completed`
      (bind _asstatic_mesh (cast `StaticMesh` _object)
        (:`then`
          (`self.OnStaticMeshLoaded` _asstatic_mesh))
        (:`CastFailed`
          _))
      (`self.K2_DestroyActor`))))

(event `AsyncLoadSkeletalMeshForComponent`
  (params (SkeletalMeshComponent :type "SkeletalMeshComponent Object Reference") (SoftObjectReference :type "Object Soft Object Reference"))
  ;[1 1 1] Async load assets and update components.
  (bind _object (`|LoadAsset` SoftObjectReference)
    (:`Completed`
      (bind _asskeletal_mesh (cast `SkeletalMesh` _object)
        (:`then`
          (`/Engine/EditorBlueprintResources/StandardMacros.IsValid` SkeletalMeshComponent
            (:`Is Valid`
              (`SkinnedMeshComponent.SetSkinnedAssetAndUpdate` SkeletalMeshComponent _asskeletal_mesh true)
              (`self.OnSkeletalMeshLoaded` _asskeletal_mesh))
            (:`Is Not Valid`
              _)))
        (:`CastFailed`
          _))
      (`self.K2_DestroyActor`))))

(event `AsyncLoadSkeletalMesh`
  (params (SoftObjectReference :type "Object Soft Object Reference"))
  ;[1 1 1] Async load assets with delegates.
  (bind _object (`|LoadAsset` SoftObjectReference)
    (:`Completed`
      (bind _asskeletal_mesh (cast `SkeletalMesh` _object)
        (:`then`
          (`self.OnSkeletalMeshLoaded` _asskeletal_mesh))
        (:`CastFailed`
          _))
      (`self.K2_DestroyActor`))))

(fn `UserConstructionScript`)