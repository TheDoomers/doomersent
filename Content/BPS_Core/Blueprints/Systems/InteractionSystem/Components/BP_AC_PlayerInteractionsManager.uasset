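; Player controller component that finds interactable objects and runs interactions with them.
; On local tick it targets BPI_InteractableObject actors by mouse or camera trace, falling back to the nearest overlapped candidate, with optional distance, overlap and line-of-sight checks.
; The target gets widget and highlight actors.
; Input runs an optional timer, cancelled if checks fail, then interacts on client, server or both, revalidating on each side.
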(event `self.ReceiveBeginPlay`
  ;[1 1 1] Begin play. Try to init component.
  (`self.InitComponent`))

(event `TryInteractWithActor (Server)`
  (params (TargetActor :type "Actor Object Reference") (TargetComponent :type "PrimitiveComponent Object Reference"))
  ;[1 1 1] Try to start interaction with actor.
  (`self.TryInteractWithActorOnServer` TargetActor TargetComponent))

(event `self.ReceiveTick`
  (params (DeltaSeconds :type "Float (single-precision)"))
  ;[1 1 1] Tick event. Try to update interaction target.
  (if (`self.IsLocalController`)
    (`/Engine/EditorBlueprintResources/StandardMacros.IsValid` (`self.InteractableActor`)
      (:`Is Valid`
        (`self.CheckInteractableActor`))
      (:`Is Not Valid`
        (`self.UpdateTargetActor`)))
    (else
      (`self.SetComponentTickEnabled` false))))

(fn `Bind_CompleteInteractionInput`
  ;[1 1 1] Try to complete interaction input for the player.
  (`KismetSystemLibrary.K2_ClearAndInvalidateTimerHandle` (`self.InteractionTimer`))
  (`self.CompleteInteractionInput`))

(fn `CheckCanInteractWithActor`
  (params (TargetActor :type "Actor Object Reference") (TargetComponent :type "PrimitiveComponent Object Reference"))
  (returns (Success :type Boolean))
  (bind _playercontroller (`self.PlayerController`))
  ;[1 1 1] Returns true if player can interact with target actor and component.
  (bind _result (message `/Game/BPS_Core/Blueprints/Systems/InteractionSystem/Interfaces/BPI_InteractableObject.HasInteractableComponents_BPI` TargetActor))
  (if _result
    (bind _success (message `/Game/BPS_Core/Blueprints/Systems/InteractionSystem/Interfaces/BPI_InteractableObject.CheckCanInteractWithComponent_BPI` TargetActor TargetComponent _playercontroller))
    (if _success
      (bind _result_2 (`self.CheckTargetActor` TargetActor TargetComponent :!label _label))
      (if _result_2
        (return true)
        (else
          _)))
    (else
      (bind _success_2 (message `/Game/BPS_Core/Blueprints/Systems/InteractionSystem/Interfaces/BPI_InteractableObject.CheckCanInteractWithActor_BPI` TargetActor _playercontroller))
      (if _success_2
        (goto _label)
        (else
          _))))
  (return false))

(fn `CheckInteractableActor`
  (returns (Success :type Boolean))
  ;[1 1 1] Check that player can interact with target actor and component. Otherwise stop interaction input.
  (bind _success (`self.CheckCanInteractWithActor` (`self.InteractableActor`) (`self.InteractableComponent`)))
  (if _success
    (return true)
    (else
      (`self.StopInteractionInput`)
      (return true))))

(fn `CheckTargetActor`
  (params (TargetActor :type "Actor Object Reference") (TargetComponent :type "PrimitiveComponent Object Reference"))
  (returns (Result :type Boolean))
  (locals (LocalTargetActor :type "Actor Object Reference") (LocalControlledPawn :type "Pawn Object Reference") (LocalActorsToIgnore :type "Array of Actor Object Reference") (LocalTargetComponent :type "PrimitiveComponent Object Reference") (LocalEndLocation :type "Vector Structure" :default (0.0 0.0 0.0)))
  ;[1 1 1] Check different interaction conditions for target actor and component.
  (set `local.LocalTargetActor` TargetActor)
  (set `local.LocalTargetComponent` TargetComponent)
  (`|ExecutionSequence`
    (:`then_0`
      (if (`self.CheckInteractionDistance`)
        (bind _output_get (set `local.LocalControlledPawn` (`Controller.K2_GetPawn` (`self.PlayerController`))))
        (`/Engine/EditorBlueprintResources/StandardMacros.IsValid` _output_get
          (:`Is Valid`
            (if (> (`KismetMathLibrary.Vector_Distance` (`Actor.K2_GetActorLocation` (`local.LocalTargetActor`)) (`Actor.K2_GetActorLocation` _output_get)) (`self.InteractionDistance`))
              (return false))))))
    (:`then_1`
      (`|ExecutionSequence`
        (:`then_0`
          (if (`self.CheckOverlappedActors`)
            (if (not (`KismetArrayLibrary.Array_Contains` (`self.OverlappedActors`) (`local.LocalTargetActor`)))
              (return false))))
        (:`then_1`
          (`|ExecutionSequence`
            (:`then_0`
              (if (`self.CheckTraceToInteractable`)
                (bind _result (`self.CheckTraceToTarget` (`local.LocalTargetActor`) (`local.LocalTargetComponent`)))
                (if (not _result)
                  (return false))))
            (:`then_1`
              (return true))))))))

(fn `CheckTraceToTarget`
  (params (TargetActor :type "Actor Object Reference") (TargetComponent :type "PrimitiveComponent Object Reference"))
  (returns (Result :type Boolean))
  (locals (LocalTargetActor :type "Actor Object Reference") (LocalTargetComponent :type "PrimitiveComponent Object Reference") (LocalControlledPawn :type "Pawn Object Reference") (LocalActorsToIgnore :type "Array of Actor Object Reference") (LocalEndLocation :type "Vector Structure") (LocalPawnLocation :type "Vector Structure" :default (0.0 0.0 0.0)) (LocalStartLocation :type "Vector Structure" :default (0.0 0.0 0.0)) (LocalResult :type Boolean :default true))
  (bind _tracecheckoffsets (`self.TraceCheckOffsets`))
  ;[1 1 1] Check trace from controlled pawn to target actor and component. Returns true if there is no blocking hit.
  (set `local.LocalTargetActor` TargetActor)
  (set `local.LocalTargetComponent` TargetComponent)
  (bind _output_get (set `local.LocalControlledPawn` (`Controller.K2_GetPawn` (`self.PlayerController`))))
  (`/Engine/EditorBlueprintResources/StandardMacros.IsValid` _output_get
    (:`Is Valid`
      (bind _output_get_2 (set `local.LocalActorsToIgnore` (`/Game/BPS_Core/Blueprints/Systems/CoreSystem/Libraries/BP_Library_CoreFunctions.GetActorsToIgnore` _output_get)))
      (`KismetArrayLibrary.Array_Add` _output_get_2 (`local.LocalTargetActor`))
      (set `local.LocalPawnLocation` (`Actor.K2_GetActorLocation` (`local.LocalControlledPawn`)))
      (bind (_success _targetlocation) (message `/Game/BPS_Core/Blueprints/Systems/InteractionSystem/Interfaces/BPI_InteractableObject.GetTraceTargetLocation_BPI` (`local.LocalTargetActor`) (`local.LocalTargetComponent`)))
      (if _success
        (set `local.LocalEndLocation` _targetlocation)
        (else
          (set `local.LocalEndLocation` (`Actor.K2_GetActorLocation` (`local.LocalTargetActor`)))))
      (if (`KismetArrayLibrary.Array_IsValidIndex` _tracecheckoffsets)
        (for _array_element _tracecheckoffsets
          (bind _output_get_3 (set `local.LocalStartLocation` (+ (`local.LocalPawnLocation`) _array_element)))
          (bind (_outhit _returnvalue) (`KismetSystemLibrary.LineTraceSingle` _output_get_3 (`local.LocalEndLocation`) "TraceTypeQuery1" false (`local.LocalActorsToIgnore`) (`self.TraceDebugType`)))
          (if _returnvalue
            (if (not (`KismetArrayLibrary.Array_Contains` (`self.TraceIgnoredClasses`) (`GameplayStatics.GetObjectClass` (`/Game/BPS_Core/Blueprints/Systems/CoreSystem/Libraries/BP_Library_CoreFunctions.GetHitActor` _outhit))))
              (if (== (`/Game/BPS_Core/Blueprints/Systems/CoreSystem/Libraries/BP_Library_CoreFunctions.GetHitLocation` _outhit) (`local.LocalEndLocation`) :`ErrorTolerance` (`self.TraceCheckTolerance`))
                (return true))
              (else
                (return true)))
            (else
              (return true))))
        (return false)
        (else
          (bind (_outhit_2 _returnvalue_2) (`KismetSystemLibrary.LineTraceSingle` (`local.LocalPawnLocation`) (`local.LocalEndLocation`) "TraceTypeQuery1" false (`local.LocalActorsToIgnore`) (`self.TraceDebugType`)))
          (if _returnvalue_2
            (if (not (`KismetArrayLibrary.Array_Contains` (`self.TraceIgnoredClasses`) (`GameplayStatics.GetObjectClass` (`/Game/BPS_Core/Blueprints/Systems/CoreSystem/Libraries/BP_Library_CoreFunctions.GetHitActor` _outhit_2))))
              (if (== (`/Game/BPS_Core/Blueprints/Systems/CoreSystem/Libraries/BP_Library_CoreFunctions.GetHitLocation` _outhit_2) (`local.LocalEndLocation`) :`ErrorTolerance` (`self.TraceCheckTolerance`))
                _
                (else
                  (return false)))))
          (return true))))))

(fn `CompleteInteractionInput`
  (returns (Success :type Boolean))
  (bind _interactableactor (`self.InteractableActor`))
  (bind _interactableactor_2 (`self.InteractableActor`))
  (bind _interactablecomponent (`self.InteractableComponent`))
  (bind _interactiontimer (`self.InteractionTimer`))
  ;[1 1 1] Complete interaction input and start interaction with target actor for player.
  (if (`KismetSystemLibrary.K2_IsTimerActiveHandle` _interactiontimer)
    (`KismetSystemLibrary.K2_ClearAndInvalidateTimerHandle` _interactiontimer))
  (`self.OnInteractionInputCompleted` self _interactableactor (`self.InteractableComponent`))
  (bind _result (message `/Game/BPS_Core/Blueprints/Systems/InteractionSystem/Interfaces/BPI_InteractableObject.HasInteractionOnClient_BPI` _interactableactor))
  (if _result
    (bind (_success _runonserver) (`self.TryInteractWithActorOnClient` _interactableactor_2 _interactablecomponent))
    (if _runonserver
      (`self.TryInteractWithActor (Server)` _interactableactor_2 _interactablecomponent :!label _label)
      (set `self.InteractableActor` null)
      (set `self.InteractableComponent` null)
      (return true))
    (else
      (goto _label))))

(fn `FindInteractionText`
  (params (InteractionType :type Name))
  (returns (Found :type Boolean) (InteractionText :type Text))
  (bind _targetactor (`self.TargetActor`))
  ;[1 1 1] Try to get interaction text from target interactable actor.
  (`/Engine/EditorBlueprintResources/StandardMacros.IsValid` _targetactor
    (:`Is Valid`
      (bind (_success _interactiontext) (message `/Game/BPS_Core/Blueprints/Systems/InteractionSystem/Interfaces/BPI_InteractableObject.GetInteractionText_BPI` _targetactor (`self.TargetComponent`) (`self.PlayerController`) InteractionType))
      (return _success _interactiontext))
    (:`Is Not Valid`
      (return false ""))))

(fn `FindPossibleTargetActorAndComponent`
  (params (TargetActor :type "Actor Object Reference") (TargetComponent :type "PrimitiveComponent Object Reference"))
  (returns (Success :type Boolean) (PossibleActor :type "Actor Object Reference") (PossibleComponent :type "PrimitiveComponent Object Reference"))
  (locals (LocalTargetActor :type "Actor Object Reference") (LocalTargetComponent :type "PrimitiveComponent Object Reference") (LocalOverlappingComponents :type "Array of PrimitiveComponent Object Reference"))
  (bind _returnvalue (`Controller.K2_GetPawn` (`self.PlayerController`)))
  ;[1 1 1] Try to find possible interactable actor and component.
  (set `local.LocalTargetActor` TargetActor)
  (bind _output_get (set `local.LocalTargetComponent` TargetComponent))
  (`/Engine/EditorBlueprintResources/StandardMacros.IsValid` _output_get
    (:`Is Valid`
      (bind _result (message `/Game/BPS_Core/Blueprints/Systems/InteractionSystem/Interfaces/BPI_InteractableObject.HasInteractableComponents_BPI` (`local.LocalTargetActor`) :!label _label))
      (if _result
        (bind _success (message `/Game/BPS_Core/Blueprints/Systems/InteractionSystem/Interfaces/BPI_InteractableObject.CheckCanInteractWithComponent_BPI` (`local.LocalTargetActor`) (`local.LocalTargetComponent`) (`self.PlayerController`)))
        (if _success
          (bind _result_2 (`self.CheckTargetActor` (`local.LocalTargetActor`) (`local.LocalTargetComponent`) :!label _label_2))
          (if _result_2
            (return true (`local.LocalTargetActor`) (`local.LocalTargetComponent`))
            (else
              _)))
        (else
          (bind _success_2 (message `/Game/BPS_Core/Blueprints/Systems/InteractionSystem/Interfaces/BPI_InteractableObject.CheckCanInteractWithActor_BPI` (`local.LocalTargetActor`) (`self.PlayerController`)))
          (if _success_2
            (goto _label_2)
            (else
              _))))
      (return false null null))
    (:`Is Not Valid`
      (`|ExecutionSequence`
        (:`then_0`
          (bind (_success_3 _component) (message `/Game/BPS_Core/Blueprints/Systems/InteractionSystem/Interfaces/BPI_InteractableObject.GetNearestInteractableComponent_BPI` (`local.LocalTargetActor`) (`self.PlayerController`)))
          (if _success_3
            (set `local.LocalTargetComponent` _component)
            (goto _label)))
        (:`then_1`
          (`|ExecutionSequence`
            (:`then_0`
              (`/Engine/EditorBlueprintResources/StandardMacros.IsValid` _returnvalue
                (:`Is Valid`
                  (bind _output_get_2 (set `local.LocalOverlappingComponents` (`Actor.GetOverlappingComponents` _returnvalue)))
                  (for _array_element _output_get_2
                    (if (== (`local.LocalTargetActor`) (`self.GetOwner` _array_element))
                      (set `local.LocalTargetComponent` _array_element)
                      (bind _result_3 (message `/Game/BPS_Core/Blueprints/Systems/InteractionSystem/Interfaces/BPI_InteractableObject.HasInteractableComponents_BPI` (`local.LocalTargetActor`)))
                      (if _result_3
                        (bind _success_4 (message `/Game/BPS_Core/Blueprints/Systems/InteractionSystem/Interfaces/BPI_InteractableObject.CheckCanInteractWithComponent_BPI` (`local.LocalTargetActor`) (`local.LocalTargetComponent`) (`self.PlayerController`)))
                        (if _success_4
                          (bind _result_4 (`self.CheckTargetActor` (`local.LocalTargetActor`) (`local.LocalTargetComponent`) :!label _label_3))
                          (if _result_4
                            (return true (`local.LocalTargetActor`) (`local.LocalTargetComponent`))))
                        (else
                          (bind _success_5 (message `/Game/BPS_Core/Blueprints/Systems/InteractionSystem/Interfaces/BPI_InteractableObject.CheckCanInteractWithActor_BPI` (`local.LocalTargetActor`) (`self.PlayerController`)))
                          (if _success_5
                            (goto _label_3)))))))))
            (:`then_1`
              (return false null null))))))))

(fn `InitComponent`
  (returns (Success :type Boolean))
  ;[1 1 1] Try to init component.
  (bind _asplayer_controller (cast `PlayerController` (`self.GetOwner`))
    (:`then`
      (bind _output_get (set `self.PlayerController` _asplayer_controller))
      (set `self.IsLocalController` (`KismetSystemLibrary.IsValid` (`PlayerController.GetHUD` _output_get)))
      (set `self.IsInitialized` true)
      (return true))
    (:`CastFailed`
      (set `self.IsInitialized` false)
      (return true))))

(fn `SetInteractionEnabled`
  (params (IsEnabled :type Boolean))
  (returns (Success :type Boolean))
  ;[1 1 1] Turn on or turn off interaction process.
  (set `self.IsEnabled` IsEnabled)
  (return true))

(fn `SetTargetActorAndComponent`
  (params (TargetActor :type "Actor Object Reference") (TargetComponent :type "PrimitiveComponent Object Reference"))
  (returns (Success :type Boolean))
  (locals (LocalInteractionWidgetClass :type "UserWidget Class Reference") (LocalTargetActor :type "Actor Object Reference") (LocalTargetComponent :type "PrimitiveComponent Object Reference"))
  (bind _interactionwidgetactor (`self.InteractionWidgetActor`))
  (bind _targetcomponent (`self.TargetComponent`))
  (bind _highlightactors (`self.HighlightActors`))
  (bind _targetactor (`local.TargetActor`))
  (bind _highlightactors_2 (`self.HighlightActors`))
  (bind _targetcomponent_2 (`self.TargetComponent`))
  (bind _interactionwidgetactor_2 (`self.InteractionWidgetActor`))
  (bind _interactionwidgetactor_3 (`self.InteractionWidgetActor`))
  ;[1 1 1] Try to set target interactable actor and component. Updates highlight components and interaction widget.
  (bind _output_get (set `local.LocalTargetActor` TargetActor))
  (bind _output_get_2 (set `local.LocalTargetComponent` TargetComponent))
  (bind (_success _targetcomponent_3) (message `/Game/BPS_Core/Blueprints/Systems/InteractionSystem/Interfaces/BPI_InteractableObject.GetTargetInteractableComponent_BPI` _output_get _output_get_2))
  (if _success
    (set `local.LocalTargetComponent` _targetcomponent_3))
  (if (or (!= (`local.LocalTargetActor`) (`self.TargetActor`)) (!= (`local.LocalTargetComponent`) (`self.TargetComponent`)))
    (bind _output_get_3 (set `self.TargetActor` (`local.LocalTargetActor`)))
    (set `self.TargetComponent` (`local.LocalTargetComponent`))
    (`/Engine/EditorBlueprintResources/StandardMacros.IsValid` _output_get_3
      (:`Is Valid`
        (`|ExecutionSequence`
          (:`then_0`
            (bind (_success_2 _widgetclass) (message `/Game/BPS_Core/Blueprints/Systems/InteractionSystem/Interfaces/BPI_InteractableObject.GetInteractionWidgetClass_BPI` (`self.TargetActor`) (`self.TargetComponent`)))
            (if _success_2
              (set `local.LocalInteractionWidgetClass` _widgetclass)
              (else
                (set `local.LocalInteractionWidgetClass` (`self.DefaultInteractionWidgetClass`))))
            (`/Engine/EditorBlueprintResources/StandardMacros.IsValid` _interactionwidgetactor
              (:`Is Valid`
                (if (!= (`local.LocalInteractionWidgetClass`) (`/Game/BPS_Core/Blueprints/Systems/InteractionSystem/Actors/BP_InteractionWidgetActor.InteractionWidgetClass` _interactionwidgetactor))
                  (`Actor.K2_DestroyActor` (`self.InteractionWidgetActor`))
                  (bind (_success_3 _scenecomponent) (message `/Game/BPS_Core/Blueprints/Systems/InteractionSystem/Interfaces/BPI_InteractableObject.GetInteractionWidgetSocket_BPI` _targetactor _targetcomponent_2 :!label _label))
                  (bind _returnvalue (`|SpawnActorFromClass` "/Game/BPS_Core/Blueprints/Systems/InteractionSystem/Actors/BP_InteractionWidgetActor.BP_InteractionWidgetActor_C" (`KismetMathLibrary.MakeTransform` (0.0 0.0 0.0)) "Undefined" "OverrideRootScale" null (`local.LocalInteractionWidgetClass`) (0.0 0.0 30.0) _targetactor (select `bool` _success_3 :`false` _targetcomponent_2 :`true` _scenecomponent :!type "SceneComponent Object Reference") null))
                  (set `self.InteractionWidgetActor` _returnvalue)
                  (else
                    (bind _output_get_4 (set `/Game/BPS_Core/Blueprints/Systems/InteractionSystem/Actors/BP_InteractionWidgetActor.TargetActor` (`local.TargetActor`) _interactionwidgetactor_2))
                    (bind (_success_4 _scenecomponent_2) (message `/Game/BPS_Core/Blueprints/Systems/InteractionSystem/Interfaces/BPI_InteractableObject.GetInteractionWidgetSocket_BPI` _output_get_4 _targetcomponent))
                    (set `/Game/BPS_Core/Blueprints/Systems/InteractionSystem/Actors/BP_InteractionWidgetActor.TargetComponent` (select `bool` _success_4 :`false` _targetcomponent :`true` _scenecomponent_2 :!type "SceneComponent Object Reference") _interactionwidgetactor_2))))
              (:`Is Not Valid`
                (goto _label))))
          (:`then_1`
            (`|ExecutionSequence`
              (:`then_0`
                (for _array_element _highlightactors_2
                  (`/Engine/EditorBlueprintResources/StandardMacros.IsValid` _array_element
                    (:`Is Valid`
                      (`Actor.K2_DestroyActor` _array_element))))
                (`KismetArrayLibrary.Array_Clear` _highlightactors_2))
              (:`then_1`
                (`|ExecutionSequence`
                  (:`then_0`
                    (bind (_success_5 _highlightcomponents) (message `/Game/BPS_Core/Blueprints/Systems/InteractionSystem/Interfaces/BPI_InteractableObject.GetHighlightComponents_BPI` (`self.TargetActor`) (`self.TargetComponent`)))
                    (if _success_5
                      (for _array_element_2 _highlightcomponents
                        (bind _output_get_5 (set `local.LocalTargetComponent` _array_element_2))
                        (bind _returnvalue_2 (`|SpawnActorFromClass` "/Game/BPS_Core/Blueprints/Systems/InteractionSystem/Actors/BP_HighlightActor.BP_HighlightActor_C" (`KismetMathLibrary.MakeTransform` (0.0 0.0 0.0)) "Undefined" "OverrideRootScale" null _output_get_5 null :!label _label_2))
                        (`KismetArrayLibrary.Array_Add` (`self.HighlightActors`) _returnvalue_2))
                      (else
                        (goto _label_2))))
                  (:`then_1`
                    (return true))))))))
      (:`Is Not Valid`
        (`|ExecutionSequence`
          (:`then_0`
            (`/Engine/EditorBlueprintResources/StandardMacros.IsValid` _interactionwidgetactor_3
              (:`Is Valid`
                (`Actor.K2_DestroyActor` _interactionwidgetactor_3))))
          (:`then_1`
            (`|ExecutionSequence`
              (:`then_0`
                (for _array_element_3 _highlightactors
                  (`/Engine/EditorBlueprintResources/StandardMacros.IsValid` _array_element_3
                    (:`Is Valid`
                      (`Actor.K2_DestroyActor` _array_element_3))))
                (`KismetArrayLibrary.Array_Clear` _highlightactors))
              (:`then_1`
                (return true)))))))))

(fn `StartInteractionInput`
  (returns (Success :type Boolean))
  (bind _targetactor (`self.TargetActor`))
  ;[1 1 1] Try to start interaction input for player.
  (`/Engine/EditorBlueprintResources/StandardMacros.IsValid` _targetactor
    (:`Is Valid`
      (bind _output_get (set `self.InteractableActor` _targetactor))
      (bind _output_get_2 (set `self.InteractableComponent` (`self.TargetComponent`)))
      (bind (_success _interactiontime) (message `/Game/BPS_Core/Blueprints/Systems/InteractionSystem/Interfaces/BPI_InteractableObject.GetInteractionTime_BPI` _output_get _output_get_2))
      (bind _output_get_3 (set `self.InteractionTime` _interactiontime))
      (if (> _output_get_3 0.0)
        (bind _returnvalue (`KismetSystemLibrary.K2_SetTimerDelegate` (`|CreateDelegate` :!event `Bind_CompleteInteractionInput`) _output_get_3))
        (set `self.InteractionTimer` _returnvalue)
        (else
          (`self.CompleteInteractionInput`)))
      (`self.OnInteractionInputStarted` self (`self.InteractableActor`) (`self.InteractableComponent`))
      (bind _asbp_character_player_jeff (cast `/Game/BPS_Core/Blueprints/Game/Characters/Player/BP_Character_Player_Jeff` (`GameplayStatics.GetPlayerPawn` 0)))
      (`/Game/BPS_Core/Blueprints/Game/Characters/Player/BP_Character_Player_Jeff.www` _asbp_character_player_jeff (`self.TargetActor`))
      (return true))
    (:`Is Not Valid`
      (return false))))

(fn `StopInteractionInput`
  (returns (Success :type Boolean))
  (bind _interactiontimer (`self.InteractionTimer`))
  ;[1 1 1] Try to stop interaction input for player.
  (if (`KismetSystemLibrary.K2_IsTimerActiveHandle` _interactiontimer)
    (`KismetSystemLibrary.K2_ClearAndInvalidateTimerHandle` _interactiontimer)
    (`self.OnInteractionInputCanceled` self (`self.InteractableActor`) (`self.InteractableComponent`)))
  (set `self.InteractableActor` null)
  (set `self.InteractableComponent` null)
  (return true))

(fn `TryAddOverlappedActor`
  (params (Actor :type "Actor Object Reference (by ref)"))
  (returns (Success :type Boolean))
  (locals (LocalActor :type "Actor Object Reference"))
  ;[1 1 1] Try to add actor to the list of interactable actors.
  (bind _output_get (set `local.LocalActor` Actor))
  (if (`KismetSystemLibrary.DoesImplementInterface` _output_get "/Game/BPS_Core/Blueprints/Systems/InteractionSystem/Interfaces/BPI_InteractableObject.BPI_InteractableObject_C")
    (`KismetArrayLibrary.Array_AddUnique` (`self.OverlappedActors`) _output_get)
    (return true)
    (else
      (return false))))

(fn `TryInteractWithActorOnClient`
  (params (TargetActor :type "Actor Object Reference") (TargetComponent :type "PrimitiveComponent Object Reference"))
  (returns (Success :type Boolean) (RunOnServer :type Boolean))
  ;[1 1 1] Try to start interaction with actor on client.
  (bind _success (`self.CheckCanInteractWithActor` TargetActor TargetComponent))
  (if _success
    (bind (_success_2 _runonserver) (message `/Game/BPS_Core/Blueprints/Systems/InteractionSystem/Interfaces/BPI_InteractableObject.TryInteractOnClient_BPI` TargetActor TargetComponent (`self.PlayerController`)))
    (if _success_2
      (`self.OnInteractionStarted` self TargetActor TargetComponent)
      (return true _runonserver)
      (else
        _)))
  (return false false))

(fn `TryInteractWithActorOnServer`
  (params (TargetActor :type "Actor Object Reference") (TargetComponent :type "PrimitiveComponent Object Reference"))
  (returns (Success :type Boolean))
  ;[1 1 1] Try to start interaction with actor on server.
  (bind _success (`self.CheckCanInteractWithActor` TargetActor TargetComponent))
  (if _success
    (bind _success_2 (message `/Game/BPS_Core/Blueprints/Systems/InteractionSystem/Interfaces/BPI_InteractableObject.TryInteractOnServer_BPI` TargetActor TargetComponent (`self.PlayerController`)))
    (if _success_2
      (`self.OnInteractionStarted` self TargetActor TargetComponent)
      (return true)
      (else
        _)))
  (return false))

(fn `TryRemoveOverlappedActor`
  (params (Actor :type "Actor Object Reference (by ref)"))
  (returns (Success :type Boolean))
  (locals (LocalActor :type "Actor Object Reference"))
  ;[1 1 1] Try to remove actor from the list of interactable actors.
  (bind _output_get (set `local.LocalActor` Actor))
  (if (`KismetSystemLibrary.DoesImplementInterface` _output_get "/Game/BPS_Core/Blueprints/Systems/InteractionSystem/Interfaces/BPI_InteractableObject.BPI_InteractableObject_C")
    (`KismetArrayLibrary.Array_RemoveItem` (`self.OverlappedActors`) _output_get)
    (return true)
    (else
      (return false))))

(fn `UpdateTargetActor`
  (returns (Success :type Boolean))
  (locals (LocalPossibleTargetActors :type "Array of Actor Object Reference") (LocalPossibleTargetComponents :type "Array of PrimitiveComponent Object Reference"))
  (bind _localpossibletargetactors (`local.LocalPossibleTargetActors`))
  (bind _possibletargetactor (`self.PossibleTargetActor`))
  (bind _possibletargetcomponent (`self.PossibleTargetComponent`))
  ;[1 1 1] Try to update target interactable actor.
  (`/Engine/EditorBlueprintResources/StandardMacros.IsValid` (`Controller.K2_GetPawn` (`self.PlayerController`))
    (:`Is Valid`
      (if (`self.IsEnabled`)
        (bind _success (`self.UpdateTargetActorByTrace`))
        (if _success
          (`|ExecutionSequence`
            (:`then_0`
              (bind (_success_2 _possibleactor _possiblecomponent) (`self.FindPossibleTargetActorAndComponent` (`self.TraceTargetActor`) (`self.TraceTargetComponent`)))
              (if _success_2
                (set `self.PossibleTargetActor` _possibleactor)
                (set `self.PossibleTargetComponent` _possiblecomponent)
                (if (or (!= (`self.PossibleTargetActor`) (`self.PrevTargetActor`)) (!= (`self.PossibleTargetComponent`) (`self.PrevTargetComponent`))) :!label _label
                  (set `self.PrevTargetActor` _possibletargetactor)
                  (set `self.PrevTargetComponent` _possibletargetcomponent)
                  (`self.SetTargetActorAndComponent` _possibletargetactor _possibletargetcomponent))
                (return true)))
            (:`then_1`
              (if (`KismetArrayLibrary.Array_IsValidIndex` (`self.OverlappedActors`)) :!label _label_2
                (for _array_element (`self.OverlappedActors`)
                  (bind (_success_3 _possibleactor_2 _possiblecomponent_2) (`self.FindPossibleTargetActorAndComponent` _array_element))
                  (if _success_3
                    (`KismetArrayLibrary.Array_Add` (`local.LocalPossibleTargetActors`) _possibleactor_2)
                    (`KismetArrayLibrary.Array_Add` (`local.LocalPossibleTargetComponents`) _possiblecomponent_2)))
                (if (`KismetArrayLibrary.Array_IsValidIndex` _localpossibletargetactors)
                  (bind _nearestactor (`/Game/BPS_Core/Blueprints/Systems/CoreSystem/Libraries/BP_Library_CoreFunctions.FindNearestActor` (`Controller.K2_GetPawn` (`self.PlayerController`)) _localpossibletargetactors))
                  (bind _output_get (set `self.PossibleTargetActor` _nearestactor))
                  (set `self.PossibleTargetComponent` (`|GetArrayItem` (`local.LocalPossibleTargetComponents`) (`KismetArrayLibrary.Array_Find` (`local.LocalPossibleTargetActors`) _output_get)))
                  (goto _label)
                  (else
                    _)))
              (set `self.PossibleTargetActor` null :!label _label_3)
              (set `self.PossibleTargetComponent` null)
              (goto _label)))
          (else
            (goto _label_2)))
        (else
          (goto _label_3))))))

(fn `UpdateTargetActorByTrace`
  (returns (Success :type Boolean))
  (locals (LocalTargetActor :type "Actor Object Reference") (LocalTargetComponent :type "PrimitiveComponent Object Reference"))
  (bind (_worldlocation _worlddirection) (`PlayerController.DeprojectMousePositionToWorld` (`self.PlayerController`)))
  (bind _playercameramanager (`PlayerController.PlayerCameraManager` (`self.PlayerController`)))
  (bind _returnvalue (`PlayerCameraManager.GetCameraLocation` _playercameramanager))
  ;[1 1 1] Try to find target interactable actor by trace.
  (if (`self.TraceToMouse`)
    (bind (_outhit _returnvalue_2) (`KismetSystemLibrary.LineTraceSingle` _worldlocation (+ _worldlocation (* _worlddirection 10000.0)) "TraceTypeQuery1"))
    (if _returnvalue_2
      (bind (_bblockinghit _binitialoverlap _time _distance _location _impactpoint _normal _impactnormal _physmat _hitactor _hitcomponent) (`GameplayStatics.BreakHitResult` _outhit))
      (bind _output_get (set `local.LocalTargetActor` _hitactor))
      (bind _output_get_2 (set `local.LocalTargetComponent` _hitcomponent))
      (if (`KismetSystemLibrary.DoesImplementInterface` _output_get "/Game/BPS_Core/Blueprints/Systems/InteractionSystem/Interfaces/BPI_InteractableObject.BPI_InteractableObject_C")
        (set `self.TraceTargetActor` _output_get)
        (set `self.TraceTargetComponent` _output_get_2)
        (return true)
        (else
          _)))
    (else
      (bind (_outhit_2 _returnvalue_3) (`KismetSystemLibrary.LineTraceSingle` _returnvalue (+ _returnvalue (* (`KismetMathLibrary.GetForwardVector` (`PlayerCameraManager.GetCameraRotation` _playercameramanager)) 10000.0)) "TraceTypeQuery1" false (`|MakeArray` (`Controller.K2_GetPawn` (`self.PlayerController`)) :!type "Actor Object Reference")))
      (if _returnvalue_3
        (bind (_bblockinghit_2 _binitialoverlap_2 _time_2 _distance_2 _location_2 _impactpoint_2 _normal_2 _impactnormal_2 _physmat_2 _hitactor_2 _hitcomponent_2) (`GameplayStatics.BreakHitResult` _outhit_2))
        (bind _output_get_3 (set `local.LocalTargetActor` _hitactor_2))
        (bind _output_get_4 (set `local.LocalTargetComponent` _hitcomponent_2))
        (if (`KismetSystemLibrary.DoesImplementInterface` _output_get_3 "/Game/BPS_Core/Blueprints/Systems/InteractionSystem/Interfaces/BPI_InteractableObject.BPI_InteractableObject_C")
          (set `self.TraceTargetActor` _output_get_3)
          (set `self.TraceTargetComponent` _output_get_4)
          (return true)
          (else
            _)))))
  (set `self.TraceTargetActor` null)
  (set `self.TraceTargetComponent` null)
  (return false))