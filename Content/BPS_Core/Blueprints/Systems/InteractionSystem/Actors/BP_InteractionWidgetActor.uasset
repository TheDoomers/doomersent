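; BP_InteractionWidgetActor is an interaction system actor that displays an interaction widget at the position of a target.
; On BeginPlay it applies an offset to its widget component, creates the widget from InteractionWidgetClass and assigns it to that component.
; Each Tick it teleports to the target component's world location, falling back to the target actor's location when no component is valid, provided the target actor is valid.
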(event `self.ReceiveBeginPlay`
  ;[1 1 1] Begin play. Create interaction widget and set relative offset for the widget component.
  (`SceneComponent.K2_SetRelativeLocation` (`self.WidgetComponent`) (`self.WidgetOffset`) false true)
  (bind _returnvalue (`|CreateWidget` (`self.InteractionWidgetClass`)))
  (set `self.InteractionWidget` _returnvalue)
  (`WidgetComponent.SetWidget` (`self.WidgetComponent`) _returnvalue))

(event `self.ReceiveTick`
  (params (DeltaSeconds :type "Float (single-precision)"))
  (bind _targetcomponent (`self.TargetComponent`))
  (bind _targetactor (`self.TargetActor`))
  ;[1 1 1] Update interaction widget location.
  (`/Engine/EditorBlueprintResources/StandardMacros.IsValid` _targetactor
    (:`Is Valid`
      (`/Engine/EditorBlueprintResources/StandardMacros.IsValid` _targetcomponent
        (:`Is Valid`
          (`self.K2_SetActorLocation` (`SceneComponent.K2_GetComponentLocation` _targetcomponent) false true))
        (:`Is Not Valid`
          (`self.K2_SetActorLocation` (`self.K2_GetActorLocation` _targetactor) false true))))))

(fn `UserConstructionScript`)