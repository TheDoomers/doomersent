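; Highlight actor for the interaction system that draws an outline over a target component by mirroring its mesh.
; On BeginPlay it snaps to the target component, then copies its static or skeletal mesh and transform, overriding every material slot with an outline material.
; Skeletal copies follow the target's animation through a leader pose component.
; Tick re-copies the mesh whenever the target's mesh asset changes.
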(event `self.ReceiveBeginPlay`
  ;[1 1 1] Begin play. Init highlight actor.
  (`self.K2_AttachToComponent` (`self.TargetComponent`) "None" "SnapToTarget" "SnapToTarget" "SnapToTarget")
  (`self.UpdateMeshes`))

(event `UpdateMeshes`
  ;[1 1 1] Update hightlight actor meshes depending on target component.
  (`|ExecutionSequence`
    (:`then_0`
      (bind _asstatic_mesh_component (cast `StaticMeshComponent` (`self.TargetComponent`)))
      (`self.UpdateStaticMesh` _asstatic_mesh_component))
    (:`then_1`
      (bind _asskeletal_mesh_component (cast `SkeletalMeshComponent` (`self.TargetComponent`)))
      (`self.UpdateSkeletalMesh` _asskeletal_mesh_component))))

(event `self.ReceiveTick`
  (params (DeltaSeconds :type "Float (single-precision)"))
  (bind _targetskeletalmeshcomponent (`self.TargetSkeletalMeshComponent`))
  (bind _targetstaticmeshcomponent (`self.TargetStaticMeshComponent`))
  ;[1 1 1] Event tick. Check and update meshes.
  (`|ExecutionSequence`
    (:`then_0`
      (`/Engine/EditorBlueprintResources/StandardMacros.IsValid` _targetstaticmeshcomponent
        (:`Is Valid`
          (if (!= (`StaticMeshComponent.StaticMesh` _targetstaticmeshcomponent) (`StaticMeshComponent.StaticMesh` (`self.StaticMesh`)))
            (`self.UpdateStaticMesh` _targetstaticmeshcomponent)))))
    (:`then_1`
      (`/Engine/EditorBlueprintResources/StandardMacros.IsValid` _targetskeletalmeshcomponent
        (:`Is Valid`
          (if (!= (`SkeletalMeshComponent.SkeletalMeshAsset` _targetskeletalmeshcomponent) (`SkeletalMeshComponent.SkeletalMeshAsset` (`self.SkeletalMesh`)))
            (`self.UpdateSkeletalMesh` _targetskeletalmeshcomponent)))))))

(fn `UpdateSkeletalMesh`
  (params (Component :type "SkeletalMeshComponent Object Reference"))
  (locals (LocalMaterials :type "Array of MaterialInterface Object Reference"))
  (bind _skeletalmesh (`self.SkeletalMesh`))
  ;[1 1 1] Update skeletal mesh depending on target component.
  (set `self.TargetSkeletalMeshComponent` Component)
  (`SkinnedMeshComponent.SetSkinnedAssetAndUpdate` _skeletalmesh (`SkeletalMeshComponent.SkeletalMeshAsset` Component) true)
  (`SkinnedMeshComponent.SetLeaderPoseComponent` _skeletalmesh Component true false)
  (`SceneComponent.K2_SetWorldTransform` _skeletalmesh (`SceneComponent.K2_GetComponentToWorld` Component) false true)
  (bind _output_get (set `local.LocalMaterials` (`MeshComponent.GetMaterials` (`self.SkeletalMesh`))))
  (for (_ _array_index) _output_get
    (`PrimitiveComponent.SetMaterial` (`self.SkeletalMesh`) _array_index "/Game/BPS_Core/Materials/Instances/Generic/MI_Outline.MI_Outline")))

(fn `UpdateStaticMesh`
  (params (Component :type "StaticMeshComponent Object Reference"))
  (locals (LocalMaterials :type "Array of MaterialInterface Object Reference"))
  (bind _staticmesh (`self.StaticMesh`))
  ;[1 1 1] Update static mesh depending on target component.
  (set `self.TargetStaticMeshComponent` Component)
  (`StaticMeshComponent.SetStaticMesh` _staticmesh (`StaticMeshComponent.StaticMesh` Component))
  (`SceneComponent.K2_SetWorldTransform` _staticmesh (`SceneComponent.K2_GetComponentToWorld` Component) false true)
  (bind _output_get (set `local.LocalMaterials` (`MeshComponent.GetMaterials` (`self.StaticMesh`))))
  (for (_ _array_index) _output_get
    (`PrimitiveComponent.SetMaterial` (`self.StaticMesh`) _array_index "/Game/BPS_Core/Materials/Instances/Generic/MI_Outline.MI_Outline")))

(fn `UserConstructionScript`)