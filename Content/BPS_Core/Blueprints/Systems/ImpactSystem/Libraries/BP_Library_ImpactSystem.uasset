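; Blueprint function library that serves as the global entry point to the impact effects system.
; It looks up the BP_AC_ImpactManager component on the Game State and prints a message if the component is missing.
; Wrapper functions forward a hit result with either preset data or a preset handle to that manager, including a replicated by-handle variant.
; Each wrapper returns the manager's result, or false when no manager is found.
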(fn `FindImpactManager`
  (returns (Found :type Boolean) (ImpactManager :type "/Game/BPS_Core/Blueprints/Systems/ImpactSystem/Components/BP_AC_ImpactManager Object Reference"))
  (locals (LocalImpactManager :type "/Game/BPS_Core/Blueprints/Systems/ImpactSystem/Components/BP_AC_ImpactManager Object Reference"))
  (bind _returnvalue (`GameplayStatics.GetGameState` null))
  ;[1 1 1] Try to find impact manager component.
  (`/Engine/EditorBlueprintResources/StandardMacros.IsValid` _returnvalue
    (:`Is Valid`
      (bind _output_get (set `local.LocalImpactManager` (`Actor.GetComponentByClass` _returnvalue "/Game/BPS_Core/Blueprints/Systems/ImpactSystem/Components/BP_AC_ImpactManager.BP_AC_ImpactManager_C")))
      (`/Engine/EditorBlueprintResources/StandardMacros.IsValid` _output_get
        (:`Is Valid`
          (return true _output_get))
        (:`Is Not Valid`
          (`KismetSystemLibrary.PrintText` null "Impact manager component is not found! \nImpact manager component should be a part of the game state class." true true (struct :`R` 1.0 :`A` 1.0) 10.0)
          (return false null))))))

(fn `PlayImpactEffects`
  (params (ImpactPresetData :type "/Game/BPS_Core/Blueprints/Systems/ImpactSystem/Structures/STR_ImpactPresetData Structure") (HitResult :type "HitResult Structure"))
  (returns (Success :type Boolean))
  ;[1 1 1] Try to play impact effects.
  (bind (_found _impactmanager) (`self.FindImpactManager` null))
  (if _found
    (bind _success (`/Game/BPS_Core/Blueprints/Systems/ImpactSystem/Components/BP_AC_ImpactManager.PlayImpactEffects` _impactmanager ImpactPresetData HitResult))
    (return _success)
    (else
      (return false))))

(fn `PlayImpactEffectsByHandle`
  (params (ImpactPresetHandle :type "DataTableRowHandle Structure") (HitResult :type "HitResult Structure"))
  (returns (Success :type Boolean))
  ;[1 1 1] Try to play impact effects by specific preset handle.
  (bind (_found _impactmanager) (`self.FindImpactManager` null))
  (if _found
    (bind _success (`/Game/BPS_Core/Blueprints/Systems/ImpactSystem/Components/BP_AC_ImpactManager.PlayImpactEffectsByHandle` _impactmanager ImpactPresetHandle HitResult))
    (return _success)
    (else
      (return false))))

(fn `PlayImpactEffectsByHandleReplicated`
  (params (ImpactPresetHandle :type "DataTableRowHandle Structure") (HitResult :type "HitResult Structure"))
  (returns (Success :type Boolean))
  ;[1 1 1] Try to play replicated impact effect by specific impact preset handle.
  (bind (_found _impactmanager) (`self.FindImpactManager` null))
  (if _found
    (bind _success (`/Game/BPS_Core/Blueprints/Systems/ImpactSystem/Components/BP_AC_ImpactManager.PlayImpactEffectsByHandleReplicated` _impactmanager ImpactPresetHandle HitResult))
    (return _success)
    (else
      (return false))))