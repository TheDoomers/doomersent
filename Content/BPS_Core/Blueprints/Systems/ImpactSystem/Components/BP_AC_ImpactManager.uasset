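; Game state component that plays surface-dependent impact effects at hit locations.
; A data table handle selects a preset, then the hit's surface type resolves through mapped names to a surface row, with "Default" and array-search fallbacks.
; The resolved data drives sound, Cascade or Niagara particles and fading normal-aligned decals, gated by a cosmetic-event check.
; A server-only entry point multicasts handle and hit result to replicate effects.
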(event `self.ReceiveBeginPlay`
  ;[1 1 1] Begin play. Init component.
  (`self.TryInitComponent`))

(event `PlayImpactEffectsByHandle (Multicast)`
  (params (ImpactPresetHandle :type "DataTableRowHandle Structure") (HitResult :type "HitResult Structure"))
  ;[1 1 1] Network events.
  (`self.PlayImpactEffectsByHandle` ImpactPresetHandle HitResult))

(fn `FindImpactSurfaceData`
  (params (ImpactPresetData :type "/Game/BPS_Core/Blueprints/Systems/ImpactSystem/Structures/STR_ImpactPresetData Structure") (SurfaceType :type "EPhysicalSurface Enum" :default "SurfaceType_Default"))
  (returns (Success :type Boolean) (ImpactSurfaceData :type "/Game/BPS_Core/Blueprints/Systems/ImpactSystem/Structures/STR_ImpactSurfaceData Structure"))
  (locals (LocalImpactPresetData :type "/Game/BPS_Core/Blueprints/Systems/ImpactSystem/Structures/STR_ImpactPresetData Structure") (LocalSurfaceType :type "EPhysicalSurface Enum" :default "SurfaceType_Default"))
  (bind ((`ImpactSurfaceDataMapped_14_3571E09442E4E10E963DD59FA69994EC` _impactsurfacedatamapped)) (break `/Game/BPS_Core/Blueprints/Systems/ImpactSystem/Structures/STR_ImpactPresetData` (`local.LocalImpactPresetData`)))
  (bind (_value _returnvalue) (`BlueprintMapLibrary.Map_Find` _impactsurfacedatamapped "Default"))
  (bind (_datatable _rowname) (break `DataTableRowHandle` _value))
  ;[1 1 1] Try to find impact surface data.
  (set `local.LocalImpactPresetData` ImpactPresetData)
  (set `local.LocalSurfaceType` SurfaceType)
  (`|ExecutionSequence`
    (:`then_0`
      (bind (_found _surfacename) (`self.FindMappedSurfaceName` (`local.LocalSurfaceType`)))
      (if _found
        (bind (_value_2 _returnvalue_2) (`BlueprintMapLibrary.Map_Find` _impactsurfacedatamapped _surfacename))
        (if _returnvalue_2
          (bind (_datatable_2 _rowname_2) (break `DataTableRowHandle` _value_2))
          (`/Engine/EditorBlueprintResources/StandardMacros.IsValid` _datatable_2
            (:`Is Valid`
              (bind _returnvalue_3 (`|GetDataTableRow` _datatable_2 _rowname_2)
                (:`then`
                  (return true _returnvalue_3)))))
          (else
            _)))
      (if _returnvalue
        (`/Engine/EditorBlueprintResources/StandardMacros.IsValid` _datatable
          (:`Is Valid`
            (bind _returnvalue_4 (`|GetDataTableRow` _datatable _rowname)
              (:`then`
                (return true _returnvalue_4)))))))
    (:`then_1`
      (`|ExecutionSequence`
        (:`then_0`
          (for _array_element (`.ImpactSurfaceData_10_3B80DA2E46B3078C3E7B1AA04C405031` (break `/Game/BPS_Core/Blueprints/Systems/ImpactSystem/Structures/STR_ImpactPresetData` (`local.LocalImpactPresetData`)))
            (if (`|EnumEquality` (`.SurfaceType_2_20AA43E7487BDA334AE2F986F6397EB9` (break `/Game/BPS_Core/Blueprints/Systems/ImpactSystem/Structures/STR_ImpactSurfaceData` _array_element)) (`local.LocalSurfaceType`))
              (return true _array_element))))
        (:`then_1`
          (return false))))))

(fn `FindMappedSurfaceName`
  (params (SurfaceType :type "EPhysicalSurface Enum" :default "SurfaceType_Default"))
  (returns (Found :type Boolean) (SurfaceName :type Name))
  (bind _mappedsurfacetypes (`self.MappedSurfaceTypes`))
  ;[1 1 1] Try to find mapped surface name.
  (bind _values (`BlueprintMapLibrary.Map_Values` _mappedsurfacetypes))
  (bind _keys (`BlueprintMapLibrary.Map_Keys` _mappedsurfacetypes))
  (for (_array_element _array_index) _values
    (if (`|EnumEquality` _array_element SurfaceType)
      (return true (`|GetArrayItem` _keys _array_index))))
  (return false "None"))

(fn `InitComponent`
  (returns (Success :type Boolean))
  ;[1 1 1] Try to init component.
  (cast `GameStateBase` (`self.GetOwner`)
    (:`then`
      (set `self.IsInitialized` true)
      (return true))
    (:`CastFailed`
      (`KismetSystemLibrary.PrintText` "Impact manager component should be a part of the game state class!" true true (struct :`R` 1.0 :`A` 1.0) 10.0)
      (return false))))

(fn `PlayImpactEffects`
  (params (ImpactPresetData :type "/Game/BPS_Core/Blueprints/Systems/ImpactSystem/Structures/STR_ImpactPresetData Structure") (HitResult :type "HitResult Structure"))
  (returns (Success :type Boolean))
  ;[1 1 1] Try to play impact effects using specific impact preset data.
  (bind (_success _impactsurfacedata) (`self.FindImpactSurfaceData` ImpactPresetData (`GameplayStatics.GetSurfaceType` HitResult)))
  (if _success
    (bind _success_2 (`self.PlayImpactSurfaceEffects` _impactsurfacedata HitResult))
    (return _success_2)
    (else
      (return false))))

(fn `PlayImpactEffectsByHandle`
  (params (ImpactPresetHandle :type "DataTableRowHandle Structure") (HitResult :type "HitResult Structure"))
  (returns (Success :type Boolean))
  (bind (_datatable _rowname) (break `DataTableRowHandle` ImpactPresetHandle))
  ;[1 1 1] Try to play impact effects by impact preset handle.
  (`/Engine/EditorBlueprintResources/StandardMacros.IsValid` _datatable
    (:`Is Valid`
      (bind _returnvalue (`|GetDataTableRow` _datatable _rowname)
        (:`then`
          (bind _success (`self.PlayImpactEffects` _returnvalue HitResult))
          (return _success))
        (:`RowNotFound`
          _)))
    (:`Is Not Valid`
      _))
  (return false))

(fn `PlayImpactEffectsByHandleReplicated`
  (params (ImpactPresetHandle :type "DataTableRowHandle Structure") (HitResult :type "HitResult Structure"))
  (returns (Success :type Boolean))
  ;[1 1 1] Try to play replicated impact effects by impact preset handle.
  (if (`KismetSystemLibrary.IsServer`)
    (`self.PlayImpactEffectsByHandle (Multicast)` ImpactPresetHandle HitResult)
    (return true)
    (else
      (return false))))

(fn `PlayImpactSurfaceEffects`
  (params (ImpactSurfaceData :type "/Game/BPS_Core/Blueprints/Systems/ImpactSystem/Structures/STR_ImpactSurfaceData Structure") (HitResult :type "HitResult Structure"))
  (returns (Success :type Boolean))
  (locals (LocalSurfaceData :type "/Game/BPS_Core/Blueprints/Systems/ImpactSystem/Structures/STR_ImpactSurfaceData Structure") (LocalHitResult :type "HitResult Structure"))
  (bind _localhitresult (`local.LocalHitResult`))
  (bind (_decalmaterial _decalsize _decallifespan _fadescreensize _fadedelaytime _fadeduration) (break `/Game/BPS_Core/Blueprints/Systems/ImpactSystem/Structures/STR_ImpactDecalData` (`.DecalData_11_183731AB4D352373A771B7B82415150A` (break `/Game/BPS_Core/Blueprints/Systems/ImpactSystem/Structures/STR_ImpactSurfaceData` (`local.LocalSurfaceData`)))))
  (bind ((`NiagaraSystem_8_9055261E4380A70AFC703BBFB4D44AF2` _niagarasystem)) (break `/Game/BPS_Core/Blueprints/Systems/ImpactSystem/Structures/STR_ImpactEffectData` (`.EffectData_10_D34932BC4DD8CF2800A19B8BB9A9B099` (break `/Game/BPS_Core/Blueprints/Systems/ImpactSystem/Structures/STR_ImpactSurfaceData` (`local.LocalSurfaceData`)))))
  (bind (_sound _volumemultiplier) (break `/Game/BPS_Core/Blueprints/Systems/ImpactSystem/Structures/STR_ImpactSoundData` (`.SoundData_9_44532693416FA59737DC639690C723D1` (break `/Game/BPS_Core/Blueprints/Systems/ImpactSystem/Structures/STR_ImpactSurfaceData` (`local.LocalSurfaceData`)))))
  (bind ((`ParticleSystem_5_A0E58EEA470598DA51BBDB85763FA467` _particlesystem)) (break `/Game/BPS_Core/Blueprints/Systems/ImpactSystem/Structures/STR_ImpactEffectData` (`.EffectData_10_D34932BC4DD8CF2800A19B8BB9A9B099` (break `/Game/BPS_Core/Blueprints/Systems/ImpactSystem/Structures/STR_ImpactSurfaceData` (`local.LocalSurfaceData`)))))
  ;[1 1 1] Try to play impact surface effects.
  (set `local.LocalSurfaceData` ImpactSurfaceData)
  (set `local.LocalHitResult` HitResult)
  (`/Engine/EditorBlueprintResources/StandardMacros.Can Execute Cosmetic Events` ; #update 1.1
    (:`True`
      (`|ExecutionSequence`
        (:`then_0`
          (`/Engine/EditorBlueprintResources/StandardMacros.IsValid` _sound
            (:`Is Valid`
              (`GameplayStatics.PlaySoundAtLocation` _sound (`/Game/BPS_Core/Blueprints/Systems/CoreSystem/Libraries/BP_Library_CoreFunctions.GetHitLocation` (`local.LocalHitResult`)) (struct) _volumemultiplier 1.0 0.0 null null null null))))
        (:`then_1`
          (`|ExecutionSequence`
            (:`then_0`
              (`/Engine/EditorBlueprintResources/StandardMacros.IsValid` _particlesystem
                (:`Is Valid`
                  (`GameplayStatics.SpawnEmitterAtLocation` _particlesystem (`/Game/BPS_Core/Blueprints/Systems/CoreSystem/Libraries/BP_Library_CoreFunctions.GetHitLocation` (`local.LocalHitResult`))))))
            (:`then_1`
              (`|ExecutionSequence`
                (:`then_0`
                  (`/Engine/EditorBlueprintResources/StandardMacros.IsValid` _niagarasystem
                    (:`Is Valid`
                      (`NiagaraFunctionLibrary.SpawnSystemAtLocation` _niagarasystem (`/Game/BPS_Core/Blueprints/Systems/CoreSystem/Libraries/BP_Library_CoreFunctions.GetHitLocation` (`local.LocalHitResult`))))))
                (:`then_1`
                  (`|ExecutionSequence`
                    (:`then_0`
                      (`/Engine/EditorBlueprintResources/StandardMacros.IsValid` _decalmaterial
                        (:`Is Valid`
                          (bind _returnvalue (`GameplayStatics.SpawnDecalAtLocation` _decalmaterial _decalsize (`/Game/BPS_Core/Blueprints/Systems/CoreSystem/Libraries/BP_Library_CoreFunctions.GetHitLocation` _localhitresult) (`KismetMathLibrary.MakeRotFromX` (`/Game/BPS_Core/Blueprints/Systems/CoreSystem/Libraries/BP_Library_CoreFunctions.GetHitNormal` _localhitresult)) _decallifespan))
                          (`DecalComponent.SetFadeScreenSize` _returnvalue _fadescreensize)
                          (`DecalComponent.SetFadeOut` _returnvalue _fadedelaytime _fadeduration true))))
                    (:`then_1`
                      (return false))))))))))))

(fn `TryInitComponent`
  (returns (Success :type Boolean))
  ;[1 1 1] Try to init component.
  (if (not (`self.IsInitialized`))
    (bind _success (`self.InitComponent`))
    (set `self.IsInitialized` _success)
    (return true)
    (else
      (return true))))