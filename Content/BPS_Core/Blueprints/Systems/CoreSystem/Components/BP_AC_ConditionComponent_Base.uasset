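; Base condition component of the BPS core system, providing overridable functions for checking gameplay conditions and producing result text.
; The default check ignores the supplied PlayerController, sets the result to true and returns it.
; The text update reads the "ResultTextFormat" entry from the condition settings' text variables, falling back to empty text.
; Getters expose the stored result and text, while child Blueprints can override the check and text update.
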(fn `CheckGameplayConditions`
  (params (PlayerController :type "PlayerController Object Reference"))
  (returns (Success :type Boolean))
  ;[1 1 1] Returns true if condition completes. Can be overridden in child class.
  (bind _output_get (set `self.ConditionResult` true))
  (return _output_get))

(fn `GetConditionResult`
  (returns (Result :type Boolean))
  ;[1 1 1] Returns condition result.
  (return (`self.ConditionResult`)))

(fn `GetConditionResultText`
  (returns (ResultText :type Text))
  ;[1 1 1] Returns condition result text.
  (return (`self.ConditionResultText`)))

(fn `UpdateConditionResultText`
  (returns (Success :type Boolean))
  (bind (_value _returnvalue) (`BlueprintMapLibrary.Map_Find` (`.TextVariables_38_F5CAB99445AD7560253D5891C6F439B3` (break `/Game/BPS_Core/Blueprints/Systems/CoreSystem/Structures/STR_ConditionSettings` (`self.ConditionSettings`))) "ResultTextFormat"))
  ;[1 1 1] Update condition result text. Can be overridden in child blueprints.
  (if _returnvalue
    (set `self.ConditionResultText` _value)
    (return true)
    (else
      (set `self.ConditionResultText` "")
      (return true))))