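; Actor component that runs global and per-player gameplay events and spawns replicated sounds and floating text.
; On BeginPlay it spawns a helper actor, which executes events that have a component class.
; Successful events, and classless ones with only a name or tag, are broadcast through played callbacks.
; Sound and floating text replicate via reliable or unreliable multicasts, with floating text spawned as timed actors.
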(event `self.ReceiveBeginPlay`
  ;[1 1 1] Begin play. Init component.
  (`self.InitComponent`))

(event `TrySpawnSoundAtLocation (Multicast)`
  (params (Sound :type "SoundBase Object Reference") (Location :type "Vector Structure"))
  ;[1 1 1] Network events.
  (`GameplayStatics.SpawnSoundAtLocation` Sound Location (struct) 1.0 1.0 0.0 null null))

(event `TrySpawnFloatingText (Multicast)`
  (params (FloatingTextClass :type "/Game/BPS_Core/Blueprints/Systems/CoreSystem/Actors/BP_FloatingText_Base Class Reference") (SpawnLocation :type "Vector Structure") (FloatingTextWidget :type "UserWidget Class Reference") (TextValue :type Text) (TextColor :type "LinearColor Structure" :default (struct :`R` 1.0 :`A` 1.0)) (TextFont :type "SlateFontInfo Structure") (LifeSpan :type "Float (double-precision)"))
  ;[1 1 1] Network events.
  (`self.TrySpawnFloatingText` FloatingTextClass SpawnLocation FloatingTextWidget TextValue TextColor TextFont LifeSpan))

(event `TrySpawnSoundAtLocationReliable (Multicast)`
  (params (Sound :type "SoundBase Object Reference") (Location :type "Vector Structure"))
  ;[1 1 1] Network events.
  (`GameplayStatics.SpawnSoundAtLocation` Sound Location (struct) 1.0 1.0 0.0 null null))

(event `TrySpawnFloatingTextReliable (Multicast)`
  (params (FloatingTextClass :type "/Game/BPS_Core/Blueprints/Systems/CoreSystem/Actors/BP_FloatingText_Base Class Reference") (SpawnLocation :type "Vector Structure") (FloatingTextWidget :type "UserWidget Class Reference") (TextValue :type Text) (TextColor :type "LinearColor Structure" :default (struct :`R` 1.0 :`A` 1.0)) (TextFont :type "SlateFontInfo Structure") (LifeSpan :type "Float (double-precision)"))
  ;[1 1 1] Network events.
  (`self.TrySpawnFloatingText` FloatingTextClass SpawnLocation FloatingTextWidget TextValue TextColor TextFont LifeSpan))

(fn `InitComponent`
  (returns (Success :type Boolean))
  ;[1 1 1] Try init component and spawn gameplay events helper actor.
  (bind _returnvalue (`|SpawnActorFromClass` "/Game/BPS_Core/Blueprints/Systems/CoreSystem/Actors/BP_GameplayEventsHelper.BP_GameplayEventsHelper_C" (`KismetMathLibrary.MakeTransform` (0.0 0.0 0.0)) "Undefined" "OverrideRootScale" null null))
  (bind _output_get (set `self.GameplayEventsHelper` _returnvalue))
  (`/Engine/EditorBlueprintResources/StandardMacros.IsValid` _output_get
    (:`Is Valid`
      (return true))
    (:`Is Not Valid`
      (return false))))

(fn `TryRunGameplayEvent`
  (params (EventSettings :type "/Game/BPS_Core/Blueprints/Systems/CoreSystem/Structures/STR_EventSettings Structure"))
  (returns (Success :type Boolean))
  (locals (LocalEventSettings :type "/Game/BPS_Core/Blueprints/Systems/CoreSystem/Structures/STR_EventSettings Structure"))
  (bind ((`EventComponentClass_40_C8DB90A84E042C3A26CF219082CD49CA` _eventcomponentclass) (`EventName_49_9592CD1249A65435D0184491FF798BBB` _eventname) (`EventTag_52_D9F5F48E49BB777EC6CBC1AC46C09581` _eventtag)) (break `/Game/BPS_Core/Blueprints/Systems/CoreSystem/Structures/STR_EventSettings` EventSettings))
  ;[1 1 1] Try to run gameplay event.
  (set `local.LocalEventSettings` EventSettings)
  (if (`KismetSystemLibrary.IsValidClass` _eventcomponentclass)
    (bind _gameplayeventshelper (`self.GameplayEventsHelper`)
      (:`then`
        (bind _success (`/Game/BPS_Core/Blueprints/Systems/CoreSystem/Actors/BP_GameplayEventsHelper.TryRunGameplayEvent` _gameplayeventshelper (`local.LocalEventSettings`)))
        (if _success
          (`self.OnGameplayEventPlayed` self (`local.LocalEventSettings`) :!label _label)
          (return true)
          (else
            (return false))))
      (:`else`
        _))
    (elif (or (!= _eventname "None") (`BlueprintGameplayTagLibrary.IsGameplayTagValid` _eventtag))
      (goto _label)
      (else
        _)))
  (return false))

(fn `TryRunPlayerGameplayEvent`
  (params (PlayerController :type "PlayerController Object Reference") (EventSettings :type "/Game/BPS_Core/Blueprints/Systems/CoreSystem/Structures/STR_EventSettings Structure"))
  (returns (Success :type Boolean))
  (locals (LocalPlayerController :type "PlayerController Object Reference") (LocalEventSettings :type "/Game/BPS_Core/Blueprints/Systems/CoreSystem/Structures/STR_EventSettings Structure"))
  (bind ((`EventComponentClass_40_C8DB90A84E042C3A26CF219082CD49CA` _eventcomponentclass) (`EventName_49_9592CD1249A65435D0184491FF798BBB` _eventname) (`EventTag_52_D9F5F48E49BB777EC6CBC1AC46C09581` _eventtag)) (break `/Game/BPS_Core/Blueprints/Systems/CoreSystem/Structures/STR_EventSettings` EventSettings))
  ;[1 1 1] Try to run player gameplay event.
  (set `local.LocalPlayerController` PlayerController)
  (set `local.LocalEventSettings` EventSettings)
  (if (`KismetSystemLibrary.IsValidClass` _eventcomponentclass)
    (bind _gameplayeventshelper (`self.GameplayEventsHelper`)
      (:`then`
        (bind _success (`/Game/BPS_Core/Blueprints/Systems/CoreSystem/Actors/BP_GameplayEventsHelper.TryRunPlayerGameplayEvent` _gameplayeventshelper (`local.LocalPlayerController`) (`local.LocalEventSettings`)))
        (if _success
          (`self.OnPlayerGameplayEventPlayed` self (`local.LocalPlayerController`) (`local.LocalEventSettings`) :!label _label)
          (return true)
          (else
            (return false))))
      (:`else`
        _))
    (elif (or (!= _eventname "None") (`BlueprintGameplayTagLibrary.IsGameplayTagValid` _eventtag))
      (goto _label)
      (else
        _)))
  (return false))

(fn `TrySpawnFloatingText`
  (params (FloatingTextClass :type "/Game/BPS_Core/Blueprints/Systems/CoreSystem/Actors/BP_FloatingText_Base Class Reference") (SpawnLocation :type "Vector Structure") (FloatingTextWidget :type "UserWidget Class Reference") (TextValue :type Text) (TextColor :type "LinearColor Structure" :default (struct :`R` 1.0 :`A` 1.0)) (TextFont :type "SlateFontInfo Structure") (LifeSpan :type "Float (double-precision)"))
  (returns (Success :type Boolean) (FloatingText :type "/Game/BPS_Core/Blueprints/Systems/CoreSystem/Actors/BP_FloatingText_Base Object Reference"))
  ;[1 1 1] Try to spawn floating text actor at location.
  (bind _returnvalue (`|SpawnActorFromClass` FloatingTextClass (`KismetMathLibrary.MakeTransform` SpawnLocation) "Undefined" "SelectDefaultAtRuntime" null FloatingTextWidget TextValue TextColor TextFont null))
  (`Actor.SetLifeSpan` _returnvalue LifeSpan)
  (`/Engine/EditorBlueprintResources/StandardMacros.IsValid` _returnvalue
    (:`Is Valid`
      (return true _returnvalue))
    (:`Is Not Valid`
      (return false null))))

(fn `TrySpawnFloatingTextReplicated`
  (params (FloatingTextClass :type "/Game/BPS_Core/Blueprints/Systems/CoreSystem/Actors/BP_FloatingText_Base Class Reference") (SpawnLocation :type "Vector Structure") (FloatingTextWidget :type "UserWidget Class Reference") (TextValue :type Text) (TextColor :type "LinearColor Structure" :default (struct :`R` 1.0 :`A` 1.0)) (TextFont :type "SlateFontInfo Structure") (LifeSpan :type "Float (double-precision)") (Reliable :type Boolean))
  (returns (Success :type Boolean))
  ;[1 1 1] Try to spawn replicated floating text at location.
  (if Reliable
    (`self.TrySpawnFloatingTextReliable (Multicast)` FloatingTextClass SpawnLocation FloatingTextWidget TextValue TextColor TextFont LifeSpan)
    (return true)
    (else
      (`self.TrySpawnFloatingText (Multicast)` FloatingTextClass SpawnLocation FloatingTextWidget TextValue TextColor TextFont LifeSpan)
      (return true))))

(fn `TrySpawnSoundAtLocationReplicated`
  (params (Sound :type "SoundBase Object Reference") (Location :type "Vector Structure") (Reliable :type Boolean))
  (returns (Success :type Boolean))
  ;[1 1 1] Try to spawn replicated sound at location.
  (if Reliable
    (`self.TrySpawnSoundAtLocationReliable (Multicast)` Sound Location)
    (return true)
    (else
      (`self.TrySpawnSoundAtLocation (Multicast)` Sound Location)
      (return true))))