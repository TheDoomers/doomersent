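; Actor component that stores an owner's customization as a map of named integers and signals when it changes.
; It can initialize on BeginPlay by applying the initial map through TryInitComponent, though InitComponent returns false, so the initialized flag is reset afterwards.
; Setters replace the whole map or write one entry, then fire the customization-changed event.
; Getters look up a value by name or return keys and values as arrays.
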(event `self.ReceiveBeginPlay`
  ;[1 1 1] Begin play. Try init component.
  (if (`self.InitOnBeginPlay`)
    (`self.TryInitComponent`)))

(fn `FindCustomizedInteger`
  (params (IntegeraName :type Name))
  (returns (Found :type Boolean) (Value :type Integer))
  (bind (_value _returnvalue) (`BlueprintMapLibrary.Map_Find` (`self.CustomizedIntegers`) IntegeraName))
  ;[1 1 1] Try to find customized integer value.
  (return _returnvalue _value))

(fn `GetCustomizedIntegerArrays`
  (returns (Keys :type "Array of Name") (Values :type "Array of Integer"))
  (bind _customizedintegers (`self.CustomizedIntegers`))
  ;[1 1 1] Returns customized integer arrays.
  (bind _keys (`BlueprintMapLibrary.Map_Keys` _customizedintegers))
  (bind _values (`BlueprintMapLibrary.Map_Values` _customizedintegers))
  (return _keys _values))

(fn `InitComponent`
  (returns (Success :type Boolean))
  ;[1 1 1] Try init component.
  (`self.SetCustomizedIntegers` (`self.InitialCustomizedIntegers`))
  (set `self.IsInitialized` true)
  (return false))

(fn `SetCustomizedInteger`
  (params (IntegerName :type Name) (IntegerValue :type Integer))
  (returns (Success :type Boolean))
  ;[1 1 1] Set customized integer and call changed event.
  (`BlueprintMapLibrary.Map_Add` (`self.CustomizedIntegers`) IntegerName IntegerValue)
  (`self.OnCustomizationChanged` self)
  (return true))

(fn `SetCustomizedIntegers`
  (params (CustomizedIntegers :type "Map of Name to Integer"))
  (returns (Success :type Boolean))
  ;[1 1 1] Set customized integers and call changed event.
  (set `self.CustomizedIntegers` CustomizedIntegers)
  (`self.OnCustomizationChanged` self)
  (return true))

(fn `TryInitComponent`
  (returns (Success :type Boolean))
  ;[1 1 1] Try init component.
  (if (not (`self.IsInitialized`))
    (bind _success (`self.InitComponent`))
    (bind _output_get (set `self.IsInitialized` _success))
    (return _output_get)
    (else
      (return true))))