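; Actor component that holds an actor's gameplay tag container, optionally initialized from preset tags on BeginPlay.
; Offers set, get, add and remove functions, plus hierarchical tag checks and tag query matching.
; Edits reassign the container to fire its RepNotify, which broadcasts OnGameplayTagsChanged with new and previous tags.
; Bulk removal also strips child tags of each given tag, unlike single-tag removal.
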(event `self.ReceiveBeginPlay`
  ;[1 1 1] Begin play. Try to init gameplay tags manager component.
  (if (`self.InitOnBeginPlay`)
    (`self.TryInitComponent`)))

(fn `AddGameplayTag`
  (params (GameplayTag :type "GameplayTag Structure"))
  (returns (Success :type Boolean))
  (locals (LocalGameplayTags :type "GameplayTagContainer Structure"))
  (bind _gameplaytags (`self.GameplayTags`))
  (bind _gameplaytags_2 (`self.GameplayTags`))
  ;[1 1 1] Add gameplay tag to the container.
  (set `local.LocalGameplayTags` _gameplaytags)
  (`BlueprintGameplayTagLibrary.AddGameplayTag` _gameplaytags GameplayTag)
  (if (!= (`local.LocalGameplayTags`) _gameplaytags_2)
    (set `self.GameplayTags` _gameplaytags_2))
  (return true))

(fn `AddGameplayTags`
  (params (GameplayTags :type "GameplayTagContainer Structure"))
  (returns (Success :type Boolean))
  (locals (LocalGameplayTags :type "GameplayTagContainer Structure") (LocalTagsToAdd :type "Array of GameplayTag Structure"))
  (bind _gameplaytags (`self.GameplayTags`))
  ;[1 1 1] Add gameplay tags to the container.
  (set `local.LocalGameplayTags` (`self.GameplayTags`))
  (bind _output_get (set `local.LocalTagsToAdd` (`BlueprintGameplayTagLibrary.BreakGameplayTagContainer` GameplayTags)))
  (for _array_element _output_get
    (`BlueprintGameplayTagLibrary.AddGameplayTag` (`self.GameplayTags`) _array_element))
  (if (!= (`local.LocalGameplayTags`) _gameplaytags)
    (set `self.GameplayTags` _gameplaytags))
  (return true))

(fn `CheckGameplayTag`
  (params (GameplayTag :type "GameplayTag Structure"))
  (returns (Result :type Boolean))
  ;[1 1 1] Returns true if gameplay tag container has specific tag.
  (return (`BlueprintGameplayTagLibrary.HasTag` (`self.GameplayTags`) GameplayTag)))

(fn `CheckGameplayTagQuery`
  (params (GameplayTagQuery :type "GameplayTagQuery Structure") (ReturnTrueIfEmpty :type Boolean))
  (returns (Result :type Boolean))
  ;[1 1 1] Returns true if gameplay tag container match specific tag query.
  (if (`BlueprintGameplayTagLibrary.IsTagQueryEmpty` GameplayTagQuery)
    (return ReturnTrueIfEmpty)
    (else
      (return (`BlueprintGameplayTagLibrary.DoesContainerMatchTagQuery` (`self.GameplayTags`) GameplayTagQuery)))))

(fn `GetGameplayTags`
  (returns (GameplayTags :type "GameplayTagContainer Structure"))
  ;[1 1 1] Returns current gameplay tags.
  (return (`self.GameplayTags`)))

(fn `InitComponent`
  (returns (Success :type Boolean))
  ;[1 1 1] Init gameplay tags.
  (bind _success (`self.SetGameplayTags` (`self.InitialGameplayTags`)))
  (set `self.IsInitialized` _success)
  (return true))

(fn `OnRep_GameplayTags`
  (bind _gameplaytags (`self.GameplayTags`))
  ;[1 1 1] Calls the on gameplay tags changed event for clients.
  (`self.OnGameplayTagsChanged` self _gameplaytags (`self.PrevGameplayTags`))
  (set `self.PrevGameplayTags` _gameplaytags))

(fn `RemoveGameplayTag`
  (params (GameplayTag :type "GameplayTag Structure"))
  (returns (Success :type Boolean))
  (locals (LocalGameplayTags :type "GameplayTagContainer Structure"))
  (bind _gameplaytags (`self.GameplayTags`))
  ;[1 1 1] Remove gameplay tag from the container.
  (set `local.LocalGameplayTags` _gameplaytags)
  (bind _returnvalue (`BlueprintGameplayTagLibrary.RemoveGameplayTag` _gameplaytags GameplayTag))
  (if _returnvalue
    (set `self.GameplayTags` (`self.GameplayTags`)))
  (return true))

(fn `RemoveGameplayTags`
  (params (GameplayTags :type "GameplayTagContainer Structure"))
  (returns (Success :type Boolean))
  (locals (LocalGameplayTags :type "GameplayTagContainer Structure") (LocalTagsToAdd :type "Array of GameplayTag Structure") (LocalTagsToCheck :type "Array of GameplayTag Structure"))
  (bind _gameplaytags (`self.GameplayTags`))
  (bind _gameplaytags_2 (`self.GameplayTags`))
  ;[1 1 1] Remove gameplay tags from the container.
  (set `local.LocalGameplayTags` (`self.GameplayTags`))
  (bind _output_get (set `local.LocalTagsToAdd` (`BlueprintGameplayTagLibrary.BreakGameplayTagContainer` GameplayTags)))
  (for _array_element _output_get
    (`BlueprintGameplayTagLibrary.RemoveGameplayTag` _gameplaytags_2 _array_element)
    (if (`BlueprintGameplayTagLibrary.HasTag` _gameplaytags_2 _array_element)
      (bind _output_get_2 (set `local.LocalTagsToCheck` (`BlueprintGameplayTagLibrary.BreakGameplayTagContainer` _gameplaytags_2)))
      (for _array_element_2 _output_get_2
        (if (`BlueprintGameplayTagLibrary.MatchesTag` _array_element_2 _array_element)
          (`BlueprintGameplayTagLibrary.RemoveGameplayTag` (`self.GameplayTags`) _array_element_2)))))
  (if (!= (`local.LocalGameplayTags`) _gameplaytags)
    (set `self.GameplayTags` _gameplaytags))
  (return true))

(fn `SetGameplayTags`
  (params (GameplayTags :type "GameplayTagContainer Structure"))
  (returns (Success :type Boolean))
  ;[1 1 1] Set gameplay tag container.
  (set `self.GameplayTags` GameplayTags)
  (return true))

(fn `TryInitComponent`
  (returns (Success :type Boolean))
  ;[1 1 1] Try to init gameplay tags manager component.
  (if (not (`self.IsInitialized`))
    (bind _success (`self.InitComponent`))
    (bind _output_get (set `self.IsInitialized` _success))
    (return _output_get)
    (else
      (return true))))