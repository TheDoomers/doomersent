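; BP_FloatingText_Base is a base actor that displays floating text in the world through a widget component.
; On BeginPlay it creates the configured FloatingTextWidget, assigns it to the component, then uses interface messages to pass itself and start the animation with text value, color and font.
; If no valid widget class is set, the actor destroys itself.
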(event `self.ReceiveBeginPlay`
  (bind _floatingtextwidget (`self.FloatingTextWidget`))
  ;[1 1 1] Begin play. Start floating text widget animation.
  (if (`KismetSystemLibrary.IsValidClass` _floatingtextwidget)
    (bind _returnvalue (`|CreateWidget` _floatingtextwidget))
    (`WidgetComponent.SetWidget` (`self.Widget`) _returnvalue)
    (message `/Game/BPS_Core/Blueprints/Systems/CoreSystem/Interfaces/BPI_UI_FloatingText.SetFloatingActor_BPI` _returnvalue self)
    (message `/Game/BPS_Core/Blueprints/Systems/CoreSystem/Interfaces/BPI_UI_FloatingText.StartFloatingText_BPI` _returnvalue (`self.TextValue`) (`self.TextColor`) (`self.TextFont`))
    (else
      (`self.K2_DestroyActor`))))

(fn `UserConstructionScript`)