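; BP_GameplayEventsHelper is a helper actor in the core system that runs gameplay events, either generally or for a given player controller.
; Each function temporarily adds the component class named in the event settings, delegates the call to it, destroys it and returns the result.
; An invalid component class makes the call return false.
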(fn `TryRunGameplayEvent`
  (params (EventSettings :type "/Game/BPS_Core/Blueprints/Systems/CoreSystem/Structures/STR_EventSettings Structure (by ref)"))
  (returns (Success :type Boolean))
  (bind ((`EventComponentClass_40_C8DB90A84E042C3A26CF219082CD49CA` _eventcomponentclass)) (break `/Game/BPS_Core/Blueprints/Systems/CoreSystem/Structures/STR_EventSettings` EventSettings))
  ;[1 1 1] Try to run gameplay event with specific event settings.
  (if (`KismetSystemLibrary.IsValidClass` _eventcomponentclass)
    (bind _returnvalue (`|AddComponentByClass` _eventcomponentclass))
    (bind _success (`/Game/BPS_Core/Blueprints/Systems/CoreSystem/Components/BP_AC_EventComponent_Base.TryRunGameplayEvent` _returnvalue EventSettings))
    (`ActorComponent.K2_DestroyComponent` _returnvalue)
    (return _success)
    (else
      (return false))))

(fn `TryRunPlayerGameplayEvent`
  (params (PlayerController :type "PlayerController Object Reference") (EventSettings :type "/Game/BPS_Core/Blueprints/Systems/CoreSystem/Structures/STR_EventSettings Structure (by ref)"))
  (returns (Success :type Boolean))
  (bind ((`EventComponentClass_40_C8DB90A84E042C3A26CF219082CD49CA` _eventcomponentclass)) (break `/Game/BPS_Core/Blueprints/Systems/CoreSystem/Structures/STR_EventSettings` EventSettings))
  ;[1 1 1] Try to run gameplay event with specific event settings for player controller.
  (if (`KismetSystemLibrary.IsValidClass` _eventcomponentclass)
    (bind _returnvalue (`|AddComponentByClass` _eventcomponentclass))
    (bind _success (`/Game/BPS_Core/Blueprints/Systems/CoreSystem/Components/BP_AC_EventComponent_Base.TryRunPlayerGameplayEvent` _returnvalue PlayerController EventSettings))
    (`ActorComponent.K2_DestroyComponent` _returnvalue)
    (return _success)
    (else
      (return false))))

(fn `UserConstructionScript`)