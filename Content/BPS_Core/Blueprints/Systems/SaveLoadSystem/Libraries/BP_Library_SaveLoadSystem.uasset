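; Blueprint function library for the save/load system, giving access to saving, loading, new game, game mode and level-opening operations.
; Most calls forward to BP_AC_SaveGameManager on the GameState; player transition saves also use the controller's save object component, found by interface message.
; Helpers gather save actors with BP_SaveLoadUpdater ones first and convert IDs and arrays to delimited strings.
; FormatStringArrayToString always returns an empty string, discarding its built value.
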(fn `CheckLastSaveGameSlot`
  (returns (Result :type Boolean) (SlotName :type String))
  ;[1 1 1] Returns true if last save game slot exists.
  (bind (_success _component) (`self.FindSaveGameManagerComponent` null))
  (if _success
    (bind (_success_2 _savegameslot) (`/Game/BPS_Core/Blueprints/Systems/SaveLoadSystem/Components/BP_AC_SaveGameManager.TryFindLastSaveGameSlot` _component))
    (return _success_2 _savegameslot)
    (else
      (return false ""))))

(fn `FindAllSaveActors`
  (returns (SaveActors :type "Array of Actor Object Reference"))
  (locals (LocalActors :type "Array of Actor Object Reference"))
  (bind _localactors (`local.LocalActors`))
  ;[1 1 1] Try to find all actors that implement save object interface.
  (bind _outactors (`GameplayStatics.GetAllActorsWithInterface` null "/Game/BPS_Core/Blueprints/Systems/SaveLoadSystem/Interfaces/BPI_SaveObject.BPI_SaveObject_C"))
  (bind _output_get (set `local.LocalActors` _outactors))
  (bind _filteredarray (`KismetArrayLibrary.FilterArray` _output_get "/Game/BPS_Core/Blueprints/Systems/SaveLoadSystem/Actors/BP_SaveLoadUpdater.BP_SaveLoadUpdater_C"))
  (for _array_element _filteredarray
    (`KismetArrayLibrary.Array_RemoveItem` _localactors _array_element)
    (`KismetArrayLibrary.Array_Insert` _localactors _array_element))
  (return _localactors))

(fn `FindSaveGameManagerComponent`
  (returns (Success :type Boolean) (Component :type "/Game/BPS_Core/Blueprints/Systems/SaveLoadSystem/Components/BP_AC_SaveGameManager Object Reference"))
  (locals (LocalSaveGameManager :type "/Game/BPS_Core/Blueprints/Systems/SaveLoadSystem/Components/BP_AC_SaveGameManager Object Reference"))
  (bind _returnvalue (`GameplayStatics.GetGameState` null))
  ;[1 1 1] Try to find save game manager component.
  (`/Engine/EditorBlueprintResources/StandardMacros.IsValid` _returnvalue
    (:`Is Valid`
      (bind _output_get (set `local.LocalSaveGameManager` (`Actor.GetComponentByClass` _returnvalue "/Game/BPS_Core/Blueprints/Systems/SaveLoadSystem/Components/BP_AC_SaveGameManager.BP_AC_SaveGameManager_C")))
      (`/Engine/EditorBlueprintResources/StandardMacros.IsValid` _output_get
        (:`Is Valid`
          (return true (`local.LocalSaveGameManager`)))
        (:`Is Not Valid`
          (`KismetSystemLibrary.PrintText` null "Save game manager component is not found! \nSave game manager component should be a part of the game state class." true true (struct :`R` 1.0 :`A` 1.0) 10.0)
          (return false null))))
    (:`Is Not Valid`
      (return false null))))

(fn `FindSaveObjectComponent`
  (params (TargetActor :type "Actor Object Reference"))
  (returns (Found :type Boolean) (Component :type "/Game/BPS_Core/Blueprints/Systems/SaveLoadSystem/Components/BP_AC_SaveObjectComponent Object Reference"))
  (locals (LocalSaveObject :type "/Game/BPS_Core/Blueprints/Systems/SaveLoadSystem/Components/BP_AC_SaveObjectComponent Object Reference"))
  ;[1 1 1] Try to find save object component.
  (bind (_success _component) (message `/Game/BPS_Core/Blueprints/Systems/SaveLoadSystem/Interfaces/BPI_SaveObject.GetSaveObjectComponent_BPI` TargetActor))
  (if _success
    (return true _component)
    (else
      (return false null))))

(fn `FormatIntegerArrayToString`
  (params (IntegerArray :type "Array of Integer"))
  (returns (StringValue :type String))
  (locals (LocalIntegerToString :type String) (LocalStringValue :type String))
  ;[1 1 1] Format integer array to string.
  (for _array_element IntegerArray
    (bind _output_get (set `local.LocalIntegerToString` (`KismetStringLibrary.Conv_IntToString` _array_element)))
    (set `local.LocalStringValue` (`KismetStringLibrary.Concat_StrStr` (`local.LocalStringValue`) _output_get ";")))
  (return (`local.LocalStringValue`)))

(fn `FormatSavedActorsToString`
  (params (ActorsArray :type "Array of Actor Object Reference"))
  (returns (StringValue :type String))
  (locals (LocalSaveIDs :type "Array of Integer"))
  ;[1 1 1] Format save ids of saved actors to string.
  (for _array_element ActorsArray
    (bind (_found _component) (`self.FindSaveObjectComponent` _array_element))
    (if _found
      (`KismetArrayLibrary.Array_Add` (`local.LocalSaveIDs`) (`/Game/BPS_Core/Blueprints/Systems/SaveLoadSystem/Components/BP_AC_SaveObjectComponent.GetSaveID_Pure` _component))))
  (bind _stringvalue (`self.FormatIntegerArrayToString` (`local.LocalSaveIDs`)))
  (return _stringvalue))

(fn `FormatStringArrayToString`
  (params (StringArray :type "Array of String"))
  (returns (StringValue :type String))
  (locals (LocalIntegerToString :type String) (LocalStringValue :type String) (LocalValue :type String))
  ;[1 1 1] Format string array to string.
  (for _array_element StringArray
    (set `local.LocalValue` (`KismetStringLibrary.Concat_StrStr` (`local.LocalValue`) _array_element ";;;")))
  (return ""))

(fn `FormatStringToIntegerArray`
  (params (StringValue :type String))
  (returns (IntegerArray :type "Array of Integer"))
  (locals (LocalIntegerArray :type "Array of Integer"))
  ;[1 1 1] Format string to integer array.
  (for _array_element (`KismetStringLibrary.ParseIntoArray` StringValue ";")
    (`KismetArrayLibrary.Array_Add` (`local.LocalIntegerArray`) (`KismetStringLibrary.Conv_StringToInt` _array_element)))
  (return (`local.LocalIntegerArray`)))

(fn `FormatStringToStringArray`
  (params (StringValue :type String))
  (returns (StringArray :type "Array of String"))
  (locals (LocalIntegerArray :type "Array of Integer"))
  ;[1 1 1] Format string to string array.
  (return (`KismetStringLibrary.ParseIntoArray` StringValue ";;;")))

(fn `GetSaveGameMode`
  (returns (Success :type Boolean) (GameModeName :type Name) (IsMultiplayer :type Boolean))
  ;[1 1 1] Returns current save game mode.
  (bind (_success _component) (`self.FindSaveGameManagerComponent` null))
  (if _success
    (bind (_gamemodename _ismultiplayer) (`/Game/BPS_Core/Blueprints/Systems/SaveLoadSystem/Components/BP_AC_SaveGameManager.GetSaveGameMode` _component))
    (return true _gamemodename _ismultiplayer)
    (else
      (return false "None" false))))

(fn `SetSaveGameMode`
  (params (GameModeName :type Name) (IsMultiplayer :type Boolean))
  (returns (Success :type Boolean))
  ;[1 1 1] Set save game mode.
  (bind (_success _component) (`self.FindSaveGameManagerComponent` null))
  (if _success
    (bind _success_2 (`/Game/BPS_Core/Blueprints/Systems/SaveLoadSystem/Components/BP_AC_SaveGameManager.SetSaveGameMode` _component GameModeName IsMultiplayer))
    (return _success_2)
    (else
      (return false))))

(fn `TryFindMappedLevelName`
  (params (MappedName :type Name))
  (returns (Success :type Boolean) (LevelName :type Name))
  ;[1 1 1] Try to find game level name from the list by specific name.
  (bind (_success _component) (`self.FindSaveGameManagerComponent` null))
  (if _success
    (bind (_success_2 _levelname) (`/Game/BPS_Core/Blueprints/Systems/SaveLoadSystem/Components/BP_AC_SaveGameManager.TryFindMappedLevelName` _component MappedName))
    (return _success_2 _levelname)
    (else
      (return false "None"))))

(fn `TryGetSaveID`
  (params (TargetActor :type "Actor Object Reference"))
  (returns (Success :type Boolean) (SaveID :type Integer))
  ;[1 1 1] Try to get save id of target actor.
  (bind (_found _component) (`self.FindSaveObjectComponent` TargetActor))
  (if _found
    (return true (`/Game/BPS_Core/Blueprints/Systems/SaveLoadSystem/Components/BP_AC_SaveObjectComponent.GetSaveID_Pure` _component))
    (else
      (return false 0))))

(fn `TryLoadGameFromSlot`
  (params (SlotName :type String))
  (returns (Success :type Boolean))
  ;[1 1 1] Try to load game from slot.
  (bind (_success _component) (`self.FindSaveGameManagerComponent` null))
  (if _success
    (bind _success_2 (`/Game/BPS_Core/Blueprints/Systems/SaveLoadSystem/Components/BP_AC_SaveGameManager.TryLoadGameFromSlot` _component SlotName))
    (return _success_2)
    (else
      (return false))))

(fn `TryLoadLastSaveGame`
  (returns (Success :type Boolean))
  ;[1 1 1] Try to load last save game.
  (bind (_success _component) (`self.FindSaveGameManagerComponent` null))
  (if _success
    (bind _success_2 (`/Game/BPS_Core/Blueprints/Systems/SaveLoadSystem/Components/BP_AC_SaveGameManager.TryLoadLastSave` _component))
    (return _success_2)
    (else
      (return false))))

(fn `TryOpenMainMenuLevel`
  (returns (Success :type Boolean))
  ;[1 1 1] Try to open main menu level.
  (bind (_success _component) (`self.FindSaveGameManagerComponent` null))
  (if _success
    (bind _success_2 (`/Game/BPS_Core/Blueprints/Systems/SaveLoadSystem/Components/BP_AC_SaveGameManager.TryOpenMainMenuLevel` _component))
    (return _success_2)
    (else
      (return false))))

(fn `TrySavePlayerTransitionData`
  (params (PlayerController :type "PlayerController Object Reference"))
  (returns (Success :type Boolean))
  ;[1 1 1] Try to create and saveplayer transition data.
  (bind (_success _component) (`self.FindSaveGameManagerComponent` null))
  (if _success
    (bind _returnvalue (`/Game/BPS_Core/Blueprints/Systems/SaveLoadSystem/Components/BP_AC_SaveGameManager.CreatePlayerTransitionSaveGame` _component))
    (bind (_found _component_2) (`self.FindSaveObjectComponent` PlayerController))
    (if _found
      (`/Game/BPS_Core/Blueprints/Systems/SaveLoadSystem/Components/BP_AC_SaveObjectComponent.TryToSaveData` _component_2 _returnvalue)
      (return true)
      (else
        _)))
  (return false))

(fn `TryStartNewGame`
  (params (LevelName :type Name))
  (returns (Success :type Boolean))
  ;[1 1 1] Try to start new game and open specific level.
  (bind (_success _component) (`self.FindSaveGameManagerComponent` null))
  (if _success
    (bind _success_2 (`/Game/BPS_Core/Blueprints/Systems/SaveLoadSystem/Components/BP_AC_SaveGameManager.TryStartNewGame` _component LevelName))
    (return _success_2)
    (else
      (return false))))