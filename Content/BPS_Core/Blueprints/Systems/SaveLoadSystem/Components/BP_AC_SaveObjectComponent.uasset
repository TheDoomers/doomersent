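; Actor component that saves and restores its owner through a SaveGame, keyed by a SaveID.
; By default it writes class, transform and a string variable map via interface messages, then on load teleports the owner and restores the map.
; Custom-logic flags skip that default step, while save and load callbacks let other code participate.
; Typed helpers convert variables to and from strings, including save-only formatting of actor lists as save IDs.
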(fn `CheckUseSaveID`
  (returns (Result :type Boolean))
  ;[1 1 1] Returns true if the component should use unique save id.
  (return (`self.UseSaveID`)))

(fn `GetSaveID`
  (returns (SaveID :type Integer))
  ;[1 1 1] Returns save id.
  (return (`self.SaveID`)))

(fn `GetSaveID_Pure`
  (returns (SaveID :type Integer))
  ;[1 1 1] Returns save id.
  (bind _saveid (`self.GetSaveID`))
  (return _saveid))

(fn `LoadActorData`
  (params (SaveGame :type "SaveGame Object Reference"))
  (returns (Success :type Boolean))
  ;[1 1 1] Try to load actor data from save game.
  (bind (_success _savedata) (message `/Game/BPS_Core/Blueprints/Systems/SaveLoadSystem/Interfaces/BPI_SaveGame_Base.GetActorSaveData_BPI` SaveGame (`self.SaveID`)))
  (if _success
    (bind ((`Transform_5_0C82CB2B44633DFA74FEB7AC2B7A3E18` _transform) (`StringVariables_15_BB7A21BF48EBC99A2C3E49A905EF09CF` _stringvariables)) (break `/Game/BPS_Core/Blueprints/Systems/SaveLoadSystem/Structures/STR_SaveData_Actor` _savedata))
    (`Actor.K2_SetActorTransform` (`self.GetOwner`) _transform false true)
    (set `self.StringVariables` _stringvariables)
    (return true)
    (else
      (return false))))

(fn `LoadBoolVariable`
  (params (VariableName :type Name))
  (returns (Success :type Boolean) (VariableValue :type Boolean))
  (bind (_value _returnvalue) (`BlueprintMapLibrary.Map_Find` (`self.StringVariables`) VariableName))
  ;[1 1 1] Load value of bool variable.
  (return _returnvalue (`KismetStringLibrary.EqualEqual_StrStr` _value "true")))

(fn `LoadByteVariable`
  (params (VariableName :type Name))
  (returns (Success :type Boolean) (VariableValue :type Byte))
  (bind (_value _returnvalue) (`BlueprintMapLibrary.Map_Find` (`self.StringVariables`) VariableName))
  ;[1 1 1] Load value of byte variable.
  (return _returnvalue (`KismetMathLibrary.Conv_IntToByte` (`KismetStringLibrary.Conv_StringToInt` _value))))

(fn `LoadFloatVariable`
  (params (VariableName :type Name))
  (returns (Success :type Boolean) (VariableValue :type "Float (double-precision)"))
  (bind (_value _returnvalue) (`BlueprintMapLibrary.Map_Find` (`self.StringVariables`) VariableName))
  ;[1 1 1] Load value of float variable.
  (return _returnvalue (`KismetStringLibrary.Conv_StringToDouble` _value)))

(fn `LoadIntegerVariable`
  (params (VariableName :type Name))
  (returns (Success :type Boolean) (VariableValue :type Integer))
  (bind (_value _returnvalue) (`BlueprintMapLibrary.Map_Find` (`self.StringVariables`) VariableName))
  ;[1 1 1] Load value of integer variable.
  (return _returnvalue (`KismetStringLibrary.Conv_StringToInt` _value)))

(fn `LoadNameVariable`
  (params (VariableName :type Name))
  (returns (Success :type Boolean) (VariableValue :type Name))
  (bind (_value _returnvalue) (`BlueprintMapLibrary.Map_Find` (`self.StringVariables`) VariableName))
  ;[1 1 1] Load value of name variable.
  (return _returnvalue (`KismetStringLibrary.Conv_StringToName` _value)))

(fn `LoadStringVariable`
  (params (VariableName :type Name))
  (returns (Success :type Boolean) (VariableValue :type String))
  (bind (_value _returnvalue) (`BlueprintMapLibrary.Map_Find` (`self.StringVariables`) VariableName))
  ;[1 1 1] Load value of string variable.
  (return _returnvalue _value))

(fn `SaveActorData`
  (params (SaveGame :type "SaveGame Object Reference"))
  (returns (Success :type Boolean))
  (bind _returnvalue (`self.GetOwner`))
  ;[1 1 1] Try to save actor data to save game.
  (bind _success (`self.SaveActorDataAdvanced` SaveGame (`GameplayStatics.GetObjectClass` _returnvalue) (`Actor.GetTransform` _returnvalue)))
  (return _success))

(fn `SaveActorDataAdvanced`
  (params (SaveGame :type "SaveGame Object Reference") (ActorClass :type "Actor Class Reference") (Transform :type "Transform Structure"))
  (returns (Success :type Boolean))
  ;[1 1 1] Try to save actor data to save game.
  (bind _success (message `/Game/BPS_Core/Blueprints/Systems/SaveLoadSystem/Interfaces/BPI_SaveGame_Base.SetActorSaveData_BPI` SaveGame (`self.SaveID`) (make `/Game/BPS_Core/Blueprints/Systems/SaveLoadSystem/Structures/STR_SaveData_Actor` ActorClass Transform (`self.StringVariables`))))
  (return _success))

(fn `SaveBoolVariable`
  (params (VariableName :type Name) (VariableValue :type Boolean))
  (returns (Success :type Boolean))
  ;[1 1 1] Save value of bool variable.
  (`BlueprintMapLibrary.Map_Add` (`self.StringVariables`) VariableName (`KismetStringLibrary.Conv_BoolToString` VariableValue))
  (return true))

(fn `SaveByteVariable`
  (params (VariableName :type Name) (VariableValue :type Byte))
  (returns (Success :type Boolean))
  ;[1 1 1] Save value of byte variable.
  (`BlueprintMapLibrary.Map_Add` (`self.StringVariables`) VariableName (`KismetStringLibrary.Conv_ByteToString` VariableValue))
  (return true))

(fn `SaveFloatVariable`
  (params (VariableName :type Name) (VariableValue :type "Float (double-precision)"))
  (returns (Success :type Boolean))
  ;[1 1 1] Save value of float variable.
  (`BlueprintMapLibrary.Map_Add` (`self.StringVariables`) VariableName (`KismetStringLibrary.Conv_DoubleToString` VariableValue))
  (return true))

(fn `SaveIntegerVariable`
  (params (VariableName :type Name) (VariableValue :type Integer))
  (returns (Success :type Boolean))
  ;[1 1 1] Save value of integer variable.
  (`BlueprintMapLibrary.Map_Add` (`self.StringVariables`) VariableName (`KismetStringLibrary.Conv_IntToString` VariableValue))
  (return true))

(fn `SaveNameVariable`
  (params (VariableName :type Name) (VariableValue :type Name))
  (returns (Success :type Boolean))
  ;[1 1 1] Save value of name variable.
  (`BlueprintMapLibrary.Map_Add` (`self.StringVariables`) VariableName (`KismetStringLibrary.Conv_NameToString` VariableValue))
  (return true))

(fn `SaveSavedActorsVariable`
  (params (VariableName :type Name) (VariableValue :type "Array of Actor Object Reference"))
  (returns (Success :type Boolean))
  ;[1 1 1] Save save ids of target list of actors.
  (bind _stringvalue (`/Game/BPS_Core/Blueprints/Systems/SaveLoadSystem/Libraries/BP_Library_SaveLoadSystem.FormatSavedActorsToString` VariableValue))
  (`BlueprintMapLibrary.Map_Add` (`self.StringVariables`) VariableName _stringvalue)
  (return true))

(fn `SaveStringArrayVariable`
  (params (VariableName :type Name) (VariableValue :type String))
  (returns (Success :type Boolean))
  ;[1 1 1] Save value of string array variable.
  (`BlueprintMapLibrary.Map_Add` (`self.StringVariables`) VariableName VariableValue)
  (return true))

(fn `SaveStringVariable`
  (params (VariableName :type Name) (VariableValue :type String))
  (returns (Success :type Boolean))
  ;[1 1 1] Save value of string variable.
  (`BlueprintMapLibrary.Map_Add` (`self.StringVariables`) VariableName VariableValue)
  (return true))

(fn `SetSaveID`
  (params (SaveID :type Integer))
  (returns (Success :type Boolean))
  ;[1 1 1] Set save id.
  (set `self.SaveID` SaveID)
  (return true))

(fn `TryToLoadData`
  (params (SaveGame :type "SaveGame Object Reference"))
  (returns (Success :type Boolean))
  (locals (LocalSaveData :type "SaveGame Object Reference"))
  (bind _localsavedata (`local.LocalSaveData`))
  ;[1 1 1] Try to load actor data.
  (set `local.LocalSaveData` SaveGame)
  (if (not (`self.UseCustomLoadLogic`))
    (bind _success (`self.LoadActorData` SaveGame))
    (if _success
      _
      (else
        (return false))))
  (`self.OnLoadData` self _localsavedata)
  (`self.OnPostLoadData` self _localsavedata)
  (return true))

(fn `TryToSaveData`
  (params (SaveGame :type "SaveGame Object Reference"))
  (returns (Success :type Boolean))
  (locals (LocalSaveData :type "SaveGame Object Reference"))
  ;[1 1 1] Try to save actor data.
  (bind _output_get (set `local.LocalSaveData` SaveGame))
  (`self.OnPreSaveData` self _output_get)
  (if (not (`self.UseCustomSaveLogic`))
    (bind _success (`self.SaveActorData` SaveGame))
    (if _success
      _
      (else
        (return false))))
  (`self.OnSaveData` self (`local.LocalSaveData`))
  (return true))