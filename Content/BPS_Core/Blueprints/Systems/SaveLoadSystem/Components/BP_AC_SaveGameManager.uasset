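; Save manager component that saves and loads games, starts new ones and moves play between levels.
; Slots are named per game mode and listed in a separate settings save.
; Actors with save-object components write per-level data, and loading respawns saved actors by ID.
; Level changes pass through a temporary transition slot read by the next level, which respawns carried-over actors and places them at a tagged transition point or PlayerStart.
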(fn `CreateNewSaveGame`
  (returns (Success :type Boolean) (SaveGame :type "SaveGame Object Reference"))
  ;[1 1 1] Try to create new save game object.
  (bind _returnvalue (`GameplayStatics.CreateSaveGameObject` (`self.SaveGameClass`)))
  (`/Engine/EditorBlueprintResources/StandardMacros.IsValid` _returnvalue
    (:`Is Valid`
      (return true _returnvalue))
    (:`Is Not Valid`
      (return false null))))

(fn `CreatePlayerTransitionSaveGame`
  (returns (ReturnValue :type "SaveGame Object Reference"))
  ;[1 1 1] Create player transition save game object.
  (bind _returnvalue (`GameplayStatics.CreateSaveGameObject` (`self.SaveGameClass`)))
  (return _returnvalue))

(fn `DeleteGameInSlot`
  (params (GameModeName :type Name) (SaveSlotName :type String))
  (returns (Success :type Boolean))
  (bind _settingssavegame (`self.GetSettingsSaveGame`))
  ;[1 1 1] Try to delete save game in slot.
  (`/Engine/EditorBlueprintResources/StandardMacros.IsValid` _settingssavegame
    (:`Is Valid`
      (bind _success (message `/Game/BPS_Core/Blueprints/Systems/SaveLoadSystem/Interfaces/BPI_SaveGame_SavesLists.RemoveSaveSlotFromList_BPI` _settingssavegame GameModeName SaveSlotName))
      (if _success
        (`self.SaveSettingsSaveGame`)
        (bind _returnvalue (`GameplayStatics.DeleteGameInSlot` (`self.MakeCombinedSaveSlotName` GameModeName SaveSlotName)))
        (return _returnvalue)
        (else
          _)))
    (:`Is Not Valid`
      _))
  (return false))

(fn `DeletePlayerTransitionSaveGame`
  (returns (Success :type Boolean))
  (bind _playertransitiondatasaveslotname (`self.PlayerTransitionDataSaveSlotName`))
  ;[1 1 1] Try to delete player transition save game.
  (bind _returnvalue (`GameplayStatics.DoesSaveGameExist` _playertransitiondatasaveslotname))
  (if _returnvalue
    (bind _returnvalue_2 (`GameplayStatics.DeleteGameInSlot` _playertransitiondatasaveslotname))
    (return _returnvalue_2)
    (else
      (return true))))

(fn `GetCurrentSaveGame`
  (returns (CurrentSaveGame :type "SaveGame Object Reference"))
  ;[1 1 1] Returns current save game.
  (return (`self.CurrentSaveGame`)))

(fn `GetCurrentSavesList`
  (returns (Success :type Boolean) (SavesList :type "/Game/BPS_Core/Blueprints/Systems/SaveLoadSystem/Structures/STR_SavesList Structure"))
  (bind _settingssavegame (`self.GetSettingsSaveGame`))
  (bind _savegamemode (`self.SaveGameMode`))
  ;[1 1 1] Returns saves list for current save game mode.
  (bind (_success _saveslist) (message `/Game/BPS_Core/Blueprints/Systems/SaveLoadSystem/Interfaces/BPI_SaveGame_SavesLists.GetSavesList_BPI` _settingssavegame _savegamemode))
  (if _success
    (return true _saveslist)
    (else
      (bind (_success_2 _saveslist_2) (message `/Game/BPS_Core/Blueprints/Systems/SaveLoadSystem/Interfaces/BPI_SaveGame_SavesLists.CreateSavesList_BPI` _settingssavegame _savegamemode))
      (return _success_2 _saveslist_2))))

(fn `GetSaveGameMode`
  (returns (GameModeName :type Name) (IsMultiplayer :type Boolean))
  ;[1 1 1] Returns current save game mode.
  (return (`self.SaveGameMode`) (`self.SaveIsMultiplayer`)))

(fn `GetSettingsSaveGame`
  (returns (SettingsSaveGame :type "SaveGame Object Reference"))
  ;[1 1 1] Returns settings save game object.
  (`/Engine/EditorBlueprintResources/StandardMacros.IsValid` (`self.SettingsSaveGame`)
    (:`Is Valid`
      _)
    (:`Is Not Valid`
      (bind _returnvalue (`GameplayStatics.LoadGameFromSlot` (`self.SettingsSaveSlotName`)))
      (`/Engine/EditorBlueprintResources/StandardMacros.IsValid` _returnvalue
        (:`Is Valid`
          (set `self.SettingsSaveGame` _returnvalue))
        (:`Is Not Valid`
          (bind _returnvalue_2 (`GameplayStatics.CreateSaveGameObject` (`self.SettingsSaveGameClass`)))
          (set `self.SettingsSaveGame` _returnvalue_2)))))
  (return (`self.SettingsSaveGame`)))

(fn `GetTransitionActors`
  (returns (Success :type Boolean) (TransitionActors :type "Array of Actor Object Reference"))
  ;[1 1 1] Returns transition actors.
  (return true (`self.TransitionActors`)))

(fn `LoadLevelData`
  (params (SaveGame :type "SaveGame Object Reference") (LevelName :type Name))
  (returns (Success :type Boolean))
  (locals (LocalSaveGame :type "SaveGame Object Reference") (LocalLoadedActors :type "Array of Actor Object Reference") (LocalSaveID :type Integer) (LocalActorData :type "/Game/BPS_Core/Blueprints/Systems/SaveLoadSystem/Structures/STR_SaveData_Actor Structure"))
  ;[1 1 1] Load current level data.
  (bind _output_get (set `local.LocalSaveGame` SaveGame))
  (message `/Game/BPS_Core/Blueprints/Systems/SaveLoadSystem/Interfaces/BPI_SaveGame_Base.LoadTempLevelData_BPI` _output_get LevelName)
  (`|ExecutionSequence`
    (:`then_0`
      (bind _saveactors (`/Game/BPS_Core/Blueprints/Systems/SaveLoadSystem/Libraries/BP_Library_SaveLoadSystem.FindAllSaveActors`))
      (for _array_element _saveactors
        (bind (_success _component) (message `/Game/BPS_Core/Blueprints/Systems/SaveLoadSystem/Interfaces/BPI_SaveObject.GetSaveObjectComponent_BPI` _array_element))
        (if _success
          (if (`/Game/BPS_Core/Blueprints/Systems/SaveLoadSystem/Components/BP_AC_SaveObjectComponent.CheckUseSaveID` _component)
            (bind _saveid (`/Game/BPS_Core/Blueprints/Systems/SaveLoadSystem/Components/BP_AC_SaveObjectComponent.GetSaveID` _component))
            (if (>= _saveid 0)
              (`Actor.K2_DestroyActor` _array_element)
              (else
                (`KismetArrayLibrary.Array_Add` (`local.LocalLoadedActors`) _array_element)
                (message `/Game/BPS_Core/Blueprints/Systems/SaveLoadSystem/Interfaces/BPI_SaveGame_Base.InitSaveActorWithID_BPI` (`local.LocalSaveGame`) _array_element _saveid)))
            (else
              (`KismetArrayLibrary.Array_Add` (`local.LocalLoadedActors`) _array_element))))))
    (:`then_1`
      (`|ExecutionSequence`
        (:`then_0`
          (bind (_success_2 _saveids _savedata) (message `/Game/BPS_Core/Blueprints/Systems/SaveLoadSystem/Interfaces/BPI_SaveGame_Base.GetSavedActorsData_BPI` (`local.LocalSaveGame`)))
          (if _success_2
            (for (_array_element_2 _array_index) _saveids
              (bind _output_get_2 (set `local.LocalSaveID` _array_element_2))
              (bind _output_get_3 (set `local.LocalActorData` (`|GetArrayItem` _savedata _array_index)))
              (if (>= _output_get_2 0)
                (bind ((`ActorClass_2_8E028EAE4FCB76A2E29782800903A34F` _actorclass) (`Transform_5_0C82CB2B44633DFA74FEB7AC2B7A3E18` _transform)) (break `/Game/BPS_Core/Blueprints/Systems/SaveLoadSystem/Structures/STR_SaveData_Actor` _output_get_3))
                (bind _returnvalue (`|SpawnActorFromClass` _actorclass _transform "AlwaysSpawn" "SelectDefaultAtRuntime" null null))
                (message `/Game/BPS_Core/Blueprints/Systems/SaveLoadSystem/Interfaces/BPI_SaveGame_Base.InitSaveActorWithID_BPI` (`local.LocalSaveGame`) _returnvalue (`local.LocalSaveID`))
                (`KismetArrayLibrary.Array_Add` (`local.LocalLoadedActors`) _returnvalue)))))
        (:`then_1`
          (`|ExecutionSequence`
            (:`then_0`
              (for _array_element_3 (`local.LocalLoadedActors`)
                (`/Engine/EditorBlueprintResources/StandardMacros.IsValid` _array_element_3
                  (:`Is Valid`
                    (bind (_success_3 _component_2) (message `/Game/BPS_Core/Blueprints/Systems/SaveLoadSystem/Interfaces/BPI_SaveObject.GetSaveObjectComponent_BPI` _array_element_3))
                    (if _success_3
                      (`/Game/BPS_Core/Blueprints/Systems/SaveLoadSystem/Components/BP_AC_SaveObjectComponent.TryToLoadData` _component_2 (`local.LocalSaveGame`)))))))
            (:`then_1`
              (return true))))))))

(fn `LoadPlayersData`
  (params (SaveGame :type "SaveGame Object Reference"))
  (returns (Success :type Boolean))
  (locals (LocalSaveGame :type "SaveGame Object Reference") (LocalLoadedActors :type "Array of Actor Object Reference") (LocalSaveID :type Integer) (LocalActorData :type "/Game/BPS_Core/Blueprints/Systems/SaveLoadSystem/Structures/STR_SaveData_Actor Structure"))
  ;[1 1 1] Try to load data for players.
  (set `local.LocalSaveGame` SaveGame)
  (bind _outactors (`GameplayStatics.GetAllActorsOfClass` "/Script/Engine.PlayerController"))
  (for _array_element _outactors
    (bind (_success _component) (message `/Game/BPS_Core/Blueprints/Systems/SaveLoadSystem/Interfaces/BPI_SaveObject.GetSaveObjectComponent_BPI` _array_element))
    (if _success
      (`/Game/BPS_Core/Blueprints/Systems/SaveLoadSystem/Components/BP_AC_SaveObjectComponent.TryToLoadData` _component (`local.LocalSaveGame`))))
  (return true))

(fn `LoadPlayerTransitionSaveGame`
  (returns (Success :type Boolean) (SaveGame :type "SaveGame Object Reference"))
  (bind _playertransitiondatasaveslotname (`self.PlayerTransitionDataSaveSlotName`))
  ;[1 1 1] Try to load player transition save game from slot.
  (bind _returnvalue (`GameplayStatics.DoesSaveGameExist` _playertransitiondatasaveslotname))
  (if _returnvalue
    (bind _returnvalue_2 (`GameplayStatics.LoadGameFromSlot` _playertransitiondatasaveslotname))
    (return true _returnvalue_2)
    (else
      (return false null))))

(fn `LoadTransitionActors`
  (params (SaveGame :type "SaveGame Object Reference") (TransitionPoint :type Name))
  (returns (Success :type Boolean))
  (locals (LocalSaveGame :type "SaveGame Object Reference") (LocalLoadedActors :type "Array of Actor Object Reference") (LocalSaveID :type Integer) (LocalActorData :type "/Game/BPS_Core/Blueprints/Systems/SaveLoadSystem/Structures/STR_SaveData_Actor Structure") (LocalTransitionPoint :type Name) (LocalTransitionPointActor :type "Actor Object Reference"))
  (bind _localtransitionpoint (`local.LocalTransitionPoint`))
  ;[1 1 1] Try to load transtion actors data.
  (bind _output_get (set `local.LocalSaveGame` SaveGame))
  (set `local.LocalTransitionPoint` TransitionPoint)
  (message `/Game/BPS_Core/Blueprints/Systems/SaveLoadSystem/Interfaces/BPI_SaveGame_Base.LoadTempLevelData_BPI` _output_get (`self.TransitionActorsLevelName`))
  (`|ExecutionSequence`
    (:`then_0`
      (bind (_success _saveids _savedata) (message `/Game/BPS_Core/Blueprints/Systems/SaveLoadSystem/Interfaces/BPI_SaveGame_Base.GetSavedActorsData_BPI` (`local.LocalSaveGame`)))
      (if _success
        (for (_array_element _array_index) _saveids
          (bind _output_get_2 (set `local.LocalSaveID` _array_element))
          (bind _output_get_3 (set `local.LocalActorData` (`|GetArrayItem` _savedata _array_index)))
          (if (>= _output_get_2 0)
            (bind _returnvalue (`|SpawnActorFromClass` (`.ActorClass_2_8E028EAE4FCB76A2E29782800903A34F` (break `/Game/BPS_Core/Blueprints/Systems/SaveLoadSystem/Structures/STR_SaveData_Actor` _output_get_3)) (`KismetMathLibrary.MakeTransform` (0.0 0.0 0.0)) "AlwaysSpawn" "SelectDefaultAtRuntime" null null))
            (message `/Game/BPS_Core/Blueprints/Systems/SaveLoadSystem/Interfaces/BPI_SaveGame_Base.InitSaveActorWithID_BPI` (`local.LocalSaveGame`) _returnvalue (`local.LocalSaveID`))
            (`KismetArrayLibrary.Array_Add` (`local.LocalLoadedActors`) _returnvalue)))))
    (:`then_1`
      (`|ExecutionSequence`
        (:`then_0`
          (bind _output_get_4 (set `self.TransitionActors` (`local.LocalLoadedActors`)))
          (if (`KismetArrayLibrary.Array_IsValidIndex` _output_get_4)
            (for _array_element_2 _output_get_4
              (`/Engine/EditorBlueprintResources/StandardMacros.IsValid` _array_element_2
                (:`Is Valid`
                  (bind (_success_2 _component) (message `/Game/BPS_Core/Blueprints/Systems/SaveLoadSystem/Interfaces/BPI_SaveObject.GetSaveObjectComponent_BPI` _array_element_2))
                  (if _success_2
                    (`/Game/BPS_Core/Blueprints/Systems/SaveLoadSystem/Components/BP_AC_SaveObjectComponent.TryToLoadData` _component (`local.LocalSaveGame`))))))
            (set `self.TransitionPointIsHandled` false)
            (`self.OnTransitActorsToPoint` self _localtransitionpoint)
            (if (not (`self.TransitionPointIsHandled`))
              (`|ExecutionSequence`
                (:`then_0`
                  (bind _outactors (`GameplayStatics.GetAllActorsWithTag` _localtransitionpoint))
                  (if (`KismetArrayLibrary.Array_IsValidIndex` _outactors)
                    (bind _output_get_5 (set `local.LocalTransitionPointActor` (`KismetArrayLibrary.Array_Random` _outactors)))
                    (for _array_element_3 (`self.TransitionActors`) :!label _label
                      (`Actor.K2_SetActorLocationAndRotation` _array_element_3 (`Actor.K2_GetActorLocation` _output_get_5) (`Actor.K2_GetActorRotation` _output_get_5) false true))
                    (message `/Game/BPS_Core/Blueprints/Systems/SaveLoadSystem/Interfaces/BPI_SaveGame_Base.ClearLevelData_BPI` (`local.LocalSaveGame`) (`self.TransitionActorsLevelName`))
                    (return true)))
                (:`then_1`
                  (bind _outactors_2 (`GameplayStatics.GetAllActorsOfClass` "/Script/Engine.PlayerStart"))
                  (if (`KismetArrayLibrary.Array_IsValidIndex` _outactors_2)
                    (set `local.LocalTransitionPointActor` (`KismetArrayLibrary.Array_Random` _outactors_2))
                    (goto _label)))))))
        (:`then_1`
          (return true))))))

(fn `MakeCombinedSaveSlotName`
  (params (GameModeName :type Name) (SaveSlotName :type String))
  (returns (Result :type String))
  ;[1 1 1] Make combined save slot name.
  (return (`KismetStringLibrary.Concat_StrStr` (`KismetStringLibrary.Conv_NameToString` GameModeName) "_" SaveSlotName)))

(fn `SaveGameToSlot`
  (params (SaveGame :type "SaveGame Object Reference") (SaveSlotName :type String))
  (returns (Success :type Boolean))
  (locals (LocalSaveGame :type "SaveGame Object Reference") (LocalSaveSlotName :type String))
  (bind _localsaveslotname (`local.LocalSaveSlotName`))
  (bind _savegamemode (`self.SaveGameMode`))
  ;[1 1 1] Try to save game to slot.
  (bind _output_get (set `local.LocalSaveGame` SaveGame))
  (bind _output_get_2 (set `local.LocalSaveSlotName` SaveSlotName))
  (`/Engine/EditorBlueprintResources/StandardMacros.IsValid` (`self.GetSettingsSaveGame`)
    (:`Is Valid`
      (message `/Game/BPS_Core/Blueprints/Systems/SaveLoadSystem/Interfaces/BPI_SaveGame_Base.SetSaveSlotData_BPI` _output_get (`self.SaveGameMode`) _output_get_2 false)
      (message `/Game/BPS_Core/Blueprints/Systems/SaveLoadSystem/Interfaces/BPI_SaveGame_Base.SetDateTime_BPI` _output_get (`KismetMathLibrary.Now`))
      (bind _success (message `/Game/BPS_Core/Blueprints/Systems/SaveLoadSystem/Interfaces/BPI_SaveGame_SavesLists.AddSaveSlotToList_BPI` (`self.GetSettingsSaveGame`) _savegamemode _localsaveslotname))
      (if _success
        (`self.SaveSettingsSaveGame`)
        (bind _returnvalue (`GameplayStatics.SaveGameToSlot` (`local.LocalSaveGame`) (`self.MakeCombinedSaveSlotName` _savegamemode _localsaveslotname)))
        (return _returnvalue)
        (else
          _)))
    (:`Is Not Valid`
      _))
  (return false))

(fn `SaveLevelData`
  (params (SaveGame :type "SaveGame Object Reference") (LevelName :type Name))
  (returns (Success :type Boolean))
  (locals (LocalSaveGame :type "SaveGame Object Reference") (LocalSavedActors :type "Array of Actor Object Reference") (LocalLevelName :type Name))
  (bind _localsavegame (`local.LocalSaveGame`))
  ;[1 1 1] Save current level data.
  (bind _output_get (set `local.LocalSaveGame` SaveGame))
  (set `local.LocalLevelName` LevelName)
  (message `/Game/BPS_Core/Blueprints/Systems/SaveLoadSystem/Interfaces/BPI_SaveGame_Base.ClearTempLevelData_BPI` _output_get)
  (bind _saveactors (`/Game/BPS_Core/Blueprints/Systems/SaveLoadSystem/Libraries/BP_Library_SaveLoadSystem.FindAllSaveActors`))
  (for _array_element _saveactors
    (bind (_success _component) (message `/Game/BPS_Core/Blueprints/Systems/SaveLoadSystem/Interfaces/BPI_SaveObject.GetSaveObjectComponent_BPI` _array_element))
    (if _success
      (`KismetArrayLibrary.Array_Add` (`local.LocalSavedActors`) _array_element)
      (if (`/Game/BPS_Core/Blueprints/Systems/SaveLoadSystem/Components/BP_AC_SaveObjectComponent.CheckUseSaveID` _component)
        (bind _saveid (`/Game/BPS_Core/Blueprints/Systems/SaveLoadSystem/Components/BP_AC_SaveObjectComponent.GetSaveID` _component))
        (if (>= _saveid 0)
          (message `/Game/BPS_Core/Blueprints/Systems/SaveLoadSystem/Interfaces/BPI_SaveGame_Base.InitSaveActor_BPI` _localsavegame _array_element)
          (else
            (message `/Game/BPS_Core/Blueprints/Systems/SaveLoadSystem/Interfaces/BPI_SaveGame_Base.InitSaveActorWithID_BPI` _localsavegame _array_element _saveid))))))
  (for _array_element_2 (`local.LocalSavedActors`)
    (bind (_success_2 _component_2) (message `/Game/BPS_Core/Blueprints/Systems/SaveLoadSystem/Interfaces/BPI_SaveObject.GetSaveObjectComponent_BPI` _array_element_2))
    (`/Game/BPS_Core/Blueprints/Systems/SaveLoadSystem/Components/BP_AC_SaveObjectComponent.TryToSaveData` _component_2 (`local.LocalSaveGame`)))
  (message `/Game/BPS_Core/Blueprints/Systems/SaveLoadSystem/Interfaces/BPI_SaveGame_Base.SaveTempLevelData_BPI` (`local.LocalSaveGame`) (`local.LocalLevelName`))
  (return true))

(fn `SavePlayerTransitionSaveGame`
  (params (SaveGame :type "SaveGame Object Reference"))
  (returns (Success :type Boolean))
  ;[1 1 1] Try to save player transition save game.
  (bind _returnvalue (`GameplayStatics.SaveGameToSlot` SaveGame (`self.PlayerTransitionDataSaveSlotName`)))
  (return _returnvalue))

(fn `SaveSettingsSaveGame`
  (returns (Success :type Boolean))
  ;[1 1 1] Save settings save game to settings slot.
  (`GameplayStatics.SaveGameToSlot` (`self.GetSettingsSaveGame`) (`self.SettingsSaveSlotName`))
  (return true))

(fn `SaveTransitionActors`
  (params (SaveGame :type "SaveGame Object Reference"))
  (returns (Success :type Boolean))
  (locals (LocalSaveGame :type "SaveGame Object Reference") (LocalLevelName :type Name) (LocalSavedActors :type "Array of Actor Object Reference"))
  (bind _localsavegame (`local.LocalSaveGame`))
  (bind _transitionactors (`self.TransitionActors`))
  ;[1 1 1] Save transition actors for the transition process.
  (bind _output_get (set `local.LocalSaveGame` SaveGame))
  (set `local.LocalLevelName` (`self.TransitionActorsLevelName`))
  (message `/Game/BPS_Core/Blueprints/Systems/SaveLoadSystem/Interfaces/BPI_SaveGame_Base.ClearTempLevelData_BPI` _output_get)
  (for _array_element (`self.TransitionActors`)
    (bind (_success _component) (message `/Game/BPS_Core/Blueprints/Systems/SaveLoadSystem/Interfaces/BPI_SaveObject.GetSaveObjectComponent_BPI` _array_element))
    (if _success
      (`KismetArrayLibrary.Array_Add` (`local.LocalSavedActors`) _array_element)
      (if (`/Game/BPS_Core/Blueprints/Systems/SaveLoadSystem/Components/BP_AC_SaveObjectComponent.CheckUseSaveID` _component)
        (bind _saveid (`/Game/BPS_Core/Blueprints/Systems/SaveLoadSystem/Components/BP_AC_SaveObjectComponent.GetSaveID` _component))
        (if (>= _saveid 0)
          (message `/Game/BPS_Core/Blueprints/Systems/SaveLoadSystem/Interfaces/BPI_SaveGame_Base.InitSaveActor_BPI` _localsavegame _array_element)
          (else
            (message `/Game/BPS_Core/Blueprints/Systems/SaveLoadSystem/Interfaces/BPI_SaveGame_Base.InitSaveActorWithID_BPI` _localsavegame _array_element _saveid))))))
  (for _array_element_2 (`local.LocalSavedActors`)
    (bind (_success_2 _component_2) (message `/Game/BPS_Core/Blueprints/Systems/SaveLoadSystem/Interfaces/BPI_SaveObject.GetSaveObjectComponent_BPI` _array_element_2))
    (`/Game/BPS_Core/Blueprints/Systems/SaveLoadSystem/Components/BP_AC_SaveObjectComponent.TryToSaveData` _component_2 (`local.LocalSaveGame`)))
  (for _array_element_3 _transitionactors
    (`Actor.K2_DestroyActor` _array_element_3))
  (`KismetArrayLibrary.Array_Clear` _transitionactors)
  (message `/Game/BPS_Core/Blueprints/Systems/SaveLoadSystem/Interfaces/BPI_SaveGame_Base.SaveTempLevelData_BPI` (`local.LocalSaveGame`) (`local.LocalLevelName`))
  (return true))

(fn `SetSaveGameMode`
  (params (GameModeName :type Name) (IsMultiplayer :type Boolean))
  (returns (Success :type Boolean))
  ;[1 1 1] Set save game mode.
  (set `self.SaveGameMode` GameModeName)
  (set `self.SaveIsMultiplayer` IsMultiplayer)
  (return true))

(fn `SetTransitionActors`
  (params (TransitionActors :type "Array of Actor Object Reference"))
  (returns (Success :type Boolean))
  ;[1 1 1] Set transition actors array.
  (set `self.TransitionActors` TransitionActors)
  (return true))

(fn `SetTransitionPointHandled`
  (params (IsHandled :type Boolean))
  (returns (Success :type Boolean))
  ;[1 1 1] Set indicator that transition is handled.
  (set `self.TransitionPointIsHandled` IsHandled)
  (return true))

(fn `TryFindLastSaveGameSlot`
  (returns (Success :type Boolean) (SaveGameSlot :type String))
  ;[1 1 1] Try to find last save game slot.
  (bind (_success _saveslist) (message `/Game/BPS_Core/Blueprints/Systems/SaveLoadSystem/Interfaces/BPI_SaveGame_SavesLists.GetSavesList_BPI` (`self.GetSettingsSaveGame`) (`self.SaveGameMode`)))
  (if _success
    (bind ((`SaveGameSlots_6_7F686ACB4DC458947A5F8B91C0F8BEEB` _savegameslots)) (break `/Game/BPS_Core/Blueprints/Systems/SaveLoadSystem/Structures/STR_SavesList` _saveslist))
    (if (`KismetArrayLibrary.Array_IsValidIndex` _savegameslots)
      (return true (`|GetArrayItem` _savegameslots))
      (else
        _)))
  (return false ""))

(fn `TryFindMappedLevelName`
  (params (MappedName :type Name))
  (returns (Success :type Boolean) (LevelName :type Name))
  (bind _value (`BlueprintMapLibrary.Map_Find` (`self.MappedLevels`) MappedName))
  ;[1 1 1] Try to find game level name from the list by specific name.
  (return (!= _value "None") _value))

(fn `TryFindSaveGameObject`
  (params (GameModeName :type Name) (SaveSlotName :type String))
  (returns (Success :type Boolean) (ReturnValue :type "SaveGame Object Reference"))
  ;[1 1 1] Try to find save game object.
  (bind _returnvalue (`GameplayStatics.LoadGameFromSlot` (`self.MakeCombinedSaveSlotName` GameModeName SaveSlotName)))
  (`/Engine/EditorBlueprintResources/StandardMacros.IsValid` _returnvalue
    (:`Is Valid`
      (return true _returnvalue))
    (:`Is Not Valid`
      (return false null))))

(fn `TryLoadCurrentLevelData`
  (returns (Success :type Boolean))
  (locals (LocalSaveGame :type "SaveGame Object Reference") (LocalLevelName :type Name :default "None") (LocalTransitionPoint :type Name :default "None"))
  (bind _transitionsaveslotname (`self.TransitionSaveSlotName`))
  (bind _localsavegame (`local.LocalSaveGame`))
  (bind _locallevelname (`local.LocalLevelName`))
  ;[1 1 1] Try to load current level data.
  (bind _returnvalue (`GameplayStatics.DoesSaveGameExist` _transitionsaveslotname))
  (if _returnvalue
    (bind _returnvalue_2 (`GameplayStatics.LoadGameFromSlot` _transitionsaveslotname))
    (`/Engine/EditorBlueprintResources/StandardMacros.IsValid` _returnvalue_2
      (:`Is Valid`
        (bind _output_get (set `local.LocalSaveGame` _returnvalue_2))
        (bind (_success _levelname _transitionpoint) (message `/Game/BPS_Core/Blueprints/Systems/SaveLoadSystem/Interfaces/BPI_SaveGame_Base.GetTransitionData_BPI` _output_get))
        (if _success
          (set `local.LocalLevelName` _levelname)
          (set `local.LocalTransitionPoint` _transitionpoint)
          (bind _returnvalue_3 (`GameplayStatics.GetCurrentLevelName` true))
          (if (== (`local.LocalLevelName`) (`KismetStringLibrary.Conv_StringToName` _returnvalue_3))
            (bind _output_get_2 (set `self.CurrentSaveGame` (`local.LocalSaveGame`)))
            (bind (_success_2 _gamemodename _saveslotname _ismultiplayer) (message `/Game/BPS_Core/Blueprints/Systems/SaveLoadSystem/Interfaces/BPI_SaveGame_Base.GetSaveSlotData_BPI` _output_get_2))
            (if _success_2
              (set `self.SaveGameMode` _gamemodename)
              (set `self.CurrentSaveSlotName` _saveslotname)
              (set `self.SaveIsMultiplayer` _ismultiplayer)
              (bind _success_3 (message `/Game/BPS_Core/Blueprints/Systems/SaveLoadSystem/Interfaces/BPI_SaveGame_Base.HasLevelData_BPI` _localsavegame _locallevelname))
              (if _success_3
                (bind _success_4 (`self.LoadLevelData` _localsavegame _locallevelname))
                (if _success_4
                  _
                  (else
                    (return false)))
                (else
                  (`self.LoadPlayersData` _localsavegame)))
              (`self.LoadTransitionActors` _localsavegame (`local.LocalTransitionPoint`))
              (`GameplayStatics.DeleteGameInSlot` (`self.TransitionSaveSlotName`))
              (return true))
            (else
              (return false)))
          (else
            (return false))))
      (:`Is Not Valid`
        (return false)))
    (else
      (return false))))

(fn `TryLoadGameFromSlot`
  (params (SlotName :type String))
  (returns (Success :type Boolean))
  ;[1 1 1] Try to load game from slot.
  (bind _returnvalue (`GameplayStatics.LoadGameFromSlot` (`self.MakeCombinedSaveSlotName` (`self.SaveGameMode`) SlotName)))
  (`/Engine/EditorBlueprintResources/StandardMacros.IsValid` _returnvalue
    (:`Is Valid`
      (bind _output_get (set `self.CurrentSaveGame` _returnvalue))
      (set `self.CurrentSaveSlotName` SlotName)
      (bind (_success _levelname) (message `/Game/BPS_Core/Blueprints/Systems/SaveLoadSystem/Interfaces/BPI_SaveGame_Base.GetTransitionData_BPI` _output_get))
      (if _success
        (`GameplayStatics.SaveGameToSlot` _output_get (`self.TransitionSaveSlotName`))
        (`GameplayStatics.OpenLevel` _levelname true (select `bool` (`self.SaveIsMultiplayer`) :`true` "listen"))
        (return true)
        (else
          (return false))))
    (:`Is Not Valid`
      (return false))))

(fn `TryLoadLastSave`
  (returns (Success :type Boolean))
  ;[1 1 1] Try to load last save game.
  (bind (_success _savegameslot) (`self.TryFindLastSaveGameSlot`))
  (if _success
    (bind _success_2 (`self.TryLoadGameFromSlot` _savegameslot))
    (return _success_2)
    (else
      (return false))))

(fn `TryOpenMainMenuLevel`
  (returns (Success :type Boolean))
  ;[1 1 1] Try to open main menu level.
  (bind (_success _levelname) (`self.TryFindMappedLevelName` "Map_Village_BackUpMenu"))
  (if _success
    (`GameplayStatics.OpenLevel` _levelname)
    (return true)
    (else
      (return false))))

(fn `TrySaveGameToSlot`
  (params (SaveSlotName :type String))
  (returns (Success :type Boolean))
  (locals (LocalCurrentLevel :type Name :default "None"))
  (bind _currentsavegame (`self.CurrentSaveGame`))
  ;[1 1 1] Try to save game to slot. Also saves current level data.
  (set `self.CurrentSaveSlotName` SaveSlotName)
  (`/Engine/EditorBlueprintResources/StandardMacros.IsValid` (`self.CurrentSaveGame`)
    (:`Is Valid`
      _)
    (:`Is Not Valid`
      (bind (_success _savegame) (`self.CreateNewSaveGame`))
      (if _success
        (set `self.CurrentSaveGame` _savegame)
        (else
          (return false)))))
  (bind _returnvalue (`GameplayStatics.GetCurrentLevelName` true))
  (bind _output_get (set `local.LocalCurrentLevel` (`KismetStringLibrary.Conv_StringToName` _returnvalue)))
  (message `/Game/BPS_Core/Blueprints/Systems/SaveLoadSystem/Interfaces/BPI_SaveGame_Base.SetTransitionData_BPI` _currentsavegame _output_get "None")
  (`self.SaveLevelData` _currentsavegame _output_get)
  (bind _success_2 (`self.SaveGameToSlot` (`self.CurrentSaveGame`) (`self.CurrentSaveSlotName`)))
  (return _success_2))

(fn `TryStartNewGame`
  (params (LevelName :type Name))
  (returns (Success :type Boolean))
  (locals (LocalLevelName :type Name))
  (bind _currentsavegame (`self.CurrentSaveGame`))
  ;[1 1 1] Try to start new game and open specific level.
  (set `local.LocalLevelName` LevelName)
  (bind (_success _savegame) (`self.CreateNewSaveGame`))
  (if _success
    (set `self.CurrentSaveGame` _savegame)
    (bind _output_get (set `self.CurrentSaveSlotName` (`self.DefaultSaveSlotName`)))
    (bind _success_2 (`self.TrySaveGameToSlot` _output_get))
    (if _success_2
      (bind _success_3 (message `/Game/BPS_Core/Blueprints/Systems/SaveLoadSystem/Interfaces/BPI_SaveGame_Base.SetTransitionData_BPI` (`self.CurrentSaveGame`) (`local.LocalLevelName`) "None"))
      (if _success_3
        (`self.SaveGameToSlot` _currentsavegame (`self.CurrentSaveSlotName`))
        (`GameplayStatics.SaveGameToSlot` _currentsavegame (`self.TransitionSaveSlotName`))
        (`GameplayStatics.OpenLevel` (`local.LocalLevelName`) true (select `bool` (`self.SaveIsMultiplayer`) :`true` "listen"))
        (return true)
        (else
          _))))
  (return false))

(fn `TryTransitToLevel`
  (params (LevelName :type Name) (TransitionPoint :type Name))
  (returns (Success :type Boolean))
  (locals (LocalLevelName :type Name) (LocalTransitionPoint :type Name))
  (bind _currentsavegame (`self.CurrentSaveGame`))
  (bind _currentsavegame_2 (`self.CurrentSaveGame`))
  ;[1 1 1] Try to transit to specific level.
  (set `local.LocalLevelName` LevelName)
  (set `local.LocalTransitionPoint` TransitionPoint)
  (if (`KismetSystemLibrary.IsValid` _currentsavegame)
    (bind (_success _gamemodename _saveslotname) (message `/Game/BPS_Core/Blueprints/Systems/SaveLoadSystem/Interfaces/BPI_SaveGame_Base.GetSaveSlotData_BPI` _currentsavegame))
    (if _success
      (bind _output_get (set `self.CurrentSaveSlotName` _saveslotname))
      (`self.SaveTransitionActors` (`self.CurrentSaveGame`) :!label _label)
      (bind _success_2 (`self.TrySaveGameToSlot` _output_get))
      (if _success_2
        (bind _success_3 (message `/Game/BPS_Core/Blueprints/Systems/SaveLoadSystem/Interfaces/BPI_SaveGame_Base.SetTransitionData_BPI` (`self.CurrentSaveGame`) (`local.LocalLevelName`) (`local.LocalTransitionPoint`)))
        (if _success_3
          (`self.SaveGameToSlot` _currentsavegame_2 (`self.CurrentSaveSlotName`))
          (`GameplayStatics.SaveGameToSlot` _currentsavegame_2 (`self.TransitionSaveSlotName`))
          (`GameplayStatics.OpenLevel` (`local.LocalLevelName`) true (select `bool` (`self.SaveIsMultiplayer`) :`true` "listen"))
          (return true)
          (else
            _))))
    (else
      (bind (_success_4 _savegame) (`self.CreateNewSaveGame`))
      (if _success_4
        (set `self.CurrentSaveGame` _savegame)
        (set `self.CurrentSaveSlotName` (`self.DefaultSaveSlotName`))
        (goto _label)
        (else
          _))))
  (return false))