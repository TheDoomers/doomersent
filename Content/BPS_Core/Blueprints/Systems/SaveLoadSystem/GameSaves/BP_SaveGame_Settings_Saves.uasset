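; BP_SaveGame_Settings_Saves is a save game object that keeps lists of save slot names grouped by game mode.
; Interface functions look up, add to and remove from SavesLists by GameModeName, writing each edited struct back by index.
; Adding moves the slot to the front without duplicates, or creates the game mode's entry if missing but then returns false.
; CreateSavesList_BPI is a stub that only returns failure.
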(fn `AddSaveSlotToList_BPI`
  (params (GameModeName :type Name) (SaveSlotName :type String))
  (returns (Success :type Boolean))
  (locals (LocalGameModeName :type Name :default "None") (LocalSaveSlot :type String) (LocalSaveSlots :type "Array of String"))
  (bind _localsaveslot (`local.LocalSaveSlot`))
  ;[1 1 1] Add save to the save list of specific game mode.
  (set `local.LocalGameModeName` GameModeName)
  (set `local.LocalSaveSlot` SaveSlotName)
  (for (_array_element _array_index) (`self.SavesLists`)
    (bind (_gamemodename _savegameslots) (break `/Game/BPS_Core/Blueprints/Systems/SaveLoadSystem/Structures/STR_SavesList` _array_element))
    (if (== _gamemodename (`local.LocalGameModeName`))
      (bind _output_get (set `local.LocalSaveSlots` _savegameslots))
      (`KismetArrayLibrary.Array_RemoveItem` _output_get _localsaveslot)
      (`KismetArrayLibrary.Array_Insert` _output_get _localsaveslot)
      (`KismetArrayLibrary.Array_Set` (`self.SavesLists`) _array_index (make `/Game/BPS_Core/Blueprints/Systems/SaveLoadSystem/Structures/STR_SavesList` (`local.LocalGameModeName`) _output_get))
      (return true)))
  (`KismetArrayLibrary.Array_Add` (`self.SavesLists`) (make `/Game/BPS_Core/Blueprints/Systems/SaveLoadSystem/Structures/STR_SavesList` (`local.LocalGameModeName`) (`|MakeArray` (`local.LocalSaveSlot`))))
  (return false))

(fn `CreateSavesList_BPI`
  (params (GameModeName :type Name))
  (returns (Success :type Boolean) (SavesList :type "/Game/BPS_Core/Blueprints/Systems/SaveLoadSystem/Structures/STR_SavesList Structure"))
  (return false))

(fn `GetSavesList_BPI`
  (params (GameModeName :type Name))
  (returns (Success :type Boolean) (SavesList :type "/Game/BPS_Core/Blueprints/Systems/SaveLoadSystem/Structures/STR_SavesList Structure"))
  ;[1 1 1] Returns saves list of specific game mode.
  (for _array_element (`self.SavesLists`)
    (if (== (`.GameModeName_7_97DEEEB844919F6828FD8E8F63BE50E4` (break `/Game/BPS_Core/Blueprints/Systems/SaveLoadSystem/Structures/STR_SavesList` _array_element)) GameModeName)
      (return true _array_element)))
  (return false))

(fn `RemoveSaveSlotFromList_BPI`
  (params (GameModeName :type Name) (SaveSlotName :type String))
  (returns (Success :type Boolean))
  (locals (LocalGameModeName :type Name) (LocalSaveSlot :type String) (LocalSaveSlots :type "Array of String"))
  ;[1 1 1] Remove save slot from the saves list for specific game mode.
  (set `local.LocalGameModeName` GameModeName)
  (set `local.LocalSaveSlot` SaveSlotName)
  (for (_array_element _array_index) (`self.SavesLists`)
    (bind (_gamemodename _savegameslots) (break `/Game/BPS_Core/Blueprints/Systems/SaveLoadSystem/Structures/STR_SavesList` _array_element))
    (if (== _gamemodename (`local.LocalGameModeName`))
      (bind _output_get (set `local.LocalSaveSlots` _savegameslots))
      (`KismetArrayLibrary.Array_RemoveItem` _output_get (`local.LocalSaveSlot`))
      (`KismetArrayLibrary.Array_Set` (`self.SavesLists`) _array_index (make `/Game/BPS_Core/Blueprints/Systems/SaveLoadSystem/Structures/STR_SavesList` (`local.LocalGameModeName`) _output_get))
      (return true)))
  (return false))