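; Base save game object that stores slot info, date/time, level transition data and per-level actor save data behind BPI interface functions.
; Actors receive save IDs, either given or from a running counter, through their save object component and are mapped by ID.
; A temporary ID-to-data map holds working actor data, which is saved into or loaded from a map keyed by level name.
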(fn `ClearLevelData_BPI`
  (params (LevelName :type Name))
  (returns (Success :type Boolean))
  ;[1 1 1] Clear level data.
  (`BlueprintMapLibrary.Map_Remove` (`self.LevelsActorsData`) LevelName)
  (return true))

(fn `ClearTempLevelData_BPI`
  (returns (Success :type Boolean))
  ;[1 1 1] Clear temporal level data.
  (set `self.SpawnedActorsCount` 0)
  (`BlueprintMapLibrary.Map_Clear` (`self.SavedActors`))
  (`BlueprintMapLibrary.Map_Clear` (`self.SavedActorsData`))
  (return true))

(fn `GetActorSaveData_BPI`
  (params (SaveID :type Integer))
  (returns (Success :type Boolean) (SaveData :type "/Game/BPS_Core/Blueprints/Systems/SaveLoadSystem/Structures/STR_SaveData_Actor Structure"))
  (bind (_value _returnvalue) (`BlueprintMapLibrary.Map_Find` (`self.SavedActorsData`) SaveID))
  ;[1 1 1] Returns actor save data.
  (return _returnvalue _value))

(fn `GetDateTime_BPI`
  (returns (Success :type Boolean) (DateTime :type "DateTime Structure"))
  ;[1 1 1] Returns value of the date time variable.
  (return true (`self.DateTime`)))

(fn `GetSavedActor_BPI`
  (params (SaveID :type Integer))
  (returns (Success :type Boolean) (SavedActor :type "Actor Object Reference"))
  (bind (_value _returnvalue) (`BlueprintMapLibrary.Map_Find` (`self.SavedActors`) SaveID))
  ;[1 1 1] Try to find saved actor by specific save ID.
  (return _returnvalue _value))

(fn `GetSavedActorsData_BPI`
  (returns (Success :type Boolean) (SaveIDs :type "Array of Integer") (SaveData :type "Array of /Game/BPS_Core/Blueprints/Systems/SaveLoadSystem/Structures/STR_SaveData_Actor Structure"))
  (bind _savedactorsdata (`self.SavedActorsData`))
  ;[1 1 1] Returns saved actors data arrays.
  (bind _keys (`BlueprintMapLibrary.Map_Keys` _savedactorsdata))
  (bind _values (`BlueprintMapLibrary.Map_Values` _savedactorsdata))
  (return true _keys _values))

(fn `GetSaveSlotData_BPI`
  (returns (Success :type Boolean) (GameModeName :type Name) (SaveSlotName :type String) (IsMultiplayer :type Boolean))
  ;[1 1 1] Returns save slot data.
  (return true (`self.GameModeName`) (`self.SaveSlotName`) (`self.IsMultiplayer`)))

(fn `GetTransitionData_BPI`
  (returns (Success :type Boolean) (LevelName :type Name) (TransitionPoint :type Name))
  ;[1 1 1] Returns transition data.
  (return true (`self.CurrentLevelName`) (`self.CurrentTransitionPoint`)))

(fn `HasLevelData_BPI`
  (params (LevelName :type Name))
  (returns (Success :type Boolean))
  ;[1 1 1] Returns true if save game has data for specific level.
  (return (`.ReturnValue` (`BlueprintMapLibrary.Map_Find` (`self.LevelsActorsData`) LevelName))))

(fn `InitSaveActor_BPI`
  (params (SaveActor :type "Actor Object Reference"))
  (returns (Success :type Boolean))
  (locals (LocalSaveActor :type "Actor Object Reference") (LocalSaveID :type Integer))
  (bind _spawnedactorscount (`self.SpawnedActorsCount`))
  (bind _output_get (set `local.LocalSaveActor` SaveActor))
  (bind _output_get_2 (set `local.LocalSaveID` _spawnedactorscount))
  (set `self.SpawnedActorsCount` (+ _spawnedactorscount 1))
  (`self.InitSaveActorWithID_BPI` _output_get _output_get_2)
  (return true))

(fn `InitSaveActorWithID_BPI`
  (params (SaveActor :type "Actor Object Reference") (SaveID :type Integer))
  (returns (Success :type Boolean))
  (locals (LocalSaveActor :type "Actor Object Reference") (LocalSaveID :type Integer))
  (bind _localsaveid (`local.LocalSaveID`))
  (bind _output_get (set `local.LocalSaveActor` SaveActor))
  (set `local.LocalSaveID` SaveID)
  (bind (_success _component) (message `/Game/BPS_Core/Blueprints/Systems/SaveLoadSystem/Interfaces/BPI_SaveObject.GetSaveObjectComponent_BPI` _output_get))
  (if _success
    (`/Game/BPS_Core/Blueprints/Systems/SaveLoadSystem/Components/BP_AC_SaveObjectComponent.SetSaveID` _component _localsaveid)
    (`BlueprintMapLibrary.Map_Add` (`self.SavedActors`) _localsaveid (`local.LocalSaveActor`))
    (return true)))

(fn `LoadTempLevelData_BPI`
  (params (LevelName :type Name))
  (returns (Success :type Boolean))
  (locals (LocalLevelActorsData :type "/Game/BPS_Core/Blueprints/Systems/SaveLoadSystem/Structures/STR_SaveLevelData_Actors Structure"))
  (bind (_value _returnvalue) (`BlueprintMapLibrary.Map_Find` (`self.LevelsActorsData`) LevelName))
  ;[1 1 1] Load temporal level data.
  (`self.ClearTempLevelData_BPI`)
  (if _returnvalue
    (bind _output_get (set `local.LocalLevelActorsData` _value))
    (set `self.SavedActorsData` (`.ActorsData_7_EF7EAE264C860D3ADCC6EFAB0C04B473` (break `/Game/BPS_Core/Blueprints/Systems/SaveLoadSystem/Structures/STR_SaveLevelData_Actors` _output_get)))
    (return true)
    (else
      (return false))))

(fn `SaveTempLevelData_BPI`
  (params (LevelName :type Name))
  (returns (Success :type Boolean))
  ;[1 1 1] Save temporal level data.
  (`BlueprintMapLibrary.Map_Add` (`self.LevelsActorsData`) LevelName (make `/Game/BPS_Core/Blueprints/Systems/SaveLoadSystem/Structures/STR_SaveLevelData_Actors` LevelName (`self.SavedActorsData`)))
  (return true))

(fn `SetActorSaveData_BPI`
  (params (SaveID :type Integer) (SaveData :type "/Game/BPS_Core/Blueprints/Systems/SaveLoadSystem/Structures/STR_SaveData_Actor Structure"))
  (returns (Success :type Boolean))
  ;[1 1 1] Set actor save data.
  (`BlueprintMapLibrary.Map_Add` (`self.SavedActorsData`) SaveID SaveData)
  (return true))

(fn `SetDateTime_BPI`
  (params (DateTime :type "DateTime Structure"))
  (returns (Success :type Boolean))
  ;[1 1 1] Set value of the date time variable.
  (set `self.DateTime` DateTime)
  (return true))

(fn `SetSaveSlotData_BPI`
  (params (GameModeName :type Name) (SaveSlotName :type String) (IsMultiplayer :type Boolean))
  (returns (Success :type Boolean))
  ;[1 1 1] Set save slot data.
  (set `self.GameModeName` GameModeName)
  (set `self.SaveSlotName` SaveSlotName)
  (set `self.IsMultiplayer` IsMultiplayer)
  (return true))

(fn `SetTransitionData_BPI`
  (params (LevelName :type Name) (TransitionPoint :type Name))
  (returns (Success :type Boolean))
  ;[1 1 1] Set transition data.
  (set `self.CurrentLevelName` LevelName)
  (set `self.CurrentTransitionPoint` TransitionPoint)
  (return true))