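; Base actor for surface overriders in the footstep system, configuring its collision to act as query-only volumes or shapes.
; On construction and again at BeginPlay, it loops over all its primitive components and makes them query-only.
; Each component gets the dedicated surface overrider object type and ignores every channel, so it blocks and overlaps nothing while carrying that type for queries.
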(event `self.ReceiveBeginPlay`
  ;[1 1 1] Init collision settings on begin play.
  (`parent.ReceiveBeginPlay`)
  (`self.InitCollisionSettings`))

(fn `InitCollisionSettings`
  ;[1 1 1] Init collision settings for primitive collision components.
  (for _array_element (`self.K2_GetComponentsByClass` "/Script/Engine.PrimitiveComponent")
    (`PrimitiveComponent.SetCollisionEnabled` _array_element "QueryOnly")
    (`PrimitiveComponent.SetCollisionObjectType` _array_element (`/Game/BPS_Core/Blueprints/Systems/FootstepSystem/Libraries/BP_Library_FootstepSystem.GetSurfaceOverriderObjectType`))
    (`PrimitiveComponent.SetCollisionResponseToAllChannels` _array_element "ECR_Ignore")))

(fn `UserConstructionScript`
  ;[1 1 1] Init collision settings.
  (`parent.UserConstructionScript`)
  (`self.InitCollisionSettings`))