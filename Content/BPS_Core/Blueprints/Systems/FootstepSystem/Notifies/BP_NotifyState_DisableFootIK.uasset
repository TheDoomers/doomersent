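; Animation notify state that switches foot IK off for the duration of an animation window in the footstep system.
; On begin it finds every BP_AC_FootstepComponent on the mesh owner and calls DisableFootIK, and on end it calls EnableFootIK on them.
; Both events act only when the owner is valid, and the notify displays as "Disable Foot IK".
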(fn `GetNotifyName`
  (returns (ReturnValue :type String))
  ;[1 1 1] Update notify name.
  (return "Disable Foot IK"))

(fn `Received_NotifyBegin`
  (params (MeshComp :type "SkeletalMeshComponent Object Reference") (Animation :type "AnimSequenceBase Object Reference") (TotalDuration :type "Float (single-precision)") (EventReference :type "AnimNotifyEventReference Structure (by ref)"))
  (returns (ReturnValue :type Boolean))
  (locals (LocalFootstepComponents :type "Array of /Game/BPS_Core/Blueprints/Systems/FootstepSystem/Components/BP_AC_FootstepComponent Object Reference"))
  (bind _returnvalue (`ActorComponent.GetOwner` MeshComp))
  ;[1 1 1] Disables foot ik on notify begin.
  (`/Engine/EditorBlueprintResources/StandardMacros.IsValid` _returnvalue
    (:`Is Valid`
      (bind _output_get (set `local.LocalFootstepComponents` (`Actor.K2_GetComponentsByClass` _returnvalue "/Game/BPS_Core/Blueprints/Systems/FootstepSystem/Components/BP_AC_FootstepComponent.BP_AC_FootstepComponent_C")))
      (for _array_element _output_get
        (`/Game/BPS_Core/Blueprints/Systems/FootstepSystem/Components/BP_AC_FootstepComponent.DisableFootIK` _array_element))
      (return true))))

(fn `Received_NotifyEnd`
  (params (MeshComp :type "SkeletalMeshComponent Object Reference") (Animation :type "AnimSequenceBase Object Reference") (EventReference :type "AnimNotifyEventReference Structure (by ref)"))
  (returns (ReturnValue :type Boolean))
  (locals (LocalFootstepComponents :type "Array of /Game/BPS_Core/Blueprints/Systems/FootstepSystem/Components/BP_AC_FootstepComponent Object Reference"))
  (bind _returnvalue (`ActorComponent.GetOwner` MeshComp))
  ;[1 1 1] Enables foot ik on notify end.
  (`/Engine/EditorBlueprintResources/StandardMacros.IsValid` _returnvalue
    (:`Is Valid`
      (bind _output_get (set `local.LocalFootstepComponents` (`Actor.K2_GetComponentsByClass` _returnvalue "/Game/BPS_Core/Blueprints/Systems/FootstepSystem/Components/BP_AC_FootstepComponent.BP_AC_FootstepComponent_C")))
      (for _array_element _output_get
        (`/Game/BPS_Core/Blueprints/Systems/FootstepSystem/Components/BP_AC_FootstepComponent.EnableFootIK` _array_element))
      (return true))))