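; Animation notify that triggers footsteps from character animations at a configured foot socket and footstep type.
; When the mesh is visible, it calls TryToPlayFootstep on every BP_AC_FootstepComponent of the mesh owner, passing sound and effect toggles.
; In the editor it also plays a 2D preview sound, either a custom override or a default chosen by footstep type.
; The notify's display name includes the foot socket.
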(fn `GetNotifyName`
  (returns (ReturnValue :type String))
  ;[1 1 1] Display notify name.
  (return (`KismetStringLibrary.Concat_StrStr` "Footstep_" (`KismetStringLibrary.Conv_NameToString` (`self.FootSocket`)))))

(fn `PlayPreviewSound`
  (bind _previewsound (`self.PreviewSound`))
  ;[1 1 1] Play preview sound in editor.
  (if (`/Game/BPS_Core/Blueprints/Systems/CoreSystem/Libraries/BP_Library_CoreFunctions.RunInEditor`)
    (if (`self.PlaySounds`)
      (`/Engine/EditorBlueprintResources/StandardMacros.IsValid` _previewsound
        (:`Is Valid`
          (`GameplayStatics.PlaySound2D` _previewsound 1.0 1.0 0.0 null null))
        (:`Is Not Valid`
          (`GameplayStatics.PlaySound2D` (select `/Game/BPS_Core/Blueprints/Systems/FootstepSystem/Enums/E_FootstepType` (`self.FootstepType`) :`NewEnumerator7` (`self.PreviewSoundDefault`) :`NewEnumerator8` (`self.PreviewSoundWalk`) :`NewEnumerator1` (`self.PreviewSoundJog`) :`NewEnumerator2` (`self.PreviewSoundRun`) :`NewEnumerator5` (`self.PreviewSoundJump`) :`NewEnumerator6` (`self.PreviewSoundLand`)) 1.0 1.0 0.0 null null))))))

(fn `Received_Notify`
  (params (MeshComp :type "SkeletalMeshComponent Object Reference") (Animation :type "AnimSequenceBase Object Reference") (EventReference :type "AnimNotifyEventReference Structure (by ref)"))
  (returns (ReturnValue :type Boolean))
  (bind _returnvalue (`ActorComponent.GetOwner` MeshComp))
  ;[1 1 1] Call footstep process for each footstep components.
  (`self.PlayPreviewSound`)
  (if (`SceneComponent.IsVisible` MeshComp)
    (`/Engine/EditorBlueprintResources/StandardMacros.IsValid` _returnvalue
      (:`Is Valid`
        (for _array_element (`Actor.K2_GetComponentsByClass` _returnvalue "/Game/BPS_Core/Blueprints/Systems/FootstepSystem/Components/BP_AC_FootstepComponent.BP_AC_FootstepComponent_C")
          (`/Game/BPS_Core/Blueprints/Systems/FootstepSystem/Components/BP_AC_FootstepComponent.TryToPlayFootstep` _array_element (`self.FootSocket`) (`self.FootstepType`) (`self.PlaySounds`) (`self.SpawnEffects`)))
        (return true)))))