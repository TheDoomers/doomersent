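; Blueprint function library of shared helpers for the footstep system built around BP_AC_FootstepComponent.
; Config getters read that component's class defaults for surface overrider and water object types and named surface types.
; Lookups find a component by foot socket, type data by footstep type, and sound, effect or decal data by mapping surface names to surface types, falling back to "Default" entries.
; It also validates preset handles and wraps two-leg pelvis translation.
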(fn `FindFootstepComponent`
  (params (TargetActor :type "Actor Object Reference") (FootSocket :type Name))
  (returns (Success :type Boolean) (Component :type "/Game/BPS_Core/Blueprints/Systems/FootstepSystem/Components/BP_AC_FootstepComponent Object Reference"))
  (locals (LocalFootstepComponent :type "Array of /Game/BPS_Core/Blueprints/Systems/FootstepSystem/Components/BP_AC_FootstepComponent Object Reference"))
  ;[1 1 1] Try to find footstep component with specific foot socket.
  (bind _output_get (set `local.LocalFootstepComponent` (`Actor.K2_GetComponentsByClass` TargetActor "/Game/BPS_Core/Blueprints/Systems/FootstepSystem/Components/BP_AC_FootstepComponent.BP_AC_FootstepComponent_C")))
  (for _array_element _output_get
    (if (== (`/Game/BPS_Core/Blueprints/Systems/FootstepSystem/Components/BP_AC_FootstepComponent.FootSocket` _array_element) FootSocket)
      (return true _array_element)))
  (return false null))

(fn `FindFootstepDecalData`
  (params (FootstepDecalsData :type "Map of Name to /Game/BPS_Core/Blueprints/Systems/FootstepSystem/Structures/STR_FootstepDecalData Structure") (SurfaceType :type "EPhysicalSurface Enum" :default "SurfaceType_Default"))
  (returns (Success :type Boolean) (OutData :type "/Game/BPS_Core/Blueprints/Systems/FootstepSystem/Structures/STR_FootstepDecalData Structure"))
  (bind _namedsurfacetypes (`self.GetNamedSurfaceTypes` null))
  (bind (_value _returnvalue) (`BlueprintMapLibrary.Map_Find` FootstepDecalsData "Default"))
  ;[1 1 1] Try to find decal data from footstep type data for target surface type.
  (bind _keys (`BlueprintMapLibrary.Map_Keys` FootstepDecalsData))
  (bind _values (`BlueprintMapLibrary.Map_Values` FootstepDecalsData))
  (for (_array_element _array_index) _keys
    (if (`BlueprintMapLibrary.Map_Contains` _namedsurfacetypes _array_element)
      (if (`|EnumEquality` SurfaceType (`BlueprintMapLibrary.Map_Find` _namedsurfacetypes _array_element))
        (return true (`|GetArrayItem` _values _array_index)))))
  (return _returnvalue _value))

(fn `FindFootstepEffectData`
  (params (FootstepEffectsData :type "Map of Name to /Game/BPS_Core/Blueprints/Systems/FootstepSystem/Structures/STR_FootstepEffectData Structure") (SurfaceType :type "EPhysicalSurface Enum" :default "SurfaceType_Default"))
  (returns (Success :type Boolean) (OutData :type "/Game/BPS_Core/Blueprints/Systems/FootstepSystem/Structures/STR_FootstepEffectData Structure"))
  (bind _namedsurfacetypes (`self.GetNamedSurfaceTypes` null))
  (bind (_value _returnvalue) (`BlueprintMapLibrary.Map_Find` FootstepEffectsData "Default"))
  ;[1 1 1] Try to find effect data from footstep type data for target surface type.
  (bind _keys (`BlueprintMapLibrary.Map_Keys` FootstepEffectsData))
  (bind _values (`BlueprintMapLibrary.Map_Values` FootstepEffectsData))
  (for (_array_element _array_index) _keys
    (if (`BlueprintMapLibrary.Map_Contains` _namedsurfacetypes _array_element)
      (if (`|EnumEquality` SurfaceType (`BlueprintMapLibrary.Map_Find` _namedsurfacetypes _array_element))
        (return true (`|GetArrayItem` _values _array_index)))))
  (return _returnvalue _value))

(fn `FindFootstepSoundData`
  (params (FootstepSoundsData :type "Map of Name to /Game/BPS_Core/Blueprints/Systems/FootstepSystem/Structures/STR_FootstepSoundData Structure") (SurfaceType :type "EPhysicalSurface Enum" :default "SurfaceType_Default"))
  (returns (Success :type Boolean) (OutData :type "/Game/BPS_Core/Blueprints/Systems/FootstepSystem/Structures/STR_FootstepSoundData Structure"))
  (bind _namedsurfacetypes (`self.GetNamedSurfaceTypes` null))
  (bind (_value _returnvalue) (`BlueprintMapLibrary.Map_Find` FootstepSoundsData "Default"))
  ;[1 1 1] Try to find sound data from footstep type data for target surface type.
  (bind _keys (`BlueprintMapLibrary.Map_Keys` FootstepSoundsData))
  (bind _values (`BlueprintMapLibrary.Map_Values` FootstepSoundsData))
  (for (_array_element _array_index) _keys
    (if (`BlueprintMapLibrary.Map_Contains` _namedsurfacetypes _array_element)
      (if (`|EnumEquality` SurfaceType (`BlueprintMapLibrary.Map_Find` _namedsurfacetypes _array_element))
        (return true (`|GetArrayItem` _values _array_index)))))
  (return _returnvalue _value))

(fn `FindFootstepTypeData`
  (params (FootstepsData :type "Map of Name to /Game/BPS_Core/Blueprints/Systems/FootstepSystem/Structures/STR_FootstepTypeData Structure") (FootstepType :type "/Game/BPS_Core/Blueprints/Systems/FootstepSystem/Enums/E_FootstepType Enum" :default "NewEnumerator7"))
  (returns (Success :type Boolean) (FootstepTypeData :type "/Game/BPS_Core/Blueprints/Systems/FootstepSystem/Structures/STR_FootstepTypeData Structure"))
  (bind (_value _returnvalue) (`BlueprintMapLibrary.Map_Find` FootstepsData "Default"))
  ;[1 1 1] Try to find footstep type data from footstep data list depending on footstep type.
  (bind _values (`BlueprintMapLibrary.Map_Values` FootstepsData))
  (for _array_element _values
    (if (`|EnumEquality` FootstepType (`.FootstepType_2_4AEA124342BB7C77AC2CF1A8C4270B4D` (break `/Game/BPS_Core/Blueprints/Systems/FootstepSystem/Structures/STR_FootstepTypeData` _array_element)))
      (return true _array_element)))
  (return _returnvalue _value))

(fn `GetNamedSurfaceTypes`
  (returns (NamedSurfaceTypes :type "Map of Name to EPhysicalSurface Enum"))
  ;[1 1 1] Returns named surface types list from the footstep system configs.
  (return (`.NamedSurfaceTypes` (defaults `/Game/BPS_Core/Blueprints/Systems/FootstepSystem/Components/BP_AC_FootstepComponent` "/Game/BPS_Core/Blueprints/Systems/FootstepSystem/Components/BP_AC_FootstepComponent.BP_AC_FootstepComponent_C"))))

(fn `GetSurfaceOverriderObjectType`
  (returns (SurfaceOverriderObjectType :type "ECollisionChannel Enum"))
  ;[1 1 1] Returns surface overrider object type from the footstep system configs.
  (return (`.SurfaceOverriderObjectType` (defaults `/Game/BPS_Core/Blueprints/Systems/FootstepSystem/Components/BP_AC_FootstepComponent` "/Game/BPS_Core/Blueprints/Systems/FootstepSystem/Components/BP_AC_FootstepComponent.BP_AC_FootstepComponent_C"))))

(fn `GetSurfaceOverriderObjectTypeQuery`
  (returns (SurfaceOverriderTypeQuery :type "EObjectTypeQuery Enum"))
  ;[1 1 1] Returns surface overrider object type query from the footstep system configs.
  (return (`.SurfaceOverriderObjectTypeQuery` (defaults `/Game/BPS_Core/Blueprints/Systems/FootstepSystem/Components/BP_AC_FootstepComponent` "/Game/BPS_Core/Blueprints/Systems/FootstepSystem/Components/BP_AC_FootstepComponent.BP_AC_FootstepComponent_C"))))

(fn `GetTwoLegsPelvisBoneTranslation`
  (params (LeftFootstepComponent :type "/Game/BPS_Core/Blueprints/Systems/FootstepSystem/Components/BP_AC_FootstepComponent Object Reference") (RightFootstepComponent :type "/Game/BPS_Core/Blueprints/Systems/FootstepSystem/Components/BP_AC_FootstepComponent Object Reference"))
  (returns (Success :type Boolean) (PelvisTranslation :type "Float (double-precision)"))
  ;[1 1 1] Returns the translation of the pelvis bone for a character with two legs.
  (bind (_success _pelvistranslation) (`/Game/BPS_Core/Blueprints/Systems/FootstepSystem/Components/BP_AC_FootstepComponent.GetTwoLegsPelvisBoneTranslation` LeftFootstepComponent RightFootstepComponent))
  (return _success _pelvistranslation))

(fn `GetWaterObjectType`
  (returns (WaterObjectType :type "ECollisionChannel Enum"))
  ;[1 1 1] Returns water object type from the footstep system configs.
  (return (`.WaterObjectType` (defaults `/Game/BPS_Core/Blueprints/Systems/FootstepSystem/Components/BP_AC_FootstepComponent` "/Game/BPS_Core/Blueprints/Systems/FootstepSystem/Components/BP_AC_FootstepComponent.BP_AC_FootstepComponent_C"))))

(fn `GetWaterObjectTypeQuery`
  (returns (WaterTypeQuery :type "EObjectTypeQuery Enum"))
  ;[1 1 1] Returns water object type query from the footstep system configs.
  (return (`.WaterObjectTypeQuery` (defaults `/Game/BPS_Core/Blueprints/Systems/FootstepSystem/Components/BP_AC_FootstepComponent` "/Game/BPS_Core/Blueprints/Systems/FootstepSystem/Components/BP_AC_FootstepComponent.BP_AC_FootstepComponent_C"))))

(fn `PresetIsValid`
  (params (Handle :type "DataTableRowHandle Structure"))
  (returns (Result :type Boolean))
  (bind (_datatable _rowname) (break `DataTableRowHandle` Handle))
  ;[1 1 1] Returns true, if footstep preset handle is valid.
  (return (and (`KismetSystemLibrary.IsValid` _datatable) (!= _rowname "None"))))