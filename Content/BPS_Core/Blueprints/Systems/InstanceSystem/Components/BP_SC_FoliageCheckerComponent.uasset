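; Scene component that detects static foliage instances around it and requests their replacement.
; On BeginPlay it spawns a BP_FoliageChecker actor with the configured sphere radius and binds its collision hit event, then destroys it on EndPlay.
; Each tick it sweeps the checker to the component's location, so hits register along the path.
; Hits on foliage instanced components derived from the project's base class call TryReplaceInstance with the hit item index.
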(event `self.ReceiveBeginPlay`
  ;[1 1 1] Begin play. Init component.
  (`self.InitComponent`))

(event `self.ReceiveEndPlay`
  (params (EndPlayReason :type "EEndPlayReason Enum" :default "Destroyed"))
  ;[1 1 1] End play. Invalidate component.
  (`self.InvalidateComponent`))

(event `self.ReceiveTick`
  (params (DeltaSeconds :type "Float (single-precision)"))
  ;[1 1 1] Event tick. Updates foliage checker location.
  (`self.UpdateCheckerLocation`))

(fn `Bind_OnHitStaticFoliage`
  (params (HitComponent :type "PrimitiveComponent Object Reference") (OtherActor :type "Actor Object Reference") (OtherComp :type "PrimitiveComponent Object Reference") (NormalImpulse :type "Vector Structure") (Hit :type "HitResult Structure (by ref)"))
  (bind (_bblockinghit _binitialoverlap _time _distance _location _impactpoint _normal _impactnormal _physmat _hitactor _hitcomponent _hitbonename _bonename _hititem) (`GameplayStatics.BreakHitResult` Hit))
  ;[1 1 1] Try to replace instance on hit event.
  (bind _asbp_fismc_foliage_instanced_component_base (cast `/Game/BPS_Core/Blueprints/Systems/InstanceSystem/Components/BP_FISMC_FoliageInstancedComponent_Base` _hitcomponent))
  (`/Game/BPS_Core/Blueprints/Systems/InstanceSystem/Components/BP_FISMC_FoliageInstancedComponent_Base.TryReplaceInstance` _asbp_fismc_foliage_instanced_component_base _hititem))

(fn `InitComponent`
  (returns (Success :type Boolean))
  ;[1 1 1] Try to init foliage checker component.
  (bind _returnvalue (`|SpawnActorFromClass` "/Game/BPS_Core/Blueprints/Systems/InstanceSystem/Actors/BP_FoliageChecker.BP_FoliageChecker_C" (`self.K2_GetComponentToWorld`) "Undefined" "MultiplyWithRoot" (`self.GetOwner`) (`self.SphereRadius`) null))
  (bind _output_get (set `self.FoliageChecker` _returnvalue))
  (add `PrimitiveComponent.OnComponentHit` (`TriggerBase.CollisionComponent` _output_get) (`|CreateDelegate` :!event `Bind_OnHitStaticFoliage`))
  (return true))

(fn `InvalidateComponent`
  (returns (Success :type Boolean))
  (bind _foliagechecker (`self.FoliageChecker`))
  ;[1 1 1] Invalidate component and destroy foliage checker actor.
  (`/Engine/EditorBlueprintResources/StandardMacros.IsValid` _foliagechecker
    (:`Is Valid`
      (`Actor.K2_DestroyActor` _foliagechecker)
      (return true))))

(fn `UpdateCheckerLocation`
  (returns (Success :type Boolean))
  (bind _foliagechecker (`self.FoliageChecker`))
  ;[1 1 1] Try to update location of the foliage checker actor.
  (`/Engine/EditorBlueprintResources/StandardMacros.IsValid` _foliagechecker
    (:`Is Valid`
      (`Actor.K2_SetActorLocation` _foliagechecker (`self.K2_GetComponentLocation`) true false)
      (return true))))