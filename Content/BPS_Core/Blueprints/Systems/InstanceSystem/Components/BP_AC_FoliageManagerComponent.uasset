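; Actor component that manages instanced foliage at runtime, adding and removing instances of a given component class by world transform.
; On BeginPlay it caches the level's InstancedFoliageActor, then searches that actor's components for an exact class match.
; Adding can run through a multicast event.
; Removal has no event wrapper and uses a zero-radius sphere overlap plus a tolerance-based transform comparison to find the instance.
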(event `self.ReceiveBeginPlay`
  ;[1 1 1] Begin play. Init component.
  (`self.InitComponent`))

(event `TryAddInstanceInTransform`
  (params (InstancedClass :type "/Game/BPS_Core/Blueprints/Systems/InstanceSystem/Components/BP_FISMC_FoliageInstancedComponent_Base Class Reference") (Transform :type "Transform Structure"))
  ;[1 1 1] Try add instance.
  (`self.AddInstanceInTransform (Multicast)` InstancedClass Transform))

(event `AddInstanceInTransform (Multicast)`
  (params (InstancedClass :type "/Game/BPS_Core/Blueprints/Systems/InstanceSystem/Components/BP_FISMC_FoliageInstancedComponent_Base Class Reference") (Transform :type "Transform Structure"))
  ;[1 1 1] Try add instance.
  (`self.AddInstanceInTransform` InstancedClass Transform))

(fn `AddInstanceInTransform`
  (params (InstancedClass :type "/Game/BPS_Core/Blueprints/Systems/InstanceSystem/Components/BP_FISMC_FoliageInstancedComponent_Base Class Reference") (Transform :type "Transform Structure (by ref)"))
  (returns (Success :type Boolean))
  (locals (LocalComponents :type "Array of /Game/BPS_Core/Blueprints/Systems/InstanceSystem/Components/BP_FISMC_FoliageInstancedComponent_Base Object Reference"))
  ;[1 1 1] Add instance for specific instanced class in target transform.
  (bind _output_get (set `local.LocalComponents` (`Actor.K2_GetComponentsByClass` (`self.GetInstancedFoliageActor`) InstancedClass)))
  (for _array_element _output_get
    (if (== (`GameplayStatics.GetObjectClass` _array_element) InstancedClass)
      (`InstancedStaticMeshComponent.AddInstance` _array_element Transform true)
      (return true))))

(fn `GetInstancedFoliageActor`
  (returns (FoliageActor :type "InstancedFoliageActor Object Reference"))
  ;[1 1 1] Returns instanced foliage actor reference.
  (`/Engine/EditorBlueprintResources/StandardMacros.IsValid` (`self.InstancedFoliageActor`)
    (:`Is Valid`
      (return (`self.InstancedFoliageActor`)))
    (:`Is Not Valid`
      (bind _outactors (`GameplayStatics.GetAllActorsOfClass` "/Script/Foliage.InstancedFoliageActor"))
      (for _array_element _outactors
        (set `self.InstancedFoliageActor` _array_element)
        (return (`self.InstancedFoliageActor`))))))

(fn `InitComponent`
  (returns (Success :type Boolean))
  ;[1 1 1] Init manager component and set reference to Instanced foliage actor.
  (set `self.InstancedFoliageActor` (`self.GetInstancedFoliageActor`))
  (return true))

(fn `RemoveInstanceInTransform`
  (params (InstancedClass :type "/Game/BPS_Core/Blueprints/Systems/InstanceSystem/Components/BP_FISMC_FoliageInstancedComponent_Base Class Reference") (Transform :type "Transform Structure"))
  (returns (Success :type Boolean))
  (locals (LocalTransform :type "Transform Structure") (LocalComponents :type "Array of /Game/BPS_Core/Blueprints/Systems/InstanceSystem/Components/BP_FISMC_FoliageInstancedComponent_Base Object Reference") (LocalInstances :type "Array of Integer"))
  ;[1 1 1] Remove instance of specific instanced class in target transform.
  (set `local.LocalTransform` Transform)
  (bind _output_get (set `local.LocalComponents` (`Actor.K2_GetComponentsByClass` (`self.GetInstancedFoliageActor`) InstancedClass)))
  (for _array_element _output_get
    (if (== (`GameplayStatics.GetObjectClass` _array_element) InstancedClass)
      (bind _output_get_2 (set `local.LocalInstances` (`InstancedStaticMeshComponent.GetInstancesOverlappingSphere` _array_element (.location Transform) 0.0 true)))
      (for _array_element_2 _output_get_2
        (if (`/Game/BPS_Core/Blueprints/Systems/InstanceSystem/Components/BP_FISMC_FoliageInstancedComponent_Base.CheckEqualTransforms` _array_element (`InstancedStaticMeshComponent.GetInstanceTransform` _array_element _array_element_2 true) (`local.LocalTransform`) 0.1)
          (`InstancedStaticMeshComponent.RemoveInstance` _array_element _array_element_2)
          (return true))))))