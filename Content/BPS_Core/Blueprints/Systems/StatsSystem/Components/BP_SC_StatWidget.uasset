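; Widget component that displays a stat bar, bound to an attribute name and tag, on its owning actor.
; On non-dedicated instances it creates the widget, passing it the attribute, bar color and owner through interface messages.
; Visibility combines a stored flag with optional hiding for the owning player's pawn.
; An optional looping timer also hides it by camera distance, or when the owner is unrendered or blocked in a line trace.
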(event `self.ReceiveBeginPlay`
  ;[1 1 1] Begin play. Try to init stat widget component.
  (if (`self.InitOnBeginPlay`)
    (`self.TryInitComponent`)))

(fn `Bind_CheckVisibilityTick`
  ;[1 1 1] Update widget visibility.
  (`self.UpdateWidgetVisibility`))

(fn `GetOwningPlayer`
  (returns (ReturnValue :type "PlayerController Object Reference"))
  (bind _statwidget (`self.StatWidget`))
  ;[1 1 1] Returns owning player.
  (`/Engine/EditorBlueprintResources/StandardMacros.IsValid` _statwidget
    (:`Is Valid`
      (return (`Widget.GetOwningPlayer` _statwidget)))
    (:`Is Not Valid`
      (return null))))

(fn `InitComponent`
  (returns (Success :type Boolean))
  ;[1 1 1] Init stat widget component.
  (if (not (`KismetSystemLibrary.IsDedicatedServer`))
    (`/Engine/EditorBlueprintResources/StandardMacros.IsValid` (`self.GetOwnerPlayer`)
      (:`Is Valid`
        (bind _success (`self.InitStatWidget`))
        (if _success
          (`|ExecutionSequence`
            (:`then_0`
              (set `self.StatWidgetVisibility` (`self.InitialVisibility`))
              (`self.SetWidgetVisibility` (`self.ShouldBeVisible`)))
            (:`then_1`
              (`|ExecutionSequence`
                (:`then_0`
                  (if (`self.UseVisibilityCheck`)
                    (`self.StartCheckVisibilityTimer`)))
                (:`then_1`
                  (bind _output_get (set `self.IsInitialized` true))
                  (return _output_get)))))
          (else
            (set `self.IsInitialized` false)
            (return false)))))))

(fn `InitStatWidget`
  (returns (Success :type Boolean))
  (bind _statwidgetclass (`self.StatWidgetClass`))
  (bind _statwidget (`self.StatWidget`))
  ;[1 1 1] Try to create and init stat widget.
  (if (`KismetSystemLibrary.IsValidClass` _statwidgetclass)
    (bind _returnvalue (`|CreateWidget` _statwidgetclass))
    (bind _output_get (set `self.StatWidget` _returnvalue))
    (`self.SetWidget` _output_get)
    (`self.SetWidgetSpace` (`self.WidgetSpace`))
    (message `/Game/BPS_Core/Blueprints/Systems/StatsSystem/Interfaces/BPI_UI_StatWidget.SetStatAttributeNameAndTag_BPI` _statwidget (`self.StatAttributeName`) (`self.StatAttributeTag`))
    (message `/Game/BPS_Core/Blueprints/Systems/StatsSystem/Interfaces/BPI_UI_StatWidget.SetProgressBarColor_BPI` _statwidget (`self.ProgressBarColor`))
    (bind _success (message `/Game/BPS_Core/Blueprints/Systems/StatsSystem/Interfaces/BPI_UI_StatWidget.SetOwnerReference_BPI` _statwidget (`self.GetOwner`)))
    (return _success)
    (else
      (return false))))

(fn `SetWidgetVisibility`
  (params (NewVisibility :type Boolean))
  (returns (Success :type Boolean))
  ;[1 1 1] Set and update widget visibility.
  (set `self.StatWidgetVisibility` NewVisibility)
  (`self.SetVisibility` (`self.ShouldBeVisible`))
  (`|ExecutionSequence`
    (:`then_0`
      (if (`self.UseVisibilityCheck`)
        (if (not (`self.HideForOwner`))
          (`self.StartCheckVisibilityTimer`)
          (else
            (`self.StopCheckVisibilityTimer` :!label _label)))
        (else
          (goto _label))))
    (:`then_1`
      (return true))))

(fn `ShouldBeVisible`
  (returns (ReturnValue :type Boolean))
  (bind _statwidgetvisibility (`self.StatWidgetVisibility`))
  (bind _statwidget (`self.StatWidget`))
  ;[1 1 1] Returns true if the stat widget should be visible.
  (if (not (`self.HideForOwner`))
    (return _statwidgetvisibility)
    (else
      (`/Engine/EditorBlueprintResources/StandardMacros.IsValid` _statwidget
        (:`Is Valid`
          (return (and _statwidgetvisibility (not (== (`Controller.K2_GetPawn` (`Widget.GetOwningPlayer` _statwidget)) (`self.GetOwner`))))))
        (:`Is Not Valid`
          (return false))))))

(fn `StartCheckVisibilityTimer`
  (returns (Success :type Boolean))
  ;[1 1 1] Start check visibility timer.
  (bind _returnvalue (`KismetSystemLibrary.K2_SetTimerDelegate` (`|CreateDelegate` :!event `Bind_CheckVisibilityTick`) (`self.CheckVisibilityTickInterval`) true))
  (set `self.CheckVisibilityTimer` _returnvalue)
  (return true))

(fn `StopCheckVisibilityTimer`
  (returns (Success :type Boolean))
  ;[1 1 1] Stop check visibility timer.
  (`KismetSystemLibrary.K2_ClearAndInvalidateTimerHandle` (`self.CheckVisibilityTimer`))
  (return true))

(fn `TryInitComponent`
  (returns (Success :type Boolean))
  ;[1 1 1] Try init stat widget component.
  (if (not (`self.IsInitialized`))
    (bind _success (`self.InitComponent`))
    (bind _output_get (set `self.IsInitialized` _success))
    (return _output_get)
    (else
      (return true))))

(fn `UpdateWidgetVisibility`
  (returns (Success :type Boolean))
  (bind _returnvalue (`self.GetOwner`))
  ;[1 1 1] Update stat widget visibility.
  (`/Engine/EditorBlueprintResources/StandardMacros.IsValid` (`self.GetOwningPlayer`)
    (:`Is Valid`
      (if (`self.ShouldBeVisible`)
        (`|ExecutionSequence`
          (:`then_0`
            (if (`self.CheckDistanceToPlayer`)
              (if (> (`KismetMathLibrary.Vector_Distance` (`Actor.K2_GetActorLocation` (`self.GetOwner`)) (`PlayerCameraManager.GetCameraLocation` (`PlayerController.PlayerCameraManager` (`self.GetOwningPlayer`)))) (`self.DistanceToPlayer`))
                (`self.SetVisibility` false)
                (return true))))
          (:`then_1`
            (`|ExecutionSequence`
              (:`then_0`
                (if (`self.CheckTraceToPlayer`)
                  (if (`Actor.WasRecentlyRendered` _returnvalue 0.2)
                    (bind (_outhit _returnvalue_2) (`KismetSystemLibrary.LineTraceSingle` (`PlayerCameraManager.GetCameraLocation` (`PlayerController.PlayerCameraManager` (`self.GetOwningPlayer`))) (`Actor.K2_GetActorLocation` _returnvalue) "TraceTypeQuery1"))
                    (if _returnvalue_2
                      (`self.SetVisibility` false :!label _label)
                      (return true))
                    (else
                      (goto _label)))))
              (:`then_1`
                (`self.SetVisibility` true)
                (return true)))))
        (else
          (`self.SetVisibility` false :!label _label_2)
          (return true))))
    (:`Is Not Valid`
      (goto _label_2))))