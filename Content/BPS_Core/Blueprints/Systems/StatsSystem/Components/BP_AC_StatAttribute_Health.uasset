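; Health stat attribute component that tracks an actor's health, max health, regeneration and alive state.
; Server-authoritative setters record causer, source and damage data, kill the owner at zero health and support revival.
; An optional damage manager component feeds damage taken into health decreases.
; Alive state replicates via OnRep and gates the inherited change timer, while parent value events are re-broadcast as health-specific events.
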(event `self.ReceiveBeginPlay`
  ;[1 1 1] Begin play. Bind health stat attribute events.
  (`parent.ReceiveBeginPlay`)
  (add `self.OnCurrentValueChanged_Server` (`|CreateDelegate` :!event `Bind_OnCurrentValueChanged_Server`))
  (add `self.OnCurrentValueChanged_Client` (`|CreateDelegate` :!event `Bind_OnCurrentValueChanged_Client`))
  (add `self.OnMaxValueChanged_Server` (`|CreateDelegate` :!event `Bind_OnMaxValueChanged_Server`))
  (add `self.OnMaxValueChanged_Client` (`|CreateDelegate` :!event `Bind_OnMaxValueChanged_Client`)))

(fn `Bind_OnCurrentValueChanged_Client`
  (params (Component :type "/Game/BPS_Core/Blueprints/Systems/StatsSystem/Components/BP_AC_StatAttribute Object Reference") (NewValue :type "Float (double-precision)") (PrevValue :type "Float (double-precision)"))
  ;[1 1 1] Calls the on health changed event for clients.
  (`self.OnHealthChanged_Client` self NewValue PrevValue))

(fn `Bind_OnCurrentValueChanged_Server`
  (params (Component :type "/Game/BPS_Core/Blueprints/Systems/StatsSystem/Components/BP_AC_StatAttribute Object Reference") (NewValue :type "Float (double-precision)") (PrevValue :type "Float (double-precision)"))
  ;[1 1 1] Calls the on health changed event for the server.
  (`self.OnHealthChanged_Server` self NewValue PrevValue (`self.LastCauser`) (`self.LastSource`) (`self.LastDamageData`)))

(fn `Bind_OnDamageTaken`
  (params (DamageManager :type "/Game/BPS_Core/Blueprints/Systems/DamageSystem/Components/BP_AC_DamageManager Object Reference") (DamageData :type "/Game/BPS_Core/Blueprints/Systems/DamageSystem/Structures/STR_DamageData Structure") (DamagedActor :type "Actor Object Reference") (EventInstigator :type "Controller Object Reference") (DamageCauser :type "Actor Object Reference") (ApplyMethod :type "/Game/BPS_Core/Blueprints/Systems/DamageSystem/Enums/E_DamageApplyMethod Enum" :default "NewEnumerator0"))
  ;[1 1 1] Decrease health on damage taken event.
  (`self.ChangeHealth` "NewEnumerator1" (`/Game/BPS_Core/Blueprints/Systems/DamageSystem/Libraries/BP_Library_DamageSystem.GetDamageValue` DamageData) false DamageCauser "NewEnumerator1" DamageData))

(fn `Bind_OnMaxValueChanged_Client`
  (params (Component :type "/Game/BPS_Core/Blueprints/Systems/StatsSystem/Components/BP_AC_StatAttribute Object Reference") (NewValue :type "Float (double-precision)") (PrevValue :type "Float (double-precision)"))
  ;[1 1 1] Calls the on max health changed event for clients.
  (`self.OnMaxHealthChanged_Client` self NewValue PrevValue))

(fn `Bind_OnMaxValueChanged_Server`
  (params (Component :type "/Game/BPS_Core/Blueprints/Systems/StatsSystem/Components/BP_AC_StatAttribute Object Reference") (NewValue :type "Float (double-precision)") (PrevValue :type "Float (double-precision)"))
  ;[1 1 1] Calls the on max health changed event for the server.
  (`self.OnMaxHealthChanged_Server` self NewValue PrevValue))

(fn `ChangeHealth`
  (params (Operation :type "/Game/BPS_Core/Blueprints/Systems/StatsSystem/Enums/E_ChangeStatOperation Enum" :default "NewEnumerator0") (Value :type "Float (double-precision)") (Percent :type Boolean) (Causer :type "Actor Object Reference") (Source :type "/Game/BPS_Core/Blueprints/Systems/StatsSystem/Enums/E_HealthChangeSource Enum" :default "NewEnumerator0") (DamageData :type "/Game/BPS_Core/Blueprints/Systems/DamageSystem/Structures/STR_DamageData Structure"))
  (returns (Success :type Boolean))
  (bind _currentvalue (`self.CurrentValue`))
  (bind _returnvalue (* Value (`self.MaxValue`)))
  ;[1 1 1] Try to change the current health variable on the server.
  (if (`KismetSystemLibrary.IsServer`)
    (bind _success (`self.SetHealth` (select `/Game/BPS_Core/Blueprints/Systems/StatsSystem/Enums/E_ChangeStatOperation` Operation :`NewEnumerator0` (+ _currentvalue (select `bool` Percent :`false` Value :`true` _returnvalue)) :`NewEnumerator1` (- _currentvalue (select `bool` Percent :`false` Value :`true` _returnvalue)) :`NewEnumerator2` Value) false Causer Source DamageData))
    (return _success)))

(fn `ChangeHealthRegeneration`
  (params (Operation :type "/Game/BPS_Core/Blueprints/Systems/StatsSystem/Enums/E_ChangeStatOperation Enum" :default "NewEnumerator0") (Value :type "Float (double-precision)") (Percent :type Boolean))
  (returns (Success :type Boolean))
  ;[1 1 1] Try to change the health regeneration variable on the server.
  (bind _success (`self.ChangeChangeValue` Operation Value Percent))
  (return _success))

(fn `ChangeMaxHealth`
  (params (Operation :type "/Game/BPS_Core/Blueprints/Systems/StatsSystem/Enums/E_ChangeStatOperation Enum" :default "NewEnumerator0") (Value :type "Float (double-precision)") (Percent :type Boolean))
  (returns (Success :type Boolean))
  ;[1 1 1] Try to change the max health variable on the server.
  (bind _success (`self.ChangeMaxValue` Operation Value Percent))
  (return _success))

(fn `CheckChangeTimerEnabled`
  (returns (Result :type Boolean))
  ;[1 1 1] Returns true if change timer should be enabled.
  (return (and (`parent.CheckChangeTimerEnabled`) (`self.OwnerIsAlive`))))

(fn `GetHealth`
  (returns (Health :type "Float (double-precision)"))
  ;[1 1 1] Returns current health value.
  (return (`self.GetCurrentValue`)))

(fn `GetHealthRegeneration`
  (returns (Regeneration :type "Float (double-precision)"))
  ;[1 1 1] Returns health regeneration value.
  (return (`self.GetChangeValue`)))

(fn `GetMaxHealth`
  (returns (MaxHealth :type "Float (double-precision)"))
  ;[1 1 1] Returns max health value.
  (return (`self.GetMaxValue`)))

(fn `InitComponent`
  (returns (Success :type Boolean))
  ;[1 1 1] Init health stat attribute component.
  (bind _success (`parent.InitComponent`))
  (if _success
    (if (`KismetSystemLibrary.IsServer`)
      (set `self.OwnerIsAlive` (> (`self.CurrentValue`) 0.0))
      (if (`self.UseDamageManager`)
        (bind _success_2 (`self.InitDamageManager`))
        (if _success_2
          _
          (else
            (return false)))))
    (return true)
    (else
      (return false))))

(fn `InitDamageManager`
  (returns (Success :type Boolean))
  ;[1 1 1] Try to init damage manager component.
  (bind (_found _component) (`/Game/BPS_Core/Blueprints/Systems/DamageSystem/Libraries/BP_Library_DamageSystem.FindDamageManager` (`self.GetOwner`)))
  (if _found
    (bind _output_get (set `self.DamageManager` _component))
    (bind _success (`/Game/BPS_Core/Blueprints/Systems/DamageSystem/Components/BP_AC_DamageManager.TryInitComponent` _output_get))
    (if _success
      (add `/Game/BPS_Core/Blueprints/Systems/DamageSystem/Components/BP_AC_DamageManager.OnDamageTaken` (`self.DamageManager`) (`|CreateDelegate` :!event `Bind_OnDamageTaken`))
      (return true)
      (else
        _)))
  (return false))

(fn `IsAlive`
  (returns (IsAlive :type Boolean))
  ;[1 1 1] Returns true if owner is alive.
  (return (`self.OwnerIsAlive`)))

(fn `KillOwner`
  (params (Causer :type "Actor Object Reference") (Source :type "/Game/BPS_Core/Blueprints/Systems/StatsSystem/Enums/E_HealthChangeSource Enum" :default "NewEnumerator0") (DamageData :type "/Game/BPS_Core/Blueprints/Systems/DamageSystem/Structures/STR_DamageData Structure"))
  (returns (Success :type Boolean))
  ;[1 1 1] Try to kill owner.
  (if (and (`KismetSystemLibrary.IsServer`) (`self.IsAlive`))
    (set `self.OwnerIsAlive` false)
    (bind _output_get (set `self.LastCauser` Causer))
    (bind _output_get_2 (set `self.LastSource` Source))
    (bind _output_get_3 (set `self.LastDamageData` DamageData))
    (bind _success (`self.SetHealth` 0.0 true _output_get _output_get_2 _output_get_3))
    (`self.OnOwnerDead` self (`self.LastCauser`) (`self.LastSource`) (`self.LastDamageData`))
    (return _success)))

(fn `OnRep_OwnerIsAlive`
  ;[1 1 1] Calls the on is alive changed event.
  (`self.OnIsAliveChanged` self (`self.IsAlive`))
  (`self.CheckChangeTimer`))

(fn `ReviveOwner`
  (params (Health :type "Float (double-precision)") (Percent :type Boolean) (Causer :type "Actor Object Reference"))
  (returns (Success :type Boolean))
  ;[1 1 1] Try to revive owner.
  (if (and (`KismetSystemLibrary.IsServer`) (not (`self.IsAlive`)))
    (set `self.OwnerIsAlive` true)
    (bind _output_get (set `self.LastCauser` Causer))
    (bind _success (`self.SetHealth` Health Percent _output_get))
    (`self.OnOwnerRevived` self (`self.LastCauser`))
    (return _success)))

(fn `SetCurrentValue`
  (params (Value :type "Float (double-precision)") (Percent :type Boolean))
  (returns (Success :type Boolean))
  ;[1 1 1] Try to set new value for the current value variable on the server.
  (bind _success (`self.SetHealth` Value Percent (`self.GetOwner`)))
  (return _success))

(fn `SetHealth`
  (params (Value :type "Float (double-precision)") (Percent :type Boolean) (Causer :type "Actor Object Reference") (Source :type "/Game/BPS_Core/Blueprints/Systems/StatsSystem/Enums/E_HealthChangeSource Enum" :default "NewEnumerator0") (DamageData :type "/Game/BPS_Core/Blueprints/Systems/DamageSystem/Structures/STR_DamageData Structure"))
  (returns (Success :type Boolean))
  (locals (LocalNewValue :type "Float (double-precision)") (LocalPrevValue :type "Float (double-precision)") (LocalCauser :type "Actor Object Reference") (LocalSource :type "/Game/BPS_Core/Blueprints/Systems/StatsSystem/Enums/E_HealthChangeSource Enum" :default "NewEnumerator0") (LocalDamageData :type "/Game/BPS_Core/Blueprints/Systems/DamageSystem/Structures/STR_DamageData Structure"))
  (bind _currentvalue (`self.CurrentValue`))
  ;[1 1 1] Try to set new value for the current value variable on the server.
  (if (`KismetSystemLibrary.IsServer`)
    (bind (_success _newvalue _prevvalue) (`self.SetCurrentValueLocal` Value Percent true))
    (if _success
      (bind _output_get (set `local.LocalNewValue` _newvalue))
      (bind _output_get_2 (set `local.LocalPrevValue` _prevvalue))
      (set `self.LastCauser` Causer)
      (set `self.LastSource` Source)
      (set `self.LastDamageData` DamageData)
      (`self.OnCurrentValueChanged_Server` self _output_get _output_get_2)
      (if (`self.ReplicateValues`)
        (set `self.ReplicatedCurrentValue` _currentvalue))
      (if (<= _currentvalue 0.0)
        (`self.KillOwner` (`self.LastCauser`) (`self.LastSource`) (`self.LastDamageData`)))
      (return true)
      (else
        (return true)))
    (else
      (return false))))

(fn `SetHealthRegeneration`
  (params (Value :type "Float (double-precision)"))
  (returns (Success :type Boolean))
  ;[1 1 1] Set health regeneration value.
  (bind _success (`self.SetChangeValue` Value))
  (return _success))

(fn `SetMaxHealth`
  (params (Value :type "Float (double-precision)"))
  (returns (Success :type Boolean))
  ;[1 1 1] Set max health value.
  (bind _success (`self.SetMaxValue` Value))
  (return _success))