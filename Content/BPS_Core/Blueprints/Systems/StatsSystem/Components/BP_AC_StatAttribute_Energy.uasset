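; Energy stat component for the StatsSystem, wrapping a generic stat attribute parent with energy-named getters, setters and change functions for current, max and regeneration values.
; Energy writes run only on the server, optionally replicate, and re-broadcast the parent's server and client change events as energy-specific events.
; Decreases can pause regeneration by disabling the change timer, then resuming it after a delay.
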(event `self.ReceiveBeginPlay`
  ;[1 1 1] Begin play. Bind energy stat attribute events.
  (`parent.ReceiveBeginPlay`)
  (add `self.OnCurrentValueChanged_Server` (`|CreateDelegate` :!event `Bind_OnCurrentValueChanged_Server`))
  (add `self.OnCurrentValueChanged_Client` (`|CreateDelegate` :!event `Bind_OnCurrentValueChanged_Client`))
  (add `self.OnMaxValueChanged_Server` (`|CreateDelegate` :!event `Bind_OnMaxValueChanged_Server`))
  (add `self.OnMaxValueChanged_Client` (`|CreateDelegate` :!event `Bind_OnMaxValueChanged_Client`)))

(fn `Bind_OnCurrentValueChanged_Client`
  (params (Component :type "/Game/BPS_Core/Blueprints/Systems/StatsSystem/Components/BP_AC_StatAttribute Object Reference") (NewValue :type "Float (double-precision)") (PrevValue :type "Float (double-precision)"))
  ;[1 1 1] Calls the on health changed event for clients.
  (`self.OnEnergyChanged_Client` self NewValue PrevValue))

(fn `Bind_OnCurrentValueChanged_Server`
  (params (Component :type "/Game/BPS_Core/Blueprints/Systems/StatsSystem/Components/BP_AC_StatAttribute Object Reference") (NewValue :type "Float (double-precision)") (PrevValue :type "Float (double-precision)"))
  ;[1 1 1] Calls the on energy changed event for the server.
  (`self.OnEnergyChanged_Server` self NewValue PrevValue))

(fn `Bind_OnMaxValueChanged_Client`
  (params (Component :type "/Game/BPS_Core/Blueprints/Systems/StatsSystem/Components/BP_AC_StatAttribute Object Reference") (NewValue :type "Float (double-precision)") (PrevValue :type "Float (double-precision)"))
  ;[1 1 1] Calls the on max health changed event for clients.
  (`self.OnMaxEnergyChanged_Client` self NewValue PrevValue))

(fn `Bind_OnMaxValueChanged_Server`
  (params (Component :type "/Game/BPS_Core/Blueprints/Systems/StatsSystem/Components/BP_AC_StatAttribute Object Reference") (NewValue :type "Float (double-precision)") (PrevValue :type "Float (double-precision)"))
  ;[1 1 1] Calls the on max health changed event for the server.
  (`self.OnMaxEnergyChanged_Server` self NewValue PrevValue))

(fn `Bind_ResumeRegeneration`
  ;[1 1 1] Resume energy regeneration.
  (`self.SetChangeTimerEnabled` true))

(fn `ChangeCurrentValue`
  (params (Operation :type "/Game/BPS_Core/Blueprints/Systems/StatsSystem/Enums/E_ChangeStatOperation Enum" :default "NewEnumerator0") (Value :type "Float (double-precision)") (Percent :type Boolean))
  (returns (Success :type Boolean))
  ;[1 1 1] Change current value and stop energy regeneration.
  (bind _success (`parent.ChangeCurrentValue` Operation Value Percent))
  (`|ExecutionSequence`
    (:`then_0`
      (if (and (`self.StopRegenOnDecrease`) (`|EnumEquality` Operation "NewEnumerator1"))
        (`self.SetChangeTimerEnabled` false)
        (`KismetSystemLibrary.K2_SetTimerDelegate` (`|CreateDelegate` :!event `Bind_ResumeRegeneration`) (`self.StopRegenTime`))))
    (:`then_1`
      (return _success))))

(fn `ChangeEnergy`
  (params (Operation :type "/Game/BPS_Core/Blueprints/Systems/StatsSystem/Enums/E_ChangeStatOperation Enum" :default "NewEnumerator0") (Value :type "Float (double-precision)") (Percent :type Boolean) (StopRegen :type Boolean))
  (returns (Success :type Boolean))
  (bind _currentvalue (`self.CurrentValue`))
  (bind _returnvalue (* Value (`self.MaxValue`)))
  ;[1 1 1] Try to change the current energy variable on the server.
  (if (`KismetSystemLibrary.IsServer`)
    (bind _success (`self.SetEnergy` (select `/Game/BPS_Core/Blueprints/Systems/StatsSystem/Enums/E_ChangeStatOperation` Operation :`NewEnumerator0` (+ _currentvalue (select `bool` Percent :`false` Value :`true` _returnvalue)) :`NewEnumerator1` (- _currentvalue (select `bool` Percent :`false` Value :`true` _returnvalue)) :`NewEnumerator2` Value) false StopRegen))
    (return _success)))

(fn `ChangeHealthRegeneration`
  (params (Operation :type "/Game/BPS_Core/Blueprints/Systems/StatsSystem/Enums/E_ChangeStatOperation Enum" :default "NewEnumerator0") (Value :type "Float (double-precision)") (Percent :type Boolean))
  (returns (Success :type Boolean))
  ;[1 1 1] Try to change the energy regeneration variable on the server.
  (bind _success (`self.ChangeChangeValue` Operation Value Percent))
  (return _success))

(fn `ChangeMaxEnergy`
  (params (Operation :type "/Game/BPS_Core/Blueprints/Systems/StatsSystem/Enums/E_ChangeStatOperation Enum" :default "NewEnumerator0") (Value :type "Float (double-precision)") (Percent :type Boolean))
  (returns (Success :type Boolean))
  ;[1 1 1] Try to change the max energy variable on the server.
  (bind _success (`self.ChangeMaxValue` Operation Value Percent))
  (return _success))

(fn `GetEnergy`
  (returns (Energy :type "Float (double-precision)"))
  ;[1 1 1] Returns current energy value.
  (return (`self.GetCurrentValue`)))

(fn `GetEnergyRegeneration`
  (returns (Regeneration :type "Float (double-precision)"))
  ;[1 1 1] Returns energy regeneration value.
  (return (`self.GetChangeValue`)))

(fn `GetMaxEnergy`
  (returns (MaxEnergy :type "Float (double-precision)"))
  ;[1 1 1] Returns max energy value.
  (return (`self.GetMaxValue`)))

(fn `SetCurrentValue`
  (params (Value :type "Float (double-precision)") (Percent :type Boolean))
  (returns (Success :type Boolean))
  ;[1 1 1] Try to set new value for the current value variable on the server.
  (bind _success (`self.SetEnergy` Value Percent))
  (return _success))

(fn `SetEnergy`
  (params (Value :type "Float (double-precision)") (Percent :type Boolean) (StopRegen :type Boolean))
  (returns (Success :type Boolean))
  (locals (LocalNewValue :type "Float (double-precision)") (LocalPrevValue :type "Float (double-precision)") (LocalStopRegen :type Boolean))
  ;[1 1 1] Try to set new value for the current value variable on the server.
  (if (`KismetSystemLibrary.IsServer`)
    (bind (_success _newvalue _prevvalue) (`self.SetCurrentValueLocal` Value Percent true))
    (if _success
      (bind _output_get (set `local.LocalNewValue` _newvalue))
      (bind _output_get_2 (set `local.LocalPrevValue` _prevvalue))
      (set `local.LocalStopRegen` StopRegen)
      (`self.OnCurrentValueChanged_Server` self _output_get _output_get_2)
      (`|ExecutionSequence`
        (:`then_0`
          (if (`self.ReplicateValues`)
            (set `self.ReplicatedCurrentValue` (`self.CurrentValue`))))
        (:`then_1`
          (`|ExecutionSequence`
            (:`then_0`
              (if (`local.LocalStopRegen`)
                (if (and (`self.StopRegenOnDecrease`) (<= (`local.LocalNewValue`) (`local.LocalPrevValue`)))
                  (`self.SetChangeTimerEnabled` false)
                  (`KismetSystemLibrary.K2_SetTimerDelegate` (`|CreateDelegate` :!event `Bind_ResumeRegeneration`) (`self.StopRegenTime`)))))
            (:`then_1`
              (return true)))))
      (else
        (return true)))
    (else
      (return false))))

(fn `SetEnergyRegeneration`
  (params (Value :type "Float (double-precision)"))
  (returns (Success :type Boolean))
  ;[1 1 1] Set energy regeneration value.
  (bind _success (`self.SetChangeValue` Value))
  (return _success))

(fn `SetMaxEnergy`
  (params (Value :type "Float (double-precision)"))
  (returns (Success :type Boolean))
  ;[1 1 1] Set max energy value.
  (bind _success (`self.SetMaxValue` Value))
  (return _success))