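; Actor component for one named or tagged stat with min, max, clamped current value and per-second change rate.
; Initial min, max and rate can come from gameplay-tagged attributes in BP_AC_AttributesManager, refreshed when attributes change.
; Setters are server-only, fire server and client events, and optionally replicate values through OnRep handlers.
; A nonzero rate drives current value via looping timer or component tick, optionally simulated on clients.
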(event `self.ReceiveBeginPlay`
  ;[1 1 1] Begin play. Init stat attribute component.
  (if (`self.InitOnBeginPlay`)
    (`self.TryInitComponent`)))

(event `self.ReceiveTick`
  (params (DeltaSeconds :type "Float (single-precision)"))
  ;[1 1 1] Event tick. Change current value on tick.
  (`self.ChangeValueTick` DeltaSeconds))

(fn `Bind_AttributesChanged`
  (params (Manager :type "/Game/BPS_Core/Blueprints/Systems/AttributesSystem/Components/BP_AC_AttributesManager Object Reference"))
  ;[1 1 1] Executes on attributes changed event.
  (`self.UpdateAttributeValues`))

(fn `Bind_ChangeTimerTick`
  ;[1 1 1] Executes on change value timer tick event.
  (`self.ChangeValueTick` (`self.ChangeTimerTickInterval`)))

(fn `ChangeChangeValue`
  (params (Operation :type "/Game/BPS_Core/Blueprints/Systems/StatsSystem/Enums/E_ChangeStatOperation Enum" :default "NewEnumerator0") (Value :type "Float (double-precision)") (Percent :type Boolean))
  (returns (Success :type Boolean))
  (bind _changevalue (`self.ChangeValue`))
  (bind _returnvalue (* Value (`self.ChangeValue`)))
  ;[1 1 1] Try to change value for the change value variable on the server.
  (if (`KismetSystemLibrary.IsServer`)
    (bind _success (`self.SetChangeValue` (select `/Game/BPS_Core/Blueprints/Systems/StatsSystem/Enums/E_ChangeStatOperation` Operation :`NewEnumerator0` (+ _changevalue (select `bool` Percent :`false` Value :`true` _returnvalue)) :`NewEnumerator1` (- _changevalue (select `bool` Percent :`false` Value :`true` _returnvalue)) :`NewEnumerator2` Value)))
    (return _success)))

(fn `ChangeCurrentValue`
  (params (Operation :type "/Game/BPS_Core/Blueprints/Systems/StatsSystem/Enums/E_ChangeStatOperation Enum" :default "NewEnumerator0") (Value :type "Float (double-precision)") (Percent :type Boolean))
  (returns (Success :type Boolean))
  (bind _currentvalue (`self.CurrentValue`))
  (bind _returnvalue (* Value (`self.MaxValue`)))
  ;[1 1 1] Try to change value for the current value variable on the server.
  (if (`KismetSystemLibrary.IsServer`)
    (bind _success (`self.SetCurrentValue` (select `/Game/BPS_Core/Blueprints/Systems/StatsSystem/Enums/E_ChangeStatOperation` Operation :`NewEnumerator0` (+ _currentvalue (`KismetMathLibrary.SelectFloat` _returnvalue Value Percent)) :`NewEnumerator1` (- _currentvalue (`KismetMathLibrary.SelectFloat` _returnvalue Value Percent)) :`NewEnumerator2` Value)))
    (return _success)))

(fn `ChangeMaxValue`
  (params (Operation :type "/Game/BPS_Core/Blueprints/Systems/StatsSystem/Enums/E_ChangeStatOperation Enum" :default "NewEnumerator0") (Value :type "Float (double-precision)") (Percent :type Boolean))
  (returns (Success :type Boolean))
  (bind _maxvalue (`self.MaxValue`))
  (bind _returnvalue (* Value (`self.MaxValue`)))
  ;[1 1 1] Try to change value for the max value variable on the server.
  (if (`KismetSystemLibrary.IsServer`)
    (bind _success (`self.SetMaxValue` (select `/Game/BPS_Core/Blueprints/Systems/StatsSystem/Enums/E_ChangeStatOperation` Operation :`NewEnumerator0` (+ _maxvalue (select `bool` Percent :`false` Value :`true` _returnvalue)) :`NewEnumerator1` (- _maxvalue (select `bool` Percent :`false` Value :`true` _returnvalue)) :`NewEnumerator2` Value)))
    (return _success)))

(fn `ChangeValueTick`
  (params (DeltaTime :type "Float (double-precision)"))
  (returns (Success :type Boolean))
  ;[1 1 1] Change current value of the stat attribute on tick.
  (bind (_success _newvalue _prevvalue) (`self.SetCurrentValueLocal` (+ (`self.CurrentValue`) (* DeltaTime (`self.ChangeValue`))) false (`self.CallClientEventOnChangeTick`)))
  (if _success
    (if (`KismetSystemLibrary.IsServer`)
      (`self.OnCurrentValueChanged_Server` self _newvalue _prevvalue)
      (return true))))

(fn `CheckChangeTimer`
  (returns (Success :type Boolean))
  ;[1 1 1] Check change timer conditions and start or stop change value ticks.
  (if (`self.CheckChangeTimerEnabled`)
    (`self.StartChangeTimer`)
    (else
      (`self.StopChangeTimer`)))
  (return true))

(fn `CheckChangeTimerEnabled`
  (returns (Result :type Boolean))
  (bind _returnvalue (!= (`self.ChangeValue`) 0.0))
  ;[1 1 1] Returns true if change timer should be enabled.
  (if (`self.ChangeTimerEnabled`)
    (if (`KismetSystemLibrary.IsServer`)
      (return _returnvalue)
      (else
        (return (and _returnvalue (`self.CallChangeTickOnClients`)))))
    (else
      (return false))))

(fn `CheckStatAttributeName`
  (params (StatAttributeName :type Name))
  (returns (Result :type Boolean))
  ;[1 1 1] Returns true if the stat attribute name matches the same one in the component.
  (return (and (!= StatAttributeName "None") (== StatAttributeName (`self.StatAttributeName`)))))

(fn `CheckStatAttributeNameOrTag`
  (params (StatAttributeName :type Name) (StatAttributeTag :type "GameplayTag Structure"))
  (returns (Result :type Boolean))
  ;[1 1 1] Returns true if the stat attribute name or tag matches the same one in the component.
  (bind _result (`self.CheckStatAttributeName` StatAttributeName))
  (if _result
    (return true)
    (else
      (bind _result_2 (`self.CheckStatAttributeTag` StatAttributeTag))
      (return _result_2))))

(fn `CheckStatAttributeTag`
  (params (StatAttributeTag :type "GameplayTag Structure"))
  (returns (Result :type Boolean))
  ;[1 1 1] Returns true if the stat attribute tag matches the same one in the component.
  (return (and (`BlueprintGameplayTagLibrary.IsGameplayTagValid` StatAttributeTag) (== StatAttributeTag (`self.StatAttributeTag`)))))

(fn `CheckStatAttributeValue`
  (params (Value :type "Float (double-precision)") (Percent :type Boolean))
  (returns (Result :type Boolean))
  (bind _currentvalue (`self.CurrentValue`))
  ;[1 1 1] Returns true if the current value is greater than or equal to the target value.
  (return (< Value (select `bool` Percent :`false` _currentvalue :`true` (* (`self.MaxValue`) _currentvalue)))))

(fn `GetChangeValue`
  (returns (Value :type "Float (double-precision)"))
  ;[1 1 1] Returns change value of the stat attribute.
  (return (`self.ChangeValue`)))

(fn `GetCurrentValue`
  (returns (Value :type "Float (double-precision)"))
  ;[1 1 1] Returns current value of the stat attribute.
  (return (`self.CurrentValue`)))

(fn `GetCurrentValue%`
  (returns (Value :type "Float (double-precision)"))
  ;[1 1 1] Returns current value percent of max value of the stat attribute.
  (return (/ (`self.CurrentValue`) (`self.GetMaxValue`))))

(fn `GetMaxValue`
  (returns (Value :type "Float (double-precision)"))
  ;[1 1 1] Returns max value of the stat attribute.
  (return (`self.MaxValue`)))

(fn `GetMinValue`
  (returns (Value :type "Float (double-precision)"))
  ;[1 1 1] Returns min value of the stat attribute.
  (return (`self.MinValue`)))

(fn `GetStatAttributeName`
  (returns (Name :type Name))
  ;[1 1 1] Returns stat attribute name.
  (return (`self.StatAttributeName`)))

(fn `GetValues`
  (returns (MinValue :type "Float (double-precision)") (MaxValue :type "Float (double-precision)") (CurrentValue :type "Float (double-precision)") (ChangeValue :type "Float (double-precision)"))
  ;[1 1 1] Returns all stat attribute values.
  (return (`self.MinValue`) (`self.MaxValue`) (`self.CurrentValue`) (`self.ChangeValue`)))

(fn `InitAttributesComponent`
  (returns (Success :type Boolean))
  ;[1 1 1] Try to find and init attribute components and attribute values.
  (bind _output_get (set `self.AttributesComponent` (`Actor.GetComponentByClass` (`self.GetOwner`) "/Game/BPS_Core/Blueprints/Systems/AttributesSystem/Components/BP_AC_AttributesManager.BP_AC_AttributesManager_C")))
  (`/Engine/EditorBlueprintResources/StandardMacros.IsValid` _output_get
    (:`Is Valid`
      (bind _success (`/Game/BPS_Core/Blueprints/Systems/AttributesSystem/Components/BP_AC_AttributesManager.TryInitComponent` _output_get))
      (if _success
        (add `/Game/BPS_Core/Blueprints/Systems/AttributesSystem/Components/BP_AC_AttributesManager.OnAttributesChanged` (`self.AttributesComponent`) (`|CreateDelegate` :!event `Bind_AttributesChanged`))
        (bind _success_2 (`self.InitAttributeValues`))
        (if _success_2
          (return true)
          (else
            _))))
    (:`Is Not Valid`
      _))
  (return false))

(fn `InitAttributeValues`
  (returns (Success :type Boolean))
  ;[1 1 1] Try to init attribute values.
  (bind _attributes (`/Game/BPS_Core/Blueprints/Systems/AttributesSystem/Components/BP_AC_AttributesManager.GetAttributes` (`self.AttributesComponent`)))
  (set `self.CurrentAttributes` _attributes)
  (`|ExecutionSequence`
    (:`then_0`
      (if (`BlueprintGameplayTagLibrary.IsGameplayTagValid` (`self.MinValueAttributeTag`))
        (bind (_success _value) (`/Game/BPS_Core/Blueprints/Systems/AttributesSystem/Components/BP_AC_AttributesManager.GetAttributeValue` (`self.AttributesComponent`) (`self.MinValueAttributeTag`)))
        (set `self.InitialMinValue` _value)))
    (:`then_1`
      (`|ExecutionSequence`
        (:`then_0`
          (if (`BlueprintGameplayTagLibrary.IsGameplayTagValid` (`self.MaxValueAttributeTag`))
            (bind (_success_2 _value_2) (`/Game/BPS_Core/Blueprints/Systems/AttributesSystem/Components/BP_AC_AttributesManager.GetAttributeValue` (`self.AttributesComponent`) (`self.MaxValueAttributeTag`)))
            (set `self.InitialMaxValue` _value_2)))
        (:`then_1`
          (`|ExecutionSequence`
            (:`then_0`
              (if (`BlueprintGameplayTagLibrary.IsGameplayTagValid` (`self.ChangeValueAttributeTag`))
                (bind (_success_3 _value_3) (`/Game/BPS_Core/Blueprints/Systems/AttributesSystem/Components/BP_AC_AttributesManager.GetAttributeValue` (`self.AttributesComponent`) (`self.ChangeValueAttributeTag`)))
                (set `self.InitialChangeValue` _value_3)))
            (:`then_1`
              (return true))))))))

(fn `InitComponent`
  (returns (Success :type Boolean))
  ;[1 1 1] Init stat attribute component.
  (if (`KismetSystemLibrary.IsServer`)
    (`|ExecutionSequence`
      (:`then_0`
        (if (`self.UseAttributes`)
          (bind _success (`self.InitAttributesComponent`))
          (if (not _success)
            (return false))))
      (:`then_1`
        (`|ExecutionSequence`
          (:`then_0`
            (`self.InitInitialValues`))
          (:`then_1`
            (set `self.IsInitialized` true :!label _label)
            (return true)))))
    (else
      (goto _label))))

(fn `InitInitialValues`
  (returns (Success :type Boolean))
  ;[1 1 1] Try to init initial values and try to start change value timer.
  (`self.SetMinValue` (`self.InitialMinValue`))
  (`self.SetMaxValue` (`self.InitialMaxValue`))
  (`self.SetCurrentValue` (`self.InitialCurrentValue`) (`self.InitialCurrentPercent`))
  (`self.SetChangeValue` (`self.InitialChangeValue`))
  (return true))

(fn `OnRep_ChangeTimerEnabled`
  ;[1 1 1] Update change timer.
  (`self.CheckChangeTimer`)
  (`self.OnChangeTimerStateChanged` null (`self.ChangeTimerEnabled`)))

(fn `OnRep_ReplicatedChangeValue`
  ;[1 1 1] Try to set change value on clients.
  (if (not (`KismetSystemLibrary.IsServer`))
    (`self.SetChangeValueLocal` (`self.ReplicatedChangeValue`))))

(fn `OnRep_ReplicatedCurrentValue`
  ;[1 1 1] Try to set current value on clients.
  (if (not (`KismetSystemLibrary.IsServer`))
    (`self.SetCurrentValueLocal` (`self.ReplicatedCurrentValue`) false true)))

(fn `OnRep_ReplicatedMaxValue`
  ;[1 1 1] Try to set max value on clients.
  (if (not (`KismetSystemLibrary.IsServer`))
    (`self.SetMaxValueLocal` (`self.ReplicatedMaxValue`))))

(fn `OnRep_ReplicatedMinValue`
  ;[1 1 1] Try to set min value on clients.
  (if (not (`KismetSystemLibrary.IsServer`))
    (`self.SetMinValueLocal` (`self.ReplicatedMinValue`))))

(fn `SetChangeTimerEnabled`
  (params (Enabled :type Boolean))
  (returns (Success :type Boolean))
  ;[1 1 1] Enable or disable change timer.
  (if (!= Enabled (`self.ChangeTimerEnabled`))
    (set `self.ChangeTimerEnabled` Enabled))
  (return true))

(fn `SetChangeValue`
  (params (Value :type "Float (double-precision)"))
  (returns (Success :type Boolean))
  (locals (LocalNewValue :type "Float (double-precision)") (LocalPrevValue :type "Float (double-precision)"))
  ;[1 1 1] Try to set new value for the change value variable on the server.
  (if (`KismetSystemLibrary.IsServer`)
    (bind (_success _newvalue _prevvalue) (`self.SetChangeValueLocal` Value))
    (if _success
      (bind _output_get (set `local.LocalNewValue` _newvalue))
      (bind _output_get_2 (set `local.LocalPrevValue` _prevvalue))
      (`self.OnChangeValueChanged_Server` self _output_get _output_get_2)
      (if (`self.ReplicateValues`)
        (set `self.ReplicatedChangeValue` (`self.ChangeValue`)))
      (return true)
      (else
        (return true)))
    (else
      (return false))))

(fn `SetChangeValueLocal`
  (params (Value :type "Float (double-precision)"))
  (returns (Success :type Boolean) (NewValue :type "Float (double-precision)") (PrevValue :type "Float (double-precision)"))
  (locals (LocalNewValue :type "Float (double-precision)") (LocalPrevValue :type "Float (double-precision)"))
  ;[1 1 1] Try to set new value for the change value variable on the local machine.
  (bind _output_get (set `local.LocalNewValue` Value))
  (bind _output_get_2 (set `local.LocalPrevValue` (`self.ChangeValue`)))
  (if (!= _output_get _output_get_2)
    (set `self.ChangeValue` (`local.LocalNewValue`))
    (`self.CheckChangeTimer`)
    (`self.OnChangeValueChanged_Client` self (`local.LocalNewValue`) (`local.LocalPrevValue`))
    (return true (`local.LocalNewValue`) (`local.LocalPrevValue`))
    (else
      (return false 0.0 0.0))))

(fn `SetCurrentValue`
  (params (Value :type "Float (double-precision)") (Percent :type Boolean))
  (returns (Success :type Boolean))
  (locals (LocalNewValue :type "Float (double-precision)" :default 0.0) (LocalPrevValue :type "Float (double-precision)" :default 0.0))
  ;[1 1 1] Try to set new value for the current value variable on the server.
  (if (`KismetSystemLibrary.IsServer`)
    (bind (_success _newvalue _prevvalue) (`self.SetCurrentValueLocal` Value Percent true))
    (if _success
      (bind _output_get (set `local.LocalNewValue` _newvalue))
      (bind _output_get_2 (set `local.LocalPrevValue` _prevvalue))
      (`self.OnCurrentValueChanged_Server` self _output_get _output_get_2)
      (if (`self.ReplicateValues`)
        (set `self.ReplicatedCurrentValue` (`self.CurrentValue`)))
      (return true)
      (else
        (return true)))
    (else
      (return false))))

(fn `SetCurrentValueLocal`
  (params (Value :type "Float (double-precision)") (Percent :type Boolean) (CallClientEvent :type Boolean))
  (returns (Success :type Boolean) (NewValue :type "Float (double-precision)") (PrevValue :type "Float (double-precision)"))
  (locals (LocalNewValue :type "Float (double-precision)") (LocalPrevValue :type "Float (double-precision)") (LocalCallClientEvent :type Boolean))
  (bind _maxvalue (`self.MaxValue`))
  ;[1 1 1] Try to set new value for the current value variable on the local machine.
  (set `local.LocalCallClientEvent` CallClientEvent)
  (bind _output_get (set `local.LocalPrevValue` (`self.CurrentValue`)))
  (bind _output_get_2 (set `local.LocalNewValue` (`KismetMathLibrary.FClamp` (`KismetMathLibrary.SelectFloat` (* Value _maxvalue) Value Percent) (`self.MinValue`) _maxvalue)))
  (if (!= _output_get_2 _output_get)
    (set `self.CurrentValue` _output_get_2)
    (if (`local.LocalCallClientEvent`)
      (`self.OnCurrentValueChanged_Client` self (`local.LocalNewValue`) (`local.LocalPrevValue`)))
    (return true (`local.LocalNewValue`) (`local.LocalPrevValue`))
    (else
      (return false 0.0 0.0))))

(fn `SetMaxValue`
  (params (Value :type "Float (double-precision)"))
  (returns (Success :type Boolean))
  (locals (LocalNewValue :type "Float (double-precision)") (LocalPrevValue :type "Float (double-precision)"))
  ;[1 1 1] Try to set new value for the max value variable on the server.
  (if (`KismetSystemLibrary.IsServer`)
    (bind (_success _newvalue _prevvalue) (`self.SetMaxValueLocal` Value))
    (if _success
      (bind _output_get (set `local.LocalNewValue` _newvalue))
      (bind _output_get_2 (set `local.LocalPrevValue` _prevvalue))
      (`self.OnMaxValueChanged_Server` self _output_get _output_get_2)
      (`self.SetCurrentValue` (`self.CurrentValue`))
      (if (`self.ReplicateValues`)
        (set `self.ReplicatedMaxValue` (`self.MaxValue`)))
      (return true)
      (else
        (return true)))
    (else
      (return false))))

(fn `SetMaxValueLocal`
  (params (Value :type "Float (double-precision)"))
  (returns (Success :type Boolean) (NewValue :type "Float (double-precision)") (PrevValue :type "Float (double-precision)"))
  (locals (LocalNewValue :type "Float (double-precision)") (LocalPrevValue :type "Float (double-precision)"))
  ;[1 1 1] Try to set new value for the max value variable on the local machine.
  (bind _output_get (set `local.LocalNewValue` Value))
  (bind _output_get_2 (set `local.LocalPrevValue` (`self.MaxValue`)))
  (if (!= _output_get _output_get_2)
    (set `self.MaxValue` (`local.LocalNewValue`))
    (`self.SetCurrentValueLocal` (`self.CurrentValue`) false true)
    (`self.OnMaxValueChanged_Client` self (`local.LocalNewValue`) (`local.LocalPrevValue`))
    (return true (`local.LocalNewValue`) (`local.LocalPrevValue`))
    (else
      (return false 0.0 0.0))))

(fn `SetMinValue`
  (params (Value :type "Float (double-precision)"))
  (returns (Success :type Boolean))
  (locals (LocalNewValue :type "Float (double-precision)") (LocalPrevValue :type "Float (double-precision)"))
  ;[1 1 1] Try to set new value for the min value variable on the server.
  (if (`KismetSystemLibrary.IsServer`)
    (bind (_success _newvalue _prevvalue) (`self.SetMinValueLocal` Value))
    (if _success
      (bind _output_get (set `local.LocalNewValue` _newvalue))
      (bind _output_get_2 (set `local.LocalPrevValue` _prevvalue))
      (`self.OnMinValueChanged_Server` self _output_get _output_get_2)
      (`self.SetCurrentValue` (`self.CurrentValue`))
      (if (`self.ReplicateValues`)
        (set `self.ReplicatedMinValue` (`self.MinValue`)))
      (return true)
      (else
        (return true)))
    (else
      (return false))))

(fn `SetMinValueLocal`
  (params (Value :type "Float (double-precision)"))
  (returns (Success :type Boolean) (NewValue :type "Float (double-precision)") (PrevValue :type "Float (double-precision)"))
  (locals (LocalNewValue :type "Float (double-precision)") (LocalPrevValue :type "Float (double-precision)"))
  ;[1 1 1] Try to set new value for the min value variable on the local machine.
  (bind _output_get (set `local.LocalNewValue` Value))
  (bind _output_get_2 (set `local.LocalPrevValue` (`self.MaxValue`)))
  (if (!= _output_get _output_get_2)
    (set `self.MinValue` (`local.LocalNewValue`))
    (`self.SetCurrentValueLocal` (`self.CurrentValue`) false true)
    (`self.OnMinValueChanged_Client` self (`local.LocalNewValue`) (`local.LocalPrevValue`))
    (return true (`local.LocalNewValue`) (`local.LocalPrevValue`))
    (else
      (return false 0.0 0.0))))

(fn `StartChangeTimer`
  (returns (Success :type Boolean))
  ;[1 1 1] Start change value ticks for the stat attribute.
  (if (> (`self.ChangeTimerTickInterval`) 0.0)
    (`self.SetComponentTickEnabled` false)
    (bind _returnvalue (`KismetSystemLibrary.K2_SetTimerDelegate` (`|CreateDelegate` :!event `Bind_ChangeTimerTick`) (`self.ChangeTimerTickInterval`) true))
    (set `self.ChangeTimer` _returnvalue)
    (else
      (`self.SetComponentTickEnabled` true)
      (`KismetSystemLibrary.K2_ClearAndInvalidateTimerHandle` (`self.ChangeTimer`))))
  (return true))

(fn `StopChangeTimer`
  (returns (Success :type Boolean))
  ;[1 1 1] Stop change value ticks for the stat attribute.
  (`KismetSystemLibrary.K2_ClearAndInvalidateTimerHandle` (`self.ChangeTimer`))
  (`self.SetComponentTickEnabled` false)
  (return true))

(fn `TryInitComponent`
  (returns (Success :type Boolean))
  ;[1 1 1] Try to init stat attribute component.
  (if (not (`self.IsInitialized`))
    (bind _success (`self.InitComponent`))
    (bind _output_get (set `self.IsInitialized` _success))
    (return _output_get)
    (else
      (return true))))

(fn `UpdateAttributeValues`
  (returns (Success :type Boolean))
  (locals (LocalChangedAttributes :type "Array of /Game/BPS_Core/Blueprints/Systems/AttributesSystem/Structures/STR_Attribute Structure"))
  ;[1 1 1] Try to update attributes and set stat attribute values.
  (bind _attributes (`/Game/BPS_Core/Blueprints/Systems/AttributesSystem/Components/BP_AC_AttributesManager.GetAttributes` (`self.AttributesComponent`)))
  (set `self.CurrentAttributes` _attributes)
  (`|ExecutionSequence`
    (:`then_0`
      (if (`BlueprintGameplayTagLibrary.IsGameplayTagValid` (`self.MinValueAttributeTag`))
        (bind (_success _value) (`/Game/BPS_Core/Blueprints/Systems/AttributesSystem/Libraries/BP_Library_Attributes.GetAttributeValue` (`self.CurrentAttributes`) (`self.MinValueAttributeTag`)))
        (`self.SetMinValue` _value)))
    (:`then_1`
      (`|ExecutionSequence`
        (:`then_0`
          (if (`BlueprintGameplayTagLibrary.IsGameplayTagValid` (`self.MaxValueAttributeTag`))
            (bind (_success_2 _value_2) (`/Game/BPS_Core/Blueprints/Systems/AttributesSystem/Libraries/BP_Library_Attributes.GetAttributeValue` (`self.CurrentAttributes`) (`self.MaxValueAttributeTag`)))
            (`self.SetMaxValue` _value_2)))
        (:`then_1`
          (`|ExecutionSequence`
            (:`then_0`
              (if (`BlueprintGameplayTagLibrary.IsGameplayTagValid` (`self.ChangeValueAttributeTag`))
                (bind (_success_3 _value_3) (`/Game/BPS_Core/Blueprints/Systems/AttributesSystem/Libraries/BP_Library_Attributes.GetAttributeValue` (`self.CurrentAttributes`) (`self.ChangeValueAttributeTag`)))
                (`self.SetChangeValue` _value_3)))
            (:`then_1`
              (return true))))))))

(fn `UseAttributes`
  (returns (Result :type Boolean))
  ;[1 1 1] Determines whether to use an attribute component.
  (return (or (`BlueprintGameplayTagLibrary.IsGameplayTagValid` (`self.MinValueAttributeTag`)) (`BlueprintGameplayTagLibrary.IsGameplayTagValid` (`self.MaxValueAttributeTag`)) (`BlueprintGameplayTagLibrary.IsGameplayTagValid` (`self.ChangeValueAttributeTag`)))))