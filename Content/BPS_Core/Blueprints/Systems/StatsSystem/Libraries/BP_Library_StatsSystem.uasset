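; Blueprint function library for the stats system that locates stat attribute components on an actor and queries them.
; Generic lookup prefers a name over a gameplay tag, returning the first matching BP_AC_StatAttribute component, while health and energy have dedicated class-based finders.
; Value checks delegate to the found component, and alive checks, including a pure wrapper, use the health component.
; Queries return false when no component is found.
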(fn `CheckActorIsAlive`
  (params (TargetActor :type "Actor Object Reference"))
  (returns (IsAlive :type Boolean))
  ;[1 1 1] Returns true if target actor is alive.
  (bind (_found _component) (`self.FindHealthStatAttributeComponent` TargetActor))
  (if _found
    (return (`/Game/BPS_Core/Blueprints/Systems/StatsSystem/Components/BP_AC_StatAttribute_Health.IsAlive` _component))
    (else
      (return false))))

(fn `CheckActorIsAlivePure`
  (params (TargetActor :type "Actor Object Reference"))
  (returns (IsAlive :type Boolean))
  ;[1 1 1] Returns true if target actor is alive.
  (bind _isalive (`self.CheckActorIsAlive` TargetActor))
  (return _isalive))

(fn `CheckStatAttributeValue`
  (params (TargetActor :type "Actor Object Reference") (StatAttributeName :type Name) (StatAttributeTag :type "GameplayTag Structure") (Value :type "Float (double-precision)") (Percent :type Boolean))
  (returns (Result :type Boolean))
  ;[1 1 1] Returns true if actor has stat attribute which current value is greater than or equal to the target value.
  (bind (_found _component) (`self.FindStatAttributeComponent` TargetActor StatAttributeName StatAttributeTag))
  (if _found
    (bind _result (`/Game/BPS_Core/Blueprints/Systems/StatsSystem/Components/BP_AC_StatAttribute.CheckStatAttributeValue` _component Value Percent))
    (return _result)
    (else
      (return false))))

(fn `FindEnergyStatAttributeComponent`
  (params (TargetActor :type "Actor Object Reference"))
  (returns (Found :type Boolean) (Component :type "/Game/BPS_Core/Blueprints/Systems/StatsSystem/Components/BP_AC_StatAttribute_Energy Object Reference"))
  (locals (LocalComponent :type "/Game/BPS_Core/Blueprints/Systems/StatsSystem/Components/BP_AC_StatAttribute_Energy Object Reference"))
  ;[1 1 1] Try to find energy stat attribute component.
  (bind _output_get (set `local.LocalComponent` (`Actor.GetComponentByClass` TargetActor "/Game/BPS_Core/Blueprints/Systems/StatsSystem/Components/BP_AC_StatAttribute_Energy.BP_AC_StatAttribute_Energy_C")))
  (`/Engine/EditorBlueprintResources/StandardMacros.IsValid` _output_get
    (:`Is Valid`
      (return true _output_get))
    (:`Is Not Valid`
      (return false null))))

(fn `FindHealthStatAttributeComponent`
  (params (TargetActor :type "Actor Object Reference"))
  (returns (Found :type Boolean) (Component :type "/Game/BPS_Core/Blueprints/Systems/StatsSystem/Components/BP_AC_StatAttribute_Health Object Reference"))
  (locals (LocalComponent :type "/Game/BPS_Core/Blueprints/Systems/StatsSystem/Components/BP_AC_StatAttribute_Health Object Reference"))
  ;[1 1 1] Try to find health stat attribute component.
  (bind _output_get (set `local.LocalComponent` (`Actor.GetComponentByClass` TargetActor "/Game/BPS_Core/Blueprints/Systems/StatsSystem/Components/BP_AC_StatAttribute_Health.BP_AC_StatAttribute_Health_C")))
  (`/Engine/EditorBlueprintResources/StandardMacros.IsValid` _output_get
    (:`Is Valid`
      (return true _output_get))
    (:`Is Not Valid`
      (return false null))))

(fn `FindStatAttributeComponent`
  (params (TargetActor :type "Actor Object Reference") (StatAttributeName :type Name) (StatAttributeTag :type "GameplayTag Structure"))
  (returns (Found :type Boolean) (Component :type "/Game/BPS_Core/Blueprints/Systems/StatsSystem/Components/BP_AC_StatAttribute Object Reference"))
  (locals (LocalTargetActor :type "Actor Object Reference") (LocalStatAttributeName :type Name) (LocalStatAttributeTag :type "GameplayTag Structure"))
  ;[1 1 1] Try to find stat attribute component by name or tag.
  (set `local.LocalTargetActor` TargetActor)
  (bind _output_get (set `local.LocalStatAttributeName` StatAttributeName))
  (bind _output_get_2 (set `local.LocalStatAttributeTag` StatAttributeTag))
  (if (!= _output_get "None")
    (bind (_found _component) (`self.FindStatAttributeComponentByName` (`local.LocalTargetActor`) (`local.LocalStatAttributeName`)))
    (return _found _component)
    (elif (`BlueprintGameplayTagLibrary.IsGameplayTagValid` _output_get_2)
      (bind (_found_2 _component_2) (`self.FindStatAttributeComponentByTag` (`local.LocalTargetActor`) (`local.LocalStatAttributeTag`)))
      (return _found_2 _component_2)
      (else
        (return false null)))))

(fn `FindStatAttributeComponentByName`
  (params (TargetActor :type "Actor Object Reference") (StatAttributeName :type Name))
  (returns (Found :type Boolean) (Component :type "/Game/BPS_Core/Blueprints/Systems/StatsSystem/Components/BP_AC_StatAttribute Object Reference"))
  ;[1 1 1] Try to find stat attribute component by name.
  (for _array_element (`Actor.K2_GetComponentsByClass` TargetActor "/Game/BPS_Core/Blueprints/Systems/StatsSystem/Components/BP_AC_StatAttribute.BP_AC_StatAttribute_C")
    (bind _result (`/Game/BPS_Core/Blueprints/Systems/StatsSystem/Components/BP_AC_StatAttribute.CheckStatAttributeName` _array_element StatAttributeName))
    (if _result
      (return true _array_element)))
  (return false null))

(fn `FindStatAttributeComponentByTag`
  (params (TargetActor :type "Actor Object Reference") (StatAttributeTag :type "GameplayTag Structure"))
  (returns (Found :type Boolean) (Component :type "/Game/BPS_Core/Blueprints/Systems/StatsSystem/Components/BP_AC_StatAttribute Object Reference"))
  ;[1 1 1] Try to find stat attribute component by tag.
  (for _array_element (`Actor.K2_GetComponentsByClass` TargetActor "/Game/BPS_Core/Blueprints/Systems/StatsSystem/Components/BP_AC_StatAttribute.BP_AC_StatAttribute_C")
    (bind _result (`/Game/BPS_Core/Blueprints/Systems/StatsSystem/Components/BP_AC_StatAttribute.CheckStatAttributeTag` _array_element StatAttributeTag))
    (if _result
      (return true _array_element)))
  (return false null))