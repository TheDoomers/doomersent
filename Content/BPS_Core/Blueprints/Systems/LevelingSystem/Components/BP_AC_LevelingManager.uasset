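; Replicated leveling component that manages experience, levels, skill points, and learned attributes and skills, with per-player save/load.
; Changes route to the server, and RepNotifies broadcast them to listeners.
; Experience, adjustable by listeners and also received through player gameplay events, drives level-ups that grant points spent on attributes or on data-table skills with level, point and attribute requirements.
; Learned attributes and skill bonuses feed the Attributes Manager as named bonus sets.
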(event Custom|TryAddExperience%20%28Server%29
  (params (ActivityLevel :type Integer) (ExperienceToAdd :type Float%20%28double-precision%29))
  ;[1 1 1] Network events.
  (LevelingManager|TryAddExperience ActivityLevel ExperienceToAdd))

(event Custom|TryAddSkillPoints%20%28Server%29
  (params (PointsToAdd :type Integer))
  ;[1 1 1] Network events.
  (LevelingManager|TryAddSkillPoints PointsToAdd))

(event Custom|TryUpLevel%20%28Server%29
  (params (RemoveExp :type Boolean))
  ;[1 1 1] Network events.
  (LevelingManager|TryUpLevel RemoveExp))

(event Custom|TryLearnAttribute%20%28Server%29
  (params (Attribute :type STR%20Attribute%20Structure) (SkillPoints :type Integer))
  ;[1 1 1] Network events.
  (LevelingManager|TryLearnAttribute Attribute SkillPoints))

(event Custom|TryLearnSkill%20%28Server%29
  (params (SkillHandle :type Data%20Table%20Row%20Handle%20Structure) (SkillLevel :type Integer))
  ;[1 1 1] Network events.
  (LevelingManager|TryLearnSkill SkillHandle SkillLevel))

(event EventBeginPlay
  ;[1 1 1] Begin play. Try init component.
  (if (Variables|Settings|GetInitOnBeginPlay)
    (LevelingManager|TryInitComponent)))

(fn TryInitComponent
  ;[1 1 1] Try to init leveling manager component.
  (if (not (Variables|State|GetIsInitialized))
    (bind _success (LevelingManager|InitComponent))
    (bind _output_get (Variables|State|SetIsInitialized _success))
    (return _output_get)
    (else
      (return true))))

(fn InitComponent
  ;[1 1 1] Try to init component and initial variables.
  (Utilities|FlowControl|Sequence
    (:then_0
      (bind _output_get (Variables|State|SetCurrentLevel (Variables|Settings|GetInitialLevel)))
      (Variables|State|SetSkillPoints (Variables|Settings|GetInitialSkillPoints))
      (bind _requiredexperience (LevelingManager|CalculateLevelExperience _output_get))
      (Variables|State|SetRequiredExperience _requiredexperience))
    (:then_1
      (Utilities|FlowControl|Sequence
        (:then_0
          (bind _values (Utilities|Map|Values (Variables|Settings|GetInitialAttributesMapped)))
          (if (Utilities|Array|IsValidIndex _values)
            (Variables|State|SetLearnedAttributes _values)
            (else
              (Variables|State|SetLearnedAttributes (Variables|Settings|GetInitialAttributes)))))
        (:then_1
          (Utilities|FlowControl|Sequence
            (:then_0
              (bind _values_2 (Utilities|Map|Values (Variables|Settings|GetInitialSkillsDataMapped)))
              (if (Utilities|Array|IsValidIndex _values_2)
                (Variables|State|SetLearnedSkillsData _values_2)
                (else
                  (Variables|State|SetLearnedSkillsData (Variables|Settings|GetInitialSkillsData)))))
            (:then_1
              (Utilities|FlowControl|Sequence
                (:then_0
                  (bind _asplayer_controller (Utilities|Casting|CastToPlayerController (Components|GetOwner)))
                  (bind _output_get_2 (Variables|State|SetPlayerController _asplayer_controller))
                  (Utilities|IsValid _output_get_2
                    (:Is%20Valid
                      (bind (_success _manager) (CallFunction|FindGameplayEventsManager))
                      (if _success
                        (EventDispatchers|BindEventtoOnPlayerGameplayEventPlayed _manager (EventDispatchers|CreateEvent :!event BindonPlayerGameplayEventPlayed))))))
                (:then_1
                  (return true))))))))))

(fn SetAttributesManager
  (params (AttributesManager :type BP%20AC%20Attributes%20Manager%20Object%20Reference))
  ;[1 1 1] Set attributes manager component reference and update learned attributes and skills.
  (bind _output_get (Variables|State|SetAttributesManager AttributesManager))
  (Utilities|IsValid _output_get
    (:Is%20Valid
      (EventDispatchers|BindEventtoOnAttributesChangedReplicated _output_get (EventDispatchers|CreateEvent :!event BindonAttributesChanged))
      (LevelingManager|UpdateLearnedAttributes)
      (LevelingManager|UpdateLearnedSkillsAttributes))))

(fn TryAddExperience
  (params (ActivityLevel :type Integer) (ExperienceToAdd :type Float%20%28double-precision%29))
  (bind _playercontroller (Variables|State|GetPlayerController))
  ;[1 1 1] Try to add experience.
  (LocalVariables|SetLocalActivityLevel ActivityLevel)
  (LocalVariables|SetLocalExperienceToAdd ExperienceToAdd)
  (if (Networking|IsServer)
    (bind _canuplevel (LevelingManager|CheckMaxLevel))
    (if _canuplevel
      (bind _output_get (Variables|State|SetCurrentExperienceToAdd ExperienceToAdd))
      (Default|CallOnAttemptAddExperience self (LocalVariables|GetLocalActivityLevel) _output_get)
      (Utilities|FlowControl|Sequence
        (:then_0
          (LevelingManager|SetCurrentExperience (+ (Variables|State|GetCurrentExperience) (Variables|State|GetCurrentExperienceToAdd))))
        (:then_1
          (Utilities|FlowControl|Sequence
            (:then_0
              (if (Variables|Settings|GetCallExperienceEvent)
                (Utilities|IsValid _playercontroller
                  (:Is%20Valid
                    (Variables|State|SetIgnoreExperienceEvent true)
                    (CallFunction|TryRunPlayerGameplayEvent _playercontroller (Utilities|Struct|MakeSTR_EventSettings "AddExperience" (Utilities|Map|MakeMap "ActivityLevel" (LocalVariables|GetLocalActivityLevel)) (Utilities|Map|MakeMap "Experience" (LocalVariables|GetLocalExperienceToAdd))))
                    (Variables|State|SetIgnoreExperienceEvent false)))))
            (:then_1
              (return true)))))
      (else
        (return true)))
    (else
      (CallFunction|TryAddExperience(Server) ActivityLevel ExperienceToAdd)
      (return true))))

(fn SetCurrentExperience
  (params (NewExperience :type Float%20%28double-precision%29))
  ;[1 1 1] Set current experienc and check level up.
  (if (and (> NewExperience 0.0) (!= NewExperience (Variables|State|GetCurrentExperience)))
    (bind _output_get (Variables|State|SetCurrentExperience NewExperience))
    (while (>= _output_get (Variables|State|GetRequiredExperience))
      (LevelingManager|TryUpLevel true))
    (return true)))

(fn SetCurrentExperiencetoAdd
  (params (ExperienceToAdd :type Float%20%28double-precision%29))
  ;[1 1 1] Set current experience to add variable. Allows to modify received experience.
  (Variables|State|SetCurrentExperienceToAdd ExperienceToAdd)
  (return true))

(fn TryUpLevel
  (params (RemoveExp :type Boolean))
  ;[1 1 1] Try to up level and update experience and skill points.
  (if (Networking|IsServer)
    (bind _canuplevel (LevelingManager|CheckMaxLevel))
    (if _canuplevel
      (bind _output_get (Variables|State|SetCurrentLevel (+ (stale _output_get) 1)))
      (if RemoveExp
        (bind _output_get_2 (Variables|State|SetCurrentExperience (- (stale _output_get_2) (Variables|State|GetRequiredExperience)))))
      (bind _requiredexperience (LevelingManager|CalculateLevelExperience (Variables|State|GetCurrentLevel)))
      (Variables|State|SetRequiredExperience _requiredexperience)
      (LevelingManager|TryAddSkillPoints (Variables|Settings|GetSkillPointsPerLevel))
      (return true)
      (else
        _))
    (else
      (CallFunction|TryUpLevel(Server) RemoveExp)))
  (return true))

(fn TryAddSkillPoints
  (params (PointsToAdd :type Integer))
  ;[1 1 1] Try to add skill points.
  (if (Networking|IsServer)
    (Variables|State|SetSkillPoints (+ (Variables|State|GetSkillPoints) PointsToAdd))
    (return true)
    (else
      (CallFunction|TryAddSkillPoints(Server) PointsToAdd)
      (return true))))

(fn CalculateLevelExperience
  (params (CurrentLevel :type Integer))
  ;[1 1 1] Calculate level experience.
  (return (|(((Level-1)*500)+1000) (Math|Conversions|ToFloat(Integer) CurrentLevel))))

(fn OnRepCurrentLevel
  (bind _currentlevel (Variables|State|GetCurrentLevel))
  ;[1 1 1] Notify all clients that level was changed.
  (Default|CallOnCurrentLevelChanged self _currentlevel (Variables|State|GetPrevLevel))
  (Variables|State|SetPrevLevel _currentlevel)
  (Default|CallOnCheckSkillRequirements self))

(fn OnRepSkillPoints
  (bind _skillpoints (Variables|State|GetSkillPoints))
  ;[1 1 1] Notify all clients that amount of skill points was changed.
  (Default|CallOnSkillPointsChanged self _skillpoints (Variables|State|GetPrevSkillPoints))
  (Variables|State|SetPrevSkillPoints _skillpoints)
  (Default|CallOnCheckSkillRequirements self))

(fn OnRepCurrentExperience
  (bind _self self)
  (bind _currentexperience (Variables|State|GetCurrentExperience))
  ;[1 1 1] Notify all clients that value of experience was changed.
  (Default|CallOnCurrentExperienceChanged _self _currentexperience (Variables|State|GetPrevExperience))
  (if (> _currentexperience (Variables|State|GetPrevExperience))
    (Default|CallOnExperienceReceived _self _currentexperience (- _currentexperience (Variables|State|GetPrevExperience))))
  (Variables|State|SetPrevExperience _currentexperience))

(fn OnRepRequiredExperience
  (bind _requiredexperience (Variables|State|GetRequiredExperience))
  ;[1 1 1] Notify that required experience value is changed.
  (Default|CallOnRequiredExperienceChanged self _requiredexperience (Variables|State|GetPrevRequiredExperience))
  (Variables|State|SetPrevRequiredExperience _requiredexperience))

(fn GetCurrentLevel
  ;[1 1 1] Returns current level.
  (return (Variables|State|GetCurrentLevel)))

(fn GetSkillPoints
  ;[1 1 1] Returns skill points.
  (return (Variables|State|GetSkillPoints)))

(fn GetCurrentExperience
  ;[1 1 1] Returns current experience.
  (return (Variables|State|GetCurrentExperience)))

(fn GetRequiredExperience
  ;[1 1 1] Returns required experience.
  (return (Variables|State|GetRequiredExperience)))

(fn CheckMaxLevel
  (bind _maxlevel (Variables|Settings|GetMaxLevel))
  ;[1 1 1] Returns true if level can be increased.
  (if (<= _maxlevel 0)
    (return true)
    (else
      (return (< (Variables|State|GetCurrentLevel) _maxlevel)))))

(fn TryLearnAttribute
  (params (Attribute :type STR%20Attribute%20Structure) (SkillPoints :type Integer))
  ;[1 1 1] Try to learn attribute and spend skill points.
  (if (Networking|IsServer)
    (if (>= (Variables|State|GetSkillPoints) SkillPoints)
      (bind _success (LevelingManager|LearnAttribute Attribute SkillPoints))
      (return _success)
      (else
        (return false)))
    (else
      (CallFunction|TryLearnAttribute(Server) Attribute SkillPoints)
      (return true))))

(fn LearnAttribute
  (params (Attribute :type STR%20Attribute%20Structure) (SkillPoints :type Integer))
  ;[1 1 1] Learn specific attribute and spend skill points on it.
  (if (>= (Variables|State|GetSkillPoints) SkillPoints)
    (CallFunction|AddAttribute (Variables|State|GetLearnedAttributes) Attribute)
    (Variables|State|SetSkillPoints (- (Variables|State|GetSkillPoints) SkillPoints))
    (LevelingManager|UpdateLearnedAttributes)
    (return true)
    (else
      (return false))))

(fn GetLearnedAttributes
  ;[1 1 1] Returns learned attributes list.
  (return (Variables|State|GetLearnedAttributes)))

(fn GetLearnedAttributesPure
  ;[1 1 1] Returns learned attributes list.
  (bind _learnedattributes (LevelingManager|GetLearnedAttributes))
  (return _learnedattributes))

(fn UpdateLearnedAttributes
  (bind _playercontroller (Variables|State|GetPlayerController))
  (bind _attributesmanager (Variables|State|GetAttributesManager))
  (bind _returnvalue (Pawn|GetControlledPawn _playercontroller))
  ;[1 1 1] Update learned attributes it in the referenced attributes manager.
  (Utilities|IsValid _attributesmanager
    (:Is%20Valid
      (LocalVariables|SetLocalAttributesManager _attributesmanager)
      (bind _success (Default|UpdateBonusAttributesSet (LocalVariables|GetLocalAttributesManager) (Utilities|Struct|MakeSTR_AttributesSet "LearnedAttributes" (Variables|State|GetLearnedAttributes)) :!label _label))
      (return _success))
    (:Is%20Not%20Valid
      (Utilities|IsValid _playercontroller
        (:Is%20Valid
          (Utilities|IsValid _returnvalue
            (:Is%20Valid
              (bind (_found _component) (CallFunction|FindAttributesManager _returnvalue))
              (if _found
                (LocalVariables|SetLocalAttributesManager _component)
                (goto _label)))))
        (:Is%20Not%20Valid
          (bind (_found_2 _component_2) (CallFunction|FindAttributesManager (Components|GetOwner)))
          (if _found_2
            (LocalVariables|SetLocalAttributesManager _component_2)
            (goto _label)))))))

(fn TryLearnSkill
  (params (SkillHandle :type Data%20Table%20Row%20Handle%20Structure) (SkillLevel :type Integer))
  ;[1 1 1] Try to learn skill to target skill level.
  (LocalVariables|SetLocalSkillHandle SkillHandle)
  (LocalVariables|SetLocalSkillLevel SkillLevel)
  (if (Networking|IsServer)
    (bind _success (LevelingManager|CheckSkillRequirements (LocalVariables|GetLocalSkillHandle) (LocalVariables|GetLocalSkillLevel)))
    (if _success
      (bind _success_2 (LevelingManager|LearnSkill (LocalVariables|GetLocalSkillHandle) (LocalVariables|GetLocalSkillLevel)))
      (return _success_2)
      (else
        (return false)))
    (else
      (CallFunction|TryLearnSkill(Server) (LocalVariables|GetLocalSkillHandle) (LocalVariables|GetLocalSkillLevel))
      (return true))))

(fn LearnSkill
  (params (SkillHandle :type Data%20Table%20Row%20Handle%20Structure) (SkillLevel :type Integer))
  ;[1 1 1] Learn skill to target level by specific skill handle.
  (bind _output_get (LocalVariables|SetLocalSkillHandle SkillHandle))
  (bind _output_get_2 (LocalVariables|SetLocalSkillLevel SkillLevel))
  (Utilities|IsValid (.DataTable (Utilities|Struct|BreakDataTableRowHandle _output_get))
    (:Is%20Valid
      (bind _returnvalue (Utilities|GetDataTableRow (.DataTable (Utilities|Struct|BreakDataTableRowHandle _output_get)) (.RowName (Utilities|Struct|BreakDataTableRowHandle _output_get)))
        (:then
          (bind (_success _requireddescription _requiredskillpoints) (CallFunction|FindLevelSkillRequirements _returnvalue _output_get_2))
          (if _success
            (if (>= (Variables|State|GetSkillPoints) _requiredskillpoints)
              (bind _output_get_3 (Variables|State|SetSkillPoints (- (stale _output_get_3) _requiredskillpoints)))
              (LevelingManager|AddSkillData (Utilities|Struct|MakeSTR_SkillData (LocalVariables|GetLocalSkillHandle) (LocalVariables|GetLocalSkillLevel)))
              (return true)
              (else
                _))))
        (:RowNotFound
          _)))
    (:Is%20Not%20Valid
      _))
  (return false))

(fn CheckSkillRequirements
  (params (SkillHandle :type Data%20Table%20Row%20Handle%20Structure) (SkillLevel :type Integer))
  (bind (_datatable _rowname) (Utilities|Struct|BreakDataTableRowHandle SkillHandle))
  (bind _playercontroller (Variables|State|GetPlayerController))
  (bind _returnvalue (Pawn|GetControlledPawn _playercontroller))
  ;[1 1 1] Returns true if skill can be learned to target skill level.
  (Utilities|IsValid _datatable
    (:Is%20Valid
      (bind _returnvalue_2 (Utilities|GetDataTableRow _datatable _rowname)
        (:then
          (bind (_success _requireddescription _requiredskillpoints _requiredlevel _requiredattributes) (CallFunction|FindLevelSkillRequirements _returnvalue_2 SkillLevel))
          (if _success
            (LocalVariables|SetLocalRequiredSkillPoints _requiredskillpoints)
            (LocalVariables|SetLocalRequiredLevel _requiredlevel)
            (LocalVariables|SetLocalRequiredAttributes _requiredattributes)
            (if (>= (Variables|State|GetSkillPoints) (LocalVariables|GetLocalRequiredSkillPoints))
              (if (>= (Variables|State|GetCurrentLevel) (LocalVariables|GetLocalRequiredLevel))
                (Utilities|IsValid _playercontroller
                  (:Is%20Valid
                    (Utilities|IsValid _returnvalue
                      (:Is%20Valid
                        (bind (_found _component) (CallFunction|FindAttributesManager _returnvalue))
                        (if _found
                          (bind _attributes (Default|GetAttributes _component))
                          (bind _result (CallFunction|CheckRequiredAttributes _attributes (LocalVariables|GetLocalRequiredAttributes)))
                          (return _result)
                          (else
                            _)))
                      (:Is%20Not%20Valid
                        _)))
                  (:Is%20Not%20Valid
                    (bind (_found_2 _component_2) (CallFunction|FindAttributesManager (Components|GetOwner)))
                    (if _found_2
                      (bind _attributes_2 (Default|GetAttributes _component_2))
                      (bind _result_2 (CallFunction|CheckRequiredAttributes _attributes_2 (LocalVariables|GetLocalRequiredAttributes)))
                      (return _result_2)
                      (else
                        _))))))))
        (:RowNotFound
          _)))
    (:Is%20Not%20Valid
      _))
  (return false))

(fn AddSkillData
  (params (SkillData :type STR%20Skill%20Data%20Structure))
  ;[1 1 1] Add or update skill data to the learned skills list.
  (for (_array_element _array_index) (Variables|State|GetLearnedSkillsData)
    (if (CallFunction|HandlesAreEqual (Utilities|Struct|BreakSTR_SkillData _array_element) (Utilities|Struct|BreakSTR_SkillData SkillData))
      (Utilities|Array|SetArrayElem (Variables|State|GetLearnedSkillsData) _array_index SkillData)
      (Variables|State|SetLearnedSkillsData (Variables|State|GetLearnedSkillsData))
      (return true)))
  (Utilities|Array|Add (Variables|State|GetLearnedSkillsData) SkillData)
  (Variables|State|SetLearnedSkillsData (Variables|State|GetLearnedSkillsData))
  (return true))

(fn FindSkillData
  (params (SkillHandle :type Data%20Table%20Row%20Handle%20Structure))
  ;[1 1 1] Find skill data in the learned skills list by skill handle.
  (for _array_element (Variables|State|GetLearnedSkillsData)
    (if (CallFunction|HandlesAreEqual (Utilities|Struct|BreakSTR_SkillData _array_element) SkillHandle)
      (return true _array_element)))
  (return false ""))

(fn CheckSkillLevel
  (params (SkillHandle :type Data%20Table%20Row%20Handle%20Structure) (SkillLevel :type Integer))
  ;[1 1 1] Returns true if current level of the skill is more or equal target skill level.
  (bind (_found _skilldata) (LevelingManager|FindSkillData SkillHandle))
  (if _found
    (return (>= (Utilities|Struct|BreakSTR_SkillData _skilldata) SkillLevel))
    (else
      (return false))))

(fn GetLearnedSkills
  ;[1 1 1] Returns learned skills data.
  (return (Variables|State|GetLearnedSkillsData)))

(fn GetLearnedSkillsPure
  ;[1 1 1] Returns learned skills data.
  (bind _skillsdata (LevelingManager|GetLearnedSkills))
  (return _skillsdata))

(fn UpdateLearnedSkillsAttributes
  (bind _playercontroller (Variables|State|GetPlayerController))
  (bind _attributesmanager (Variables|State|GetAttributesManager))
  (bind _returnvalue (Pawn|GetControlledPawn _playercontroller))
  ;[1 1 1] Update learned skills and bonus attributes in the referenced attributes manager.
  (Utilities|IsValid _attributesmanager
    (:Is%20Valid
      (LocalVariables|SetLocalAttributesManager _attributesmanager)
      (for _array_element (Variables|State|GetLearnedSkillsData) :!label _label
        (bind (_success _skillinstance) (CallFunction|MakeSkillInstance (.SkillHandle (Utilities|Struct|BreakSTR_SkillData _array_element))))
        (if _success
          (LocalVariables|SetLocalSkillInstance _skillinstance)
          (bind _output_get (LocalVariables|SetLocalSkillLevel (.SkillLevel (Utilities|Struct|BreakSTR_SkillData _array_element))))
          (bind _resultattribute (CallFunction|MultiplyAttribute (Utilities|Struct|BreakSTR_SkillInstance _skillinstance) (Math|Conversions|ToFloat(Integer) _output_get)))
          (CallFunction|AddAttribute (LocalVariables|GetLocalBonusAttributes) _resultattribute)
          (if (Utilities|Array|IsValidIndex (.CustomSkillLevels (Utilities|Struct|BreakSTR_SkillInstance (LocalVariables|GetLocalSkillInstance))) (- (LocalVariables|GetLocalSkillLevel) 1))
            (CallFunction|AddAttributes (LocalVariables|GetLocalBonusAttributes) (Utilities|Struct|BreakSTR_SkillLevelData (Utilities|Array|Get(acopy) (.CustomSkillLevels (Utilities|Struct|BreakSTR_SkillInstance (LocalVariables|GetLocalSkillInstance))) (- (LocalVariables|GetLocalSkillLevel) 1))))
            (else
              (bind _resultattributes (CallFunction|MultiplyAttributes (Utilities|Struct|BreakSTR_SkillLevelData (.DefaultLevelData (Utilities|Struct|BreakSTR_SkillInstance (LocalVariables|GetLocalSkillInstance)))) (Math|Conversions|ToFloat(Integer) (LocalVariables|GetLocalSkillLevel))))
              (CallFunction|AddAttributes (LocalVariables|GetLocalBonusAttributes) _resultattributes)))))
      (bind _success_2 (Default|UpdateBonusAttributesSet (LocalVariables|GetLocalAttributesManager) (Utilities|Struct|MakeSTR_AttributesSet "SkillsAttributes" (LocalVariables|GetLocalBonusAttributes))))
      (return _success_2))
    (:Is%20Not%20Valid
      (Utilities|IsValid _playercontroller
        (:Is%20Valid
          (Utilities|IsValid _returnvalue
            (:Is%20Valid
              (bind (_found _component) (CallFunction|FindAttributesManager _returnvalue))
              (if _found
                (LocalVariables|SetLocalAttributesManager _component)
                (goto _label)))))
        (:Is%20Not%20Valid
          (bind (_found_2 _component_2) (CallFunction|FindAttributesManager (Components|GetOwner)))
          (if _found_2
            (LocalVariables|SetLocalAttributesManager _component_2)
            (goto _label)))))))

(fn SaveLevelingData
  (params (SaveGame :type Save%20Game%20Object%20Reference))
  ;[1 1 1] Try to save leveling data.
  (bind _asplayer_controller (Utilities|Casting|CastToPlayerController (Components|GetOwner))
    (:then
      (bind _success (Class|BPISaveGameLevelingSystem|SetPlayerLevelingSaveDataBPI(Message) SaveGame (CallFunction|GetNetworkedPlayerID _asplayer_controller) (Utilities|Struct|MakeSTR_SaveData_LevelingSystem (Variables|State|GetCurrentLevel) (Variables|State|GetSkillPoints) (Variables|State|GetCurrentExperience) (Variables|State|GetLearnedAttributes) (Variables|State|GetLearnedSkillsData))))
      (return _success))
    (:CastFailed
      (return false))))

(fn LoadLevelingData
  (params (SaveGame :type Save%20Game%20Object%20Reference))
  ;[1 1 1] Try to load leveling data.
  (bind _asplayer_controller (Utilities|Casting|CastToPlayerController (Components|GetOwner))
    (:then
      (bind (_success _savedata) (Class|BPISaveGameLevelingSystem|GetPlayerLevelingSaveDataBPI(Message) SaveGame (CallFunction|GetNetworkedPlayerID _asplayer_controller)))
      (if _success
        (bind _output_get (Variables|State|SetCurrentLevel (.CurrentLevel (Utilities|Struct|BreakSTR_SaveData_LevelingSystem _savedata))))
        (Variables|State|SetSkillPoints (.SkillPoints (Utilities|Struct|BreakSTR_SaveData_LevelingSystem _savedata)))
        (Variables|State|SetCurrentExperience (.CurrentExperience (Utilities|Struct|BreakSTR_SaveData_LevelingSystem _savedata)))
        (Variables|State|SetLearnedAttributes (.LearnedAttributes (Utilities|Struct|BreakSTR_SaveData_LevelingSystem _savedata)))
        (Variables|State|SetLearnedSkillsData (.LearnedSkillsData (Utilities|Struct|BreakSTR_SaveData_LevelingSystem _savedata)))
        (bind _requiredexperience (LevelingManager|CalculateLevelExperience _output_get))
        (Variables|State|SetRequiredExperience _requiredexperience)
        (Utilities|FlowControl|Sequence
          (:then_0
            (LevelingManager|UpdateLearnedAttributes)
            (LevelingManager|UpdateLearnedSkillsAttributes))
          (:then_1
            (Utilities|FlowControl|Sequence
              (:then_0
                (bind _asplayer_controller_2 (Utilities|Casting|CastToPlayerController (Components|GetOwner))
                  (:then
                    (Variables|State|SetPlayerController _asplayer_controller_2))
                  (:CastFailed
                    _))
                (Variables|State|SetIsInitialized true))
              (:then_1
                (return true)))))
        (else
          (return false))))
    (:CastFailed
      (return false))))

(fn BindonAttributesChanged
  (params (Manager :type BP%20AC%20Attributes%20Manager%20Object%20Reference))
  ;[1 1 1] Check skill requirements when the attributes of referenced attributes manager is changed.
  (Default|CallOnCheckSkillRequirements self))

(fn BindonPlayerGameplayEventPlayed
  (params (Manager :type BP%20AC%20Gameplay%20Events%20Manager%20Object%20Reference) (PlayerController :type Player%20Controller%20Object%20Reference) (EventSettings :type STR%20Event%20Settings%20Structure))
  (bind (_eventname _integervariables _floatvariables) (Utilities|Struct|BreakSTR_EventSettings EventSettings))
  ;[1 1 1] Add exeperience when the add experience player gameplay event is called.
  (if (not (Variables|State|GetIgnoreExperienceEvent))
    (if (== PlayerController (Variables|State|GetPlayerController))
      (switch name _eventname
        (:AddExperience
          (LevelingManager|TryAddExperience (.Value (Utilities|Map|Find _integervariables "ActivityLevel")) (.Value (Utilities|Map|Find _floatvariables "Experience"))))))))

(fn OnRepLearnedSkillsData
  ;[1 1 1] Update learned skills attributes.
  (if (Networking|IsServer)
    (LevelingManager|UpdateLearnedSkillsAttributes))
  (Default|CallOnLearnedSkillsDataChanged self))