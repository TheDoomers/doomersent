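; Blueprint function library for the leveling system, giving static access to an actor's experience and skill learning.
; Actor-facing functions locate the BP_AC_LevelingManager component and forward calls to it, with Find variants reporting success and Get variants returning just the value.
; Skill helpers build instances from data table handles and resolve max level and per-level requirements, preferring custom level entries over the skill's defaults.
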(fn `FindCurrentExperience`
  (params (TargetActor :type "Actor Object Reference"))
  (returns (Success :type Boolean) (CurrentExperience :type "Float (double-precision)"))
  ;[1 1 1] Returns current amount of the actor experience.
  (bind (_found _manager) (`self.FindLevelingManager` TargetActor))
  (if _found
    (return true (`/Game/BPS_Core/Blueprints/Systems/LevelingSystem/Components/BP_AC_LevelingManager.GetCurrentExperience` _manager))
    (else
      (return false 0.0))))

(fn `FindLevelingManager`
  (params (TargetActor :type "Actor Object Reference"))
  (returns (Found :type Boolean) (Manager :type "/Game/BPS_Core/Blueprints/Systems/LevelingSystem/Components/BP_AC_LevelingManager Object Reference"))
  (locals (LocalLevelingManager :type "/Game/BPS_Core/Blueprints/Systems/LevelingSystem/Components/BP_AC_LevelingManager Object Reference"))
  ;[1 1 1] Try to find leveling manager component.
  (bind _output_get (set `local.LocalLevelingManager` (`Actor.GetComponentByClass` TargetActor "/Game/BPS_Core/Blueprints/Systems/LevelingSystem/Components/BP_AC_LevelingManager.BP_AC_LevelingManager_C")))
  (`/Engine/EditorBlueprintResources/StandardMacros.IsValid` _output_get
    (:`Is Valid`
      (return true _output_get))
    (:`Is Not Valid`
      (return false null))))

(fn `FindLevelSkillRequirements`
  (params (SkillInstance :type "/Game/BPS_Core/Blueprints/Systems/LevelingSystem/Structures/STR_SkillInstance Structure (by ref)") (SkillLevel :type Integer))
  (returns (Success :type Boolean) (RequiredDescription :type Text) (RequiredSkillPoints :type Integer) (RequiredLevel :type Integer) (RequiredAttributes :type "Array of /Game/BPS_Core/Blueprints/Systems/AttributesSystem/Structures/STR_Attribute Structure"))
  (locals (LocalSkillLevelData :type "/Game/BPS_Core/Blueprints/Systems/LevelingSystem/Structures/STR_SkillLevelData Structure"))
  (bind ((`DefaultLevelData_39_2303B8974C954A5CF5FAC896ECADC03A` _defaultleveldata) (`CustomSkillLevels_40_2680CBDC440DFBD81E0819A0D9E1E2DC` _customskilllevels)) (break `/Game/BPS_Core/Blueprints/Systems/LevelingSystem/Structures/STR_SkillInstance` SkillInstance))
  (bind _returnvalue (- SkillLevel 1))
  (bind _maxlevel (`self.GetMaxSkillLevel` SkillInstance))
  ;[1 1 1] Try to find requirements to learn the skill level.
  (if (or (<= _maxlevel 0) (<= SkillLevel _maxlevel))
    (if (`KismetArrayLibrary.Array_IsValidIndex` _customskilllevels _returnvalue)
      (bind _output_get (set `local.LocalSkillLevelData` (`|GetArrayItem` _customskilllevels _returnvalue)))
      (else
        (set `local.LocalSkillLevelData` _defaultleveldata)))
    (bind ((`RequiredDescription_13_56A242A242968381FA4BEFB03372FEAE` _requireddescription) (`RequiredSkillPoints_31_AE8AA0394ADE60D0018FA180007A7835` _requiredskillpoints) (`RequiredLevel_32_FCCF069548DC9CB76FD7E0844F48CBFA` _requiredlevel) (`RequiredAttributes_33_8D9F6D0E472E1ABB02883F93633D36D6` _requiredattributes)) (break `/Game/BPS_Core/Blueprints/Systems/LevelingSystem/Structures/STR_SkillLevelData` _output_get))
    (return true _requireddescription _requiredskillpoints _requiredlevel _requiredattributes)
    (else
      (return false "" 0 0))))

(fn `FindRequiredExperience`
  (params (TargetActor :type "Actor Object Reference"))
  (returns (Success :type Boolean) (RequiredExperience :type "Float (double-precision)"))
  ;[1 1 1] Returns required amount of experience of the actor that is required to next level.
  (bind (_found _manager) (`self.FindLevelingManager` TargetActor))
  (if _found
    (return true (`/Game/BPS_Core/Blueprints/Systems/LevelingSystem/Components/BP_AC_LevelingManager.GetRequiredExperience` _manager))
    (else
      (return false 0.0))))

(fn `GetCurrentExperience`
  (params (TargetActor :type "Actor Object Reference"))
  (returns (CurrentExperience :type "Float (double-precision)"))
  ;[1 1 1] Returns current amount of the actor experience.
  (bind (_success _currentexperience) (`self.FindCurrentExperience` TargetActor))
  (return _currentexperience))

(fn `GetMaxSkillLevel`
  (params (SkillInstance :type "/Game/BPS_Core/Blueprints/Systems/LevelingSystem/Structures/STR_SkillInstance Structure (by ref)"))
  (returns (MaxLevel :type Integer))
  (locals (LocalMaxLevel :type Integer))
  (bind ((`MaxLevel_29_42AB9EB94AED25F17E93DF9A8945D9F7` _maxlevel) (`CustomSkillLevels_40_2680CBDC440DFBD81E0819A0D9E1E2DC` _customskilllevels)) (break `/Game/BPS_Core/Blueprints/Systems/LevelingSystem/Structures/STR_SkillInstance` SkillInstance))
  ;[1 1 1] Returns max skill level of the skill.
  (if (`KismetArrayLibrary.Array_IsValidIndex` _customskilllevels)
    (set `local.LocalMaxLevel` (`KismetArrayLibrary.Array_Length` _customskilllevels))
    (else
      (bind _output_get (set `local.LocalMaxLevel` _maxlevel))))
  (return _output_get))

(fn `GetRequiredExperience`
  (params (TargetActor :type "Actor Object Reference"))
  (returns (RequiredExperience :type "Float (double-precision)"))
  ;[1 1 1] Returns required amount of experience of the actor that is required to next level.
  (bind (_success _requiredexperience) (`self.FindRequiredExperience` TargetActor))
  (return _requiredexperience))

(fn `MakeSkillInstance`
  (params (SkillHandle :type "DataTableRowHandle Structure"))
  (returns (Success :type Boolean) (SkillInstance :type "/Game/BPS_Core/Blueprints/Systems/LevelingSystem/Structures/STR_SkillInstance Structure"))
  (bind (_datatable _rowname) (break `DataTableRowHandle` SkillHandle))
  ;[1 1 1] Make skill instance from skill handle.
  (`/Engine/EditorBlueprintResources/StandardMacros.IsValid` _datatable
    (:`Is Valid`
      (bind _returnvalue (`|GetDataTableRow` _datatable _rowname)
        (:`then`
          (return true _returnvalue))
        (:`RowNotFound`
          _)))
    (:`Is Not Valid`
      _))
  (return false))

(fn `TryAddExperience`
  (params (TargetActor :type "Actor Object Reference") (ActivityLevel :type Integer) (ExperienceToAdd :type "Float (double-precision)"))
  (returns (Success :type Boolean))
  ;[1 1 1] Try add a specific amount of the experience to the actor.
  (bind (_found _manager) (`self.FindLevelingManager` TargetActor))
  (if _found
    (bind _success (`/Game/BPS_Core/Blueprints/Systems/LevelingSystem/Components/BP_AC_LevelingManager.TryAddExperience` _manager ActivityLevel ExperienceToAdd))
    (return _success)))

(fn `TryLearnSkill`
  (params (TargetActor :type "Actor Object Reference") (SkillHandle :type "DataTableRowHandle Structure") (SkillLevel :type Integer :default 1))
  (returns (Success :type Boolean))
  ;[1 1 1] Try to learn skill for target actor.
  (bind (_found _manager) (`self.FindLevelingManager` TargetActor))
  (if _found
    (bind _success (`/Game/BPS_Core/Blueprints/Systems/LevelingSystem/Components/BP_AC_LevelingManager.TryLearnSkill` _manager SkillHandle SkillLevel))
    (return _success)
    (else
      (return false))))