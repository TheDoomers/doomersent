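; Actor component that manages the level's day-night cycle, exposing time and part of day with replication and save/load support.
; On init it finds the single BP_DayNightCycleActor, warning if there isn't exactly one, and re-broadcasts its change events.
; Setters run on the server or forward from clients by RPC.
; A looping server timer refreshes replicated SyncedTimeOfDay, whose OnRep corrects clients' local cycle actor.
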(event `self.ReceiveBeginPlay`
  ;[1 1 1] Begin play. Init component.
  (`self.TryInitComponent`))

(event `TrySetTimeOfDay (Server)`
  (params (TimeOfDay :type "/Game/BPS_Core/Blueprints/Systems/DayNightCycleSystem/Structures/STR_TimeOfDay Structure"))
  ;[1 1 1] Set time of day events.
  (`self.TrySetTimeOfDay` TimeOfDay))

(event `TrySetPartOfDay (Server)`
  (params (PartOfDay :type "/Game/BPS_Core/Blueprints/Systems/DayNightCycleSystem/Enums/E_PartOfDay Enum" :default "NewEnumerator0"))
  ;[1 1 1] Set time of day events.
  (`self.TrySetPartOfDay` PartOfDay))

(fn `Bind_OnPartOfDayChanged`
  (params (DayNightCycleActor :type "/Game/BPS_Core/Blueprints/Systems/DayNightCycleSystem/Actors/BP_DayNightCycleActor Object Reference") (PartOfDay :type "/Game/BPS_Core/Blueprints/Systems/DayNightCycleSystem/Enums/E_PartOfDay Enum" :default "NewEnumerator0"))
  ;[1 1 1] Notify that part of day was changed.
  (`self.OnPartOfDayChanged` self PartOfDay))

(fn `Bind_OnTimeOfDayChanged`
  (params (DayNightCycleActor :type "/Game/BPS_Core/Blueprints/Systems/DayNightCycleSystem/Actors/BP_DayNightCycleActor Object Reference") (TimeOfDay :type "/Game/BPS_Core/Blueprints/Systems/DayNightCycleSystem/Structures/STR_TimeOfDay Structure"))
  ;[1 1 1] Notify that time of day was changed.
  (`self.OnTimeOfDayChanged` self TimeOfDay))

(fn `Bind_SyncTimerTick`
  (bind _daynightcycleactor (`self.DayNightCycleActor`))
  ;[1 1 1] Try to sync tyme of day.
  (`/Engine/EditorBlueprintResources/StandardMacros.IsValid` _daynightcycleactor
    (:`Is Valid`
      (set `self.SyncedTimeOfDay` (`/Game/BPS_Core/Blueprints/Systems/DayNightCycleSystem/Actors/BP_DayNightCycleActor.GetTimeOfDay` _daynightcycleactor)))))

(fn `GetPartOfDay`
  (returns (PartOfDay :type "/Game/BPS_Core/Blueprints/Systems/DayNightCycleSystem/Enums/E_PartOfDay Enum"))
  (bind _daynightcycleactor (`self.DayNightCycleActor`))
  ;[1 1 1] Returns current part of the day.
  (`/Engine/EditorBlueprintResources/StandardMacros.IsValid` _daynightcycleactor
    (:`Is Valid`
      (return (`/Game/BPS_Core/Blueprints/Systems/DayNightCycleSystem/Actors/BP_DayNightCycleActor.GetPartOfDay` _daynightcycleactor)))))

(fn `GetTimeOfDay`
  (returns (TimeOfDay :type "/Game/BPS_Core/Blueprints/Systems/DayNightCycleSystem/Structures/STR_TimeOfDay Structure"))
  (bind _daynightcycleactor (`self.DayNightCycleActor`))
  ;[1 1 1] Returns current time of the day.
  (`/Engine/EditorBlueprintResources/StandardMacros.IsValid` _daynightcycleactor
    (:`Is Valid`
      (return (`/Game/BPS_Core/Blueprints/Systems/DayNightCycleSystem/Actors/BP_DayNightCycleActor.GetTimeOfDay` _daynightcycleactor)))))

(fn `InitComponent`
  (returns (Success :type Boolean))
  ;[1 1 1] Try init component and bind events.
  (bind _outactors (`GameplayStatics.GetAllActorsOfClass` "/Game/BPS_Core/Blueprints/Systems/DayNightCycleSystem/Actors/BP_DayNightCycleActor.BP_DayNightCycleActor_C"))
  (if (== (`KismetArrayLibrary.Array_Length` _outactors) 1)
    (for _array_element _outactors
      (bind _output_get (set `self.DayNightCycleActor` _array_element))
      (add `/Game/BPS_Core/Blueprints/Systems/DayNightCycleSystem/Actors/BP_DayNightCycleActor.OnTimeOfDayChanged` _output_get (`|CreateDelegate` :!event `Bind_OnTimeOfDayChanged`))
      (add `/Game/BPS_Core/Blueprints/Systems/DayNightCycleSystem/Actors/BP_DayNightCycleActor.OnPartOfDayChanged` _output_get (`|CreateDelegate` :!event `Bind_OnPartOfDayChanged`))
      (if (`KismetSystemLibrary.IsServer`)
        (set `self.SyncedTimeOfDay` (`/Game/BPS_Core/Blueprints/Systems/DayNightCycleSystem/Actors/BP_DayNightCycleActor.GetTimeOfDay` _output_get))
        (`KismetSystemLibrary.K2_SetTimerDelegate` (`|CreateDelegate` :!event `Bind_SyncTimerTick`) 10.0 true))
      (bind _output_get_2 (set `self.IsInitialized` true))
      (return _output_get_2))
    (else
      (if (`self.ShowInitializationWarning`)
        (`KismetSystemLibrary.PrintText` "The only one Day Night Cycle Actor should be placed on the level!" true true (struct :`R` 1.0 :`A` 1.0) 10.0))
      (return false))))

(fn `LoadDayNightCycleData`
  (params (SaveGame :type "SaveGame Object Reference"))
  (returns (Success :type Boolean))
  ;[1 1 1] Try to load data.
  (bind (_success _savedata) (message `/Game/BPS_Core/Blueprints/Systems/DayNightCycleSystem/Interfaces/BPI_SaveGame_DayNightCycle.GetDayNightCycleData_BPI` SaveGame))
  (if _success
    (`self.TryInitComponent`)
    (bind _success_2 (`self.TrySetTimeOfDay` (`.TimeOfDay_2_17B122B447F2F514120F3AA740B50114` (break `/Game/BPS_Core/Blueprints/Systems/DayNightCycleSystem/Structures/STR_SaveData_DayNightCycle` _savedata))))
    (return _success_2)))

(fn `OnRep_SyncedTimeOfDay`
  (bind _daynightcycleactor (`self.DayNightCycleActor`))
  (if (not (`KismetSystemLibrary.IsServer`))
    (`/Engine/EditorBlueprintResources/StandardMacros.IsValid` _daynightcycleactor
      (:`Is Valid`
        (`/Game/BPS_Core/Blueprints/Systems/DayNightCycleSystem/Actors/BP_DayNightCycleActor.TrySetTimeOfDay` _daynightcycleactor (`self.SyncedTimeOfDay`))))))

(fn `SaveDayNightCycleData`
  (params (SaveGame :type "SaveGame Object Reference"))
  (returns (Success :type Boolean))
  ;[1 1 1] Try to save data.
  (bind _success (message `/Game/BPS_Core/Blueprints/Systems/DayNightCycleSystem/Interfaces/BPI_SaveGame_DayNightCycle.SetDayNightCycleData_BPI` SaveGame (make `/Game/BPS_Core/Blueprints/Systems/DayNightCycleSystem/Structures/STR_SaveData_DayNightCycle` (`self.GetTimeOfDay`))))
  (return _success))

(fn `TryInitComponent`
  (returns (Success :type Boolean))
  ;[1 1 1] Try init component.
  (if (not (`self.IsInitialized`))
    (bind _success (`self.InitComponent`))
    (set `self.IsInitialized` _success)
    (return true)
    (else
      (return true))))

(fn `TrySetPartOfDay`
  (params (PartOfDay :type "/Game/BPS_Core/Blueprints/Systems/DayNightCycleSystem/Enums/E_PartOfDay Enum" :default "NewEnumerator0"))
  (returns (Success :type Boolean))
  (bind _daynightcycleactor (`self.DayNightCycleActor`))
  ;[1 1 1] Try to set part of a day.
  (if (`KismetSystemLibrary.IsServer`)
    (`/Engine/EditorBlueprintResources/StandardMacros.IsValid` _daynightcycleactor
      (:`Is Valid`
        (`/Game/BPS_Core/Blueprints/Systems/DayNightCycleSystem/Actors/BP_DayNightCycleActor.TrySetPartOfDay` _daynightcycleactor PartOfDay)
        (return true))
      (:`Is Not Valid`
        (return false)))
    (else
      (`self.TrySetPartOfDay (Server)` PartOfDay)
      (return true))))

(fn `TrySetTimeOfDay`
  (params (TimeOfDay :type "/Game/BPS_Core/Blueprints/Systems/DayNightCycleSystem/Structures/STR_TimeOfDay Structure"))
  (returns (Success :type Boolean))
  (bind _daynightcycleactor (`self.DayNightCycleActor`))
  ;[1 1 1] Try to set time of a day.
  (if (`KismetSystemLibrary.IsServer`)
    (bind _output_get (set `self.SyncedTimeOfDay` TimeOfDay))
    (`/Engine/EditorBlueprintResources/StandardMacros.IsValid` _daynightcycleactor
      (:`Is Valid`
        (`/Game/BPS_Core/Blueprints/Systems/DayNightCycleSystem/Actors/BP_DayNightCycleActor.TrySetTimeOfDay` _daynightcycleactor _output_get)
        (return true))
      (:`Is Not Valid`
        (return false)))
    (else
      (`self.TrySetTimeOfDay (Server)` TimeOfDay)
      (return true))))