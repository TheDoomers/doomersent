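; Day-night cycle actor that runs an in-game clock over a configurable real-seconds day length and drives the sky lighting.
; Tick advances a normalized day value that rotates the sun, samples sun and skylight intensity curves, and refreshes the sky sphere.
; The hours/minutes/seconds clock updates on tick or by a looping scaled-minute timer, broadcasting time and part-of-day changes.
; Construction resolves the initial time from a part-of-day map and previews the lighting.
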(event `self.ReceiveBeginPlay`
  ;[1 1 1] Begin play. Set initial time of day.
  (`self.TrySetTimeOfDay` (`self.InitialTimeOfDay`))
  (if (not (`self.UpdateTimeOfDayOnTick`))
    (`self.StartMinuteTimer`)))

(event `StartMinuteTimer`
  ;[1 1 1] Update time of day and
  (`KismetSystemLibrary.K2_SetTimerDelegate` (delegate `MinuteTimerTick`) (`self.MinuteTickTime`) true))

(event `MinuteTimerTick`
  ;[1 1 1] Update time of day and
  (`self.UpdateTimeOfDay`))

(event `self.ReceiveTick`
  (params (DeltaSeconds :type "Float (single-precision)"))
  ;[1 1 1] Update time of day and
  (bind _output_get (set `self.CurrentSeconds` (mod (+ (`self.CurrentSeconds`) DeltaSeconds) (`self.RealSecondsInDay`))))
  (set `self.TimeOfDayValue` (/ _output_get (`self.RealSecondsInDay`)))
  (`self.UpdateLightActors`)
  (if (`self.UpdateTimeOfDayOnTick`)
    (`self.UpdateTimeOfDay`)))

(fn `FindTimeOfDay`
  (params (PartOfDay :type "/Game/BPS_Core/Blueprints/Systems/DayNightCycleSystem/Enums/E_PartOfDay Enum" :default "NewEnumerator0"))
  (returns (Success :type Boolean) (Value :type "/Game/BPS_Core/Blueprints/Systems/DayNightCycleSystem/Structures/STR_TimeOfDay Structure"))
  (bind (_value _returnvalue) (`BlueprintMapLibrary.Map_Find` (`self.PartOfDayTimes`) PartOfDay))
  ;[1 1 1] Find time of day by part of day.
  (return _returnvalue _value))

(fn `GetPartOfDay`
  (returns (PartOfDay :type "/Game/BPS_Core/Blueprints/Systems/DayNightCycleSystem/Enums/E_PartOfDay Enum"))
  ;[1 1 1] Returns current part of day.
  (return (`self.CurrentPartOfDay`)))

(fn `GetTimeOfDay`
  (returns (TimeOfDay :type "/Game/BPS_Core/Blueprints/Systems/DayNightCycleSystem/Structures/STR_TimeOfDay Structure"))
  ;[1 1 1] Returns time of the day.
  (return (`self.CurrentTimeOfDay`)))

(fn `TryChangeTimeOfDay`
  (params (NewTimeOfDay :type "/Game/BPS_Core/Blueprints/Systems/DayNightCycleSystem/Structures/STR_TimeOfDay Structure"))
  (returns (Success :type Boolean))
  (locals (LocalTimeOfDay :type "/Game/BPS_Core/Blueprints/Systems/DayNightCycleSystem/Structures/STR_TimeOfDay Structure"))
  (bind (_hours _minutes _seconds) (break `/Game/BPS_Core/Blueprints/Systems/DayNightCycleSystem/Structures/STR_TimeOfDay` NewTimeOfDay))
  (bind (_hours_2 _minutes_2 _seconds_2) (break `/Game/BPS_Core/Blueprints/Systems/DayNightCycleSystem/Structures/STR_TimeOfDay` (`self.CurrentTimeOfDay`)))
  ;[1 1 1] Try to change time of day.
  (set `local.LocalTimeOfDay` NewTimeOfDay)
  (if (or (!= _hours _hours_2) (!= _minutes _minutes_2) (!= _seconds _seconds_2))
    (bind _output_get (set `self.CurrentTimeOfDay` (`local.LocalTimeOfDay`)))
    (`self.OnTimeOfDayChanged` self _output_get)
    (`self.UpdatePartOfDay`)
    (return true)
    (else
      (return false))))

(fn `TrySetPartOfDay`
  (params (NewPartOfDay :type "/Game/BPS_Core/Blueprints/Systems/DayNightCycleSystem/Enums/E_PartOfDay Enum" :default "NewEnumerator0"))
  (returns (Success :type Boolean))
  (bind (_value _returnvalue) (`BlueprintMapLibrary.Map_Find` (`self.PartOfDayTimes`) NewPartOfDay))
  ;[1 1 1] Try to set part of day.
  (if _returnvalue
    (bind _success (`self.TrySetTimeOfDay` _value))
    (return _success)
    (else
      (return false))))

(fn `TrySetTimeOfDay`
  (params (NewTimeOfDay :type "/Game/BPS_Core/Blueprints/Systems/DayNightCycleSystem/Structures/STR_TimeOfDay Structure"))
  (returns (Success :type Boolean))
  (locals (LocalSecondsAmount :type Integer :default 0) (LocalMaxSecondsAmount :type Integer :default 0))
  (bind _minutes (`/Game/BPS_Core/Blueprints/Systems/DayNightCycleSystem/Libraries/BP_Library_DayNightCycle.GetMinutesInHour`))
  (bind _seconds (`/Game/BPS_Core/Blueprints/Systems/DayNightCycleSystem/Libraries/BP_Library_DayNightCycle.GetSecondsInMinute`))
  ;[1 1 1] Try to set time of day variables and update light actors.
  (bind _result (`/Game/BPS_Core/Blueprints/Systems/DayNightCycleSystem/Libraries/BP_Library_DayNightCycle.CorrectTimeOfDay` NewTimeOfDay))
  (`self.TryChangeTimeOfDay` _result)
  (`self.UpdateLightActors`)
  (bind (_hours _minutes_2 _seconds_2) (break `/Game/BPS_Core/Blueprints/Systems/DayNightCycleSystem/Structures/STR_TimeOfDay` _result))
  (bind _output_get (set `local.LocalSecondsAmount` (+ (* _hours _minutes _seconds) (* _minutes_2 _seconds) _seconds_2)))
  (bind _output_get_2 (set `local.LocalMaxSecondsAmount` (* (`/Game/BPS_Core/Blueprints/Systems/DayNightCycleSystem/Libraries/BP_Library_DayNightCycle.GetHoursInDay`) _minutes _seconds)))
  (bind _output_get_3 (set `self.TimeOfDayValue` (/ (`KismetMathLibrary.Conv_IntToDouble` _output_get) (`KismetMathLibrary.Conv_IntToDouble` _output_get_2))))
  (set `self.CurrentSeconds` (* _output_get_3 (`self.RealSecondsInDay`)))
  (return true))

(fn `UpdateLightActors`
  (returns (Success :type Boolean))
  (bind _skysphereactor (`self.SkySphereActor`))
  (bind _sunlightactor (`self.SunLightActor`))
  (bind _skylightactor (`self.SkyLightActor`))
  ;[1 1 1] Update light actors depending on time of day value.
  (`|ExecutionSequence`
    (:`then_0`
      (`/Engine/EditorBlueprintResources/StandardMacros.IsValid` _sunlightactor
        (:`Is Valid`
          (`LightComponent.SetIntensity` (`Light.LightComponent` _sunlightactor) (`CurveFloat.GetFloatValue` (`self.SunLightIntensityCurve`) (`self.TimeOfDayValue`)))
          (`self.K2_SetActorRotation` (`self.SunLightActor`) (`KismetMathLibrary.ComposeRotators` (`self.MidnightRotation`) (`KismetMathLibrary.MakeRotator` 0.0 (`KismetMathLibrary.Lerp` 0.0 360.0 (`self.TimeOfDayValue`)) (`self.SunYawRotation`))) true))))
    (:`then_1`
      (`|ExecutionSequence`
        (:`then_0`
          (`/Engine/EditorBlueprintResources/StandardMacros.IsValid` _skylightactor
            (:`Is Valid`
              (`SkyLightComponent.SetIntensity` (`SkyLight.LightComponent` _skylightactor) (`CurveFloat.GetFloatValue` (`self.SkyLightIntensityCurve`) (`self.TimeOfDayValue`))))))
        (:`then_1`
          (`|ExecutionSequence`
            (:`then_0`
              (`/Engine/EditorBlueprintResources/StandardMacros.IsValid` _skysphereactor
                (:`Is Valid`
                  (`/Engine/EngineSky/BP_Sky_Sphere.UpdateSunDirection` _skysphereactor))))
            (:`then_1`
              (return true))))))))

(fn `UpdatePartOfDay`
  (returns (Success :type Boolean))
  (locals (LocalPartOfDay :type "/Game/BPS_Core/Blueprints/Systems/DayNightCycleSystem/Enums/E_PartOfDay Enum" :default "NewEnumerator0"))
  (bind _timeofdayvalue (`self.TimeOfDayValue`))
  (bind _localpartofday (`local.LocalPartOfDay`))
  ;[1 1 1] Update part of day.
  (if (>= _timeofdayvalue 0.75)
    (if (== _timeofdayvalue 0.75)
      (set `local.LocalPartOfDay` "NewEnumerator7")
      (else
        (set `local.LocalPartOfDay` "NewEnumerator5")))
    (elif (>= _timeofdayvalue 0.5)
      (if (== _timeofdayvalue 0.5)
        (set `local.LocalPartOfDay` "NewEnumerator3")
        (else
          (set `local.LocalPartOfDay` "NewEnumerator2")))
      (elif (>= _timeofdayvalue 0.25)
        (if (== _timeofdayvalue 0.25)
          (set `local.LocalPartOfDay` "NewEnumerator6")
          (else
            (set `local.LocalPartOfDay` "NewEnumerator1")))
        (elif (== _timeofdayvalue 0.0)
          (set `local.LocalPartOfDay` "NewEnumerator4")
          (else
            (set `local.LocalPartOfDay` "NewEnumerator8"))))))
  (if (`|EnumInequality` _localpartofday (`self.CurrentPartOfDay`))
    (set `self.CurrentPartOfDay` _localpartofday)
    (`self.OnPartOfDayChanged` self (`self.CurrentPartOfDay`))
    (return true)))

(fn `UpdateTimeOfDay`
  (returns (Success :type Boolean))
  (locals (LocalSecondsAmount :type Integer :default 0) (LocalHours :type Integer :default 0) (LocalMinutes :type Integer :default 0) (LocalSeconds :type Integer :default 0))
  (bind _seconds (`/Game/BPS_Core/Blueprints/Systems/DayNightCycleSystem/Libraries/BP_Library_DayNightCycle.GetSecondsInMinute`))
  (bind _returnvalue (* (`/Game/BPS_Core/Blueprints/Systems/DayNightCycleSystem/Libraries/BP_Library_DayNightCycle.GetMinutesInHour`) _seconds))
  ;[1 1 1] Update time of day and update light actors.
  (bind _output_get (set `local.LocalSecondsAmount` (`KismetMathLibrary.Round` (* (`/Game/BPS_Core/Blueprints/Systems/DayNightCycleSystem/Libraries/BP_Library_DayNightCycle.GetSecondsInDay`) (`self.TimeOfDayValue`)))))
  (bind _output_get_2 (set `local.LocalHours` (/ _output_get _returnvalue)))
  (bind _output_get_3 (set `local.LocalMinutes` (/ (mod _output_get _returnvalue) _seconds)))
  (bind _output_get_4 (set `local.LocalSeconds` (mod _output_get _seconds)))
  (bind _success (`self.TryChangeTimeOfDay` (make `/Game/BPS_Core/Blueprints/Systems/DayNightCycleSystem/Structures/STR_TimeOfDay` _output_get_2 _output_get_3 _output_get_4)))
  (if _success
    (`self.UpdateLightActors`)
    (return true)
    (else
      (return false))))

(fn `UserConstructionScript`
  ;[1 1 1] Construction script. Init components and variables.
  (set `self.MinuteTickTime` (* (`/Game/BPS_Core/Blueprints/Systems/DayNightCycleSystem/Libraries/BP_Library_DayNightCycle.GetSecondsInMinute`) (/ (`self.RealSecondsInDay`) (`KismetMathLibrary.Conv_IntToDouble` (`/Game/BPS_Core/Blueprints/Systems/DayNightCycleSystem/Libraries/BP_Library_DayNightCycle.GetSecondsInDay`)))))
  (bind (_success _value) (`self.FindTimeOfDay` (`self.InitialPartOfDay`)))
  (if _success
    (bind _output_get (set `self.InitialTimeOfDay` _value)))
  (bind _result (`/Game/BPS_Core/Blueprints/Systems/DayNightCycleSystem/Libraries/BP_Library_DayNightCycle.CorrectTimeOfDay` _output_get))
  (`self.TrySetTimeOfDay` _result)
  (`/Engine/EditorBlueprintResources/StandardMacros.IsValid` (`self.SunLightActor`)
    (:`Is Valid`
      (`self.UpdateLightActors`))))