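; Blueprint function library that gives global access to the day-night cycle system.
; Getters and setters for time and part of day find BP_AC_DayNightCycleManager on the Game State and forward to it, reporting failure or returning defaults when absent.
; Helpers build, wrap and convert time-of-day structs to day fractions.
; CheckTimeOfDay compares those fractions to test whether the current time lies in a range, including ranges crossing midnight.
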(fn `CheckTimeOfDay`
  (params (FromTime :type "/Game/BPS_Core/Blueprints/Systems/DayNightCycleSystem/Structures/STR_TimeOfDay Structure") (ToTime :type "/Game/BPS_Core/Blueprints/Systems/DayNightCycleSystem/Structures/STR_TimeOfDay Structure"))
  (returns (Result :type Boolean))
  (locals (LocalFromFraction :type "Float (double-precision)" :default 0.0) (LocalToFraction :type "Float (double-precision)" :default 0.0))
  (bind _returnvalue (`self.GetTimeOfDayFraction` (`self.GetTimeOfDayPure` null)))
  ;[1 1 1] Returns true if current time of day is in specific time range.
  (bind _result (`self.CorrectTimeOfDay` FromTime))
  (bind _result_2 (`self.CorrectTimeOfDay` ToTime))
  (bind _output_get (set `local.LocalFromFraction` (`self.GetTimeOfDayFraction` _result)))
  (bind _output_get_2 (set `local.LocalToFraction` (`self.GetTimeOfDayFraction` _result_2)))
  (if (< _output_get _output_get_2)
    (return (`KismetMathLibrary.InRange_FloatFloat` _returnvalue (`local.LocalFromFraction`) (`local.LocalToFraction`)))
    (else
      (return (not (`KismetMathLibrary.InRange_FloatFloat` _returnvalue (`local.LocalToFraction`) (`local.LocalFromFraction`) false false))))))

(fn `CorrectTimeOfDay`
  (params (TimeOfDay :type "/Game/BPS_Core/Blueprints/Systems/DayNightCycleSystem/Structures/STR_TimeOfDay Structure (by ref)"))
  (returns (Result :type "/Game/BPS_Core/Blueprints/Systems/DayNightCycleSystem/Structures/STR_TimeOfDay Structure"))
  (bind (_hours _minutes _seconds) (break `/Game/BPS_Core/Blueprints/Systems/DayNightCycleSystem/Structures/STR_TimeOfDay` TimeOfDay))
  ;[1 1 1] Correct time of day structure.
  (bind _structout (setmembers `/Game/BPS_Core/Blueprints/Systems/DayNightCycleSystem/Structures/STR_TimeOfDay` :`StructRef` TimeOfDay :`Hours` (mod _hours (`self.GetHoursInDay` null)) :`Minutes` (mod _minutes (`self.GetMinutesInHour` null)) :`Seconds` (mod _seconds (`self.GetSecondsInMinute` null))))
  (return _structout))

(fn `FindDayNightCycleManager`
  (returns (Found :type Boolean) (Manager :type "/Game/BPS_Core/Blueprints/Systems/DayNightCycleSystem/Components/BP_AC_DayNightCycleManager Object Reference"))
  (locals (LocalManager :type "/Game/BPS_Core/Blueprints/Systems/DayNightCycleSystem/Components/BP_AC_DayNightCycleManager Object Reference"))
  ;[1 1 1] Try to find day night manager component.
  (bind _output_get (set `local.LocalManager` (`Actor.GetComponentByClass` (`GameplayStatics.GetGameState` null) "/Game/BPS_Core/Blueprints/Systems/DayNightCycleSystem/Components/BP_AC_DayNightCycleManager.BP_AC_DayNightCycleManager_C")))
  (`/Engine/EditorBlueprintResources/StandardMacros.IsValid` _output_get
    (:`Is Valid`
      (return true _output_get))
    (:`Is Not Valid`
      (return false null))))

(fn `GetHoursInDay`
  (returns (Hours :type Integer))
  ;[1 1 1] Returns hours in a day.
  (return 24))

(fn `GetMinutesInHour`
  (returns (Minutes :type Integer))
  ;[1 1 1] Returns minutes in an hour.
  (return 60))

(fn `GetPartOfDay`
  (returns (Success :type Boolean) (PartOfDay :type "/Game/BPS_Core/Blueprints/Systems/DayNightCycleSystem/Enums/E_PartOfDay Enum"))
  ;[1 1 1] Returns current part of day.
  (bind (_found _manager) (`self.FindDayNightCycleManager` null))
  (if _found
    (return true (`/Game/BPS_Core/Blueprints/Systems/DayNightCycleSystem/Components/BP_AC_DayNightCycleManager.GetPartOfDay` _manager))
    (else
      (return false "NewEnumerator0"))))

(fn `GetPartOfDayPure`
  (returns (PartOfDay :type "/Game/BPS_Core/Blueprints/Systems/DayNightCycleSystem/Enums/E_PartOfDay Enum"))
  ;[1 1 1] Returns current part of day.
  (bind (_found _manager) (`self.FindDayNightCycleManager` null))
  (if _found
    (return (`/Game/BPS_Core/Blueprints/Systems/DayNightCycleSystem/Components/BP_AC_DayNightCycleManager.GetPartOfDay` _manager))
    (else
      (return "NewEnumerator0"))))

(fn `GetSecondsInDay`
  (returns (SecondsInDay :type Integer))
  ;[1 1 1] Returns seconds in a day.
  (return (* (`self.GetHoursInDay` null) (`self.GetMinutesInHour` null) (`self.GetSecondsInMinute` null))))

(fn `GetSecondsInMinute`
  (returns (Seconds :type Integer))
  ;[1 1 1] Returns seconds in a minute.
  (return 60))

(fn `GetTimeOfDay`
  (returns (Success :type Boolean) (TimeOfDay :type "/Game/BPS_Core/Blueprints/Systems/DayNightCycleSystem/Structures/STR_TimeOfDay Structure"))
  ;[1 1 1] Returns current time of day.
  (bind (_found _manager) (`self.FindDayNightCycleManager` null))
  (if _found
    (return true (`/Game/BPS_Core/Blueprints/Systems/DayNightCycleSystem/Components/BP_AC_DayNightCycleManager.GetTimeOfDay` _manager))
    (else
      (return false))))

(fn `GetTimeOfDayFraction`
  (params (TimeOfDay :type "/Game/BPS_Core/Blueprints/Systems/DayNightCycleSystem/Structures/STR_TimeOfDay Structure"))
  (returns (ReturnValue :type "Float (double-precision)"))
  (bind (_hours _minutes _seconds) (break `/Game/BPS_Core/Blueprints/Systems/DayNightCycleSystem/Structures/STR_TimeOfDay` TimeOfDay))
  (bind _seconds_2 (`self.GetSecondsInMinute` null))
  ;[1 1 1] Returns fraction of day depending on time of day.
  (return (/ (`KismetMathLibrary.Conv_IntToDouble` (+ (* _hours (`self.GetMinutesInHour` null) _seconds_2) (* _minutes _seconds_2) _seconds)) (`KismetMathLibrary.Conv_IntToDouble` (`self.GetSecondsInDay` null)))))

(fn `GetTimeOfDayPure`
  (returns (TimeOfDay :type "/Game/BPS_Core/Blueprints/Systems/DayNightCycleSystem/Structures/STR_TimeOfDay Structure"))
  ;[1 1 1] Returns current time of day.
  (bind (_found _manager) (`self.FindDayNightCycleManager` null))
  (if _found
    (return (`/Game/BPS_Core/Blueprints/Systems/DayNightCycleSystem/Components/BP_AC_DayNightCycleManager.GetTimeOfDay` _manager))
    (else
      (return))))

(fn `MakeTimeOfDay`
  (params (Hours :type Integer) (Minutes :type Integer) (Seconds :type Integer))
  (returns (TimeOfDay :type "/Game/BPS_Core/Blueprints/Systems/DayNightCycleSystem/Structures/STR_TimeOfDay Structure"))
  ;[1 1 1] Make time of day structure.
  (return (make `/Game/BPS_Core/Blueprints/Systems/DayNightCycleSystem/Structures/STR_TimeOfDay` (`KismetMathLibrary.Clamp` Hours 0 (`self.GetHoursInDay` null)) (`KismetMathLibrary.Clamp` Minutes 0 (`self.GetMinutesInHour` null)) (`KismetMathLibrary.Clamp` Seconds 0 (`self.GetSecondsInMinute` null)))))

(fn `TrySetPartOfDay`
  (params (PartOfDay :type "/Game/BPS_Core/Blueprints/Systems/DayNightCycleSystem/Enums/E_PartOfDay Enum" :default "NewEnumerator0"))
  (returns (Success :type Boolean))
  ;[1 1 1] Try to set part of day.
  (bind (_found _manager) (`self.FindDayNightCycleManager` null))
  (if _found
    (bind _success (`/Game/BPS_Core/Blueprints/Systems/DayNightCycleSystem/Components/BP_AC_DayNightCycleManager.TrySetPartOfDay` _manager PartOfDay))
    (return _success)
    (else
      (return false))))

(fn `TrySetTimeOfDay`
  (params (TimeOfDay :type "/Game/BPS_Core/Blueprints/Systems/DayNightCycleSystem/Structures/STR_TimeOfDay Structure"))
  (returns (Success :type Boolean))
  ;[1 1 1] Try to set time of day.
  (bind (_found _manager) (`self.FindDayNightCycleManager` null))
  (if _found
    (bind _success (`/Game/BPS_Core/Blueprints/Systems/DayNightCycleSystem/Components/BP_AC_DayNightCycleManager.TrySetTimeOfDay` _manager TimeOfDay))
    (return _success)
    (else
      (return false))))