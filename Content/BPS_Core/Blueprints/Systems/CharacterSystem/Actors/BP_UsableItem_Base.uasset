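; Base actor for usable items that characters holster or equip, including melee hit detection.
; Initializes from a data table row, async-loads soft meshes, and uses RepNotify variables to update meshes and socket attachment.
; During melee traces, Tick traces between previous and current positions of "Trace"-prefixed sockets, reporting each hit actor once.
; Child classes can override notify and state hooks; destruction waits until allowed.
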(event `self.ReceiveBeginPlay`
  ;[1 1 1] Begin play. Try to init usable item.
  (`self.InitUsableItem`)
  (`self.InitSoftStaticMesh`)
  (`self.InitSoftSkeletalMesh`))

(event `self.ReceiveTick`
  (params (DeltaSeconds :type "Float (single-precision)"))
  ;[1 1 1] Tick event. Try hit actors.
  (if (`self.TraceInProcess`)
    (`self.TryHitActors`)
    (else
      (`self.SetActorTickEnabled` false))))

(event `InitSoftStaticMesh`
  (bind (_value _returnvalue) (`BlueprintMapLibrary.Map_Find` (`.SoftObjects_50_A6F1060F47C5DEA16A3FD3AF7E38C230` (break `/Game/BPS_Core/Blueprints/Systems/CharacterSystem/Structures/Usable/STR_UsableItemInstance` (`self.UsableItemData`))) "StaticMesh"))
  ;[1 1 1] Init soft static and skeletal mesh references.
  (if _returnvalue
    (`/Game/BPS_Core/Blueprints/Systems/AsyncLoadSystem/Libraries/BP_Library_AsyncLoad.AsyncLoadStaticMeshForComponent` (`self.StaticMeshComponent`) _value)))

(event `InitSoftSkeletalMesh`
  (bind (_value _returnvalue) (`BlueprintMapLibrary.Map_Find` (`.SoftObjects_50_A6F1060F47C5DEA16A3FD3AF7E38C230` (break `/Game/BPS_Core/Blueprints/Systems/CharacterSystem/Structures/Usable/STR_UsableItemInstance` (`self.UsableItemData`))) "SkeletalMesh"))
  ;[1 1 1] Init soft static and skeletal mesh references.
  (if _returnvalue
    (`/Game/BPS_Core/Blueprints/Systems/AsyncLoadSystem/Libraries/BP_Library_AsyncLoad.AsyncLoadSkeletalMeshForComponent` (`self.SkeletalMeshComponent`) _value)))

(fn `AttachToComponent`
  (params (Component :type "SceneComponent Object Reference") (SocketName :type Name))
  (returns (Success :type Boolean))
  ;[1 1 1] Set component and socket name to attach usable item.
  (set `self.AttachComponent` Component)
  (set `self.AttachSocketName` SocketName)
  (return true))

(fn `CreateTraceLocations`
  (returns (Locations :type "Array of Vector Structure"))
  (locals (LocalLocations :type "Array of Vector Structure"))
  (bind _staticmeshcomponent (`self.StaticMeshComponent`))
  (bind _skeletalmeshcomponent (`self.SkeletalMeshComponent`))
  ;[1 1 1] Create array of trace locations.
  (for _array_element (`SceneComponent.GetAllSocketNames` _staticmeshcomponent)
    (if (`KismetStringLibrary.StartsWith` (`KismetStringLibrary.Conv_NameToString` _array_element) "Trace")
      (`KismetArrayLibrary.Array_Add` (`local.LocalLocations`) (`SceneComponent.GetSocketLocation` _staticmeshcomponent _array_element))))
  (for _array_element_2 (`SceneComponent.GetAllSocketNames` _skeletalmeshcomponent)
    (if (`KismetStringLibrary.StartsWith` (`KismetStringLibrary.Conv_NameToString` _array_element_2) "Trace")
      (`KismetArrayLibrary.Array_Add` (`local.LocalLocations`) (`SceneComponent.GetSocketLocation` _skeletalmeshcomponent _array_element_2))))
  (if (not (`KismetArrayLibrary.Array_IsValidIndex` (`local.LocalLocations`)))
    (`KismetArrayLibrary.Array_Add` (`local.LocalLocations`) (`SceneComponent.K2_GetComponentLocation` (`self.DefaultSceneRoot`))))
  (return (`local.LocalLocations`)))

(fn `FindUsableSocketTransform`
  (params (ComponentTag :type Name) (SocketName :type Name))
  (returns (Found :type Boolean) (Transform :type "Transform Structure"))
  (locals (LocalSocketName :type Name))
  ;[1 1 1] Find transform of specific socket of the component.
  (set `local.LocalSocketName` SocketName)
  (for _array_element (`self.GetComponentsByTag` "/Script/Engine.SceneComponent" ComponentTag)
    (return true (`SceneComponent.GetSocketTransform` _array_element (`local.LocalSocketName`) "RTS_World")))
  (return false))

(fn `GetDefaultSocketData`
  (returns (DefaultSocket :type "/Game/BPS_Core/Blueprints/Systems/CoreSystem/Structures/STR_SocketData Structure"))
  ;[1 1 1] Returns default socket data.
  (return (`.DefaultSocket_61_0167332943AA821ED6F05E93A96263A6` (break `/Game/BPS_Core/Blueprints/Systems/CharacterSystem/Structures/Usable/STR_UsableItemInstance` (`self.UsableItemData`)))))

(fn `GetEquippedState`
  (returns (IsEquipped :type Boolean))
  ;[1 1 1] Returns current equipped state.
  (return (`self.IsEquipped`)))

(fn `GetEquippedTag`
  (returns (EquippedTag :type Name))
  ;[1 1 1] Returns current equipped tag.
  (return (`self.EquippedTag`)))

(fn `GetHolsterTag`
  (returns (HolsterTag :type Name))
  ;[1 1 1] Returns current holster tag.
  (return (`self.HolsterTag`)))

(fn `GetItemTypeTag`
  (returns (ItemTypeTag :type "GameplayTag Structure"))
  ;[1 1 1] Returns item type tag.
  (return (`.ItemTypeTag_5_637484B64522FEF1EB760098759D15A1` (break `/Game/BPS_Core/Blueprints/Systems/CharacterSystem/Structures/Usable/STR_UsableItemInstance` (`self.UsableItemData`)))))

(fn `InitUsableItem`
  (returns (Success :type Boolean))
  (locals (LocalStaticMesh :type "StaticMesh Object Reference") (LocalSkeletalMesh :type "SkeletalMesh Object Reference") (LocalRelativeTransform :type "Transform Structure") (LocalDefaultUsableTag :type Name) (LocalDefaultVisibility :type Boolean))
  (bind _localstaticmesh (`local.LocalStaticMesh`))
  (bind _localskeletalmesh (`local.LocalSkeletalMesh`))
  (bind (_datatable _rowname) (break `DataTableRowHandle` (`self.UsableItemHandle`)))
  ;[1 1 1] Init usable item data.
  (`/Engine/EditorBlueprintResources/StandardMacros.IsValid` _datatable
    (:`Is Valid`
      (bind _returnvalue (`|GetDataTableRow` _datatable _rowname)
        (:`then`
          (bind _output_get (set `self.UsableItemData` _returnvalue))
          (bind ((`StaticMesh_10_0D2DD0604A04872D360EDAB8E1EB95BB` _staticmesh) (`SkeletalMesh_16_1B4B1E174F2572C8D4E837AD0ABA8170` _skeletalmesh) (`DefaultUsableTag_67_E00A0B97497A1E1FEF60D98A95A6C8DB` _defaultusabletag) (`DefaultVisibility_64_43400AAB46802BCFE23E099ED4602FC8` _defaultvisibility) (`RelativeTransform_21_DB62816E465CBA6D2039E5A329B190AF` _relativetransform)) (break `/Game/BPS_Core/Blueprints/Systems/CharacterSystem/Structures/Usable/STR_UsableItemInstance` _output_get))
          (set `local.LocalStaticMesh` _staticmesh)
          (set `local.LocalSkeletalMesh` _skeletalmesh)
          (set `local.LocalDefaultUsableTag` _defaultusabletag)
          (set `local.LocalDefaultVisibility` _defaultvisibility)
          (set `local.LocalRelativeTransform` _relativetransform)
          (`|ExecutionSequence`
            (:`then_0`
              (`/Engine/EditorBlueprintResources/StandardMacros.IsValid` _localstaticmesh
                (:`Is Valid`
                  (set `self.StaticMesh` _localstaticmesh))))
            (:`then_1`
              (`|ExecutionSequence`
                (:`then_0`
                  (`/Engine/EditorBlueprintResources/StandardMacros.IsValid` _localskeletalmesh
                    (:`Is Valid`
                      (set `self.SkeletalMesh` _localskeletalmesh))))
                (:`then_1`
                  (`|ExecutionSequence`
                    (:`then_0`
                      (set `self.RelativeTransform` (`local.LocalRelativeTransform`)))
                    (:`then_1`
                      (`|ExecutionSequence`
                        (:`then_0`
                          (`KismetArrayLibrary.Array_Add` (`self.Tags`) (`local.LocalDefaultUsableTag`))
                          (`self.SetActorHiddenInGame` (not (`local.LocalDefaultVisibility`))))
                        (:`then_1`
                          (return true))))))))))))))

(fn `OnRep_AttachComponent`
  ;[1 1 1] Update relative transform of the usable item.
  (`self.UpdateAttachSettings`))

(fn `OnRep_AttachSocketName`
  ;[1 1 1] Update relative transform of the usable item.
  (`self.UpdateAttachSettings`))

(fn `OnRep_RelativeTransform`
  ;[1 1 1] Update relative transform of the usable item.
  (`self.UpdateAttachSettings`))

(fn `OnRep_SkeletalMesh`
  ;[1 1 1] Update skeletal mesh component on all clients.
  (`SkinnedMeshComponent.SetSkinnedAssetAndUpdate` (`self.SkeletalMeshComponent`) (`self.SkeletalMesh`) true))

(fn `OnRep_StaticMesh`
  ;[1 1 1] Update static mesh component on all clients.
  (`StaticMeshComponent.SetStaticMesh` (`self.StaticMeshComponent`) (`self.StaticMesh`)))

(fn `PlayUsableNotify`
  (params (NotifyName :type Name))
  (returns (Success :type Boolean))
  ;[1 1 1] Play specific notify of the item.
  ; Can be overridden in child classes.
  (return true))

(fn `SetCanBeDestroyed`
  (params (CanBeDestroyed :type Boolean))
  (returns (Success :type Boolean))
  ;[1 1 1] Set can be destroyed flag.
  (bind _output_get (set `self.CanBeDestroyed` CanBeDestroyed))
  (if (and _output_get (`self.ShouldBeDestroyed`))
    (`self.K2_DestroyActor`))
  (return true))

(fn `SetDefaultVisibility`
  (returns (Success :type Boolean))
  ;[1 1 1] Set default visibility for usable item.
  (`self.SetActorHiddenInGame` (not (`.DefaultVisibility_64_43400AAB46802BCFE23E099ED4602FC8` (break `/Game/BPS_Core/Blueprints/Systems/CharacterSystem/Structures/Usable/STR_UsableItemInstance` (`self.UsableItemData`)))))
  (return true))

(fn `SetEquippedState`
  (params (NewEquipped :type Boolean))
  (returns (Success :type Boolean))
  ;[1 1 1] Set equipped state for usable item.
  (set `self.IsEquipped` NewEquipped)
  (return true))

(fn `SetEquippedTag`
  (params (EquippedTag :type Name))
  (returns (Success :type Boolean))
  ;[1 1 1] Set current equipped tag.
  (set `self.EquippedTag` EquippedTag)
  (return true))

(fn `SetHolsterTag`
  (params (HolsterTag :type Name))
  (returns (Success :type Boolean))
  ;[1 1 1] Set current holster tag.
  (set `self.HolsterTag` HolsterTag)
  (return true))

(fn `SetUsableState`
  (params (StateName :type Name) (StateValue :type Boolean))
  (returns (Success :type Boolean))
  ;[1 1 1] Set specific state of the item.
  ; Can be overridden in child classes.
  (return true))

(fn `StartMeleeTrace`
  (params (TraceDamageData :type "/Game/BPS_Core/Blueprints/Systems/CharacterSystem/Structures/Character/STR_TraceDamageData Structure") (TraceSettings :type "/Game/BPS_Core/Blueprints/Systems/CoreSystem/Structures/STR_TraceSettings Structure") (ActorsToIgnore :type "Array of Actor Object Reference"))
  (returns (Success :type Boolean))
  ;[1 1 1] Start melee trace process.
  (set `self.TraceDamageData` TraceDamageData)
  (set `self.TraceSettings` TraceSettings)
  (set `self.TraceActorsToIgnore` ActorsToIgnore)
  (`KismetArrayLibrary.Array_Clear` (`self.HitActors`))
  (bind _output_get (set `self.TraceInProcess` true))
  (`self.SetActorTickEnabled` _output_get)
  (bind _locations (`self.CreateTraceLocations`))
  (set `self.PrevTraceLocations` _locations)
  (`self.TryHitActors`)
  (return true))

(fn `StopMeleeTrace`
  (returns (Success :type Boolean))
  ;[1 1 1] Stop melee trace process.
  (bind _output_get (set `self.TraceInProcess` false))
  (`self.SetActorTickEnabled` _output_get)
  (return true))

(fn `Try Melee Trace`
  (params (TraceDamageData :type "/Game/BPS_Core/Blueprints/Systems/CharacterSystem/Structures/Character/STR_TraceDamageData Structure") (StartLocations :type "Array of Vector Structure (by ref)") (EndLocations :type "Array of Vector Structure (by ref)") (TraceSettings :type "/Game/BPS_Core/Blueprints/Systems/CoreSystem/Structures/STR_TraceSettings Structure") (ActorsToIgnore :type "Array of Actor Object Reference (by ref)"))
  (returns (Success :type Boolean))
  (locals (LocalTraceDamageData :type "/Game/BPS_Core/Blueprints/Systems/CharacterSystem/Structures/Character/STR_TraceDamageData Structure") (LocalHitResult :type "HitResult Structure") (LocalHitActor :type "Actor Object Reference"))
  ;[1 1 1] Try hit actors using specific settings.
  (set `local.LocalTraceDamageData` TraceDamageData)
  (if (not (`self.TraceInProcess`))
    (`KismetArrayLibrary.Array_Clear` (`self.HitActors`)))
  (bind _hits (`/Game/BPS_Core/Blueprints/Systems/CoreSystem/Libraries/BP_Library_CoreFunctions.FindMultiTraceHits` StartLocations EndLocations TraceSettings ActorsToIgnore))
  (bind _actorhits (`/Game/BPS_Core/Blueprints/Systems/CoreSystem/Libraries/BP_Library_CoreFunctions.RemoveSameActorHits` _hits))
  (for _array_element _actorhits
    (set `local.LocalHitResult` _array_element)
    (bind _output_get (set `local.LocalHitActor` (`.HitActor` (`GameplayStatics.BreakHitResult` _array_element))))
    (if (not (`KismetArrayLibrary.Array_Contains` (`self.HitActors`) _output_get))
      (`KismetArrayLibrary.Array_Add` (`self.HitActors`) (`local.LocalHitActor`))
      (`self.OnTraceHit` self (`local.LocalHitActor`) (`local.LocalHitResult`) (`local.LocalTraceDamageData`))))
  (return true))

(fn `TryDestroyActor`
  (returns (Success :type Boolean))
  ;[1 1 1] Try to destroy usable item actor.
  (set `self.ShouldBeDestroyed` true)
  (if (`self.CanBeDestroyed`)
    (`self.K2_DestroyActor`))
  (return true))

(fn `TryHitActors`
  (returns (Success :type Boolean))
  (locals (LocalHitResult :type "HitResult Structure") (LocalHitActor :type "Actor Object Reference"))
  ;[1 1 1] Try hit actors using trace settings.
  (bind _locations (`self.CreateTraceLocations`))
  (bind _hits (`/Game/BPS_Core/Blueprints/Systems/CoreSystem/Libraries/BP_Library_CoreFunctions.FindMultiTraceHits` (`self.PrevTraceLocations`) _locations (`self.TraceSettings`) (`self.TraceActorsToIgnore`)))
  (set `self.PrevTraceLocations` _locations)
  (bind _actorhits (`/Game/BPS_Core/Blueprints/Systems/CoreSystem/Libraries/BP_Library_CoreFunctions.RemoveSameActorHits` _hits))
  (for _array_element _actorhits
    (set `local.LocalHitResult` _array_element)
    (bind _output_get (set `local.LocalHitActor` (`.HitActor` (`GameplayStatics.BreakHitResult` _array_element))))
    (if (not (`KismetArrayLibrary.Array_Contains` (`self.HitActors`) _output_get))
      (`KismetArrayLibrary.Array_Add` (`self.HitActors`) (`local.LocalHitActor`))
      (`self.OnTraceHit` self (`local.LocalHitActor`) (`local.LocalHitResult`) (`self.TraceDamageData`))))
  (return true))

(fn `UpdateAttachSettings`
  (returns (Success :type Boolean))
  (bind _attachcomponent (`self.AttachComponent`))
  ;[1 1 1] Attach usable item actor to attach component reference and update relative transform.
  (`/Engine/EditorBlueprintResources/StandardMacros.IsValid` _attachcomponent
    (:`Is Valid`
      (`self.K2_AttachToComponent` _attachcomponent (`self.AttachSocketName`) "SnapToTarget" "SnapToTarget" "SnapToTarget")
      (`self.K2_SetActorRelativeTransform` (`self.RelativeTransform`) false true)
      (return true))))

(fn `UserConstructionScript`
  ;[1 1 1] Construction script.
  (`self.InitUsableItem`))