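; Blueprint function library for the character system, giving shortcuts to character-related manager components and trace damage data.
; Find helpers look up Character, Interaction, Locomotion and Usable manager components on an actor.
; Wrappers use them to check critical hits and start or stop interactions for an actor or controller's pawn, with Oriented variants allowing client animations without network delay.
; Other getters read trace damage overrides, modifiers and a random min-max multiplier.
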(fn `CheckCharacterCriticalHit`
  (params (TargetActor :type "Actor Object Reference") (HitResult :type "HitResult Structure"))
  (returns (CriticalHit :type Boolean))
  ;[1 1 1] Returns true if hit is critical for the character.
  (bind (_found _component) (`self.FindCharacterManager` TargetActor))
  (if _found
    (bind _criticalhit (`/Game/BPS_Core/Blueprints/Systems/CharacterSystem/Components/BP_AC_CharacterManager.CheckCriticalHit` _component HitResult))
    (return _criticalhit)
    (else
      (return false))))

(fn `FindCharacterManager`
  (params (TargetActor :type "Actor Object Reference"))
  (returns (Found :type Boolean) (Component :type "/Game/BPS_Core/Blueprints/Systems/CharacterSystem/Components/BP_AC_CharacterManager Object Reference"))
  (locals (LocalCharacterManager :type "/Game/BPS_Core/Blueprints/Systems/CharacterSystem/Components/BP_AC_CharacterManager Object Reference"))
  ;[1 1 1] Try to find character manager component.
  (bind _output_get (set `local.LocalCharacterManager` (`Actor.GetComponentByClass` TargetActor "/Game/BPS_Core/Blueprints/Systems/CharacterSystem/Components/BP_AC_CharacterManager.BP_AC_CharacterManager_C")))
  (`/Engine/EditorBlueprintResources/StandardMacros.IsValid` _output_get
    (:`Is Valid`
      (return true _output_get))
    (:`Is Not Valid`
      (return false null))))

(fn `FindInteractionManager`
  (params (TargetActor :type "Actor Object Reference"))
  (returns (Found :type Boolean) (Component :type "/Game/BPS_Core/Blueprints/Systems/CharacterSystem/Components/BP_AC_InteractionManager Object Reference"))
  (locals (LocalInteractionManager :type "/Game/BPS_Core/Blueprints/Systems/CharacterSystem/Components/BP_AC_InteractionManager Object Reference"))
  ;[1 1 1] Try to find interaction manager component.
  (`/Engine/EditorBlueprintResources/StandardMacros.IsValid` TargetActor
    (:`Is Valid`
      (bind _output_get (set `local.LocalInteractionManager` (`Actor.GetComponentByClass` TargetActor "/Game/BPS_Core/Blueprints/Systems/CharacterSystem/Components/BP_AC_InteractionManager.BP_AC_InteractionManager_C")))
      (`/Engine/EditorBlueprintResources/StandardMacros.IsValid` _output_get
        (:`Is Valid`
          (return true _output_get))
        (:`Is Not Valid`
          (return false null))))))

(fn `FindLocomotionManager`
  (params (TargetActor :type "Actor Object Reference"))
  (returns (Found :type Boolean) (Component :type "/Game/BPS_Core/Blueprints/Systems/CharacterSystem/Components/BP_AC_LocomotionManager Object Reference"))
  (locals (LocalLocomotionManager :type "/Game/BPS_Core/Blueprints/Systems/CharacterSystem/Components/BP_AC_LocomotionManager Object Reference"))
  ;[1 1 1] Try to find locomotion manager component.
  (bind _output_get (set `local.LocalLocomotionManager` (`Actor.GetComponentByClass` TargetActor "/Game/BPS_Core/Blueprints/Systems/CharacterSystem/Components/BP_AC_LocomotionManager.BP_AC_LocomotionManager_C")))
  (`/Engine/EditorBlueprintResources/StandardMacros.IsValid` _output_get
    (:`Is Valid`
      (return true _output_get))
    (:`Is Not Valid`
      (return false null))))

(fn `FindUsableManager`
  (params (TargetActor :type "Actor Object Reference"))
  (returns (Found :type Boolean) (Component :type "/Game/BPS_Core/Blueprints/Systems/CharacterSystem/Components/BP_AC_UsableManager Object Reference"))
  (locals (LocalInteractionManager :type "/Game/BPS_Core/Blueprints/Systems/CharacterSystem/Components/BP_AC_InteractionManager Object Reference") (LocalUsableManager :type "/Game/BPS_Core/Blueprints/Systems/CharacterSystem/Components/BP_AC_UsableManager Object Reference"))
  ;[1 1 1] Try to find usable manager component.
  (bind _output_get (set `local.LocalUsableManager` (`Actor.GetComponentByClass` TargetActor "/Game/BPS_Core/Blueprints/Systems/CharacterSystem/Components/BP_AC_UsableManager.BP_AC_UsableManager_C")))
  (`/Engine/EditorBlueprintResources/StandardMacros.IsValid` _output_get
    (:`Is Valid`
      (return true _output_get))
    (:`Is Not Valid`
      (return false null))))

(fn `GetCustomTraceDamageData`
  (params (TraceDamageData :type "/Game/BPS_Core/Blueprints/Systems/CharacterSystem/Structures/Character/STR_TraceDamageData Structure"))
  (returns (CustomDamageData :type "/Game/BPS_Core/Blueprints/Systems/DamageSystem/Structures/STR_DamageData Structure"))
  ;[1 1 1] Returns custom damage data.
  (return (`.CustomDamageData_9_3E88E8F44C646302206A8AB4ACA170A9` (break `/Game/BPS_Core/Blueprints/Systems/CharacterSystem/Structures/Character/STR_TraceDamageData` TraceDamageData))))

(fn `GetTraceDamageDataModifiers`
  (params (TraceDamageData :type "/Game/BPS_Core/Blueprints/Systems/CharacterSystem/Structures/Character/STR_TraceDamageData Structure"))
  (returns (DamageModifiers :type "GameplayTagContainer Structure"))
  ;[1 1 1] Returns damage modifiers.
  (return (`.DamageModifiers_11_15B7AB1D4BFED40BFAEBCE8062D038A0` (break `/Game/BPS_Core/Blueprints/Systems/CharacterSystem/Structures/Character/STR_TraceDamageData` TraceDamageData))))

(fn `GetTraceDamageDataMultiplier`
  (params (TraceDamageData :type "/Game/BPS_Core/Blueprints/Systems/CharacterSystem/Structures/Character/STR_TraceDamageData Structure"))
  (returns (DamageMultiplier :type "Float (double-precision)"))
  (bind ((`MinDamageMultiplier_12_017882D2497404BC525C1C991EE0C3F6` _mindamagemultiplier) (`MaxDamageMultiplier_13_E611B3C34A975256F124EF8D7674C06C` _maxdamagemultiplier)) (break `/Game/BPS_Core/Blueprints/Systems/CharacterSystem/Structures/Character/STR_TraceDamageData` TraceDamageData))
  ;[1 1 1] Returns random damage multiplier in range of min and max values.
  (return (`KismetMathLibrary.RandomFloatInRange` _mindamagemultiplier _maxdamagemultiplier)))

(fn `TryStartInteraction`
  (params (InteractingActor :type "Actor Object Reference") (InteractionTag :type "GameplayTag Structure") (SubType :type Name) (TargetActor :type "Actor Object Reference"))
  (returns (Success :type Boolean))
  ;[1 1 1] Try to start interaction for interacting actor.
  (bind (_found _component) (`self.FindInteractionManager` InteractingActor))
  (if _found
    (bind _success (`/Game/BPS_Core/Blueprints/Systems/CharacterSystem/Components/BP_AC_InteractionManager.TryStartInteraction` _component InteractionTag SubType TargetActor))
    (return _success)))

(fn `TryStartInteractionForController`
  (params (Controller :type "Controller Object Reference") (InteractionTag :type "GameplayTag Structure") (SubType :type Name) (TargetActor :type "Actor Object Reference"))
  (returns (Success :type Boolean))
  (bind _returnvalue (`Controller.K2_GetPawn` Controller))
  ;[1 1 1] Try to start interaction for pawn of target controller.
  (`/Engine/EditorBlueprintResources/StandardMacros.IsValid` _returnvalue
    (:`Is Valid`
      (bind (_found _component) (`self.FindInteractionManager` _returnvalue))
      (if _found
        (bind _success (`/Game/BPS_Core/Blueprints/Systems/CharacterSystem/Components/BP_AC_InteractionManager.TryStartInteraction` _component InteractionTag SubType TargetActor))
        (return _success)
        (else
          _)))
    (:`Is Not Valid`
      _))
  (return false))

(fn `TryStartInteractionForControllerOriented`
  (params (Controller :type "Controller Object Reference") (InteractionTag :type "GameplayTag Structure") (SubType :type Name) (TargetActor :type "Actor Object Reference"))
  (returns (Success :type Boolean))
  (bind _returnvalue (`Controller.K2_GetPawn` Controller))
  ;[1 1 1] Try to start interaction for pawn of target controller. If allowed starts animations on client without networking delay.
  (`/Engine/EditorBlueprintResources/StandardMacros.IsValid` _returnvalue
    (:`Is Valid`
      (bind (_found _component) (`self.FindInteractionManager` _returnvalue))
      (if _found
        (bind _success (`/Game/BPS_Core/Blueprints/Systems/CharacterSystem/Components/BP_AC_InteractionManager.TryStartInteractionOriented` _component InteractionTag SubType TargetActor))
        (return _success)
        (else
          _)))
    (:`Is Not Valid`
      _))
  (return false))

(fn `TryStartInteractionOriented`
  (params (InteractingActor :type "Actor Object Reference") (InteractionTag :type "GameplayTag Structure") (SubType :type Name) (TargetActor :type "Actor Object Reference"))
  (returns (Success :type Boolean))
  ;[1 1 1] Try to start interaction for interacting actor. If allowed starts animations on client without networking delay.
  (bind (_found _component) (`self.FindInteractionManager` InteractingActor))
  (if _found
    (bind _success (`/Game/BPS_Core/Blueprints/Systems/CharacterSystem/Components/BP_AC_InteractionManager.TryStartInteractionOriented` _component InteractionTag SubType TargetActor))
    (return _success)))

(fn `TryStopInteraction`
  (params (InteractingActor :type "Actor Object Reference") (InBlendOutTime :type "Float (double-precision)" :default 0.25))
  (returns (Success :type Boolean))
  ;[1 1 1] Try to stop interaction for interacting actor.
  (bind (_found _component) (`self.FindInteractionManager` InteractingActor))
  (if _found
    (`/Game/BPS_Core/Blueprints/Systems/CharacterSystem/Components/BP_AC_InteractionManager.StopAnimation (Multicast)` _component InBlendOutTime)
    (return false)))

(fn `TryStopInteractionForController`
  (params (Controller :type "Controller Object Reference") (InBlendOutTime :type "Float (double-precision)" :default 0.25))
  (returns (Success :type Boolean))
  (bind _returnvalue (`Controller.K2_GetPawn` Controller))
  ;[1 1 1] Try to stop interaction for pawn of target controller.
  (`/Engine/EditorBlueprintResources/StandardMacros.IsValid` _returnvalue
    (:`Is Valid`
      (bind (_found _component) (`self.FindInteractionManager` _returnvalue))
      (if _found
        (`/Game/BPS_Core/Blueprints/Systems/CharacterSystem/Components/BP_AC_InteractionManager.StopAnimation (Multicast)` _component InBlendOutTime)
        (return true)
        (else
          _)))
    (:`Is Not Valid`
      _))
  (return false))

(fn `UseCustomTraceDamageData`
  (params (TraceDamageData :type "/Game/BPS_Core/Blueprints/Systems/CharacterSystem/Structures/Character/STR_TraceDamageData Structure"))
  (returns (UseCustom :type Boolean))
  ;[1 1 1] Returns true if damage data should be overridden.
  (return (`.OverrideDamageData_14_4D370E3549ED5FBD068650B79ECA659C` (break `/Game/BPS_Core/Blueprints/Systems/CharacterSystem/Structures/Character/STR_TraceDamageData` TraceDamageData))))