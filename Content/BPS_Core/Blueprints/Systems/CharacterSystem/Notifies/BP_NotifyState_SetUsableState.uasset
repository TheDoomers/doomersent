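; Anim notify state that sets a named state on a usable item for the span of an animation window.
; Begin and end apply separate values for the configured state name.
; It looks up the selected item by tag through the mesh owner's usable manager component.
; Without a manager, it treats the owner itself as the usable item, so it also works in item animations.
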(fn `GetNotifyName`
  (returns (ReturnValue :type String))
  ;[1 1 1] Update notify name.
  (return "Set Usable State"))

(fn `Received_NotifyBegin`
  (params (MeshComp :type "SkeletalMeshComponent Object Reference") (Animation :type "AnimSequenceBase Object Reference") (TotalDuration :type "Float (single-precision)") (EventReference :type "AnimNotifyEventReference Structure (by ref)"))
  (returns (ReturnValue :type Boolean))
  (locals (LocalUsableManager :type "/Game/BPS_Core/Blueprints/Systems/CharacterSystem/Components/BP_AC_UsableManager Object Reference"))
  (bind _returnvalue (`ActorComponent.GetOwner` MeshComp))
  ;[1 1 1] Try to set state for usable item on notify begin.
  (`/Engine/EditorBlueprintResources/StandardMacros.IsValid` _returnvalue
    (:`Is Valid`
      (bind _output_get (set `local.LocalUsableManager` (`Actor.GetComponentByClass` _returnvalue "/Game/BPS_Core/Blueprints/Systems/CharacterSystem/Components/BP_AC_UsableManager.BP_AC_UsableManager_C")))
      (`/Engine/EditorBlueprintResources/StandardMacros.IsValid` _output_get
        (:`Is Valid`
          (bind (_found _usableitem) (`/Game/BPS_Core/Blueprints/Systems/CharacterSystem/Components/BP_AC_UsableManager.FindSelectedItem` _output_get (`self.UsableTag`)))
          (if _found
            (`/Game/BPS_Core/Blueprints/Systems/CharacterSystem/Actors/BP_UsableItem_Base.SetUsableState` _usableitem (`self.StateName`) (`self.BeginStateValue`))
            (return true)))
        (:`Is Not Valid`
          (bind _asbp_usable_item_base (cast `/Game/BPS_Core/Blueprints/Systems/CharacterSystem/Actors/BP_UsableItem_Base` _returnvalue))
          (`/Game/BPS_Core/Blueprints/Systems/CharacterSystem/Actors/BP_UsableItem_Base.SetUsableState` _asbp_usable_item_base (`self.StateName`) (`self.BeginStateValue`))
          (return true))))))

(fn `Received_NotifyEnd`
  (params (MeshComp :type "SkeletalMeshComponent Object Reference") (Animation :type "AnimSequenceBase Object Reference") (EventReference :type "AnimNotifyEventReference Structure (by ref)"))
  (returns (ReturnValue :type Boolean))
  (locals (LocalUsableManager :type "/Game/BPS_Core/Blueprints/Systems/CharacterSystem/Components/BP_AC_UsableManager Object Reference"))
  (bind _returnvalue (`ActorComponent.GetOwner` MeshComp))
  ;[1 1 1] Try to set state for usable item on notify end.
  (`/Engine/EditorBlueprintResources/StandardMacros.IsValid` _returnvalue
    (:`Is Valid`
      (bind _output_get (set `local.LocalUsableManager` (`Actor.GetComponentByClass` _returnvalue "/Game/BPS_Core/Blueprints/Systems/CharacterSystem/Components/BP_AC_UsableManager.BP_AC_UsableManager_C")))
      (`/Engine/EditorBlueprintResources/StandardMacros.IsValid` _output_get
        (:`Is Valid`
          (bind (_found _usableitem) (`/Game/BPS_Core/Blueprints/Systems/CharacterSystem/Components/BP_AC_UsableManager.FindSelectedItem` _output_get (`self.UsableTag`)))
          (if _found
            (`/Game/BPS_Core/Blueprints/Systems/CharacterSystem/Actors/BP_UsableItem_Base.SetUsableState` _usableitem (`self.StateName`) (`self.EndStateValue`))
            (return true)))
        (:`Is Not Valid`
          (bind _asbp_usable_item_base (cast `/Game/BPS_Core/Blueprints/Systems/CharacterSystem/Actors/BP_UsableItem_Base` _returnvalue))
          (`/Game/BPS_Core/Blueprints/Systems/CharacterSystem/Actors/BP_UsableItem_Base.SetUsableState` _asbp_usable_item_base (`self.StateName`) (`self.EndStateValue`))
          (return true))))))