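; Animation notify that adds or removes interaction tags on the animated character at a point in an animation.
; It finds the BP_AC_InteractionManager component on the mesh owner and, based on a boolean, adds or removes the configured tag set.
; It shows as "Set Interaction Tags" in the animation editor.
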(fn `GetNotifyName`
  (returns (ReturnValue :type String))
  ;[1 1 1] Update item name.
  (return "Set Interaction Tags"))

(fn `Received_Notify`
  (params (MeshComp :type "SkeletalMeshComponent Object Reference") (Animation :type "AnimSequenceBase Object Reference") (EventReference :type "AnimNotifyEventReference Structure (by ref)"))
  (returns (ReturnValue :type Boolean))
  (locals (LocalInteractionManager :type "/Game/BPS_Core/Blueprints/Systems/CharacterSystem/Components/BP_AC_InteractionManager Object Reference"))
  (bind _returnvalue (`ActorComponent.GetOwner` MeshComp))
  (bind _interactiontags (`self.InteractionTags`))
  ;[1 1 1] Set interaction tags for the character.
  (`/Engine/EditorBlueprintResources/StandardMacros.IsValid` _returnvalue
    (:`Is Valid`
      (bind _output_get (set `local.LocalInteractionManager` (`Actor.GetComponentByClass` _returnvalue "/Game/BPS_Core/Blueprints/Systems/CharacterSystem/Components/BP_AC_InteractionManager.BP_AC_InteractionManager_C")))
      (`/Engine/EditorBlueprintResources/StandardMacros.IsValid` _output_get
        (:`Is Valid`
          (if (`self.InteractionTagsValue`)
            (`/Game/BPS_Core/Blueprints/Systems/CharacterSystem/Components/BP_AC_InteractionManager.AddInteractionTags` _output_get _interactiontags)
            (else
              (`/Game/BPS_Core/Blueprints/Systems/CharacterSystem/Components/BP_AC_InteractionManager.RemoveInteractionTags` _output_get _interactiontags)))
          (return true))))))