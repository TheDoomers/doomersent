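; Animation notify state that opens and closes a trace-damage window on the owning actor for the span of the notify.
; With a UsableTag set, it starts and stops tracing on that usable through the owner's Usable Manager.
; Otherwise it uses the Character Manager, passing socket data to trace from.
; Both paths forward the damage data and optional custom trace settings on begin.
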(fn `GetNotifyName`
  (returns (ReturnValue :type String))
  ;[1 1 1] Update notify name.
  (return "Trace Damage"))

(fn `Received_NotifyBegin`
  (params (MeshComp :type "SkeletalMeshComponent Object Reference") (Animation :type "AnimSequenceBase Object Reference") (TotalDuration :type "Float (single-precision)") (EventReference :type "AnimNotifyEventReference Structure (by ref)"))
  (returns (ReturnValue :type Boolean))
  (locals (LocalUsableManager :type "/Game/BPS_Core/Blueprints/Systems/CharacterSystem/Components/BP_AC_UsableManager Object Reference") (LocalSocketData :type "Array of /Game/BPS_Core/Blueprints/Systems/CoreSystem/Structures/STR_SocketData Structure"))
  (bind _returnvalue (`ActorComponent.GetOwner` MeshComp))
  ;[1 1 1] Try to start trace damage process.
  (`/Engine/EditorBlueprintResources/StandardMacros.IsValid` _returnvalue
    (:`Is Valid`
      (if (!= (`self.UsableTag`) "None")
        (bind (_found _component) (`/Game/BPS_Core/Blueprints/Systems/CharacterSystem/Libraries/BP_Library_CharacterSystem.FindUsableManager` _returnvalue self))
        (if _found
          (`/Game/BPS_Core/Blueprints/Systems/CharacterSystem/Components/BP_AC_UsableManager.StartTraceDamage` _component (`self.UsableTag`) (`self.TraceDamageData`) (`self.OverrideTraceSettings`) (`self.CustomTraceSettings`))
          (return true))
        (else
          (bind (_found_2 _component_2) (`/Game/BPS_Core/Blueprints/Systems/CharacterSystem/Libraries/BP_Library_CharacterSystem.FindCharacterManager` _returnvalue self))
          (if _found_2
            (bind _output_get (set `local.LocalSocketData` (`self.SocketData`)))
            (`/Game/BPS_Core/Blueprints/Systems/CharacterSystem/Components/BP_AC_CharacterManager.StartTraceDamage` _component_2 _output_get (`self.TraceDamageData`) (`self.OverrideTraceSettings`) (`self.CustomTraceSettings`))
            (return true)))))))

(fn `Received_NotifyEnd`
  (params (MeshComp :type "SkeletalMeshComponent Object Reference") (Animation :type "AnimSequenceBase Object Reference") (EventReference :type "AnimNotifyEventReference Structure (by ref)"))
  (returns (ReturnValue :type Boolean))
  (locals (LocalUsableManager :type "/Game/BPS_Core/Blueprints/Systems/CharacterSystem/Components/BP_AC_UsableManager Object Reference"))
  (bind _returnvalue (`ActorComponent.GetOwner` MeshComp))
  ;[1 1 1] Try to stop trace damage process.
  (`/Engine/EditorBlueprintResources/StandardMacros.IsValid` _returnvalue
    (:`Is Valid`
      (if (!= (`self.UsableTag`) "None")
        (bind (_found _component) (`/Game/BPS_Core/Blueprints/Systems/CharacterSystem/Libraries/BP_Library_CharacterSystem.FindUsableManager` _returnvalue self))
        (if _found
          (`/Game/BPS_Core/Blueprints/Systems/CharacterSystem/Components/BP_AC_UsableManager.StopTraceDamage` _component (`self.UsableTag`))
          (return true))
        (else
          (bind (_found_2 _component_2) (`/Game/BPS_Core/Blueprints/Systems/CharacterSystem/Libraries/BP_Library_CharacterSystem.FindCharacterManager` _returnvalue self))
          (if _found_2
            (`/Game/BPS_Core/Blueprints/Systems/CharacterSystem/Components/BP_AC_CharacterManager.StopTraceDamage` _component_2)
            (return true)))))))