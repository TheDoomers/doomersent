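; Animation notify that triggers trace-based damage from an animation, either for a specific usable item or for the owning character.
; When a UsableTag is set it calls TryTraceDamage on the owner's usable manager, otherwise on its character manager.
; It forwards its damage data, optional trace setting overrides, offsets and distance, leaving the trace to the manager component.
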(fn `GetNotifyName`
  (returns (ReturnValue :type String))
  ;[1 1 1] Update notify name.
  (return "Trace Damage"))

(fn `Received_Notify`
  (params (MeshComp :type "SkeletalMeshComponent Object Reference") (Animation :type "AnimSequenceBase Object Reference") (EventReference :type "AnimNotifyEventReference Structure (by ref)"))
  (returns (ReturnValue :type Boolean))
  (locals (LocalUsableManager :type "/Game/BPS_Core/Blueprints/Systems/CharacterSystem/Components/BP_AC_UsableManager Object Reference") (LocalTraceOffsets :type "Array of Vector Structure"))
  (bind _returnvalue (`ActorComponent.GetOwner` MeshComp))
  ;[1 1 1] Try to execute trace damage function for specific usable item or for character.
  (`/Engine/EditorBlueprintResources/StandardMacros.IsValid` _returnvalue
    (:`Is Valid`
      (if (!= (`self.UsableTag`) "None")
        (bind (_found _component) (`/Game/BPS_Core/Blueprints/Systems/CharacterSystem/Libraries/BP_Library_CharacterSystem.FindUsableManager` _returnvalue))
        (if _found
          (bind _output_get (set `local.LocalTraceOffsets` (`self.TraceOffsets`)))
          (`/Game/BPS_Core/Blueprints/Systems/CharacterSystem/Components/BP_AC_UsableManager.TryTraceDamage` _component (`self.UsableTag`) (`self.TraceDamageData`) (`self.OverrideTraceSettings`) (`self.TraceSettings`) _output_get (`self.TraceDistance`))
          (return true))
        (else
          (bind (_found_2 _component_2) (`/Game/BPS_Core/Blueprints/Systems/CharacterSystem/Libraries/BP_Library_CharacterSystem.FindCharacterManager` _returnvalue))
          (if _found_2
            (bind _output_get_2 (set `local.LocalTraceOffsets` (`self.TraceOffsets`)))
            (`/Game/BPS_Core/Blueprints/Systems/CharacterSystem/Components/BP_AC_CharacterManager.TryTraceDamage` _component_2 (`self.TraceDamageData`) (`self.OverrideTraceSettings`) (`self.TraceSettings`) _output_get_2 (`self.TraceDistance`))
            (return true)))))))