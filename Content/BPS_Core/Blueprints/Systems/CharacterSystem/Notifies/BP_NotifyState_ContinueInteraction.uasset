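; Anim notify state that opens a window during an animation in which the owning character can continue an interaction.
; On begin it registers each ContinueInteractionData entry with the owner's BP_AC_InteractionManager component, then immediately tries to continue the interaction.
; On end it removes those entries from the manager by interaction type.
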(fn `GetNotifyName`
  (returns (ReturnValue :type String))
  ;[1 1 1] Update notify name.
  (return "Continue Interaction"))

(fn `Received_NotifyBegin`
  (params (MeshComp :type "SkeletalMeshComponent Object Reference") (Animation :type "AnimSequenceBase Object Reference") (TotalDuration :type "Float (single-precision)") (EventReference :type "AnimNotifyEventReference Structure (by ref)"))
  (returns (ReturnValue :type Boolean))
  (locals (LocalInteractionManager :type "/Game/BPS_Core/Blueprints/Systems/CharacterSystem/Components/BP_AC_InteractionManager Object Reference"))
  (bind _returnvalue (`ActorComponent.GetOwner` MeshComp))
  ;[1 1 1] Adds continue interaction settings and try start continue interaction on notify begin.
  (`/Engine/EditorBlueprintResources/StandardMacros.IsValid` _returnvalue
    (:`Is Valid`
      (bind _output_get (set `local.LocalInteractionManager` (`Actor.GetComponentByClass` _returnvalue "/Game/BPS_Core/Blueprints/Systems/CharacterSystem/Components/BP_AC_InteractionManager.BP_AC_InteractionManager_C")))
      (`/Engine/EditorBlueprintResources/StandardMacros.IsValid` _output_get
        (:`Is Valid`
          (for _array_element (`self.ContinueInteractionData`)
            (`/Game/BPS_Core/Blueprints/Systems/CharacterSystem/Components/BP_AC_InteractionManager.AddContinueInteractionData` _output_get _array_element))
          (`/Game/BPS_Core/Blueprints/Systems/CharacterSystem/Components/BP_AC_InteractionManager.TryContinueInteraction` _output_get)
          (return true))))))

(fn `Received_NotifyEnd`
  (params (MeshComp :type "SkeletalMeshComponent Object Reference") (Animation :type "AnimSequenceBase Object Reference") (EventReference :type "AnimNotifyEventReference Structure (by ref)"))
  (returns (ReturnValue :type Boolean))
  (locals (LocalInteractionManager :type "/Game/BPS_Core/Blueprints/Systems/CharacterSystem/Components/BP_AC_InteractionManager Object Reference"))
  (bind _returnvalue (`ActorComponent.GetOwner` MeshComp))
  ;[1 1 1] Removes continue interaction settings on notify end.
  (`/Engine/EditorBlueprintResources/StandardMacros.IsValid` _returnvalue
    (:`Is Valid`
      (bind _output_get (set `local.LocalInteractionManager` (`Actor.GetComponentByClass` _returnvalue "/Game/BPS_Core/Blueprints/Systems/CharacterSystem/Components/BP_AC_InteractionManager.BP_AC_InteractionManager_C")))
      (`/Engine/EditorBlueprintResources/StandardMacros.IsValid` _output_get
        (:`Is Valid`
          (for _array_element (`self.ContinueInteractionData`)
            (`/Game/BPS_Core/Blueprints/Systems/CharacterSystem/Components/BP_AC_InteractionManager.RemoveContinueInteractionData` _output_get (`.InteractionType_2_DEAEC2164D64A686C7E5B9ADC0AE6138` (break `/Game/BPS_Core/Blueprints/Systems/CharacterSystem/Structures/Interactions/STR_ContinueInteractionData` _array_element))))
          (return true))))))