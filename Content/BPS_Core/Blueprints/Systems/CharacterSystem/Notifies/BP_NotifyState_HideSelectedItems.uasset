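; Animation notify state that hides a character's selected usable items for the duration of an animation window.
; On begin and end it finds the usable manager on the mesh owner and asks it to hide, then show, the selected items.
; Separate start and end delay settings offset each toggle, and an EquippedOnly option is passed through to filter which items are affected.
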(fn `GetNotifyName`
  (returns (ReturnValue :type String))
  ;[1 1 1] Update notify name.
  (return "Hide Selected Items"))

(fn `Received_NotifyBegin`
  (params (MeshComp :type "SkeletalMeshComponent Object Reference") (Animation :type "AnimSequenceBase Object Reference") (TotalDuration :type "Float (single-precision)") (EventReference :type "AnimNotifyEventReference Structure (by ref)"))
  (returns (ReturnValue :type Boolean))
  (bind _returnvalue (`ActorComponent.GetOwner` MeshComp))
  ;[1 1 1] Hide selected usable items.
  (`/Engine/EditorBlueprintResources/StandardMacros.IsValid` _returnvalue
    (:`Is Valid`
      (bind (_found _component) (`/Game/BPS_Core/Blueprints/Systems/CharacterSystem/Libraries/BP_Library_CharacterSystem.FindUsableManager` _returnvalue self))
      (if _found
        (`/Game/BPS_Core/Blueprints/Systems/CharacterSystem/Components/BP_AC_UsableManager.SetSelectedItemsHiddenDelayed` _component (`self.StartDelayTime`) (`self.EquippedOnly`) true)
        (return true)))))

(fn `Received_NotifyEnd`
  (params (MeshComp :type "SkeletalMeshComponent Object Reference") (Animation :type "AnimSequenceBase Object Reference") (EventReference :type "AnimNotifyEventReference Structure (by ref)"))
  (returns (ReturnValue :type Boolean))
  (bind _returnvalue (`ActorComponent.GetOwner` MeshComp))
  ;[1 1 1] Show selected usable items.
  (`/Engine/EditorBlueprintResources/StandardMacros.IsValid` _returnvalue
    (:`Is Valid`
      (bind (_found _component) (`/Game/BPS_Core/Blueprints/Systems/CharacterSystem/Libraries/BP_Library_CharacterSystem.FindUsableManager` _returnvalue self))
      (if _found
        (`/Game/BPS_Core/Blueprints/Systems/CharacterSystem/Components/BP_AC_UsableManager.SetSelectedItemsHiddenDelayed` _component (`self.EndDelayTime`) (`self.EquippedOnly`) false)
        (return true)))))