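; Animation notify state that plays an attached sound on the skeletal mesh for the span of the notify, skipped on dedicated servers.
; On begin it stops the owner's audio components carrying SoundTag, then spawns the sound with volume and pitch multipliers and tags the new component.
; On end, if StopOnEnd is set, it stops tagged sounds, or prints a red on-screen error naming the animation when the tag is missing.
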(fn `GetNotifyName`
  (returns (ReturnValue :type String))
  ;[1 1 1] Update notify name.
  (return "Play Sound"))

(fn `Received_NotifyBegin`
  (params (MeshComp :type "SkeletalMeshComponent Object Reference") (Animation :type "AnimSequenceBase Object Reference") (TotalDuration :type "Float (single-precision)") (EventReference :type "AnimNotifyEventReference Structure (by ref)"))
  (returns (ReturnValue :type Boolean))
  (bind _returnvalue (`ActorComponent.GetOwner` MeshComp))
  (bind _soundtag (`self.SoundTag`))
  ;[1 1 1] Start to play sound with specific sound tag. Stop sounds with the sound tag.
  (`/Engine/EditorBlueprintResources/StandardMacros.IsValid` _returnvalue
    (:`Is Valid`
      (if (not (`KismetSystemLibrary.IsDedicatedServer` _returnvalue))
        (for _array_element (`Actor.GetComponentsByTag` _returnvalue "/Script/Engine.AudioComponent" _soundtag)
          (`AudioComponent.Stop` _array_element))
        (bind _returnvalue_2 (`GameplayStatics.SpawnSoundAttached` (`self.SoundAsset`) MeshComp "None" (0.0 0.0 0.0) (struct) "KeepRelativeOffset" true (`self.VolumeMultiplier`) (`self.PitchMultiplier`) 0.0 null null))
        (`/Engine/EditorBlueprintResources/StandardMacros.IsValid` _returnvalue_2
          (:`Is Valid`
            (`/Game/BPS_Core/Blueprints/Systems/CoreSystem/Libraries/BP_Library_CoreFunctions.AddComponentTag` _returnvalue_2 _soundtag _returnvalue)
            (return true)))))))

(fn `Received_NotifyEnd`
  (params (MeshComp :type "SkeletalMeshComponent Object Reference") (Animation :type "AnimSequenceBase Object Reference") (EventReference :type "AnimNotifyEventReference Structure (by ref)"))
  (returns (ReturnValue :type Boolean))
  (bind _returnvalue (`ActorComponent.GetOwner` MeshComp))
  ;[1 1 1] Stop started sound on end if requried.
  (`/Engine/EditorBlueprintResources/StandardMacros.IsValid` _returnvalue
    (:`Is Valid`
      (if (not (`KismetSystemLibrary.IsDedicatedServer` _returnvalue))
        (if (`self.StopOnEnd`)
          (if (`/Game/BPS_Core/Blueprints/Systems/CoreSystem/Libraries/BP_Library_CoreFunctions.NameIsValid` (`self.SoundTag`) Animation)
            (for _array_element (`Actor.GetComponentsByTag` _returnvalue "/Script/Engine.AudioComponent" (`self.SoundTag`))
              (`AudioComponent.Stop` _array_element))
            (else
              (`KismetSystemLibrary.PrintString` null (`KismetStringLibrary.Concat_StrStr` "SoundTag is not set in the PlaySound notify in the " (`KismetSystemLibrary.GetDisplayName` Animation) " animation!") true true (struct :`R` 1.0 :`A` 1.0) 10.0)
              (return false))))
        (return true)))))