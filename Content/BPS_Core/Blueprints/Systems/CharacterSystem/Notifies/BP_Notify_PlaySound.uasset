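; BP_Notify_PlaySound is an animation notify that plays a tagged sound attached to the animated mesh, replacing any earlier sound with the same tag.
; When cosmetic events can execute, it stops every audio component on the mesh's owner carrying the sound tag.
; It then spawns the sound asset with configurable volume and pitch, and tags the new component so later notifies can stop it.
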(fn `GetNotifyName`
  (returns (ReturnValue :type String))
  ;[1 1 1] Update notify name.
  (return "Play Sound"))

(fn `Received_Notify`
  (params (MeshComp :type "SkeletalMeshComponent Object Reference") (Animation :type "AnimSequenceBase Object Reference") (EventReference :type "AnimNotifyEventReference Structure (by ref)"))
  (returns (ReturnValue :type Boolean))
  (bind _returnvalue (`ActorComponent.GetOwner` MeshComp))
  (bind _soundtag (`self.SoundTag`))
  ;[1 1 1] Try to play sound with specific sound tag. Stop sounds with the sound tag.
  (`/Engine/EditorBlueprintResources/StandardMacros.Can Execute Cosmetic Events`
    (:`True`
      (`/Engine/EditorBlueprintResources/StandardMacros.IsValid` _returnvalue
        (:`Is Valid`
          (for _array_element (`Actor.GetComponentsByTag` _returnvalue "/Script/Engine.AudioComponent" _soundtag)
            (`AudioComponent.Stop` _array_element))
          (bind _returnvalue_2 (`GameplayStatics.SpawnSoundAttached` (`self.SoundAsset`) MeshComp "None" (0.0 0.0 0.0) (struct) "KeepRelativeOffset" true (`self.VolumeMultiplier`) (`self.PitchMultiplier`) 0.0 null null))
          (`/Engine/EditorBlueprintResources/StandardMacros.IsValid` _returnvalue_2
            (:`Is Valid`
              (`/Game/BPS_Core/Blueprints/Systems/CoreSystem/Libraries/BP_Library_CoreFunctions.AddComponentTag` _returnvalue_2 _soundtag)
              (return true))))))))