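; Anim notify that triggers a named notify on a usable item during an animation.
; It looks for a BP_AC_UsableManager on the mesh owner and forwards NotifyName to the selected item found by UsableTag.
; Without a manager, it casts the owner to BP_UsableItem_Base and calls PlayUsableNotify on it directly, so item animations can use it too.
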(fn `GetNotifyName`
  (returns (ReturnValue :type String))
  ;[1 1 1] Update notify name.
  (return "Play Usable Notify"))

(fn `Received_Notify`
  (params (MeshComp :type "SkeletalMeshComponent Object Reference") (Animation :type "AnimSequenceBase Object Reference") (EventReference :type "AnimNotifyEventReference Structure (by ref)"))
  (returns (ReturnValue :type Boolean))
  (locals (LocalUsableManager :type "/Game/BPS_Core/Blueprints/Systems/CharacterSystem/Components/BP_AC_UsableManager Object Reference"))
  (bind _returnvalue (`ActorComponent.GetOwner` MeshComp))
  ;[1 1 1] Try to play usable item notify.
  (`/Engine/EditorBlueprintResources/StandardMacros.IsValid` _returnvalue
    (:`Is Valid`
      (bind _output_get (set `local.LocalUsableManager` (`Actor.GetComponentByClass` _returnvalue "/Game/BPS_Core/Blueprints/Systems/CharacterSystem/Components/BP_AC_UsableManager.BP_AC_UsableManager_C")))
      (`/Engine/EditorBlueprintResources/StandardMacros.IsValid` _output_get
        (:`Is Valid`
          (bind (_found _usableitem) (`/Game/BPS_Core/Blueprints/Systems/CharacterSystem/Components/BP_AC_UsableManager.FindSelectedItem` _output_get (`self.UsableTag`)))
          (if _found
            (`/Game/BPS_Core/Blueprints/Systems/CharacterSystem/Actors/BP_UsableItem_Base.PlayUsableNotify` _usableitem (`self.NotifyName`))
            (return true)))
        (:`Is Not Valid`
          (bind _asbp_usable_item_base (cast `/Game/BPS_Core/Blueprints/Systems/CharacterSystem/Actors/BP_UsableItem_Base` _returnvalue))
          (`/Game/BPS_Core/Blueprints/Systems/CharacterSystem/Actors/BP_UsableItem_Base.PlayUsableNotify` _asbp_usable_item_base (`self.NotifyName`))
          (return true))))))