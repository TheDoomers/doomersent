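; Anim notify state that temporarily overrides a usable item's socket, visibility and destructibility during part of an animation.
; On begin, it finds the owner's usable manager and tagged item, attaches it to the configured socket and applies the hidden and destroy-permission settings.
; On end, it optionally attempts to destroy the item, then calls restores for its default socket and visibility and re-enables destruction, even when destruction was requested.
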(fn `GetNotifyName`
  (returns (ReturnValue :type String))
  ;[1 1 1] Update notify name.
  (return "Override Usable Item"))

(fn `Received_NotifyBegin`
  (params (MeshComp :type "SkeletalMeshComponent Object Reference") (Animation :type "AnimSequenceBase Object Reference") (TotalDuration :type "Float (single-precision)") (EventReference :type "AnimNotifyEventReference Structure (by ref)"))
  (returns (ReturnValue :type Boolean))
  (bind _returnvalue (`ActorComponent.GetOwner` MeshComp))
  ;[1 1 1] Attach weapon to start weapon socket.
  (`/Engine/EditorBlueprintResources/StandardMacros.IsValid` _returnvalue
    (:`Is Valid`
      (bind (_found _component) (`/Game/BPS_Core/Blueprints/Systems/CharacterSystem/Libraries/BP_Library_CharacterSystem.FindUsableManager` _returnvalue self))
      (if _found
        (bind (_found_2 _usableitem) (`/Game/BPS_Core/Blueprints/Systems/CharacterSystem/Components/BP_AC_UsableManager.FindUsableItem` _component (`self.UsableTag`)))
        (if _found_2
          (`/Game/BPS_Core/Blueprints/Systems/CharacterSystem/Components/BP_AC_UsableManager.AttachUsableItemToSocket` _component _usableitem (`self.SocketData`))
          (`Actor.SetActorHiddenInGame` _usableitem (`self.NewHidden`))
          (`/Game/BPS_Core/Blueprints/Systems/CharacterSystem/Actors/BP_UsableItem_Base.SetCanBeDestroyed` _usableitem (`self.CanBeDestroyed`))
          (return true))))))

(fn `Received_NotifyEnd`
  (params (MeshComp :type "SkeletalMeshComponent Object Reference") (Animation :type "AnimSequenceBase Object Reference") (EventReference :type "AnimNotifyEventReference Structure (by ref)"))
  (returns (ReturnValue :type Boolean))
  (bind _returnvalue (`ActorComponent.GetOwner` MeshComp))
  ;[1 1 1] Attach weapon to end weapon socket.
  (`/Engine/EditorBlueprintResources/StandardMacros.IsValid` _returnvalue
    (:`Is Valid`
      (bind (_found _component) (`/Game/BPS_Core/Blueprints/Systems/CharacterSystem/Libraries/BP_Library_CharacterSystem.FindUsableManager` _returnvalue self))
      (if _found
        (bind (_found_2 _usableitem) (`/Game/BPS_Core/Blueprints/Systems/CharacterSystem/Components/BP_AC_UsableManager.FindUsableItem` _component (`self.UsableTag`)))
        (if _found_2
          (if (`self.DestroyOnEnd`)
            (`/Game/BPS_Core/Blueprints/Systems/CharacterSystem/Actors/BP_UsableItem_Base.TryDestroyActor` _usableitem))
          (`/Game/BPS_Core/Blueprints/Systems/CharacterSystem/Components/BP_AC_UsableManager.AttachUsableItemToSocket` _component _usableitem (`/Game/BPS_Core/Blueprints/Systems/CharacterSystem/Actors/BP_UsableItem_Base.GetDefaultSocketData` _usableitem))
          (`/Game/BPS_Core/Blueprints/Systems/CharacterSystem/Actors/BP_UsableItem_Base.SetDefaultVisibility` _usableitem)
          (`/Game/BPS_Core/Blueprints/Systems/CharacterSystem/Actors/BP_UsableItem_Base.SetCanBeDestroyed` _usableitem true)
          (return true))))))