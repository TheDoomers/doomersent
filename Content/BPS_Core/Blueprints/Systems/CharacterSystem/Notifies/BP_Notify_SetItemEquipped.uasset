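; BP_Notify_SetItemEquipped is an animation notify that sets the equipped state of usable items at a chosen animation frame.
; It finds the BP_AC_UsableManager component on the mesh's owner and passes it the configured equipped flag.
; A set usable tag targets that specific item, while a tag of None applies the state to all selected usable items.
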(fn `GetNotifyName`
  (returns (ReturnValue :type String))
  ;[1 1 1] Update notify name.
  (return "Set Item Equipped"))

(fn `Received_Notify`
  (params (MeshComp :type "SkeletalMeshComponent Object Reference") (Animation :type "AnimSequenceBase Object Reference") (EventReference :type "AnimNotifyEventReference Structure (by ref)"))
  (returns (ReturnValue :type Boolean))
  (locals (LocalUsableManager :type "/Game/BPS_Core/Blueprints/Systems/CharacterSystem/Components/BP_AC_UsableManager Object Reference"))
  (bind _returnvalue (`ActorComponent.GetOwner` MeshComp))
  (bind _newequipped (`self.NewEquipped`))
  ;[1 1 1] Try to set equipped state for specific usable item. If usable tag is not set then sets equipped state for all selected usable items.
  (`/Engine/EditorBlueprintResources/StandardMacros.IsValid` _returnvalue
    (:`Is Valid`
      (bind _output_get (set `local.LocalUsableManager` (`Actor.GetComponentByClass` _returnvalue "/Game/BPS_Core/Blueprints/Systems/CharacterSystem/Components/BP_AC_UsableManager.BP_AC_UsableManager_C")))
      (`/Engine/EditorBlueprintResources/StandardMacros.IsValid` _output_get
        (:`Is Valid`
          (if (== (`self.UsableTag`) "None")
            (`/Game/BPS_Core/Blueprints/Systems/CharacterSystem/Components/BP_AC_UsableManager.SetItemsAreEquipped` _output_get _newequipped)
            (else
              (`/Game/BPS_Core/Blueprints/Systems/CharacterSystem/Components/BP_AC_UsableManager.SetItemEquipped` _output_get (`self.UsableTag`) _newequipped)))
          (return true))))))