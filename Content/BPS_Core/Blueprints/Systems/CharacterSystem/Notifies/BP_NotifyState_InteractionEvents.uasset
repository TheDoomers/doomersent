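; Animation notify state that fires interaction events on the animated character at the start and end of its window.
; Begin and end each find an interaction manager component for the mesh owner and call PlayInteractionEvent with separate start or end event name and subtype properties.
; If no manager is found, no event plays.
; It displays as "Interaction Events" in the animation editor.
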(fn `GetNotifyName`
  (returns (ReturnValue :type String))
  ;[1 1 1] Update notify name.
  (return "Interaction Events"))

(fn `Received_NotifyBegin`
  (params (MeshComp :type "SkeletalMeshComponent Object Reference") (Animation :type "AnimSequenceBase Object Reference") (TotalDuration :type "Float (single-precision)") (EventReference :type "AnimNotifyEventReference Structure (by ref)"))
  (returns (ReturnValue :type Boolean))
  (locals (LocalUsableManager :type "/Game/BPS_Core/Blueprints/Systems/CharacterSystem/Components/BP_AC_UsableManager Object Reference") (LocalSocketData :type "Array of /Game/BPS_Core/Blueprints/Systems/CoreSystem/Structures/STR_SocketData Structure"))
  (bind _returnvalue (`ActorComponent.GetOwner` MeshComp))
  ;[1 1 1] Try to play interaction event for the charater on notify begin.
  (bind (_found _component) (`/Game/BPS_Core/Blueprints/Systems/CharacterSystem/Libraries/BP_Library_CharacterSystem.FindInteractionManager` _returnvalue _returnvalue))
  (if _found
    (bind _success (`/Game/BPS_Core/Blueprints/Systems/CharacterSystem/Components/BP_AC_InteractionManager.PlayInteractionEvent` _component (`self.StartEventName`) (`self.StartSubType`)))
    (return _success)))

(fn `Received_NotifyEnd`
  (params (MeshComp :type "SkeletalMeshComponent Object Reference") (Animation :type "AnimSequenceBase Object Reference") (EventReference :type "AnimNotifyEventReference Structure (by ref)"))
  (returns (ReturnValue :type Boolean))
  (locals (LocalUsableManager :type "/Game/BPS_Core/Blueprints/Systems/CharacterSystem/Components/BP_AC_UsableManager Object Reference"))
  (bind _returnvalue (`ActorComponent.GetOwner` MeshComp))
  ;[1 1 1] Try to play interaction event for the charater on notify end.
  (bind (_found _component) (`/Game/BPS_Core/Blueprints/Systems/CharacterSystem/Libraries/BP_Library_CharacterSystem.FindInteractionManager` _returnvalue _returnvalue))
  (if _found
    (bind _success (`/Game/BPS_Core/Blueprints/Systems/CharacterSystem/Components/BP_AC_InteractionManager.PlayInteractionEvent` _component (`self.EndEventName`) (`self.EndSubType`)))
    (return _success)))