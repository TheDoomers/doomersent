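; Interactable campfire building that opens crafting for the player who uses it.
; It implements the interaction interface at actor level, gated by CanInteract, supplying an interaction time and widget socket while component-level queries return false.
; On server interaction it finds the player's controller manager and passes its CraftingComponent to TryOpenCrafting.
; It then multicasts a cosmetic sound, even if opening fails.
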(event `PlayInteractionEffects (Multicast)`
  ;[1 1 1] Network cosmetic effects.
  (`/Engine/EditorBlueprintResources/StandardMacros.Can Execute Cosmetic Events`
    (:`True`
      (`GameplayStatics.PlaySoundAtLocation` (`self.InteractionSound`) (`self.K2_GetActorLocation`) (struct) 1.0 1.0 0.0 null null null null))))

(fn `CheckCanInteractWithActor_BPI`
  (params (PlayerController :type "PlayerController Object Reference"))
  (returns (Success :type Boolean))
  ;[1 1 1] Returns true if player can interact with the actor.
  (return (`self.CanInteract`)))

(fn `CheckCanInteractWithComponent_BPI`
  (params (TargetComponent :type "PrimitiveComponent Object Reference") (PlayerController :type "PlayerController Object Reference"))
  (returns (Success :type Boolean))
  (return false))

(fn `GetHighlightComponents_BPI`
  (params (TargetComponent :type "PrimitiveComponent Object Reference"))
  (returns (Success :type Boolean) (HighlightComponents :type "Array of PrimitiveComponent Object Reference"))
  (return false))

(fn `GetInteractionText_BPI`
  (params (TargetComponent :type "PrimitiveComponent Object Reference") (PlayerController :type "PlayerController Object Reference") (InteractionType :type Name))
  (returns (Success :type Boolean) (InteractionText :type Text))
  (return false ""))

(fn `GetInteractionTime_BPI`
  (params (TargetComponent :type "PrimitiveComponent Object Reference"))
  (returns (Success :type Boolean) (InteractionTime :type "Float (double-precision)"))
  ;[1 1 1] Returns interaction time.
  (return true (`self.InteractionTime`)))

(fn `GetInteractionWidgetClass_BPI`
  (params (TargetComponent :type "PrimitiveComponent Object Reference"))
  (returns (Success :type Boolean) (WidgetClass :type "UserWidget Class Reference"))
  (return false null))

(fn `GetInteractionWidgetSocket_BPI`
  (params (TargetComponent :type "PrimitiveComponent Object Reference"))
  (returns (Success :type Boolean) (SceneComponent :type "SceneComponent Object Reference"))
  ;[1 1 1] Returns interaction widget socket.
  (return true (`self.InteractionWidgetSocket`)))

(fn `GetNearestInteractableComponent_BPI`
  (params (PlayerController :type "PlayerController Object Reference"))
  (returns (Success :type Boolean) (Component :type "PrimitiveComponent Object Reference"))
  (return false null))

(fn `GetTargetInteractableComponent_BPI`
  (params (PossibleComponent :type "PrimitiveComponent Object Reference"))
  (returns (Success :type Boolean) (TargetComponent :type "PrimitiveComponent Object Reference"))
  (return false null))

(fn `GetTraceTargetLocation_BPI`
  (params (TargetComponent :type "PrimitiveComponent Object Reference"))
  (returns (Success :type Boolean) (TargetLocation :type "Vector Structure"))
  (return false (0.0 0.0 0.0)))

(fn `HasInteractableComponents_BPI`
  (returns (Result :type Boolean))
  (return false))

(fn `HasInteractionOnClient_BPI`
  (returns (Result :type Boolean))
  (return false))

(fn `SetCanInteract_BPI`
  (params (NewCanInteract :type Boolean))
  (returns (Success :type Boolean))
  ;[1 1 1] Set value of the can interact variable.
  (set `self.CanInteract` NewCanInteract)
  (return true))

(fn `TryInteractOnClient_BPI`
  (params (TargetComponent :type "PrimitiveComponent Object Reference") (PlayerController :type "PlayerController Object Reference"))
  (returns (Success :type Boolean) (RunOnServer :type Boolean))
  (return false false))

(fn `TryInteractOnServer_BPI`
  (params (TargetComponent :type "PrimitiveComponent Object Reference") (PlayerController :type "PlayerController Object Reference"))
  (returns (Success :type Boolean))
  ;[1 1 1] Try open crafting for the player.
  (bind (_found _manager) (`/Game/BPS_Core/Blueprints/Game/Libraries/BP_Library_TopDownGame.FindPlayerControllerManager` PlayerController))
  (if _found
    (bind _success (`/Game/BPS_Core/Blueprints/Game/Components/PlayerController/BP_AC_PlayerControllerManager.TryOpenCrafting` _manager (`self.CraftingComponent`) null))
    (`self.PlayInteractionEffects (Multicast)`) ; #update 1.1
    (return _success)))

(fn `TryRunInteractionEvent_BPI`
  (params (PlayerController :type "PlayerController Object Reference") (EventName :type Name) (SubType :type Name) (Options :type String))
  (returns (Success :type Boolean))
  (return false))

(fn `UserConstructionScript`
  (`parent.UserConstructionScript`))