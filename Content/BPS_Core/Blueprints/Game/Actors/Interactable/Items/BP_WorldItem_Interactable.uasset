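; A world item that players pick up through the BPI interaction interface, showing a "Pick up {Name}" prompt with zero interaction time.
; Server interaction fires OnItemInteracted, then passes the item to the player's items manager via TryPickUpItem.
; BeginPlay selects the pickup sound from the item's TakeGroup gameplay tags.
; The actor itself is the interactable, gated by a CanInteract flag that persists through SaveObjectComponent.
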(event `self.ReceiveBeginPlay`
  ;[1 1 1] Begin play event.
  (`parent.ReceiveBeginPlay`)
  (`self.UpdatePickUpSound`))

(event `self.SaveObjectComponent.OnPreSaveData`
  (params (Component :type "/Game/BPS_Core/Blueprints/Systems/SaveLoadSystem/Components/BP_AC_SaveObjectComponent Object Reference") (SaveGame :type "SaveGame Object Reference"))
  ;[1 1 1] Save and load events.
  (`/Game/BPS_Core/Blueprints/Systems/SaveLoadSystem/Components/BP_AC_SaveObjectComponent.SaveBoolVariable` Component "CanInteract" (`self.CanInteract`)))

(event `self.SaveObjectComponent.OnPostLoadData`
  (params (Component :type "/Game/BPS_Core/Blueprints/Systems/SaveLoadSystem/Components/BP_AC_SaveObjectComponent Object Reference") (SaveGame :type "SaveGame Object Reference"))
  ;[1 1 1] Save and load events.
  (bind (_success _variablevalue) (`/Game/BPS_Core/Blueprints/Systems/SaveLoadSystem/Components/BP_AC_SaveObjectComponent.LoadBoolVariable` Component "CanInteract"))
  (set `self.CanInteract` _variablevalue))

(fn `CheckCanInteractWithActor_BPI`
  (params (PlayerController :type "PlayerController Object Reference"))
  (returns (Success :type Boolean))
  ;[1 1 1] Returns true if player can interact with the actor.
  (return (`self.CanInteract`)))

(fn `CheckCanInteractWithComponent_BPI`
  (params (TargetComponent :type "PrimitiveComponent Object Reference") (PlayerController :type "PlayerController Object Reference"))
  (returns (Success :type Boolean))
  (return false))

(fn `GetHighlightComponents_BPI`
  (params (TargetComponent :type "PrimitiveComponent Object Reference"))
  (returns (Success :type Boolean) (HighlightComponents :type "Array of PrimitiveComponent Object Reference"))
  (return false))

(fn `GetInteractionText_BPI`
  (params (TargetComponent :type "PrimitiveComponent Object Reference") (PlayerController :type "PlayerController Object Reference") (InteractionType :type Name))
  (returns (Success :type Boolean) (InteractionText :type Text))
  ;[1 1 1] Returns interaction text.
  (return true (`|FormatText` "Pick up {Name}" (`/Game/BPS_Core/Blueprints/Systems/ItemsSystem/Libraries/BP_Library_ItemsSystem.GetItemName` (`self.GetWorldItemData`)))))

(fn `GetInteractionTime_BPI`
  (params (TargetComponent :type "PrimitiveComponent Object Reference"))
  (returns (Success :type Boolean) (InteractionTime :type "Float (double-precision)"))
  ;[1 1 1] Returns interactable time.
  (return true 0.0))

(fn `GetInteractionWidgetClass_BPI`
  (params (TargetComponent :type "PrimitiveComponent Object Reference"))
  (returns (Success :type Boolean) (WidgetClass :type "UserWidget Class Reference"))
  (return false null))

(fn `GetInteractionWidgetSocket_BPI`
  (params (TargetComponent :type "PrimitiveComponent Object Reference"))
  (returns (Success :type Boolean) (SceneComponent :type "SceneComponent Object Reference"))
  (return false null))

(fn `GetNearestInteractableComponent_BPI`
  (params (PlayerController :type "PlayerController Object Reference"))
  (returns (Success :type Boolean) (Component :type "PrimitiveComponent Object Reference"))
  ;[1 1 1] Returns nearest interactable component.
  (return true (`self.StaticMesh`)))

(fn `GetTargetInteractableComponent_BPI`
  (params (PossibleComponent :type "PrimitiveComponent Object Reference"))
  (returns (Success :type Boolean) (TargetComponent :type "PrimitiveComponent Object Reference"))
  (return false null))

(fn `GetTraceTargetLocation_BPI`
  (params (TargetComponent :type "PrimitiveComponent Object Reference"))
  (returns (Success :type Boolean) (TargetLocation :type "Vector Structure"))
  (return false (0.0 0.0 0.0)))

(fn `HasInteractableComponents_BPI`
  (returns (Result :type Boolean))
  (return false))

(fn `HasInteractionOnClient_BPI`
  (returns (Result :type Boolean))
  (return false))

(fn `SetCanInteract_BPI`
  (params (NewCanInteract :type Boolean))
  (returns (Success :type Boolean))
  ;[1 1 1] Set value of the can interact variable.
  (set `self.CanInteract` NewCanInteract)
  (return true))

(fn `TryInteractOnClient_BPI`
  (params (TargetComponent :type "PrimitiveComponent Object Reference") (PlayerController :type "PlayerController Object Reference"))
  (returns (Success :type Boolean) (RunOnServer :type Boolean))
  (return false false))

(fn `TryInteractOnServer_BPI`
  (params (TargetComponent :type "PrimitiveComponent Object Reference") (PlayerController :type "PlayerController Object Reference"))
  (returns (Success :type Boolean))
  ;[1 1 1] Try to start interaction with actor on server.
  (`self.OnItemInteracted` self PlayerController)
  (bind (_found _component) (`/Game/BPS_Core/Blueprints/Systems/ItemsSystem/Libraries/BP_Library_ItemsSystem.FindPlayerItemsManager` PlayerController))
  (if _found
    (bind _success (`/Game/BPS_Core/Blueprints/Systems/ItemsSystem/Components/BP_AC_PlayerItemsManager.TryPickUpItem` _component self))
    (return _success)
    (else
      (return false))))

(fn `TryRunInteractionEvent_BPI`
  (params (PlayerController :type "PlayerController Object Reference") (EventName :type Name) (SubType :type Name) (Options :type String))
  (returns (Success :type Boolean))
  (return false))

(fn `UpdatePickUpSound`
  (returns (Success :type Boolean))
  (locals (LocalItemData :type "/Game/BPS_Core/Blueprints/Systems/ItemsSystem/Structures/STR_ItemData Structure") (LocalItemTag :type "GameplayTag Structure"))
  (bind _itemdata (`self.GetWorldItemData`))
  ;[1 1 1] Update pick up sound for item.
  (set `local.LocalItemData` _itemdata)
  (for _array_element (`BlueprintGameplayTagLibrary.BreakGameplayTagContainer` (`/Game/BPS_Core/Blueprints/Systems/ItemsSystem/Libraries/BP_Library_ItemsSystem.GetItemTags` _itemdata))
    (bind _output_get (set `local.LocalItemTag` _array_element))
    (if (`BlueprintGameplayTagLibrary.MatchesTag` _array_element (struct :`TagName` "ItemsSystem.Item.TakeGroup"))
      (bind (_value _returnvalue) (`BlueprintMapLibrary.Map_Find` (`self.PickUpSounds`) _output_get))
      (if _returnvalue
        (set `self.PickUpSound` _value)
        (return true)))))

(fn `UserConstructionScript`
  (`parent.UserConstructionScript`))