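; Base zombie character with randomized modular meshes following a leader pose, saved health, energy and loot, and a lootable corpse.
; Damage raises aggression, spawns blood and plays directional hit reactions, while hits on listed bones drain balance toward a temporary ragdoll knockout.
; BehaviorManager events drive combat state and attack interactions through InteractionManager.
; Timers after death or losing the chase target destroy it based on a player-range check.
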(fn `CheckCanInteractWithActor_BPI`
  (params (PlayerController :type "PlayerController Object Reference"))
  (returns (Success :type Boolean))
  ;[1 1 1] Returns true if player can interact with the actor.
  (return (not (`/Game/BPS_Core/Blueprints/Systems/StatsSystem/Components/BP_AC_StatAttribute_Health.IsAlive` (`self.Stat_Health`)))))

(fn `CheckCanInteractWithComponent_BPI`
  (params (TargetComponent :type "PrimitiveComponent Object Reference") (PlayerController :type "PlayerController Object Reference"))
  (returns (Success :type Boolean))
  (return false))

(fn `GetCasterAimVariables_BPI`
  (returns (Success :type Boolean) (StartLocation :type "Vector Structure") (Rotation :type "Rotator Structure"))
  (return true (`SceneComponent.K2_GetComponentLocation` (`self.LaunchStart`)) (`/Game/BPS_Core/Blueprints/Systems/CharacterSystem/Components/BP_AC_LocomotionManager.GetAimRotation` (`self.LocomotionManager`))))

(fn `GetCasterLaunchSpeed_BPI`
  (returns (Success :type Boolean) (IsOverridden :type Boolean) (OverriddenSpeed :type "Float (double-precision)"))
  (return true false 0.0))

(fn `GetCasterLaunchTransform_BPI`
  (returns (Success :type Boolean) (Transform :type "Transform Structure"))
  (return true (`SceneComponent.K2_GetComponentToWorld` (`self.LaunchStart`))))

(fn `GetHighlightComponents_BPI`
  (params (TargetComponent :type "PrimitiveComponent Object Reference"))
  (returns (Success :type Boolean) (HighlightComponents :type "Array of PrimitiveComponent Object Reference"))
  ;[1 1 1] Returns highlight components.
  (return true (`|MakeArray` (`self.Mesh`) (`self.HatSkeletal`) (`self.BodySkeletal`) (`self.PantsSkeletal`) (`self.FeetSkeletal`) :!type "PrimitiveComponent Object Reference")))

(fn `GetInteractionText_BPI`
  (params (TargetComponent :type "PrimitiveComponent Object Reference") (PlayerController :type "PlayerController Object Reference") (InteractionType :type Name))
  (returns (Success :type Boolean) (InteractionText :type Text))
  (return false ""))

(fn `GetInteractionTime_BPI`
  (params (TargetComponent :type "PrimitiveComponent Object Reference"))
  (returns (Success :type Boolean) (InteractionTime :type "Float (double-precision)"))
  ;[1 1 1] Returns interaction time.
  (return true 1.0))

(fn `GetInteractionWidgetClass_BPI`
  (params (TargetComponent :type "PrimitiveComponent Object Reference"))
  (returns (Success :type Boolean) (WidgetClass :type "UserWidget Class Reference"))
  (return false null))

(fn `GetInteractionWidgetSocket_BPI`
  (params (TargetComponent :type "PrimitiveComponent Object Reference"))
  (returns (Success :type Boolean) (SceneComponent :type "SceneComponent Object Reference"))
  ;[1 1 1] Returns interaction widget socket.
  (return true (`self.Mesh`)))

(fn `GetNearestInteractableComponent_BPI`
  (params (PlayerController :type "PlayerController Object Reference"))
  (returns (Success :type Boolean) (Component :type "PrimitiveComponent Object Reference"))
  (return false null))

(fn `GetSaveObjectComponent_BPI`
  (returns (Success :type Boolean) (Component :type "/Game/BPS_Core/Blueprints/Systems/SaveLoadSystem/Components/BP_AC_SaveObjectComponent Object Reference"))
  ;[1 1 1] Returns save object component.
  (return true (`self.SaveObjectComponent`)))

(fn `GetTargetInteractableComponent_BPI`
  (params (PossibleComponent :type "PrimitiveComponent Object Reference"))
  (returns (Success :type Boolean) (TargetComponent :type "PrimitiveComponent Object Reference"))
  (return false null))

(fn `GetTraceTargetLocation_BPI`
  (params (TargetComponent :type "PrimitiveComponent Object Reference"))
  (returns (Success :type Boolean) (TargetLocation :type "Vector Structure"))
  (return false (0.0 0.0 0.0)))

(fn `HasInteractableComponents_BPI`
  (returns (Result :type Boolean))
  (return false))

(fn `HasInteractionOnClient_BPI`
  (returns (Result :type Boolean))
  (return false))

(fn `OnRep_BodySkeletalMesh`
  ;[1 1 1] Update body skeletal mesh for all clients.
)

(fn `OnRep_FeetSkeletalMesh`
  ;[1 1 1] Update feet skeletal mesh for all clients.
  (`/Game/BPS_Core/Blueprints/Systems/AsyncLoadSystem/Libraries/BP_Library_AsyncLoad.AsyncLoadSkeletalMeshForComponent` (`self.FeetSkeletal`) (`self.FeetSkeletalMesh`)))

(fn `OnRep_HeadSkeletalMesh`
  (`/Game/BPS_Core/Blueprints/Systems/AsyncLoadSystem/Libraries/BP_Library_AsyncLoad.AsyncLoadSkeletalMeshForComponent` (`self.Mesh`) (`self.HeadSkeletalMesh`)))

(fn `OnRep_PantsSkeletalMesh`
  ;[1 1 1] Update pants skeletal mesh for all clients.
  (`/Game/BPS_Core/Blueprints/Systems/AsyncLoadSystem/Libraries/BP_Library_AsyncLoad.AsyncLoadSkeletalMeshForComponent` null))

(fn `SetCanInteract_BPI`
  (params (NewCanInteract :type Boolean))
  (returns (Success :type Boolean))
  (return false))

(fn `TryInteractOnClient_BPI`
  (params (TargetComponent :type "PrimitiveComponent Object Reference") (PlayerController :type "PlayerController Object Reference"))
  (returns (Success :type Boolean) (RunOnServer :type Boolean))
  (return false false))

(fn `TryInteractOnServer_BPI`
  (params (TargetComponent :type "PrimitiveComponent Object Reference") (PlayerController :type "PlayerController Object Reference"))
  (returns (Success :type Boolean))
  ;[1 1 1] Try to start interaction with actor on server.
  (bind (_found _manager) (`/Game/BPS_Core/Blueprints/Game/Libraries/BP_Library_TopDownGame.FindPlayerControllerManager` PlayerController))
  (if _found
    (`/Game/BPS_Core/Blueprints/Game/Components/PlayerController/BP_AC_PlayerControllerManager.TryOpenLootContainer` _manager (`self.LootContainer`))
    (return true)))

(fn `TryRunInteractionEvent_BPI`
  (params (PlayerController :type "PlayerController Object Reference") (EventName :type Name) (SubType :type Name) (Options :type String))
  (returns (Success :type Boolean))
  (return false))

(fn `UserConstructionScript`
  ;[1 1 1] Construction script. Init components and variables.
  (`SkeletalMeshComponent.SetSkeletalMeshAsset` (`self.BodySkeletal`) (`|GetArrayItem` (`self.Body`) (`KismetMathLibrary.RandomIntegerInRange` 0 4)))
  (`SkeletalMeshComponent.SetSkeletalMeshAsset` (`self.PantsSkeletal`) (`|GetArrayItem` (`self.Pants`) (`KismetMathLibrary.RandomIntegerInRange` 0 4)))
  (`SkinnedMeshComponent.SetLeaderPoseComponent` (`self.BodySkeletal`) (`self.Mesh`) true false)
  (`SkinnedMeshComponent.SetLeaderPoseComponent` (`self.PantsSkeletal`) (`self.Mesh`) true false)
  (`SkinnedMeshComponent.SetLeaderPoseComponent` (`self.FeetSkeletal`) (`self.Mesh`) true false)
  (`SkinnedMeshComponent.SetLeaderPoseComponent` (`self.HatSkeletal`) (`self.Mesh`) true false)
  (`SkinnedMeshComponent.SetLeaderPoseComponent` (`self.NewZombie`) (`self.Mesh`) true false))