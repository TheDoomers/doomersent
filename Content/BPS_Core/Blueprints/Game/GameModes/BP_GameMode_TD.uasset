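; Top-down game mode that restores saved level data and sets up joining players and their pawns.
; On begin play the save game manager component loads current level data, and new players are initialized from the current save through their PlayerControllerManager component.
; Restarts initialize the pawn after a short delay.
; Pawn spawning reuses a living, unpossessed PlayerCharacter-tagged pawn before falling back to default spawning, except at Play-From-Here starts.
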(event `self.ReceiveBeginPlay`
  ;[1 1 1] Begin play event. Try to load level data from transition save.
  (bind (_success _component) (`/Game/BPS_Core/Blueprints/Systems/SaveLoadSystem/Libraries/BP_Library_SaveLoadSystem.FindSaveGameManagerComponent`))
  (if _success
    (`/Game/BPS_Core/Blueprints/Systems/SaveLoadSystem/Components/BP_AC_SaveGameManager.TryLoadCurrentLevelData` _component)))

(event `self.HandleStartingNewPlayer`
  (params (NewPlayer :type "PlayerController Object Reference"))
  ;[1 1 1] Try to initializa game for player.
  (`KismetSystemLibrary.Delay` 0.0)
  (bind (_success _component) (`/Game/BPS_Core/Blueprints/Systems/SaveLoadSystem/Libraries/BP_Library_SaveLoadSystem.FindSaveGameManagerComponent`))
  (if _success
    (`/Game/BPS_Core/Blueprints/Game/Components/PlayerController/BP_AC_PlayerControllerManager.TryInitGameForPlayer` (`self.GetComponentByClass` NewPlayer "/Game/BPS_Core/Blueprints/Game/Components/PlayerController/BP_AC_PlayerControllerManager.BP_AC_PlayerControllerManager_C") (`/Game/BPS_Core/Blueprints/Systems/SaveLoadSystem/Components/BP_AC_SaveGameManager.GetCurrentSaveGame` _component))))

(event `self.K2_OnRestartPlayer`
  (params (NewPlayer :type "Controller Object Reference"))
  ;[1 1 1] Try to restart player and init player pawn.
  (`KismetSystemLibrary.Delay` 1.0)
  (`/Game/BPS_Core/Blueprints/Game/Components/PlayerController/BP_AC_PlayerControllerManager.TryInitPlayerPawn` (`self.GetComponentByClass` NewPlayer "/Game/BPS_Core/Blueprints/Game/Components/PlayerController/BP_AC_PlayerControllerManager.BP_AC_PlayerControllerManager_C")))

(fn `SpawnDefaultPawnFor`
  (params (NewPlayer :type "Controller Object Reference") (StartSpot :type "Actor Object Reference"))
  (returns (ReturnValue :type "Pawn Object Reference"))
  ;[1 1 1] Try to find available playable character for player or spawn new in player start or in respawn point.
  (cast `PlayerStartPIE` StartSpot
    (:`then`
      _)
    (:`CastFailed`
      (bind _outactors (`GameplayStatics.GetAllActorsOfClassWithTag` "/Script/Engine.Pawn" "PlayerCharacter"))
      (for _array_element _outactors
        (bind _isalive (`/Game/BPS_Core/Blueprints/Systems/StatsSystem/Libraries/BP_Library_StatsSystem.CheckActorIsAlive` _array_element))
        (if _isalive
          (if (not (`Pawn.IsPlayerControlled` _array_element))
            (return _array_element))))))
  (bind _returnvalue (`parent.SpawnDefaultPawnFor` NewPlayer StartSpot))
  (return _returnvalue))

(fn `UserConstructionScript`)