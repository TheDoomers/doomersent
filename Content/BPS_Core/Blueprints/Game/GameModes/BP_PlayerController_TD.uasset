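; Top-down player controller that routes player input, spawns a top-down plane actor and handles the player's save data.
; Enhanced Input actions forward to PlayerControllerManager for HUD, menus, crafting, building, camera and dialogue replies; map panning goes to MapManager, while map zoom is unwired.
; Client character initialization spawns the plane targeting the pawn, and level changes update its CharacterManager.
; SaveObjectComponent events save and load tags, narrative, leveling and customization.
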(event `self.LevelingManager.OnCurrentLevelChanged`
  (params (Manager :type "/Game/BPS_Core/Blueprints/Systems/LevelingSystem/Components/BP_AC_LevelingManager Object Reference") (NewLevel :type Integer) (PrevLevel :type Integer))
  (bind _returnvalue (`self.K2_GetPawn`))
  ;[1 1 1] Component events.
  (`/Engine/EditorBlueprintResources/StandardMacros.IsValid` _returnvalue
    (:`Is Valid`
      (bind (_found _component) (`/Game/BPS_Core/Blueprints/Systems/CharacterSystem/Libraries/BP_Library_CharacterSystem.FindCharacterManager` _returnvalue))
      (if _found
        (`/Game/BPS_Core/Blueprints/Systems/CharacterSystem/Components/BP_AC_CharacterManager.SetCharacterLevel` _component NewLevel)))))

(event `self.PlayerControllerManager.OnCharacterInitialized_Client`
  (params (Manager :type "/Game/BPS_Core/Blueprints/Game/Components/PlayerController/BP_AC_PlayerControllerManager Object Reference") (Character :type "Character Object Reference"))
  ;[1 1 1] Component events.
  (`self.CreateTopDownPlane`))

(event `CreateTopDownPlane`
  (bind _returnvalue (`self.K2_GetPawn`))
  ;[1 1 1] Component events.
  (`/Engine/EditorBlueprintResources/StandardMacros.IsValid` _returnvalue
    (:`Is Valid`
      (`|SpawnActorFromClass` "/Game/BPS_Core/Blueprints/Game/Actors/Misc/BP_TopDownPlaneActor.BP_TopDownPlaneActor_C" (`KismetMathLibrary.MakeTransform` (`self.K2_GetActorLocation` _returnvalue)) "Undefined" "OverrideRootScale" null _returnvalue (0.0 0.0 0.0) null))))

(event `self.SaveObjectComponent.OnSaveData`
  (params (Component :type "/Game/BPS_Core/Blueprints/Systems/SaveLoadSystem/Components/BP_AC_SaveObjectComponent Object Reference") (SaveGame :type "SaveGame Object Reference"))
  ;[1 1 1] Save and load events.
  (`/Game/BPS_Core/Blueprints/Systems/CoreSystem/Libraries/BP_Library_CoreFunctions.SavePlayerTags` self SaveGame)
  (`/Game/BPS_Core/Blueprints/Systems/NarrativeSystem/Components/BP_AC_NarrativeManager.SaveNarrativeData` (`self.NarrativeManager`) SaveGame)
  (`/Game/BPS_Core/Blueprints/Systems/LevelingSystem/Components/BP_AC_LevelingManager.SaveLevelingData` (`self.LevelingManager`) SaveGame)
  (message `/Game/BPS_Core/Blueprints/Game/GameModes/BPI_SaveGame_PlayerData.SetPlayerSaveData_BPI` SaveGame (`/Game/BPS_Core/Blueprints/Systems/CoreSystem/Libraries/BP_Library_CoreFunctions.GetNetworkedPlayerID` self) (make `/Game/BPS_Core/Blueprints/Game/Structures/STR_SaveData_Player_TD` (`/Game/BPS_Core/Blueprints/Systems/CoreSystem/Components/BP_AC_CustomizationManager.CustomizedIntegers` (`self.CustomizationManager`)))))

(event `self.SaveObjectComponent.OnLoadData`
  (params (Component :type "/Game/BPS_Core/Blueprints/Systems/SaveLoadSystem/Components/BP_AC_SaveObjectComponent Object Reference") (SaveGame :type "SaveGame Object Reference"))
  ;[1 1 1] Save and load events.
  (`/Game/BPS_Core/Blueprints/Systems/CoreSystem/Libraries/BP_Library_CoreFunctions.LoadPlayerTags` self SaveGame)
  (`/Game/BPS_Core/Blueprints/Systems/NarrativeSystem/Components/BP_AC_NarrativeManager.LoadNarrativeData` (`self.NarrativeManager`) SaveGame)
  (`/Game/BPS_Core/Blueprints/Systems/LevelingSystem/Components/BP_AC_LevelingManager.LoadLevelingData` (`self.LevelingManager`) SaveGame)
  (bind (_success _savedata) (message `/Game/BPS_Core/Blueprints/Game/GameModes/BPI_SaveGame_PlayerData.GetPlayerSaveData_BPI` SaveGame (`/Game/BPS_Core/Blueprints/Systems/CoreSystem/Libraries/BP_Library_CoreFunctions.GetNetworkedPlayerID` self)))
  (if _success
    (`/Game/BPS_Core/Blueprints/Systems/CoreSystem/Components/BP_AC_CustomizationManager.SetCustomizedIntegers` (`self.CustomizationManager`) (`.CustomizationVariables_5_AA17F65C4BF88417523495BD706862F9` (break `/Game/BPS_Core/Blueprints/Game/Structures/STR_SaveData_Player_TD` _savedata)))))

(event `EnhancedInput|/Game/BPS_Core/Blueprints/Systems/InputsSystem/InputActions/IA_ToggleHUD`
  (params (ActionValue :type Boolean) (ElapsedSeconds :type "Float (double-precision)") (TriggeredSeconds :type "Float (double-precision)") (InputAction :type "InputAction Object Reference" :default "/Game/BPS_Core/Blueprints/Systems/InputsSystem/InputActions/IA_ToggleHUD.IA_ToggleHUD"))
  ;[1 1 1] Open / close interface events.
  (:`Triggered`
    (`/Game/BPS_Core/Blueprints/Game/Components/PlayerController/BP_AC_PlayerControllerManager.HandleInput_ToggleHUD` (`self.PlayerControllerManager`))))

(event `EnhancedInput|/Game/BPS_Core/Blueprints/Systems/InputsSystem/InputActions/IA_PauseMenu`
  (params (ActionValue :type Boolean) (ElapsedSeconds :type "Float (double-precision)") (TriggeredSeconds :type "Float (double-precision)") (InputAction :type "InputAction Object Reference" :default "/Game/BPS_Core/Blueprints/Systems/InputsSystem/InputActions/IA_PauseMenu.IA_PauseMenu"))
  ;[1 1 1] Open / close pause menu.
  (:`Triggered`
    (`/Game/BPS_Core/Blueprints/Game/Components/PlayerController/BP_AC_PlayerControllerManager.HandleInput_PauseMenu` (`self.PlayerControllerManager`))))

(event `EnhancedInput|/Game/BPS_Core/Blueprints/Game/Inputs/IA_Crafting_Process`
  (params (ActionValue :type Boolean) (ElapsedSeconds :type "Float (double-precision)") (TriggeredSeconds :type "Float (double-precision)") (InputAction :type "InputAction Object Reference" :default "/Game/BPS_Core/Blueprints/Game/Inputs/IA_Crafting_Process.IA_Crafting_Process"))
  (bind _playercontrollermanager (`self.PlayerControllerManager`))
  ;[1 1 1] Crafting process inputs.
  (:`Started`
    (`/Game/BPS_Core/Blueprints/Game/Components/PlayerController/BP_AC_PlayerControllerManager.PressCraftingInput` _playercontrollermanager))
  (:`Completed`
    (`/Game/BPS_Core/Blueprints/Game/Components/PlayerController/BP_AC_PlayerControllerManager.ReleaseCraftingInput` _playercontrollermanager)))

(event `EnhancedInput|/Game/BPS_Core/Blueprints/Systems/InputsSystem/InputActions/IA_ToggleInventory`
  (params (ActionValue :type Boolean) (ElapsedSeconds :type "Float (double-precision)") (TriggeredSeconds :type "Float (double-precision)") (InputAction :type "InputAction Object Reference" :default "/Game/BPS_Core/Blueprints/Systems/InputsSystem/InputActions/IA_ToggleInventory.IA_ToggleInventory"))
  ;[1 1 1] Open / close interface events.
  (:`Triggered`
    (`/Game/BPS_Core/Blueprints/Game/Components/PlayerController/BP_AC_PlayerControllerManager.HandleInput_ToggleInventory` (`self.PlayerControllerManager`))))

(event `EnhancedInput|/Game/BPS_Core/Blueprints/Systems/InputsSystem/InputActions/IA_ToggleJournal`
  (params (ActionValue :type Boolean) (ElapsedSeconds :type "Float (double-precision)") (TriggeredSeconds :type "Float (double-precision)") (InputAction :type "InputAction Object Reference" :default "/Game/BPS_Core/Blueprints/Systems/InputsSystem/InputActions/IA_ToggleJournal.IA_ToggleJournal"))
  ;[1 1 1] Open / close interface events.
  (:`Triggered`
    (`/Game/BPS_Core/Blueprints/Game/Components/PlayerController/BP_AC_PlayerControllerManager.HandleInput_ToggleJournal` (`self.PlayerControllerManager`))))

(event `EnhancedInput|/Game/BPS_Core/Blueprints/Game/Inputs/IA_Crafting_Process`
  (params (ActionValue :type Boolean) (ElapsedSeconds :type "Float (double-precision)") (TriggeredSeconds :type "Float (double-precision)") (InputAction :type "InputAction Object Reference" :default "/Game/BPS_Core/Blueprints/Game/Inputs/IA_Crafting_Process.IA_Crafting_Process"))
  (bind _playercontrollermanager (`self.PlayerControllerManager`))
  ;[1 1 1] Crafting process inputs.
  (:`Triggered`
    (`/Game/BPS_Core/Blueprints/Game/Components/PlayerController/BP_AC_PlayerControllerManager.HandleInput_Crafting` _playercontrollermanager))
  (:`Completed`
    (`/Game/BPS_Core/Blueprints/Game/Components/PlayerController/BP_AC_PlayerControllerManager.ReleaseCraftingInput` _playercontrollermanager)))

(event `EnhancedInput|/Game/BPS_Core/Blueprints/Systems/InputsSystem/InputActions/IA_ToggleMap`
  (params (ActionValue :type Boolean) (ElapsedSeconds :type "Float (double-precision)") (TriggeredSeconds :type "Float (double-precision)") (InputAction :type "InputAction Object Reference" :default "/Game/BPS_Core/Blueprints/Systems/InputsSystem/InputActions/IA_ToggleMap.IA_ToggleMap"))
  ;[1 1 1] Open / close interface events.
  (:`Triggered`
    (`/Game/BPS_Core/Blueprints/Game/Components/PlayerController/BP_AC_PlayerControllerManager.HandleInput_ToggleMap` (`self.PlayerControllerManager`))))

(event `EnhancedInput|/Game/BPS_Core/Blueprints/Game/Inputs/IA_SelectDialogueReply1`
  (params (ActionValue :type Boolean) (ElapsedSeconds :type "Float (double-precision)") (TriggeredSeconds :type "Float (double-precision)") (InputAction :type "InputAction Object Reference" :default "/Game/BPS_Core/Blueprints/Game/Inputs/IA_SelectDialogueReply1.IA_SelectDialogueReply1"))
  ;[1 1 1] Dialogue reply selection inputs.
  (:`Triggered`
    (`/Game/BPS_Core/Blueprints/Game/Components/PlayerController/BP_AC_PlayerControllerManager.HandleInput_SelectDialogueReply` (`self.PlayerControllerManager`) 0)))

(event `EnhancedInput|/Game/BPS_Core/Blueprints/Game/Inputs/IA_SelectDialogueReply2`
  (params (ActionValue :type Boolean) (ElapsedSeconds :type "Float (double-precision)") (TriggeredSeconds :type "Float (double-precision)") (InputAction :type "InputAction Object Reference" :default "/Game/BPS_Core/Blueprints/Game/Inputs/IA_SelectDialogueReply2.IA_SelectDialogueReply2"))
  ;[1 1 1] Dialogue reply selection inputs.
  (:`Triggered`
    (`/Game/BPS_Core/Blueprints/Game/Components/PlayerController/BP_AC_PlayerControllerManager.HandleInput_SelectDialogueReply` (`self.PlayerControllerManager`) 1)))

(event `EnhancedInput|/Game/BPS_Core/Blueprints/Game/Inputs/IA_Building_Toggle`
  (params (ActionValue :type Boolean) (ElapsedSeconds :type "Float (double-precision)") (TriggeredSeconds :type "Float (double-precision)") (InputAction :type "InputAction Object Reference" :default "/Game/BPS_Core/Blueprints/Game/Inputs/IA_Building_Toggle.IA_Building_Toggle"))
  ;[1 1 1] Building process inputs.
  (:`Triggered`
    (`/Game/BPS_Core/Blueprints/Game/Components/PlayerController/BP_AC_PlayerControllerManager.HandleInput_ToggleBuilding` (`self.PlayerControllerManager`))))

(event `EnhancedInput|/Game/BPS_Core/Blueprints/Systems/InputsSystem/InputActions/IA_Camera_RotationMode`
  (params (ActionValue :type Boolean) (ElapsedSeconds :type "Float (double-precision)") (TriggeredSeconds :type "Float (double-precision)") (InputAction :type "InputAction Object Reference" :default "/Game/BPS_Core/Blueprints/Systems/InputsSystem/InputActions/IA_Camera_RotationMode.IA_Camera_RotationMode"))
  (bind _playercontrollermanager (`self.PlayerControllerManager`))
  ;[1 1 1] Camera rotation mode input.
  (:`Triggered`
    (`/Game/BPS_Core/Blueprints/Game/Components/PlayerController/BP_AC_PlayerControllerManager.HandleInput_CameraMode` _playercontrollermanager))
  (:`Completed`
    (`/Game/BPS_Core/Blueprints/Game/Components/PlayerController/BP_AC_PlayerControllerManager.ReleaseCameraModeInput` _playercontrollermanager)))

(event `EnhancedInput|/Game/BPS_Core/Blueprints/Game/Inputs/IA_SelectDialogueReply3`
  (params (ActionValue :type Boolean) (ElapsedSeconds :type "Float (double-precision)") (TriggeredSeconds :type "Float (double-precision)") (InputAction :type "InputAction Object Reference" :default "/Game/BPS_Core/Blueprints/Game/Inputs/IA_SelectDialogueReply3.IA_SelectDialogueReply3"))
  ;[1 1 1] Dialogue reply selection inputs.
  (:`Triggered`
    (`/Game/BPS_Core/Blueprints/Game/Components/PlayerController/BP_AC_PlayerControllerManager.HandleInput_SelectDialogueReply` (`self.PlayerControllerManager`) 2)))

(event `EnhancedInput|/Game/BPS_Core/Blueprints/Game/Inputs/IA_Building_Process`
  (params (ActionValue :type Boolean) (ElapsedSeconds :type "Float (double-precision)") (TriggeredSeconds :type "Float (double-precision)") (InputAction :type "InputAction Object Reference" :default "/Game/BPS_Core/Blueprints/Game/Inputs/IA_Building_Process.IA_Building_Process"))
  (bind _playercontrollermanager (`self.PlayerControllerManager`))
  ;[1 1 1] Building process inputs.
  (:`Started`
    (`/Game/BPS_Core/Blueprints/Game/Components/PlayerController/BP_AC_PlayerControllerManager.HandleInput_BuildingProcessPressed` _playercontrollermanager))
  (:`Completed`
    (`/Game/BPS_Core/Blueprints/Game/Components/PlayerController/BP_AC_PlayerControllerManager.HandleInput_BuildingProcessReleased` _playercontrollermanager)))

(event `EnhancedInput|/Game/BPS_Core/Blueprints/Game/Inputs/IA_SelectDialogueReply4`
  (params (ActionValue :type Boolean) (ElapsedSeconds :type "Float (double-precision)") (TriggeredSeconds :type "Float (double-precision)") (InputAction :type "InputAction Object Reference" :default "/Game/BPS_Core/Blueprints/Game/Inputs/IA_SelectDialogueReply4.IA_SelectDialogueReply4"))
  ;[1 1 1] Dialogue reply selection inputs.
  (:`Triggered`
    (`/Game/BPS_Core/Blueprints/Game/Components/PlayerController/BP_AC_PlayerControllerManager.HandleInput_SelectDialogueReply` (`self.PlayerControllerManager`) 3)))

(event `EnhancedInput|/Game/BPS_Core/Blueprints/Game/Inputs/IA_Building_Complete`
  (params (ActionValue :type Boolean) (ElapsedSeconds :type "Float (double-precision)") (TriggeredSeconds :type "Float (double-precision)") (InputAction :type "InputAction Object Reference" :default "/Game/BPS_Core/Blueprints/Game/Inputs/IA_Building_Complete.IA_Building_Complete"))
  ;[1 1 1] Building process inputs.
  (:`Triggered`
    (`/Game/BPS_Core/Blueprints/Game/Components/PlayerController/BP_AC_PlayerControllerManager.HandleInput_CompleteBuild` (`self.PlayerControllerManager`))))

(event `EnhancedInput|/Game/BPS_Core/Blueprints/Systems/InputsSystem/InputActions/IA_Map_Navigation`
  (params (ActionValue :type "Vector2D Structure") (ElapsedSeconds :type "Float (double-precision)") (TriggeredSeconds :type "Float (double-precision)") (InputAction :type "InputAction Object Reference" :default "/Game/BPS_Core/Blueprints/Systems/InputsSystem/InputActions/IA_Map_Navigation.IA_Map_Navigation"))
  ;[1 1 1] Map navigation inputs.
  (:`Triggered`
    (`/Game/BPS_Core/Blueprints/Systems/MapSystem/Components/BP_AC_MapManager.ChangeMapRenderOffset` (`self.MapManager`) ActionValue)))

(event `EnhancedInput|/Game/BPS_Core/Blueprints/Game/Inputs/IA_SelectDialogueReply5`
  (params (ActionValue :type Boolean) (ElapsedSeconds :type "Float (double-precision)") (TriggeredSeconds :type "Float (double-precision)") (InputAction :type "InputAction Object Reference" :default "/Game/BPS_Core/Blueprints/Game/Inputs/IA_SelectDialogueReply5.IA_SelectDialogueReply5"))
  ;[1 1 1] Dialogue reply selection inputs.
  (:`Triggered`
    (`/Game/BPS_Core/Blueprints/Game/Components/PlayerController/BP_AC_PlayerControllerManager.HandleInput_SelectDialogueReply` (`self.PlayerControllerManager`) 4)))

(event `EnhancedInput|/Game/BPS_Core/Blueprints/Game/Inputs/IA_Building_Rotation`
  (params (ActionValue :type "Float (double-precision)") (ElapsedSeconds :type "Float (double-precision)") (TriggeredSeconds :type "Float (double-precision)") (InputAction :type "InputAction Object Reference" :default "/Game/BPS_Core/Blueprints/Game/Inputs/IA_Building_Rotation.IA_Building_Rotation"))
  ;[1 1 1] Building process inputs.
  (:`Triggered`
    (`/Game/BPS_Core/Blueprints/Game/Components/PlayerController/BP_AC_PlayerControllerManager.HandleInput_BuildingRotation` (`self.PlayerControllerManager`) ActionValue)))

(event `EnhancedInput|/Game/BPS_Core/Blueprints/Systems/InputsSystem/InputActions/IA_Map_Zoom`
  (params (ActionValue :type "Float (double-precision)") (ElapsedSeconds :type "Float (double-precision)") (TriggeredSeconds :type "Float (double-precision)") (InputAction :type "InputAction Object Reference" :default "/Game/BPS_Core/Blueprints/Systems/InputsSystem/InputActions/IA_Map_Zoom.IA_Map_Zoom"))
  ;[1 1 1] Map navigation inputs.
)

(fn `GetSaveObjectComponent_BPI`
  (returns (Success :type Boolean) (Component :type "/Game/BPS_Core/Blueprints/Systems/SaveLoadSystem/Components/BP_AC_SaveObjectComponent Object Reference"))
  ;[1 1 1] Returns save object component reference.
  (return true (`self.SaveObjectComponent`)))

(fn `UserConstructionScript`)