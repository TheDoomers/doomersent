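; Settings save game that keeps per-game-mode lists of save slot names in a SavesLists array of structs.
; Interface functions find or create a list by game mode name, and add or remove slots within it.
; Adding moves the slot to the front, keeping newest first without duplicates, and creates the list if missing.
; Edits rebuild the struct and write it back into the array.
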(fn `AddSaveSlotToList_BPI`
  (params (GameModeName :type Name) (SaveSlotName :type String))
  (returns (Success :type Boolean))
  (locals (LocalGameModeName :type Name) (LocalSaveSlot :type String) (LocalSaveSlots :type "Array of String"))
  (bind _localsaveslot (`local.LocalSaveSlot`))
  ;[1 1 1] Try to add save slot to the list of saved games for specific game mode.
  (set `local.LocalGameModeName` GameModeName)
  (set `local.LocalSaveSlot` SaveSlotName)
  (for (_array_element _array_index) (`self.SavesLists`)
    (bind (_gamemodename _savegameslots) (break `/Game/BPS_Core/Blueprints/Systems/SaveLoadSystem/Structures/STR_SavesList` _array_element))
    (if (== _gamemodename (`local.LocalGameModeName`))
      (bind _output_get (set `local.LocalSaveSlots` _savegameslots))
      (`KismetArrayLibrary.Array_RemoveItem` _output_get _localsaveslot)
      (`KismetArrayLibrary.Array_Insert` _output_get _localsaveslot)
      (`KismetArrayLibrary.Array_Set` (`self.SavesLists`) _array_index (make `/Game/BPS_Core/Blueprints/Systems/SaveLoadSystem/Structures/STR_SavesList` (`local.LocalGameModeName`) _output_get))
      (return true)))
  (`KismetArrayLibrary.Array_Add` (`self.SavesLists`) (make `/Game/BPS_Core/Blueprints/Systems/SaveLoadSystem/Structures/STR_SavesList` (`local.LocalGameModeName`) (`|MakeArray` (`local.LocalSaveSlot`))))
  (return true))

(fn `CreateSavesList_BPI`
  (params (GameModeName :type Name))
  (returns (Success :type Boolean) (SavesList :type "/Game/BPS_Core/Blueprints/Systems/SaveLoadSystem/Structures/STR_SavesList Structure"))
  (locals (LocalSavesList :type "/Game/BPS_Core/Blueprints/Systems/SaveLoadSystem/Structures/STR_SavesList Structure"))
  (bind ((`STR_SavesList` _str_saveslist)) (make `/Game/BPS_Core/Blueprints/Systems/SaveLoadSystem/Structures/STR_SavesList` :`GameModeName` GameModeName))
  ;[1 1 1] Create saves list for specific game mode.
  (for _array_element (`self.SavesLists`)
    (if (== (`.GameModeName_7_97DEEEB844919F6828FD8E8F63BE50E4` (break `/Game/BPS_Core/Blueprints/Systems/SaveLoadSystem/Structures/STR_SavesList` _array_element)) GameModeName)
      (return true _array_element)))
  (bind _output_get (set `local.LocalSavesList` _str_saveslist))
  (`KismetArrayLibrary.Array_Add` (`self.SavesLists`) _str_saveslist)
  (return true _output_get))

(fn `GetSavesList_BPI`
  (params (GameModeName :type Name))
  (returns (Success :type Boolean) (SavesList :type "/Game/BPS_Core/Blueprints/Systems/SaveLoadSystem/Structures/STR_SavesList Structure"))
  ;[1 1 1] Try to find saves list for specific game mode.
  (for _array_element (`self.SavesLists`)
    (if (== (`.GameModeName_7_97DEEEB844919F6828FD8E8F63BE50E4` (break `/Game/BPS_Core/Blueprints/Systems/SaveLoadSystem/Structures/STR_SavesList` _array_element)) GameModeName)
      (return true _array_element)))
  (return false))

(fn `RemoveSaveSlotFromList_BPI`
  (params (GameModeName :type Name) (SaveSlotName :type String))
  (returns (Success :type Boolean))
  (locals (LocalGameModeName :type Name) (LocalSaveSlot :type String) (LocalSaveSlots :type "Array of String"))
  ;[1 1 1] Try to remove save slot from the list of saved games for specific game mode.
  (set `local.LocalGameModeName` GameModeName)
  (set `local.LocalSaveSlot` SaveSlotName)
  (for (_array_element _array_index) (`self.SavesLists`)
    (bind (_gamemodename _savegameslots) (break `/Game/BPS_Core/Blueprints/Systems/SaveLoadSystem/Structures/STR_SavesList` _array_element))
    (if (== _gamemodename (`local.LocalGameModeName`))
      (bind _output_get (set `local.LocalSaveSlots` _savegameslots))
      (`KismetArrayLibrary.Array_RemoveItem` _output_get (`local.LocalSaveSlot`))
      (`KismetArrayLibrary.Array_Set` (`self.SavesLists`) _array_index (make `/Game/BPS_Core/Blueprints/Systems/SaveLoadSystem/Structures/STR_SavesList` (`local.LocalGameModeName`) _output_get))
      (return true)))
  (return false))