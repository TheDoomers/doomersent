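; Save game class for the TD game mode, storing world, level and player state behind BPI getter and setter functions.
; Attributes, world items, containers and crafting use working maps keyed by save ID, archived with actor data into per-level maps by level name.
; Player data, quests, notes, tags and leveling are keyed by player ID; day-night and game tags are global.
; Level functions mostly extend parent logic; non-player leveling is stubbed to fail.
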(fn `CheckPlayerSaveData_BPI`
  (params (PlayerID :type String))
  (returns (Success :type Boolean))
  ;[1 1 1] Returns true if the save has a save data for specific player.
  (return (`.ReturnValue` (`BlueprintMapLibrary.Map_Find` (`self.PlayersData`) PlayerID))))

(fn `ClearLevelData_BPI`
  (params (LevelName :type Name))
  (returns (Success :type Boolean))
  (locals (LocalLevelName :type Name :default "None"))
  ;[1 1 1] Remove specific level data from the arrays.
  (bind _output_get (set `local.LocalLevelName` LevelName))
  (`parent.ClearLevelData_BPI` _output_get)
  (`|ExecutionSequence`
    (:`then_0`
      (`|ExecutionSequence`
        (:`then_0`
          (`BlueprintMapLibrary.Map_Remove` (`self.LevelsAttributesData`) (`local.LocalLevelName`)))
        (:`then_1`
          (`|ExecutionSequence`
            (:`then_0`
              (`BlueprintMapLibrary.Map_Remove` (`self.LevelsWorldItemsData`) (`local.LocalLevelName`)))
            (:`then_1`
              (`|ExecutionSequence`
                (:`then_0`
                  (`BlueprintMapLibrary.Map_Remove` (`self.LevelsContainersData`) (`local.LocalLevelName`)))
                (:`then_1`
                  (`|ExecutionSequence`
                    (:`then_0`
                      (`BlueprintMapLibrary.Map_Remove` (`self.LevelsCraftingData`) (`local.LocalLevelName`)))))))))))
    (:`then_1`
      (return true))))

(fn `ClearTempLevelData_BPI`
  (returns (Success :type Boolean))
  ;[1 1 1] Clear temp level data.
  (`parent.ClearTempLevelData_BPI`)
  (`|ExecutionSequence`
    (:`then_0`
      (`|ExecutionSequence`
        (:`then_0`
          (`BlueprintMapLibrary.Map_Clear` (`self.SavedAttributesData`)))
        (:`then_1`
          (`|ExecutionSequence`
            (:`then_0`
              (`BlueprintMapLibrary.Map_Clear` (`self.SavedWorldItemsData`)))
            (:`then_1`
              (`|ExecutionSequence`
                (:`then_0`
                  (`BlueprintMapLibrary.Map_Clear` (`self.SavedContainersData`)))
                (:`then_1`
                  (`|ExecutionSequence`
                    (:`then_0`
                      (`BlueprintMapLibrary.Map_Clear` (`self.SavedCraftingData`)))))))))))
    (:`then_1`
      (return true))))

(fn `GetAttributesSaveData_BPI`
  (params (SaveID :type Integer))
  (returns (Success :type Boolean) (SaveData :type "/Game/BPS_Core/Blueprints/Systems/AttributesSystem/Structures/STR_SaveData_Attributes Structure"))
  (bind (_value _returnvalue) (`BlueprintMapLibrary.Map_Find` (`self.SavedAttributesData`) SaveID))
  ;[1 1 1] Returns save data of attributes manager with specific save ID.
  (return _returnvalue _value))

(fn `GetContainerSaveData_BPI`
  (params (SaveID :type Integer))
  (returns (Success :type Boolean) (SaveData :type "/Game/BPS_Core/Blueprints/Systems/ItemsSystem/Structures/STR_SaveData_Container Structure"))
  (bind (_value _returnvalue) (`BlueprintMapLibrary.Map_Find` (`self.SavedContainersData`) SaveID))
  ;[1 1 1] Returns save data of container with specific save ID.
  (return _returnvalue _value))

(fn `GetCraftingSaveData_BPI`
  (params (SaveID :type Integer))
  (returns (Success :type Boolean) (SaveData :type "/Game/BPS_Core/Blueprints/Systems/ItemsSystem/Structures/STR_SaveData_Crafting Structure"))
  (bind (_value _returnvalue) (`BlueprintMapLibrary.Map_Find` (`self.SavedCraftingData`) SaveID))
  ;[1 1 1] Returns save data of crafting component with specific save ID.
  (return _returnvalue _value))

(fn `GetDayNightCycleData_BPI`
  (returns (Success :type Boolean) (SaveData :type "/Game/BPS_Core/Blueprints/Systems/DayNightCycleSystem/Structures/STR_SaveData_DayNightCycle Structure"))
  ;[1 1 1] Returns save data of day night cycle system.
  (return true (`self.DayNightCycleData`)))

(fn `GetGameTagsSaveData_BPI`
  (returns (Success :type Boolean) (SaveData :type "/Game/BPS_Core/Blueprints/Systems/CoreSystem/Structures/STR_SaveData_GameplayTags Structure"))
  ;[1 1 1] Returns save data of game tags.
  (return true (`self.GameTags`)))

(fn `GetJournalNotesSaveData_BPI`
  (params (PlayerID :type String))
  (returns (Success :type Boolean) (SaveData :type "/Game/BPS_Core/Blueprints/Systems/NarrativeSystem/Structures/STR_SaveData_JournalNotes Structure"))
  (bind (_value _returnvalue) (`BlueprintMapLibrary.Map_Find` (`self.PlayersJournalNotes`) PlayerID))
  ;[1 1 1] Returns save data of journal notes for player with specific player ID.
  (return _returnvalue _value))

(fn `GetLevelingSaveData_BPI`
  (params (SaveID :type Integer))
  (returns (Success :type Boolean) (SaveData :type "/Game/BPS_Core/Blueprints/Systems/LevelingSystem/Structures/STR_SaveData_LevelingSystem Structure"))
  (return false))

(fn `GetPlayerLevelingSaveData_BPI`
  (params (PlayerID :type String))
  (returns (Success :type Boolean) (SaveData :type "/Game/BPS_Core/Blueprints/Systems/LevelingSystem/Structures/STR_SaveData_LevelingSystem Structure"))
  (bind (_value _returnvalue) (`BlueprintMapLibrary.Map_Find` (`self.PlayersLevelingData`) PlayerID))
  ;[1 1 1] Returns save data of leveling for player with specific player ID.
  (return _returnvalue _value))

(fn `GetPlayerSaveData_BPI`
  (params (PlayerID :type String))
  (returns (Success :type Boolean) (SaveData :type "/Game/BPS_Core/Blueprints/Game/Structures/STR_SaveData_Player_TD Structure"))
  (bind (_value _returnvalue) (`BlueprintMapLibrary.Map_Find` (`self.PlayersData`) PlayerID))
  ;[1 1 1] Returns save data of player with specific player ID.
  (return _returnvalue _value))

(fn `GetPlayerTagsSaveData_BPI`
  (params (PlayerID :type String))
  (returns (Success :type Boolean) (SaveData :type "/Game/BPS_Core/Blueprints/Systems/CoreSystem/Structures/STR_SaveData_GameplayTags Structure"))
  (bind (_value _returnvalue) (`BlueprintMapLibrary.Map_Find` (`self.PlayersTags`) PlayerID))
  ;[1 1 1] Returns save data for tags of player with specific player ID.
  (return _returnvalue _value))

(fn `GetQuestsSaveData_BPI`
  (params (PlayerID :type String))
  (returns (Success :type Boolean) (SaveData :type "/Game/BPS_Core/Blueprints/Systems/NarrativeSystem/Structures/STR_SaveData_Quests Structure"))
  (bind (_value _returnvalue) (`BlueprintMapLibrary.Map_Find` (`self.PlayersQuests`) PlayerID))
  ;[1 1 1] Returns quest data for the player controller.
  (return _returnvalue _value))

(fn `GetWorldItemSaveData_BPI`
  (params (SaveID :type Integer))
  (returns (Success :type Boolean) (SaveData :type "/Game/BPS_Core/Blueprints/Systems/ItemsSystem/Structures/STR_SaveData_WorldItem Structure"))
  (bind (_value _returnvalue) (`BlueprintMapLibrary.Map_Find` (`self.SavedWorldItemsData`) SaveID))
  ;[1 1 1] Returns save data of world item with specific save ID.
  (return _returnvalue _value))

(fn `LoadTempLevelData_BPI`
  (params (LevelName :type Name))
  (returns (Success :type Boolean))
  (locals (LocalLevelName :type Name :default "None"))
  ;[1 1 1] Load temp level data.
  (bind _output_get (set `local.LocalLevelName` LevelName))
  (bind _success (`parent.LoadTempLevelData_BPI` _output_get))
  (if _success
    (`|ExecutionSequence`
      (:`then_0`
        (`|ExecutionSequence`
          (:`then_0`
            (set `self.SavedActorsData` (`.ActorsData_7_EF7EAE264C860D3ADCC6EFAB0C04B473` (break `/Game/BPS_Core/Blueprints/Systems/SaveLoadSystem/Structures/STR_SaveLevelData_Actors` (`BlueprintMapLibrary.Map_Find` (`self.LevelsActorsData`) (`local.LocalLevelName`))))))
          (:`then_1`
            (`|ExecutionSequence`
              (:`then_0`
                (set `self.SavedAttributesData` (`.SaveData_6_41ADA04B444CC3E4DF383D95359DD371` (break `/Game/BPS_Core/Blueprints/Systems/AttributesSystem/Structures/STR_SaveLevelData_Attributes` (`BlueprintMapLibrary.Map_Find` (`self.LevelsAttributesData`) (`local.LocalLevelName`))))))
              (:`then_1`
                (`|ExecutionSequence`
                  (:`then_0`
                    (set `self.SavedWorldItemsData` (`.WorldItems_10_7B9639D04664F6E56D2E51841FE917FC` (break `/Game/BPS_Core/Blueprints/Systems/ItemsSystem/Structures/STR_SaveLevelData_WorldItems` (`BlueprintMapLibrary.Map_Find` (`self.LevelsWorldItemsData`) (`local.LocalLevelName`))))))
                  (:`then_1`
                    (`|ExecutionSequence`
                      (:`then_0`
                        (set `self.SavedContainersData` (`.Containers_12_7B9639D04664F6E56D2E51841FE917FC` (break `/Game/BPS_Core/Blueprints/Systems/ItemsSystem/Structures/STR_SaveLevelData_Containers` (`BlueprintMapLibrary.Map_Find` (`self.LevelsContainersData`) (`local.LocalLevelName`))))))
                      (:`then_1`
                        (`|ExecutionSequence`
                          (:`then_0`
                            (set `self.SavedCraftingData` (`.CraftingComponents_14_7B9639D04664F6E56D2E51841FE917FC` (break `/Game/BPS_Core/Blueprints/Systems/ItemsSystem/Structures/STR_SaveLevelData_Crafting` (`BlueprintMapLibrary.Map_Find` (`self.LevelsCraftingData`) (`local.LocalLevelName`))))))))))))))))
      (:`then_1`
        (return true)))
    (else
      (return false))))

(fn `SaveTempLevelData_BPI`
  (params (LevelName :type Name))
  (returns (Success :type Boolean))
  (locals (LocalLevelName :type Name :default "None"))
  (bind _locallevelname (`local.LocalLevelName`))
  (bind _locallevelname_2 (`local.LocalLevelName`))
  (bind _locallevelname_3 (`local.LocalLevelName`))
  (bind _locallevelname_4 (`local.LocalLevelName`))
  (bind _locallevelname_5 (`local.LocalLevelName`))
  ;[1 1 1] Save temp level data.
  (set `local.LocalLevelName` LevelName)
  (`|ExecutionSequence`
    (:`then_0`
      (`|ExecutionSequence`
        (:`then_0`
          (`BlueprintMapLibrary.Map_Add` (`self.LevelsActorsData`) _locallevelname (make `/Game/BPS_Core/Blueprints/Systems/SaveLoadSystem/Structures/STR_SaveLevelData_Actors` _locallevelname (`self.SavedActorsData`))))
        (:`then_1`
          (`|ExecutionSequence`
            (:`then_0`
              (`BlueprintMapLibrary.Map_Add` (`self.LevelsAttributesData`) _locallevelname_4 (make `/Game/BPS_Core/Blueprints/Systems/AttributesSystem/Structures/STR_SaveLevelData_Attributes` _locallevelname_4 (`self.SavedAttributesData`))))
            (:`then_1`
              (`|ExecutionSequence`
                (:`then_0`
                  (`BlueprintMapLibrary.Map_Add` (`self.LevelsWorldItemsData`) _locallevelname_5 (make `/Game/BPS_Core/Blueprints/Systems/ItemsSystem/Structures/STR_SaveLevelData_WorldItems` _locallevelname_5 (`self.SavedWorldItemsData`))))
                (:`then_1`
                  (`|ExecutionSequence`
                    (:`then_0`
                      (`BlueprintMapLibrary.Map_Add` (`self.LevelsContainersData`) _locallevelname_2 (make `/Game/BPS_Core/Blueprints/Systems/ItemsSystem/Structures/STR_SaveLevelData_Containers` _locallevelname_2 (`self.SavedContainersData`))))
                    (:`then_1`
                      (`|ExecutionSequence`
                        (:`then_0`
                          (`BlueprintMapLibrary.Map_Add` (`self.LevelsCraftingData`) _locallevelname_3 (make `/Game/BPS_Core/Blueprints/Systems/ItemsSystem/Structures/STR_SaveLevelData_Crafting` _locallevelname_3 (`self.SavedCraftingData`))))))))))))))
    (:`then_1`
      (return true))))

(fn `SetAttributesSaveData_BPI`
  (params (SaveID :type Integer) (SaveData :type "/Game/BPS_Core/Blueprints/Systems/AttributesSystem/Structures/STR_SaveData_Attributes Structure"))
  (returns (Success :type Boolean))
  ;[1 1 1] Set attributes save data with target save ID.
  (`BlueprintMapLibrary.Map_Add` (`self.SavedAttributesData`) SaveID SaveData)
  (return true))

(fn `SetContainerSaveData_BPI`
  (params (SaveID :type Integer) (SaveData :type "/Game/BPS_Core/Blueprints/Systems/ItemsSystem/Structures/STR_SaveData_Container Structure"))
  (returns (Success :type Boolean))
  ;[1 1 1] Set save data for container with specific save ID.
  (`BlueprintMapLibrary.Map_Add` (`self.SavedContainersData`) SaveID SaveData)
  (return true))

(fn `SetCraftingSaveData_BPI`
  (params (SaveID :type Integer) (SaveData :type "/Game/BPS_Core/Blueprints/Systems/ItemsSystem/Structures/STR_SaveData_Crafting Structure"))
  (returns (Success :type Boolean))
  ;[1 1 1] Set save data of crafting component with specific save ID.
  (`BlueprintMapLibrary.Map_Add` (`self.SavedCraftingData`) SaveID SaveData)
  (return true))

(fn `SetDayNightCycleData_BPI`
  (params (SaveData :type "/Game/BPS_Core/Blueprints/Systems/DayNightCycleSystem/Structures/STR_SaveData_DayNightCycle Structure"))
  (returns (Success :type Boolean))
  ;[1 1 1] Set save data of the day night cycle system.
  (set `self.DayNightCycleData` SaveData)
  (return true))

(fn `SetGameTagsSaveData_BPI`
  (params (SaveData :type "/Game/BPS_Core/Blueprints/Systems/CoreSystem/Structures/STR_SaveData_GameplayTags Structure"))
  (returns (Success :type Boolean))
  ;[1 1 1] Set save data of game tags.
  (set `self.GameTags` SaveData)
  (return true))

(fn `SetJournalNotesSaveData_BPI`
  (params (PlayerID :type String) (SaveData :type "/Game/BPS_Core/Blueprints/Systems/NarrativeSystem/Structures/STR_SaveData_JournalNotes Structure"))
  (returns (Success :type Boolean))
  ;[1 1 1] Set save data of journal notes for player with specific player ID.
  (`BlueprintMapLibrary.Map_Add` (`self.PlayersJournalNotes`) PlayerID SaveData)
  (return true))

(fn `SetLevelingSaveData_BPI`
  (params (SaveID :type Integer) (SaveData :type "/Game/BPS_Core/Blueprints/Systems/LevelingSystem/Structures/STR_SaveData_LevelingSystem Structure"))
  (returns (Success :type Boolean))
  (return false))

(fn `SetPlayerLevelingSaveData_BPI`
  (params (PlayerID :type String) (SaveData :type "/Game/BPS_Core/Blueprints/Systems/LevelingSystem/Structures/STR_SaveData_LevelingSystem Structure"))
  (returns (Success :type Boolean))
  ;[1 1 1] Set save data of leveling for player with specific player ID.
  (`BlueprintMapLibrary.Map_Add` (`self.PlayersLevelingData`) PlayerID SaveData)
  (return true))

(fn `SetPlayerSaveData_BPI`
  (params (PlayerID :type String) (SaveData :type "/Game/BPS_Core/Blueprints/Game/Structures/STR_SaveData_Player_TD Structure"))
  (returns (Success :type Boolean))
  ;[1 1 1] Set player save data.
  (`BlueprintMapLibrary.Map_Add` (`self.PlayersData`) PlayerID SaveData)
  (return true))

(fn `SetPlayerTagsSaveData_BPI`
  (params (PlayerID :type String) (SaveData :type "/Game/BPS_Core/Blueprints/Systems/CoreSystem/Structures/STR_SaveData_GameplayTags Structure"))
  (returns (Success :type Boolean))
  ;[1 1 1] Set save data for tags of player with specific player ID.
  (`BlueprintMapLibrary.Map_Add` (`self.PlayersTags`) PlayerID SaveData)
  (return true))

(fn `SetQuestsSaveData_BPI`
  (params (PlayerID :type String) (SaveData :type "/Game/BPS_Core/Blueprints/Systems/NarrativeSystem/Structures/STR_SaveData_Quests Structure"))
  (returns (Success :type Boolean))
  ;[1 1 1] Set quests save data for the player controller.
  (`BlueprintMapLibrary.Map_Add` (`self.PlayersQuests`) PlayerID SaveData)
  (return true))

(fn `SetWorldItemSaveData_BPI`
  (params (SaveID :type Integer) (SaveData :type "/Game/BPS_Core/Blueprints/Systems/ItemsSystem/Structures/STR_SaveData_WorldItem Structure"))
  (returns (Success :type Boolean))
  ;[1 1 1] Set save data for world item with specific save ID.
  (`BlueprintMapLibrary.Map_Add` (`self.SavedWorldItemsData`) SaveID SaveData)
  (return true))