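; BP_GameState_TD is the TD game state Blueprint that saves and loads game-wide state.
; Its SaveObjectComponent's save and load events pass the save game to game tag routines and to the DayNightCycleManager for day-night cycle data.
; Interface functions expose the save object component and the TD attribute settings data table to other systems.
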(event `self.SaveObjectComponent.OnSaveData`
  (params (Component :type "/Game/BPS_Core/Blueprints/Systems/SaveLoadSystem/Components/BP_AC_SaveObjectComponent Object Reference") (SaveGame :type "SaveGame Object Reference"))
  ;[1 1 1] Save and load events.
  (`/Game/BPS_Core/Blueprints/Systems/CoreSystem/Libraries/BP_Library_CoreFunctions.SaveGameTags` SaveGame)
  (`/Game/BPS_Core/Blueprints/Systems/DayNightCycleSystem/Components/BP_AC_DayNightCycleManager.SaveDayNightCycleData` (`self.DayNightCycleManager`) SaveGame))

(event `self.SaveObjectComponent.OnLoadData`
  (params (Component :type "/Game/BPS_Core/Blueprints/Systems/SaveLoadSystem/Components/BP_AC_SaveObjectComponent Object Reference") (SaveGame :type "SaveGame Object Reference"))
  ;[1 1 1] Save and load events.
  (`/Game/BPS_Core/Blueprints/Systems/CoreSystem/Libraries/BP_Library_CoreFunctions.LoadGameTags` SaveGame)
  (`/Game/BPS_Core/Blueprints/Systems/DayNightCycleSystem/Components/BP_AC_DayNightCycleManager.LoadDayNightCycleData` (`self.DayNightCycleManager`) SaveGame))

(fn `GetAttributesSettingsDataTable_BPI`
  (returns (Success :type Boolean) (DataTable :type "DataTable Object Reference"))
  ;[1 1 1] Returns attribute settings data table.
  (return true "/Game/BPS_Core/Blueprints/Game/DataTables/DT_AttributeSettings_TD.DT_AttributeSettings_TD"))

(fn `GetSaveObjectComponent_BPI`
  (returns (Success :type Boolean) (Component :type "/Game/BPS_Core/Blueprints/Systems/SaveLoadSystem/Components/BP_AC_SaveObjectComponent Object Reference"))
  ;[1 1 1] Returns save object component.
  (return true (`self.SaveObjectComponent`)))

(fn `UserConstructionScript`)